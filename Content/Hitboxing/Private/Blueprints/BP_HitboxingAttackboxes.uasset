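; BP_HitboxingAttackboxes is a Blueprint that exercises the Hitboxing attackbox system by reporting the hits it registers.
; On BeginPlay it enables its Attackboxes and assigns OnHit as the hit event.
; OnHit prints the attacker and its attackbox alongside the struck object and its hurtbox as a debug string.
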(event `self.ReceiveBeginPlay`
  (`FTJHitboxingAttackboxes.Enable` (`self.Attackboxes`))
  (add `FTJHitboxingAttackboxes.HitEvent` (`self.Attackboxes`) (delegate `OnHit`)))

(event `OnHit`
  (params (InHit :type "FTJHitboxingHit Structure (by ref)"))
  (`KismetSystemLibrary.PrintString` (`KismetStringLibrary.Concat_StrStr` (`KismetSystemLibrary.GetDisplayName` InHit_Attackboxer) "." (`KismetStringLibrary.Conv_NameToString` InHit_Attackbox) " > " (`KismetSystemLibrary.GetDisplayName` InHit_Hurtboxer) "." (`KismetStringLibrary.Conv_NameToString` InHit_Hurtbox))))

(fn `UserConstructionScript`)