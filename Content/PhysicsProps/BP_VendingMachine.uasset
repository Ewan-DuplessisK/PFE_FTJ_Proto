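; BP_VendingMachine is a physics prop vending machine that dispenses snacks when kicked, until its Ammo runs out.
; Each kick spends one Ammo and spawns SpawnNum BP_Snack actors, each with a voice sound, randomly offset within a cone around the actor's right vector.
; A timeline then animates the mesh with a lift and pitch tilt, relative to the transform cached at BeginPlay.
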(event `self.ReceiveBeginPlay`
  (bind _staticmesh (`self.StaticMesh`))
  (set `self.Old Location` (`SceneComponent.K2_GetComponentLocation` _staticmesh))
  (set `self.Old Rotation` (`SceneComponent.K2_GetComponentRotation` _staticmesh)))

(event `self.IsKicked`
  (bind _returnvalue (`self.K2_GetActorLocation`))
  (bind _old_location (`self.Old Location`))
  (bind (_old_rotation_roll _old_rotation_pitch _old_rotation_yaw) (`KismetMathLibrary.BreakRotator` (`self.Old Rotation`)))
  (bind (_spawnoffset_x _spawnoffset_y _spawnoffset_z) (`KismetMathLibrary.BreakVector` (`self.SpawnOffset`)))
  (bind (_returnvalue_x _returnvalue_y) (`KismetMathLibrary.BreakVector` (+ (* (`KismetMathLibrary.RandomUnitVectorInConeInDegrees` (`self.GetActorRightVector`) (`self.SpawnAngle`)) _spawnoffset_y) _returnvalue)))
  (if (> (`self.Ammo`) 0)
    (for _ (range 1 (+ (`self.SpawnNum`) 1))
      (`GameplayStatics.PlaySound2D` "/Game/Sound/Vending_Machine/SW_VendingVoice.SW_VendingVoice" 1.0 1.0 0.0 null null false)
      (`|SpawnActorFromClass` "/Game/WeaponsGTP/BP_Snack.BP_Snack_C" (`KismetMathLibrary.MakeTransform` (`KismetMathLibrary.MakeVector` _returnvalue_x _returnvalue_y (+ _spawnoffset_z (.z _returnvalue))) (`SceneComponent.RelativeRotation` (`self.Arrow`))) "AdjustIfPossibleButAlwaysSpawn" "MultiplyWithRoot" null null))
    (`/Engine/EditorBlueprintResources/StandardMacros.DecrementInt` (`self.Ammo`)
      (:`  `
        (bind (_direction _location _rotation) (`Timeline|Anim` :!via `PlayFromStart`)
          (:`Update`
            (`SceneComponent.K2_SetWorldLocationAndRotation` (`self.StaticMesh`) (`KismetMathLibrary.VLerp` _old_location (+ _old_location (0.0 0.0 20.0)) _location) (`KismetMathLibrary.RLerp` (`self.Old Rotation`) (`KismetMathLibrary.MakeRotator` _old_rotation_roll (+ _old_rotation_pitch 10.0) _old_rotation_yaw) _rotation) false false)))))))

(fn `UserConstructionScript`)