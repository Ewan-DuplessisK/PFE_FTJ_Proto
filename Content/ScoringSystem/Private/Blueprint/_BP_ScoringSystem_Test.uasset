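; Test Blueprint for the scoring system that exercises a Score object and shows its state on screen.
; Every tick it prints the current score, multiplier and multiplier percentage as one string.
; Pressing P raises the score and multiplier percentage through the enumeration-based message variant.
; The plain and text-message increase variants are present but unwired, so they never run.
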(event `self.ReceiveTick`
  (params (DeltaSeconds :type "Float (single-precision)"))
  (`KismetSystemLibrary.PrintString` (`KismetStringLibrary.Concat_StrStr` (`KismetStringLibrary.Conv_IntToString` (`FTJ_ScoringSystem_ScoreBase.GetScore` (`self.Score`))) " - " "x" (`KismetStringLibrary.Conv_IntToString` (`FTJ_ScoringSystem_ScoreBase.GetMultiplier` (`self.Score`))) " - " (`KismetStringLibrary.Conv_IntToString` (`FTJ_ScoringSystem_ScoreBase.GetMultiplierPercentage` (`self.Score`))) "%")))

(event `Key|P`
  (params (Key :type "Key Structure"))
  (:`Pressed`
    (`FTJ_ScoringSystem_Score.IncreaseWithEnumeration` (`self.Score`) 1 55 "Test")))

(fn `UserConstructionScript`)