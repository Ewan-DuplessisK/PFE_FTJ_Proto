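; BP_AIManagerTest is a test AI manager for Enemy_Base actors.
; Its Construction Script finds every Enemy_Base and rebuilds unique lists of talking and sitting enemies from their EnemyState.
; BeginPlay, Tick and the AttackSystem function do no work.
; Unconnected AttackSystem nodes sketch a single-attacker scheme that claims CurrentAttacker and halves or restores RunSpeed, but none of it runs.
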(event `self.ReceiveTick`
  (params (DeltaSeconds :type "Float (single-precision)")))

(event `self.ReceiveBeginPlay`
  (`|ExecutionSequence`))

(fn `AttackSystem`)

(fn `UserConstructionScript`
  (`KismetArrayLibrary.Array_Clear` (`self.EnemySitting`))
  (`KismetArrayLibrary.Array_Clear` (`self.EnemyTalking`))
  (bind _outactors (`GameplayStatics.GetAllActorsOfClass` "/Script/FTJ_Proto.Enemy_Base"))
  (for _array_element _outactors
    (`|ExecutionSequence`
      (:`then_0`
        (if (`|EnumEquality` (`Enemy_Base.EnemyState` _array_element) "TALKING")
          (`KismetArrayLibrary.Array_AddUnique` (`self.EnemyTalking`) _array_element)))
      (:`then_1`
        (if (`|EnumEquality` (`Enemy_Base.EnemyState` _array_element) "SITTING")
          (`KismetArrayLibrary.Array_AddUnique` (`self.EnemySitting`) _array_element))))))