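; Enemy AI character for Coworker and R&D types, with stats loaded from DT_EnemyAI by type.
; BeginPlay converts the starting EnemyState into Blackboard keys, pairs talking partners and finds the AI manager and player.
; Pawn sensing and talk events update the Blackboard, while QTE events toggle Walking and NavWalking.
; Launching stops AI logic and sets ragdoll collision, landing enables physics, and enemy overlaps trigger velocity-scaled launches.
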(event `QTE End`
  (bind _charactermovement (`self.CharacterMovement`))
  ;[0 0.4964 1 0.5] QTE Enemy Speed
  (`/Engine/EditorBlueprintResources/StandardMacros.IsValid` _charactermovement
    (:`Is Valid`
      (`CharacterMovementComponent.SetMovementMode` _charactermovement "MOVE_NavWalking" 0)
      (set `self.QTE Ended` true)
      (`KismetSystemLibrary.PrintString` (`KismetSystemLibrary.GetDisplayName` self)))))

(event `QTE Begin`
  (bind _charactermovement (`self.CharacterMovement`))
  ;[0 0.4964 1 0.5] QTE Enemy Speed
  (`/Engine/EditorBlueprintResources/StandardMacros.IsValid` _charactermovement
    (:`Is Valid`
      (`CharacterMovementComponent.SetMovementMode` _charactermovement "MOVE_Walking" 0)
      (set `self.QTE Ended` false)
      (`KismetSystemLibrary.PrintString` (`KismetSystemLibrary.GetDisplayName` self)))))

(event `self.PawnSensing.OnSeePawn`
  (params (Pawn :type "Pawn Object Reference"))
  ;[1 0 0.9698] Player Detection
  (cast `/Game/FullBPProto/BP_CharaSystems` Pawn)
  (`BlackboardComponent.SetValueAsBool` (`AIBlueprintHelperLibrary.GetBlackboard` (`AIBlueprintHelperLibrary.GetAIController` self)) (`self.hasSeenPlayerKey`) true))

(event `CanTalk`
  (bind _cantalkwithotherkey (`self.CanTalkWithOtherKey`))
  ;[1 1 1] Can Talk Event
  (if (`self.bCanTalk`)
    (`BlackboardComponent.SetValueAsBool` (`AIBlueprintHelperLibrary.GetBlackboard` (`AIBlueprintHelperLibrary.GetAIController` self)) _cantalkwithotherkey true)
    (`KismetSystemLibrary.PrintString` "CanTalkWithOther? True" true true (struct :`R` 1.0 :`B` 0.029831 :`A` 1.0))
    (else
      (`BlackboardComponent.SetValueAsBool` (`AIBlueprintHelperLibrary.GetBlackboard` (`AIBlueprintHelperLibrary.GetAIController` self)) _cantalkwithotherkey false))))

(event `self.ReceiveBeginPlay`
  (bind _talkingto (`self.TalkingTo`))
  (bind _asenemy_base (cast `Enemy_Base` _talkingto :!pure true))
  (bind _talkingto_2 (`Enemy_Base.TalkingTo` _asenemy_base))
  (`|ExecutionSequence`
    (:`then_0`
      ;[1 0.8897 0] Enemy State Detection
      (switch `EEnemyType` (`self.EnemyState`)
        (:`PATROL`
          (set `self.E_Patrol` true))
        (:`CHASE`
          (set `self.E_Chase` true))
        (:`SITTING`
          (set `self.E_Sit` true))
        (:`TALKING`
          (set `self.E_Talk` true))
        (:`CHARGE`
          (set `self.E_Charge` true))
        (:`GRAB`
          (set `self.E_Grab` true))
        (:`STUN`
          (set `self.E_Stun` true))))
    (:`then_1`
      ;[0.04394 1 0] Talking To system. Position & switch other actor
      (if (`|EnumEquality` (`self.EnemyState`) "TALKING")
        (set `self.TalkingToPosition` (`self.K2_GetActorLocation` (`self.TalkingTo`)))))
    (:`then_2`
      ;[1 0.4987 0.3582] Set Functions
      (`self.SetVariables`)
      (`self.Patrol`)
      (`self.Chase`)
      (`self.Talking`)
      (`self.Sit`)
      (`self.Charge`)
      (`self.Grab`)
      (`self.Stun`))
    (:`then_3`
      (`/Engine/EditorBlueprintResources/StandardMacros.IsValid` _talkingto
        (:`Is Valid`
          (`/Engine/EditorBlueprintResources/StandardMacros.IsValid` _talkingto_2
            (:`Is Valid`
              (if (== _talkingto_2 self)
                (set `Enemy_Base.EnemyState` "TALKING" _asenemy_base :!label _label)
                (else
                  (`KismetSystemLibrary.PrintString` "[ERROR] Talking to Multiple Enemy" true true (struct :`R` 1.0 :`A` 1.0) 99.0))))
            (:`Is Not Valid`
              (set `Enemy_Base.TalkingTo` self _asenemy_base)
              (goto _label))))))
    (:`then_4`
      ;[0.6213 1 0.6308] Get the Player & AIManager
      (bind _returnvalue (`GameplayStatics.GetActorOfClass` "/Game/IA_System/BP_EnemyAIManager.BP_EnemyAIManager_C"))
      (`/Engine/EditorBlueprintResources/StandardMacros.IsValid` _returnvalue
        (:`Is Valid`
          (set `self.AIManager` _returnvalue)
          (bind _returnvalue_2 (`GameplayStatics.GetActorOfClass` "/Game/FullBPProto/BP_CharaSystems.BP_CharaSystems_C"))
          (`/Engine/EditorBlueprintResources/StandardMacros.IsValid` _returnvalue_2
            (:`Is Valid`
              (set `self.Player` _returnvalue_2))
            (:`Is Not Valid`
              (`KismetSystemLibrary.PrintString` "[ERROR] No Player or Wrong Player REF" true true (struct :`R` 1.0 :`B` 0.00876 :`A` 1.0) 99.0))))
        (:`Is Not Valid`
          (`KismetSystemLibrary.PrintString` "[ERROR] No AIManager on the Level" true true (struct :`R` 1.0 :`B` 0.00876 :`A` 1.0) 99.0))))))

(event `Launched`
  (params (Force :type "Vector Structure"))
  (`BrainComponent.StopLogic` (`AIController.BrainComponent` (`AIBlueprintHelperLibrary.GetAIController` self)) "Dead")
  (`PrimitiveComponent.SetCollisionProfileName` (`self.Mesh`) "Ragdoll" true))

(event `self.OnLanded`
  (params (Hit :type "HitResult Structure (by ref)"))
  (if true
    (`PrimitiveComponent.SetSimulatePhysics` (`self.Mesh`) true)
    (else
      (`CharacterMovementComponent.SetMovementMode` (`self.CharacterMovement`) "MOVE_None" 0))))

(event `self.Capsule.OnComponentBeginOverlap`
  (params (OverlappedComponent :type "PrimitiveComponent Object Reference") (OtherActor :type "Actor Object Reference") (OtherComp :type "PrimitiveComponent Object Reference") (OtherBodyIndex :type Integer) (bFromSweep :type Boolean) (SweepResult :type "HitResult Structure (by ref)"))
  (bind _returnvalue (`self.GetVelocity`))
  ; Physics enabled objects collisions
  ; If the object is moving and not detecting itself
  (if true
    (if (!= OtherActor self)
      ; Colliding with an enemy
      (bind _asenemy_base (cast `Enemy_Base` OtherActor))
      (if (not (`Enemy_Base.isLaunched` _asenemy_base))
        (`self.Launched` (* _returnvalue 0.8))
        ; Reduce actor speed after transmitting force
        (`PrimitiveComponent.SetAllPhysicsLinearVelocity` (`self.CapsuleComponent`) (* _returnvalue 0.5) false)))))

(fn `Charge`
  (if (`self.E_Charge`)
    (`BlackboardComponent.SetValueAsBool` (`AIBlueprintHelperLibrary.GetBlackboard` (`AIBlueprintHelperLibrary.GetAIController` self)) "ECharge" true)))

(fn `Chase`
  (if (`self.E_Chase`)
    (`BlackboardComponent.SetValueAsBool` (`AIBlueprintHelperLibrary.GetBlackboard` (`AIBlueprintHelperLibrary.GetAIController` self)) "playerAction?" true)))

(fn `Grab`
  (if (`self.E_Grab`)
    (`BlackboardComponent.SetValueAsBool` (`AIBlueprintHelperLibrary.GetBlackboard` (`AIBlueprintHelperLibrary.GetAIController` self)) "EGrab" true)))

(fn `Patrol`
  (if (`self.E_Patrol`)
    (`BlackboardComponent.SetValueAsBool` (`AIBlueprintHelperLibrary.GetBlackboard` (`AIBlueprintHelperLibrary.GetAIController` self)) "EPatrol" true)))

(fn `SetVariables`
  (switch `/Game/IA_System/E_EnemyTypeCRD` (`self.Enemy Type`)
    (:`NewEnumerator1`
      (bind _returnvalue (`|GetDataTableRow` "/Game/IA_System/DT_EnemyAI.DT_EnemyAI" "Coworker")
        (:`then`
          (bind (_walkspeed _runspeed _maxhealth _damages _chargedistance _speedcharge _grabdistance _qteinputrequired _timeafkafterqte _stunduration) (break `/Game/IA_System/S_EnemyAI` _returnvalue))
          (set `self.WalkSpeed` _walkspeed)
          (set `self.RunSpeed` _runspeed)
          (set `self.MaxHealth` _maxhealth)
          (set `self.Damages` _damages)
          (set `self.ChargeDistance` _chargedistance)
          (set `self.SpeedCharge` _speedcharge)
          (set `self.GrabDistance` _grabdistance)
          (set `self.QTEInputRequired` _qteinputrequired)
          (set `self.TimeAFKAfterQTE` _timeafkafterqte)
          (set `self.StunDuration` _stunduration))))
    (:`NewEnumerator2`
      (bind _returnvalue_2 (`|GetDataTableRow` "/Game/IA_System/DT_EnemyAI.DT_EnemyAI" "R&D")
        (:`then`
          (bind (_walkspeed_2 _runspeed_2 _maxhealth_2 _damages_2 _chargedistance_2 _speedcharge_2 _grabdistance_2 _qteinputrequired_2 _timeafkafterqte_2 _stunduration_2) (break `/Game/IA_System/S_EnemyAI` _returnvalue_2))
          (set `self.WalkSpeed` _walkspeed_2)
          (set `self.RunSpeed` _runspeed_2)
          (set `self.MaxHealth` _maxhealth_2)
          (set `self.Damages` _damages_2)
          (set `self.ChargeDistance` _chargedistance_2)
          (set `self.SpeedCharge` _speedcharge_2)
          (set `self.GrabDistance` _grabdistance_2)
          (set `self.QTEInputRequired` _qteinputrequired_2)
          (set `self.TimeAFKAfterQTE` _timeafkafterqte_2)
          (set `self.StunDuration` _stunduration_2))))
    (:`NewEnumerator0`
      (`KismetSystemLibrary.PrintString` "You Need to Select a Enemy Type" true true (struct :`R` 1.0 :`G` 0.014146 :`A` 1.0) 10.0))))

(fn `Sit`
  (if (`self.E_Sit`)
    (`BlackboardComponent.SetValueAsBool` (`AIBlueprintHelperLibrary.GetBlackboard` (`AIBlueprintHelperLibrary.GetAIController` self)) "ESit" true)))

(fn `Stun`
  (if (`self.E_Stun`)
    (`BlackboardComponent.SetValueAsBool` (`AIBlueprintHelperLibrary.GetBlackboard` (`AIBlueprintHelperLibrary.GetAIController` self)) "EStun" true)))

(fn `Talking`
  (if (`self.E_Talk`)
    (`BlackboardComponent.SetValueAsBool` (`AIBlueprintHelperLibrary.GetBlackboard` (`AIBlueprintHelperLibrary.GetAIController` self)) "ETalk" true)))

(fn `UserConstructionScript`)