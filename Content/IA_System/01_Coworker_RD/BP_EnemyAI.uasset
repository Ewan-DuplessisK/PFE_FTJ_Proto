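; Enemy AI character for Coworker and R&D types, feeding its starting state, attack type and player awareness into Blackboard keys.
; BeginPlay loads stats from a data table, finds the player and AI manager, and pairs talking enemies.
; A looping timer line-traces the player for ranged attack range.
; When launched, it passes damped velocity to enemies and props it hits; on landing it teleports away after a delay and notifies the manager.
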(event `self.ReceiveTick`
  (params (DeltaSeconds :type "Float (single-precision)"))
  (`self.PlayerAction Exec`))

(event `self.ReceiveBeginPlay`
  (`|ExecutionSequence`
    (:`then_0`
      (`self.EnemyState Detection`)
      (`self.Set Functions`)
      (`self.Get Player and Manager`)
      (`self.Set Enemy Attack Type`))
    (:`then_1`
      (`self.Talking To`)
      (`self.Position / Switch Talking`))
    (:`then_2`
      (`KismetSystemLibrary.K2_SetTimerDelegate` (delegate `Distance Attack`) 0.3 true))))

(event `self.PawnSensing.OnSeePawn`
  (params (Pawn :type "Pawn Object Reference"))
  ;[1 0 0.9698] Player Detection
  (cast `Game_Character` Pawn)
  (`BlackboardComponent.SetValueAsBool` (`AIBlueprintHelperLibrary.GetBlackboard` (`AIBlueprintHelperLibrary.GetAIController` self)) (`self.hasSeenPlayerKey`) true))

(event `self.OnLanded`
  (params (Hit :type "HitResult Structure (by ref)"))
  ;[1 0.1021 0 0.5] Launch / Ragdoll / Death
  (`KismetSystemLibrary.Delay` (`self.Delay For TP After Enemy Death`))
  (`PrimitiveComponent.SetSimulatePhysics` (`self.Mesh`) false)
  (`self.K2_SetActorLocation` (`self.DeathTpPosition`))
  (`PrimitiveComponent.SetCollisionProfileName` (`self.Mesh`) "BlockAllDynamic" true)
  (`SceneComponent.K2_SetRelativeLocation` (`self.Mesh`) (0.0 0.0 -90.0) false true)
  (`SceneComponent.K2_SetRelativeRotation` (`self.Mesh`) (struct :`Yaw` -90.0) false false)
  (`ActorComponent.Deactivate` (`self.PawnSensing`))
  (bind _asbp_aimanager (cast `/Game/IA_System/BP_AIManager` (`self.AIManager`)))
  (`AIManager.NotifyOutOfRange` _asbp_aimanager self))

(event `self.CapsulePhysics.OnComponentBeginOverlap`
  (params (OverlappedComponent :type "PrimitiveComponent Object Reference") (OtherActor :type "Actor Object Reference") (OtherComp :type "PrimitiveComponent Object Reference") (OtherBodyIndex :type Integer) (bFromSweep :type Boolean) (SweepResult :type "HitResult Structure (by ref)"))
  (bind _returnvalue (`self.GetVelocity`))
  (bind _returnvalue_2 (* _returnvalue 0.8))
  ;[1 0.1021 0 0.5] Launch / Ragdoll / Death
  ;; Physics enabled objects collisions
  ;; If the object is moving and not detecting itself
  (if (`self.isLaunched`)
    (if (!= OtherActor self)
      ;; Colliding with an enemy
      (bind _asenemy_base (cast `Enemy_Base` OtherActor)
        (:`then`
          (if (not (`Enemy_Base.isLaunched` _asenemy_base))
            (`self.Launched` _asenemy_base _returnvalue_2)
            ;; Reduce actor speed after transmitting force
            (`PrimitiveComponent.SetAllPhysicsLinearVelocity` (`self.CapsuleComponent`) (* _returnvalue 0.5) false :!label _label)))
        (:`CastFailed`
          ;; Colliding with a prop
          (bind _asphysics_props (cast `Physics_Props` OtherActor))
          (if (not (`Physics_Props.isLaunched` _asphysics_props))
            (`Physics_Props.Launched` _asphysics_props _returnvalue_2)
            (goto _label)))))))

(event `Distance Attack`
  ;[0 1 0.08625] Distance Attack
  (if (and (`Game_Character.PlayerAction` (cast `/Game/PlayerCharacter/BP_CharaSystems` (`self.Player`) :!pure true)) (`self.DistanceAttack?`))
    (bind _outhit (`KismetSystemLibrary.LineTraceSingleForObjects` :`Start` (`self.K2_GetActorLocation`) :`End` (`self.K2_GetActorLocation` (`self.Player`)) :`ObjectTypes` (`|MakeArray` "ObjectTypeQuery3" "ObjectTypeQuery1" "ObjectTypeQuery2" :!type "EObjectTypeQuery Enum") :`DrawDebugType` "ForOneFrame"))
    (bind (_bblockinghit _binitialoverlap _time _distance _location _impactpoint _normal _impactnormal _physmat _hitactor) (`GameplayStatics.BreakHitResult` _outhit))
    ;;[1 0 0] PRINT
    (`KismetSystemLibrary.PrintString` (`KismetStringLibrary.Concat_StrStr` "Player Distance :" (`KismetStringLibrary.Conv_DoubleToString` _distance) " - " "Attack Distance Set :" (`KismetStringLibrary.Conv_DoubleToString` (`self.AttackDistanceRange`))))
    (if (== _hitactor (`GameplayStatics.GetPlayerPawn` 0))
      (if (< _distance (`self.AttackDistanceRange`))
        (`MovementComponent.StopMovementImmediately` (`self.CharacterMovement`))
        (`BlackboardComponent.SetValueAsBool` (`AIBlueprintHelperLibrary.GetBlackboard` (`AIBlueprintHelperLibrary.GetAIController` self)) (`self.playerInDistanceAttackRangeKey`) true)
        (else
          (`BlackboardComponent.SetValueAsBool` (`AIBlueprintHelperLibrary.GetBlackboard` (`AIBlueprintHelperLibrary.GetAIController` self)) (`self.playerInDistanceAttackRangeKey`) false))))))

(fn `AFK`
  (if (`self.E_AFK`)
    (`BlackboardComponent.SetValueAsBool` (`AIBlueprintHelperLibrary.GetBlackboard` (`AIBlueprintHelperLibrary.GetAIController` self)) "EAFK" true)))

(fn `Chase`
  (if (`self.E_Chase`)
    (`BlackboardComponent.SetValueAsBool` (`AIBlueprintHelperLibrary.GetBlackboard` (`AIBlueprintHelperLibrary.GetAIController` self)) "playerAction?" true)))

(fn `EnemyState Detection`
  ;[1 0.8897 0] Enemy State Detection
  (switch `EEnemyType` (`self.EnemyState`)
    (:`PATROL`
      (set `self.E_Patrol` true))
    (:`CHASE`
      (set `self.E_Chase` true))
    (:`SITTING`
      (set `self.E_Sit` true))
    (:`TALKING`
      (set `self.E_Talk` true))
    (:`AFK`
      (set `self.E_AFK` true))))

(fn `Get Player and Manager`
  ;[0.6213 1 0.6308] Get the Player & AIManager
  (bind _returnvalue (`GameplayStatics.GetActorOfClass` "/Game/IA_System/BP_AIManager.BP_AIManager_C"))
  (`/Engine/EditorBlueprintResources/StandardMacros.IsValid` _returnvalue
    (:`Is Valid`
      (set `self.AIManager` _returnvalue)
      (bind _returnvalue_2 (`GameplayStatics.GetActorOfClass` "/Game/PlayerCharacter/BP_CharaSystems.BP_CharaSystems_C"))
      (`/Engine/EditorBlueprintResources/StandardMacros.IsValid` _returnvalue_2
        (:`Is Valid`
          (set `self.Player` _returnvalue_2))
        (:`Is Not Valid`
          (`KismetSystemLibrary.PrintString` "[ERROR] No Player or Wrong Player REF" true true (struct :`R` 1.0 :`B` 0.00876 :`A` 1.0) 99.0))))
    (:`Is Not Valid`
      (`KismetSystemLibrary.PrintString` "[ERROR] No AIManager on the Level" true true (struct :`R` 1.0 :`B` 0.00876 :`A` 1.0) 99.0))))

(fn `Patrol`
  (if (`self.E_Patrol`)
    (`BlackboardComponent.SetValueAsBool` (`AIBlueprintHelperLibrary.GetBlackboard` (`AIBlueprintHelperLibrary.GetAIController` self)) "EPatrol" true)))

(fn `PlayerAction Exec`
  (if (`Game_Character.PlayerAction` (cast `/Game/PlayerCharacter/BP_CharaSystems` (`GameplayStatics.GetPlayerPawn` 0) :!pure true))
    (`/Engine/EditorBlueprintResources/StandardMacros.DoOnce` false
      (:`Completed`
        (`BlackboardComponent.SetValueAsBool` (`AIBlueprintHelperLibrary.GetBlackboard` (`AIBlueprintHelperLibrary.GetAIController` self)) (`self.playerActionKey`) true)))))

(fn `Position / Switch Talking`
  (bind _talkingto (`self.TalkingTo`))
  (bind _asenemy_base (cast `Enemy_Base` _talkingto :!pure true))
  (bind _talkingto_2 (`Enemy_Base.TalkingTo` _asenemy_base))
  (`/Engine/EditorBlueprintResources/StandardMacros.IsValid` _talkingto
    (:`Is Valid`
      (`/Engine/EditorBlueprintResources/StandardMacros.IsValid` _talkingto_2
        (:`Is Valid`
          (if (== _talkingto_2 self)
            (set `Enemy_Base.EnemyState` "TALKING" _asenemy_base :!label _label)
            (else
              (`KismetSystemLibrary.PrintString` "[ERROR] Talking to Multiple Enemy" true true (struct :`R` 1.0 :`A` 1.0) 99.0))))
        (:`Is Not Valid`
          (set `Enemy_Base.TalkingTo` self _asenemy_base)
          (goto _label))))))

(fn `QTE Begin`
  (bind _charactermovement (`self.CharacterMovement`))
  (`/Engine/EditorBlueprintResources/StandardMacros.IsValid` _charactermovement
    (:`Is Valid`
      (`CharacterMovementComponent.SetMovementMode` _charactermovement "MOVE_Walking" 0)
      (set `self.QTE Ended` false))))

(fn `QTE End`
  (bind _charactermovement (`self.CharacterMovement`))
  (`/Engine/EditorBlueprintResources/StandardMacros.IsValid` _charactermovement
    (:`Is Valid`
      (`CharacterMovementComponent.SetMovementMode` _charactermovement "MOVE_NavWalking" 0)
      (set `self.QTE Ended` true))))

(fn `Set Enemy Attack Type`
  (switch `/Game/IA_System/E_AttackType` (`self.Attack Type`)
    (:`NewEnumerator1`
      (`BlackboardComponent.SetValueAsBool` (`AIBlueprintHelperLibrary.GetBlackboard` (`AIBlueprintHelperLibrary.GetAIController` self)) "CQCAttack?" true)
      (set `self.MeleeAttack?` true)
      (set `self.DistanceAttack?` false))
    (:`NewEnumerator0`
      (`BlackboardComponent.SetValueAsBool` (`AIBlueprintHelperLibrary.GetBlackboard` (`AIBlueprintHelperLibrary.GetAIController` self)) "DistanceAttack?" true)
      (set `self.DistanceAttack?` true)
      (set `self.MeleeAttack?` false))))

(fn `Set Functions`
  (`self.SetVariables`)
  (`self.Patrol`)
  (`self.Chase`)
  (`self.Talking`)
  (`self.Sit`)
  (`self.AFK`))

(fn `SetVariables`
  (switch `/Game/IA_System/E_EnemyTypeCRD` (`self.Enemy Type`)
    (:`NewEnumerator1`
      (bind _returnvalue (`|GetDataTableRow` "/Game/DataAssets/Data_Enemies/DT_EnemyAI.DT_EnemyAI" (`self.Coworker Row Name`))
        (:`then`
          (bind (_walkspeed _runspeed _maxhealth _cqcdamages _cqcinvincibilitytime _distancedamages _distanceinvincibilitytime _attackdistancerange _qteinputrequired _timeafkafterqte) (break `/Game/IA_System/S_EnemyAI` _returnvalue))
          (set `self.WalkSpeed` _walkspeed)
          (set `self.RunSpeed` _runspeed)
          (set `self.MaxHealth` _maxhealth)
          (set `self.CQCDamages` _cqcdamages)
          (set `self.CQCInvincibilityTime` _cqcinvincibilitytime)
          (set `self.DistanceDamages` _distancedamages)
          (set `self.DistanceInvincibilityTime` _distanceinvincibilitytime)
          (set `self.AttackDistanceRange` _attackdistancerange)
          (set `self.QTEInputRequired` _qteinputrequired)
          (set `self.TimeAFKAfterQTE` _timeafkafterqte))))
    (:`NewEnumerator2`
      (bind _returnvalue_2 (`|GetDataTableRow` "/Game/DataAssets/Data_Enemies/DT_EnemyAI.DT_EnemyAI" (`self.R&D Row Name`))
        (:`then`
          (bind (_walkspeed_2 _runspeed_2 _maxhealth_2 _cqcdamages_2 _cqcinvincibilitytime_2 _distancedamages_2 _distanceinvincibilitytime_2 _attackdistancerange_2 _qteinputrequired_2 _timeafkafterqte_2) (break `/Game/IA_System/S_EnemyAI` _returnvalue_2))
          (set `self.WalkSpeed` _walkspeed_2)
          (set `self.RunSpeed` _runspeed_2)
          (set `self.MaxHealth` _maxhealth_2)
          (set `self.CQCDamages` _cqcdamages_2)
          (set `self.CQCInvincibilityTime` _cqcinvincibilitytime_2)
          (set `self.DistanceDamages` _distancedamages_2)
          (set `self.DistanceInvincibilityTime` _distanceinvincibilitytime_2)
          (set `self.AttackDistanceRange` _attackdistancerange_2)
          (set `self.QTEInputRequired` _qteinputrequired_2)
          (set `self.TimeAFKAfterQTE` _timeafkafterqte_2))))
    (:`NewEnumerator0`
      (`KismetSystemLibrary.PrintString` "You Need to Select a Enemy Type" true true (struct :`R` 1.0 :`G` 0.014146 :`A` 1.0) 10.0))))

(fn `Sit`
  (if (`self.E_Sit`)
    (`BlackboardComponent.SetValueAsBool` (`AIBlueprintHelperLibrary.GetBlackboard` (`AIBlueprintHelperLibrary.GetAIController` self)) "ESit" true)))

(fn `Talking`
  (if (`self.E_Talk`)
    (`BlackboardComponent.SetValueAsBool` (`AIBlueprintHelperLibrary.GetBlackboard` (`AIBlueprintHelperLibrary.GetAIController` self)) "ETalk" true)))

(fn `Talking To`
  (if (`|EnumEquality` (`self.EnemyState`) "TALKING")
    (set `self.TalkingToPosition` (`self.K2_GetActorLocation` (`self.TalkingTo`)))))

(fn `UserConstructionScript`)