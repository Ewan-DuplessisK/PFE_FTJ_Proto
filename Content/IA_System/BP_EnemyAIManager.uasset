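; BP_EnemyAIManager is an enemy AI manager that limits attacks to one Enemy_Base at a time.
; Its construction script sorts level enemies into talking and sitting lists by EnemyState.
; While enabled, Tick scans all enemies and, for each one attacking, clears IsAttacking and deactivates PlayerInRangeSphere on the others.
; Coworker_RD enemies whose QTE has ended get that sphere reactivated immediately.
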(event `self.ReceiveTick`
  (params (DeltaSeconds :type "Float (single-precision)"))
  (if (`self.ManagerAttackEnable`)
    (`self.AttackSystem`)))

(fn `AttackSystem`
  (bind _enemyattacking (`self.EnemyAttacking`))
  (bind _outactors (`GameplayStatics.GetAllActorsOfClass` "/Script/FTJ_Proto.Enemy_Base"))
  (for _array_element _outactors
    (if (`Enemy_Base.IsAttacking` _array_element)
      (`KismetArrayLibrary.Array_Add` _enemyattacking _array_element)
      (set `self.Current Attacker` (`|GetArrayItem` _enemyattacking))
      (`KismetArrayLibrary.Array_Clear` _enemyattacking)
      (for _array_element_2 _outactors
        (if (!= _array_element_2 (`self.Current Attacker`))
          (`|ExecutionSequence`
            (:`then_0`
              (set `Enemy_Base.IsAttacking` false _array_element_2))
            (:`then_1`
              (`ActorComponent.Deactivate` (`Enemy_Base.PlayerInRangeSphere` _array_element_2))
              (bind _asbp_enemy_ai_coworker_rd (cast `/Game/IA_System/01_Coworker_RD/BP_EnemyAI_Coworker_RD` _array_element_2))
              (if (`/Game/IA_System/01_Coworker_RD/BP_EnemyAI_Coworker_RD.QTE Ended` _asbp_enemy_ai_coworker_rd)
                (`ActorComponent.Activate` (`Enemy_Base.PlayerInRangeSphere` _array_element_2) false)))))))))

(fn `UserConstructionScript`
  (`KismetArrayLibrary.Array_Clear` (`self.EnemySitting`))
  (`KismetArrayLibrary.Array_Clear` (`self.EnemyTalking`))
  (bind _outactors (`GameplayStatics.GetAllActorsOfClass` "/Script/FTJ_Proto.Enemy_Base"))
  (for _array_element _outactors
    (`|ExecutionSequence`
      (:`then_0`
        (if (`|EnumEquality` (`Enemy_Base.EnemyState` _array_element) "TALKING")
          (`KismetArrayLibrary.Array_AddUnique` (`self.EnemyTalking`) _array_element)))
      (:`then_1`
        (if (`|EnumEquality` (`Enemy_Base.EnemyState` _array_element) "SITTING")
          (`KismetArrayLibrary.Array_AddUnique` (`self.EnemySitting`) _array_element))))))