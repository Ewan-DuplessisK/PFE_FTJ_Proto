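; BP_ProjectileEnemy is an enemy ranged projectile that damages the player character on sphere overlap.
; It reads damage and invincibility time from the first BP_EnemyAI found at BeginPlay, not necessarily its shooter.
; An exact BP_CharaSystems hit with a valid life widget applies damage, refreshes the widget and destroys the projectile.
; Non-character overlaps destroy it immediately, while subclass overlaps destroy it after a delay without damage.
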(event `self.ReceiveBeginPlay`
  (bind _returnvalue (`GameplayStatics.GetActorOfClass` "/Game/IA_System/01_Coworker_RD/BP_EnemyAI.BP_EnemyAI_C")))

(event `self.Sphere collision.OnComponentBeginOverlap`
  (params (OverlappedComponent :type "PrimitiveComponent Object Reference") (OtherActor :type "Actor Object Reference") (OtherComp :type "PrimitiveComponent Object Reference") (OtherBodyIndex :type Integer) (bFromSweep :type Boolean) (SweepResult :type "HitResult Structure (by ref)"))
  (bind _asbp_chara_systems (cast `/Game/PlayerCharacter/BP_CharaSystems` OtherActor)
    (:`then`
      (if (== (`GameplayStatics.GetObjectClass` OtherActor) "/Game/PlayerCharacter/BP_CharaSystems.BP_CharaSystems_C")
        (bind _playerlifewidget (`/Game/PlayerCharacter/BP_CharaSystems.PlayerLifeWidget` _asbp_chara_systems)
          (:`then`
            (`/Game/PlayerCharacter/BP_CharaSystems.Damages` _asbp_chara_systems (`Enemy_Base.DistanceDamages` (stale `self.ReceiveBeginPlay` _returnvalue)) (`Enemy_Base.DistanceInvincibilityTime` (stale `self.ReceiveBeginPlay` _returnvalue)))
            (`/Game/UI/W_PlayerLife.Update LIfe` _playerlifewidget))
          (:`else`))
        (else
          (`KismetSystemLibrary.Delay` 3.0))))
    (:`CastFailed`
      _))
  (`self.K2_DestroyActor`))

(fn `UserConstructionScript`)