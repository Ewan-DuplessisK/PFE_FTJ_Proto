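; Game mode for the AI system that spawns coworker enemies (BP_EnemyAI_Coworker_RD) on request from the player character.
; Tick polls the player's WrkRDSpawn flag, spawns one at the first BP_EnemyAISpawner found with randomized height scale, then clears the flag.
; A DoOnce reset after a short delay throttles spawning.
; BeginPlay stores the initial coworker count in EnemyCwrkNumber, which is not updated on spawn.
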(event `self.ReceiveTick`
  (params (DeltaSeconds :type "Float (single-precision)"))
  (bind _asbp_fpsaisystem (cast `/Game/IA_System/BP_FPSAISystem` (`GameplayStatics.GetPlayerCharacter` 0) :!pure true))
  (`|ExecutionSequence`
    (:`then_0`
      (if (`/Game/IA_System/BP_FPSAISystem.WrkRDSpawn` _asbp_fpsaisystem)
        (bind _returnvalue (`GameplayStatics.GetActorOfClass` "/Game/IA_System/BP_EnemyAISpawner.BP_EnemyAISpawner_C"))
        (`/Engine/EditorBlueprintResources/StandardMacros.DoOnce` false :!label _label
          (:`Completed`
            (bind _returnvalue_2 (`self.K2_GetActorLocation` _returnvalue))
            (bind _returnvalue_3 (`|SpawnActorFromClass` "/Game/IA_System/01_Coworker_RD/BP_EnemyAI_Coworker_RD.BP_EnemyAI_Coworker_RD_C" (`KismetMathLibrary.Conv_VectorToTransform` _returnvalue_2) "Undefined" "MultiplyWithRoot" null null))
            (`self.K2_SetActorTransform` _returnvalue_3 (`KismetMathLibrary.MakeTransform` _returnvalue_2 (struct) (`KismetMathLibrary.MakeVector` 1.0 1.0 (`KismetMathLibrary.RandomFloatInRange` 0.75 1.2))) false false)
            (`KismetSystemLibrary.PrintString` "Enemy CWR Spawn !" true true (struct :`G` 0.752667 :`B` 1.0 :`A` 1.0))
            (set `/Game/IA_System/BP_FPSAISystem.WrkRDSpawn` false _asbp_fpsaisystem)
            (`KismetSystemLibrary.Delay` 0.2)
            (goto _label :!via `Reset`)))))))

(event `self.ReceiveBeginPlay`
  (bind _outactors (`GameplayStatics.GetAllActorsOfClass` "/Game/IA_System/01_Coworker_RD/BP_EnemyAI_Coworker_RD.BP_EnemyAI_Coworker_RD_C"))
  (set `self.EnemyCwrkNumber` (`KismetArrayLibrary.Array_Length` _outactors)))

(fn `UserConstructionScript`)