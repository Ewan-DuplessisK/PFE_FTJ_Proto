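; Accountant enemy AI character that loads its speeds, health, damage and talking time from DT_EnemyAI on BeginPlay.
; Pawn sensing sets a Blackboard seen-player flag for BP_FPSAISystem pawns.
; Range-sphere overlaps toggle the attack-range flag, though the check passes actors not equal to BP_FPSAISystem.
; StartConvo and EndConvo handle facing and talk-sphere activation, but the overlap-driven conversation is disconnected and CanTalk is marked useless.
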(event `self.ReceiveBeginPlay`
  (`self.SetVariables`))

(event `self.PlayerInRangeSphere.OnComponentBeginOverlap`
  (params (OverlappedComponent :type "PrimitiveComponent Object Reference") (OtherActor :type "Actor Object Reference") (OtherComp :type "PrimitiveComponent Object Reference") (OtherBodyIndex :type Integer) (bFromSweep :type Boolean) (SweepResult :type "HitResult Structure (by ref)"))
  ;[0 0.9686 1] Is the player in enemy attack range
  (if (not (== OtherActor "/Game/IA_System/BP_FPSAISystem.BP_FPSAISystem"))
    (set `self.isPlayerInAttackRange?` true)
    (`BlackboardComponent.SetValueAsBool` (`AIBlueprintHelperLibrary.GetBlackboard` self) "playerInAttackRange?" true)))

(event `self.PlayerInRangeSphere.OnComponentEndOverlap`
  (params (OverlappedComponent :type "PrimitiveComponent Object Reference") (OtherActor :type "Actor Object Reference") (OtherComp :type "PrimitiveComponent Object Reference") (OtherBodyIndex :type Integer))
  ;[0 0.9686 1] Is the player in enemy attack range
  (if (not (== OtherActor "/Game/IA_System/BP_FPSAISystem.BP_FPSAISystem"))
    (set `self.isPlayerInAttackRange?` false)
    (`BlackboardComponent.SetValueAsBool` (`AIBlueprintHelperLibrary.GetBlackboard` self) "playerInAttackRange?" false)))

(event `CanTalk`
  ;[1 1 1] [Useless] [Need BT CanTalk] Can Talk Event
  (if (`self.CanTalk?`)
    (`BlackboardComponent.SetValueAsBool` (`AIBlueprintHelperLibrary.GetBlackboard` (`AIBlueprintHelperLibrary.GetAIController` self)) "CanTalkWithOther?" true)
    (else
      (`BlackboardComponent.SetValueAsBool` (`AIBlueprintHelperLibrary.GetBlackboard` (`AIBlueprintHelperLibrary.GetAIController` self)) "CanTalkWithOther?" false))))

(event `self.PawnSensing.OnSeePawn`
  (params (Pawn :type "Pawn Object Reference"))
  ;[1 0 0.9698] Player Detection
  (cast `/Game/IA_System/BP_FPSAISystem` Pawn)
  (`BlackboardComponent.SetValueAsBool` (`AIBlueprintHelperLibrary.GetBlackboard` (`AIBlueprintHelperLibrary.GetAIController` self)) "hasSeenPlayer?" true))

(event `self.Talkingsphere.OnComponentBeginOverlap`
  (params (OverlappedComponent :type "PrimitiveComponent Object Reference") (OtherActor :type "Actor Object Reference") (OtherComp :type "PrimitiveComponent Object Reference") (OtherBodyIndex :type Integer) (bFromSweep :type Boolean) (SweepResult :type "HitResult Structure (by ref)"))
  (if (!= OtherActor self)
    _))

(event `StartConvo`
  (params (`Other AI` :type "/Game/IA_System/01_Coworker_RD/BP_EnemyAI_Coworker_RD Object Reference"))
  (`MovementComponent.StopMovementImmediately` (`self.CharacterMovement`))
  (`ActorComponent.Deactivate` (`self.Talkingsphere`))
  (`self.K2_SetActorRotation` (`KismetMathLibrary.FindLookAtRotation` (`self.K2_GetActorLocation`) (`self.K2_GetActorLocation` `Other AI`))))

(event `EndConvo`
  (`ActorComponent.Activate` (`self.Talkingsphere`) false))

(fn `SetVariables`
  (bind _returnvalue (`|GetDataTableRow` "/Game/IA_System/DT_EnemyAI.DT_EnemyAI" "Accountant")
    (:`then`
      (bind (_walkspeed _runspeed _health _damages _talkingtime) (break `/Game/IA_System/S_EnemyAI` _returnvalue))
      (set `self.WalkSpeed` _walkspeed)
      (set `self.RunSpeed` _runspeed)
      (set `self.Health` _health)
      (set `self.Damages` _damages)
      (set `self.TalkingTime` _talkingtime))))

(fn `UserConstructionScript`)