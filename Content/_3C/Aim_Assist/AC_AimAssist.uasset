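; Aim-assist component that computes a corrected crosshair screen position, using zone radii from S_CombatFeel.
; A 60 Hz timer sphere-traces pawns from screen center and picks the hit closest to center in screen space.
; Within the bend zone, BPI_Damageable targets can snap to weak or base spots; others snap or bend proportionally toward the hit.
; GetCrosshairLocation exposes the result, optionally mirrored to a debug HUD; the magnetic zone only sets state.
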(event `self.ReceiveBeginPlay`
  (bind _returnvalue (`GameplayStatics.GetPlayerController` 0))
  (bind _debug_hud_ref (`self.Debug HUD Ref`))
  (bind ((`AimAssistSearchRadius_39_51EBD4B4489622AE1A441A9EFC22E1C7` _aimassistsearchradius) (`AimAssistStartOffset_41_220F1AFC4308764AD64EA8AD97383D4B` _aimassiststartoffset) (`AimAssistRange_43_0EA751BC40CC14F469D3E19C992B85CB` _aimassistrange) (`AimHeadshotRadius_52_A03BCE474CDCC6FFE8DF9A9D2FD79129` _aimheadshotradius) (`AimBaseShotRadius_49_D7106A6346AA900AB812B5AD21F65FC1` _aimbaseshotradius) (`AimBendZoneRadius_46_B059DA824AE278AC7185949816F54A82` _aimbendzoneradius) (`AimMagneticRadius_54_25D6227840BC9E9FE64A5C8535ECD312` _aimmagneticradius)) (break `/Game/_3C/Data_3C/S_CombatFeel` (`self.Combat Feel Struct Ref`)))
  (bind ((`AimHeadshotRadius_52_A03BCE474CDCC6FFE8DF9A9D2FD79129` _aimheadshotradius_2) (`AimBaseShotRadius_49_D7106A6346AA900AB812B5AD21F65FC1` _aimbaseshotradius_2) (`AimBendZoneRadius_46_B059DA824AE278AC7185949816F54A82` _aimbendzoneradius_2) (`AimMagneticRadius_54_25D6227840BC9E9FE64A5C8535ECD312` _aimmagneticradius_2)) (break `/Game/_3C/Data_3C/S_CombatFeel` (`self.Combat Feel Struct Ref`)))
  (`|ExecutionSequence`
    (:`then_0`
      (set `self.Debug Active ?` (`.DebugActive?_56_EC1916A14429D29BD4C219926B4A9B00` (break `/Game/_3C/Data_3C/S_CombatFeel` (`self.Combat Feel Struct Ref`))))
      (if (`self.Debug Active ?`)
        (`PlayerController.ClientSetHUD` _returnvalue "/Game/_3C/FPS_Hud/BPH_AimingSys_Debug.BPH_AimingSys_Debug_C")
        (set `self.Debug HUD Ref` (cast `/Game/_3C/FPS_Hud/BPH_AimingSys_Debug` (`PlayerController.GetHUD` _returnvalue) :!pure true))
        (set `/Game/_3C/FPS_Hud/BPH_AimingSys_Debug.Headshot Zone Radius` _aimheadshotradius_2 _debug_hud_ref)
        (set `/Game/_3C/FPS_Hud/BPH_AimingSys_Debug.Base Shot Zone Radius` _aimbaseshotradius_2 _debug_hud_ref)
        (set `/Game/_3C/FPS_Hud/BPH_AimingSys_Debug.Bend Zone Radius` _aimbendzoneradius_2 _debug_hud_ref)
        (set `/Game/_3C/FPS_Hud/BPH_AimingSys_Debug.Magnetic Zone Radius` _aimmagneticradius_2 _debug_hud_ref)))
    (:`then_1`
      ;[0.75 0.75 0.75 0.75] Settings from Struct "S_CombatFeel"
      (set `self.Search Trace Sphere Radius` _aimassistsearchradius)
      (set `self.Search Trace Start Offset` _aimassiststartoffset)
      (set `self.Search Trace Range` _aimassistrange)
      (set `self.Aim Bend Zone Radius` _aimbendzoneradius)
      (set `self.Aim Base Shot Radius` _aimbaseshotradius)
      (set `self.Aim Headshot Radius` _aimheadshotradius)
      (set `self.Aim Magnetic Radius` _aimmagneticradius))
    (:`then_2`
      (`KismetSystemLibrary.K2_SetTimerDelegate` (delegate `Execute System`) 0.016667 true) ; Time(60 FPS) = 1/60 = 0.016667\nor (30 FPS) = 1/30 = 0.033333
    )))

(event `Execute System`
  (bind (_was_pawn_found _pawn_screen_location _pdoesimplementinterface _base_spot_screen_location _weak_spot_screen_location) (`self.Pawn Search`))
  (bind _adjustedposition (`self.Set Crosshair Screen Location` _was_pawn_found _pawn_screen_location _pdoesimplementinterface _base_spot_screen_location _weak_spot_screen_location))
  (set `self.Croshair Screen Location` _adjustedposition)
  (if (`self.Debug Active ?`)
    (set `/Game/_3C/FPS_Hud/BPH_AimingSys_Debug.Main Crosshair Location` (`self.Croshair Screen Location`) (`self.Debug HUD Ref`))))

(fn `Get Crosshair Location`
  (returns (`Croshair Screen Location` :type "Vector2D Structure"))
  (return (`self.Croshair Screen Location`)))

(fn `Pawn Search`
  (returns (`Was Pawn Found` :type Boolean) (`Pawn Screen Location` :type "Vector2D Structure") (pDoesImplementInterface :type Boolean) (`Base spot Screen Location` :type "Vector2D Structure") (`Weak spot Screen Location` :type "Vector2D Structure"))
  (locals (`L Engaged Pawn Screen Loc` :type "Vector2D Structure") (`L Engaged Pawn` :type "Actor Object Reference"))
  (bind _l_engaged_pawn (`local.L Engaged Pawn`))
  (bind _l_engaged_pawn_screen_loc (`local.L Engaged Pawn Screen Loc`))
  (bind _returnvalue (`KismetSystemLibrary.DoesImplementInterface` (`local.L Engaged Pawn`) "/Game/_3C/BPI_Damageable.BPI_Damageable_C"))
  (bind (_worldposition _worlddirection) (`GameplayStatics.DeprojectScreenToWorld` (`GameplayStatics.GetPlayerController` 0) (* (`WidgetLayoutLibrary.GetViewportSize`) 0.5)))
  (bind (_bblockinghit _binitialoverlap _time _distance _location _impactpoint _normal _impactnormal _physmat _hitactor) (`GameplayStatics.BreakHitResult` (`|GetArrayItem` (`self.Hit Pawns`) (`KismetMathLibrary.MinOfFloatArray` (`self.Hit Pawns Distance to Center`)))))
  (bind (_outhits _returnvalue_2) (`KismetSystemLibrary.SphereTraceMultiForObjects` (+ _worldposition (* _worlddirection (`self.Search Trace Start Offset`))) (+ _worldposition (* _worlddirection (`self.Search Trace Range`))) (`self.Search Trace Sphere Radius`) (`|MakeArray` "ObjectTypeQuery3" :!type "EObjectTypeQuery Enum") false (`|MakeArray` (`GameplayStatics.GetPlayerPawn` 0) :!type "Actor Object Reference") "None" false))
  (set `self.Hit Pawns` _outhits)
  (if _returnvalue_2
    (for _array_element (`self.Hit Pawns`)
      (`KismetArrayLibrary.Array_Add` (`self.Hit Pawns Distance to Center`) (`KismetMathLibrary.Distance2D` (* (`WidgetLayoutLibrary.GetViewportSize`) 0.5) (`GameplayStatics.ProjectWorldToScreen` (`GameplayStatics.GetPlayerController` 0) (`.ImpactPoint` (`GameplayStatics.BreakHitResult` _array_element))))))
    (set `local.L Engaged Pawn Screen Loc` (`GameplayStatics.ProjectWorldToScreen` (`GameplayStatics.GetPlayerController` 0) _impactpoint))
    (set `local.L Engaged Pawn` _hitactor)
    (if _returnvalue
      (bind _screen_location (message `/Game/_3C/BPI_Damageable.Get Weak Spot Screen Loc` _l_engaged_pawn))
      (bind _screen_location_2 (message `/Game/_3C/BPI_Damageable.Get Base Spot Screen Loc` _l_engaged_pawn))
      (return true _l_engaged_pawn_screen_loc _returnvalue _screen_location_2 _screen_location)
      (else
        (return true _l_engaged_pawn_screen_loc _returnvalue (0.0 0.0) (0.0 0.0))))
    (else
      (return false (-1.0 -1.0) false (0.0 0.0) (0.0 0.0)))))

(fn `Set Crosshair Screen Location`
  (params (`bPaw Found` :type Boolean) (InLocation :type "Vector2D Structure") (bDoesImplementInterface :type Boolean) (BaseSpotLocation :type "Vector2D Structure") (WeakSpotLocation :type "Vector2D Structure"))
  (returns (AdjustedPosition :type "Vector2D Structure"))
  (locals (`L Pawn In Location` :type "Vector2D Structure") (`L Viewport Center Location` :type "Vector2D Structure") (`L Pawn Distance to Center` :type "Float (double-precision)") (`L Pawn Found` :type Boolean :default false) (`L Does Implement Interface` :type Boolean) (`L Base Spot Location` :type "Vector2D Structure") (`L Weak Spot Location` :type "Vector2D Structure"))
  (bind _returnvalue (/ (`WidgetLayoutLibrary.GetViewportSize`) 2.0))
  (set `local.L Pawn Found` `bPaw Found`)
  (set `local.L Does Implement Interface` bDoesImplementInterface)
  (set `local.L Base Spot Location` BaseSpotLocation)
  (set `local.L Weak Spot Location` WeakSpotLocation)
  (bind _output_get (set `local.L Pawn In Location` InLocation))
  (set `local.L Viewport Center Location` _returnvalue)
  (set `local.L Pawn Distance to Center` (`KismetMathLibrary.Distance2D` _output_get _returnvalue))
  (if (and (`local.L Pawn Found`) (<= (`local.L Pawn Distance to Center`) (`self.Aim Bend Zone Radius`)))
    (if (`local.L Does Implement Interface`)
      (if (<= (`KismetMathLibrary.Distance2D` (`local.L Weak Spot Location`) (`local.L Viewport Center Location`)) (`self.Aim Headshot Radius`))
        (set `self.Current State` "NewEnumerator5")
        (return (`local.L Weak Spot Location`))
        (elif (<= (`KismetMathLibrary.Distance2D` (`local.L Base Spot Location`) (`local.L Viewport Center Location`)) (`self.Aim Base Shot Radius`))
          (set `self.Current State` "NewEnumerator4")
          (return (`local.L Base Spot Location`))
          (else
            (`KismetSystemLibrary.PrintString` "False" true true (struct :`R` 1.0 :`A` 1.0)))))
      (else
        (set `self.Current State` "NewEnumerator0")
        (if (<= (`local.L Pawn Distance to Center`) (`self.Aim Base Shot Radius`))
          (set `self.Current State` "NewEnumerator3")
          (return (`local.L Pawn In Location`))
          (else
            (set `self.Current State` "NewEnumerator2")
            (return (+ (`local.L Viewport Center Location`) (* (`KismetMathLibrary.Normal2D` (- (`local.L Pawn In Location`) (`local.L Viewport Center Location`))) (/ (* (`self.Aim Base Shot Radius`) (- (`self.Aim Bend Zone Radius`) (`local.L Pawn Distance to Center`))) (- (`self.Aim Bend Zone Radius`) (`self.Aim Base Shot Radius`))))))))))
    (else
      (set `self.Current State` (select `bool` (<= (`local.L Pawn Distance to Center`) (`self.Aim Magnetic Radius`)) :`false` "NewEnumerator0" :`true` "NewEnumerator1" :!type "/Game/_3C/E_AimingSys_State Enum"))
      (return (`local.L Viewport Center Location`)))))