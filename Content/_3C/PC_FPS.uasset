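; First-person player controller that adds the FPS input context and drives movement, look and a quick 180 turn on the BP_FPS pawn.
; BeginPlay copies FOV, pitch limits, sensitivity, inversion and tilt settings from a camera-feel struct.
; Strafe and look input feed a roll tilt that Tick decays, clamps and applies to the camera.
; A timeline lerps the turn; shoot, interact, throw, kick and ultimate inputs are empty stubs.
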(event `EnhancedInput|/Game/_3C/Inputs/Actions/IA_Shoot`
  (params (ActionValue :type Boolean) (ElapsedSeconds :type "Float (double-precision)") (TriggeredSeconds :type "Float (double-precision)") (InputAction :type "InputAction Object Reference" :default "/Game/_3C/Inputs/Actions/IA_Shoot.IA_Shoot")))

(event `EnhancedInput|/Game/_3C/Inputs/Actions/IA_Interact`
  (params (ActionValue :type Boolean) (ElapsedSeconds :type "Float (double-precision)") (TriggeredSeconds :type "Float (double-precision)") (InputAction :type "InputAction Object Reference" :default "/Game/_3C/Inputs/Actions/IA_Interact.IA_Interact")))

(event `EnhancedInput|/Game/_3C/Inputs/Actions/IA_Throw`
  (params (ActionValue :type Boolean) (ElapsedSeconds :type "Float (double-precision)") (TriggeredSeconds :type "Float (double-precision)") (InputAction :type "InputAction Object Reference" :default "/Game/_3C/Inputs/Actions/IA_Throw.IA_Throw")))

(event `EnhancedInput|/Game/_3C/Inputs/Actions/IA_Kick`
  (params (ActionValue :type Boolean) (ElapsedSeconds :type "Float (double-precision)") (TriggeredSeconds :type "Float (double-precision)") (InputAction :type "InputAction Object Reference" :default "/Game/_3C/Inputs/Actions/IA_Kick.IA_Kick")))

(event `EnhancedInput|/Game/_3C/Inputs/Actions/IA_Ultimate`
  (params (ActionValue :type Boolean) (ElapsedSeconds :type "Float (double-precision)") (TriggeredSeconds :type "Float (double-precision)") (InputAction :type "InputAction Object Reference" :default "/Game/_3C/Inputs/Actions/IA_Ultimate.IA_Ultimate")))

(event `self.ReceiveTick`
  (params (DeltaSeconds :type "Float (single-precision)"))
  (`self.Head Tilt` DeltaSeconds))

(event `self.ReceiveBeginPlay`
  (bind _returnvalue (`GameplayStatics.GetPlayerCameraManager` 0))
  (bind ((`TitRecoverySpeed_41_B0EAD35C44C2B8DC530A72B308D0893B` _titrecoveryspeed) (`MaxTilt_40_48D4C2F74564D063DEBC7ABA5BB316FE` _maxtilt)) (break `/Game/_3C/Data_3C/S_FPSCameraFeel` (`self.Camera Feel Structure Ref`)))
  (bind ((`InvertCam_28_90E7021E4B9690B321581A938CF1278B` _invertcam) (`ViewPitchMin_34_1401A7A94B9759766D93A8BF0EDF6337` _viewpitchmin) (`ViewPitchMax_35_D2DEF8154FD9D617C127778BFC7FEC8E` _viewpitchmax)) (break `/Game/_3C/Data_3C/S_FPSCameraFeel` (`self.Camera Feel Structure Ref`)))
  (bind ((`HorizontalCamSpeed_48_BCC115954F2DC5CE029858B577AE2287` _horizontalcamspeed) (`VerticalCamSpeed_47_BDA38A3643667DFE78A0778FF1A6268E` _verticalcamspeed) (`TiltClamp_51_1A1E3FEB4354BFAA12EEA98BBA7D8D3B` _tiltclamp)) (break `/Game/_3C/Data_3C/S_FPSCameraFeel` (`self.Camera Feel Structure Ref`)))
  (bind _asbp_fps (cast `/Game/_3C/BP_FPS` (`GameplayStatics.GetPlayerPawn` 0) :!pure true))
  ;[0.5 0.5 1 0.75] Add IMC
  (`EnhancedInputSubsystemInterface.AddMappingContext` (subsystem `EnhancedInputLocalPlayerSubsystem`) "/Game/_3C/Inputs/IMC_FPS.IMC_FPS" 0 (struct))
  ;[0.005 0.005 0.005 0.75] Clamp Camera
  (set `PlayerCameraManager.ViewPitchMin` _viewpitchmin _returnvalue)
  (set `PlayerCameraManager.ViewPitchMax` _viewpitchmax _returnvalue)
  ;[0.25 0.25 0.25 0.75] Camera Settings from Struct ("S_FPSCameraFeel")
  (set `self.Inverted Cam` _invertcam)
  (`CameraComponent.SetFieldOfView` (`/Game/_3C/BP_FPS.Camera` _asbp_fps) (`.FOV_5_3BBB83674770A4A3F1B4E99A3A546ABD` (break `/Game/_3C/Data_3C/S_FPSCameraFeel` (`self.Camera Feel Structure Ref`))))
  (set `self.Player Ref` _asbp_fps)
  (set `self.Tilt Recover Speed` _titrecoveryspeed)
  (set `self.Max Tilt` _maxtilt)
  ;[0.25 0.25 0.25 0.75] Camera Speed
  (set `self.Horizontal Cam Speed` _horizontalcamspeed)
  (set `self.Vertical Cam Speed` _verticalcamspeed)
  (set `self.Tilt Clamp` _tiltclamp))

(event `EnhancedInput|/Game/_3C/Inputs/Actions/IA_Move`
  (params (ActionValue :type "Vector2D Structure") (ElapsedSeconds :type "Float (double-precision)") (TriggeredSeconds :type "Float (double-precision)") (InputAction :type "InputAction Object Reference" :default "/Game/_3C/Inputs/Actions/IA_Move.IA_Move"))
  (bind _returnvalue (`self.K2_GetPawn`))
  (bind _returnvalue_2 (`self.GetControlRotation`))
  (bind (_returnvalue_x _returnvalue_y) (`KismetMathLibrary.BreakVector` (`KismetMathLibrary.GetForwardVector` _returnvalue_2)))
  ;[0.5 0.5 0.5] Basic Movement
  ;;[1 0 0] Movement
  (:`Triggered`
    (`Pawn.AddMovementInput` _returnvalue (`KismetMathLibrary.Normal` (`KismetMathLibrary.MakeVector` _returnvalue_x _returnvalue_y)) ActionValue_X false) ; Forward
    (`Pawn.AddMovementInput` _returnvalue (`KismetMathLibrary.GetRightVector` _returnvalue_2) ActionValue_Y false) ; Right
    ;;[0.65 0 0.65] Camera Tilt (For Movement)
    (set `self.Tilt` (+ (* ActionValue_Y (* (`self.Tilt Recover Speed`) 0.05)) (`self.Tilt`)))))

(event `Head Tilt`
  (params (`Delta Time` :type "Float (double-precision)"))
  (bind _player_ref (`self.Player Ref`))
  (bind _tilt (`self.Tilt`))
  (bind _tilt_clamp (`self.Tilt Clamp`))
  (bind _camera (`/Game/_3C/BP_FPS.Camera` _player_ref))
  (bind _returnvalue (- _tilt (* _tilt (`self.Tilt Recover Speed`) `Delta Time`)))
  ;[0.75 0.45 0.15] Head Tilt (Event Tick)
  (`/Engine/EditorBlueprintResources/StandardMacros.IsValid` _player_ref
    (:`Is Valid`
      (set `self.Tilt` (select `bool` (< _returnvalue 0.0) :`false` (`KismetMathLibrary.FClamp` _returnvalue _tilt_clamp (`self.Max Tilt`)) :`true` (`KismetMathLibrary.FClamp` _returnvalue (* (`self.Max Tilt`) -1.0) _tilt_clamp)))
      (`SceneComponent.K2_SetWorldRotation` _camera (`self.GetControlRotation`) false false)
      (`SceneComponent.K2_AddRelativeRotation` _camera (`KismetMathLibrary.MakeRotator` (`self.Tilt`)) false false))))

(event `EnhancedInput|/Game/_3C/Inputs/Actions/IA_180Turn`
  (params (ActionValue :type Boolean) (ElapsedSeconds :type "Float (double-precision)") (TriggeredSeconds :type "Float (double-precision)") (InputAction :type "InputAction Object Reference" :default "/Game/_3C/Inputs/Actions/IA_180Turn.IA_180Turn"))
  (bind (_returnvalue_roll _returnvalue_pitch _returnvalue_yaw) (`KismetMathLibrary.BreakRotator` (`self.GetControlRotation`)))
  (bind _180_rotation (`self.180_Rotation`))
  ;[0.2 1 0.2] 180 Rotation
  (:`Triggered`
    (`MovementComponent.StopMovementImmediately` (`Character.CharacterMovement` (`self.Player Ref`)))
    (bind _output_get (set `self.Temp Rota` (select `bool` (< _returnvalue_yaw 0.0) :`false` (`KismetMathLibrary.MakeRotator` _returnvalue_roll _returnvalue_pitch (+ _returnvalue_yaw _180_rotation)) :`true` (`KismetMathLibrary.MakeRotator` _returnvalue_roll _returnvalue_pitch (+ _returnvalue_yaw (* _180_rotation -1.0))))))
    (bind (_direction _rota_speed) (`Timeline|180 Rotation Speed Timeline` :!via `PlayFromStart`)
      (:`Update`
        (`self.SetControlRotation` (`KismetMathLibrary.RLerp` (`self.GetControlRotation`) _output_get _rota_speed true))))))

(event `EnhancedInput|/Game/_3C/Inputs/Actions/IA_Look`
  (params (ActionValue :type "Vector2D Structure") (ElapsedSeconds :type "Float (double-precision)") (TriggeredSeconds :type "Float (double-precision)") (InputAction :type "InputAction Object Reference" :default "/Game/_3C/Inputs/Actions/IA_Look.IA_Look"))
  (bind _tilt_clamp (`self.Tilt Clamp`))
  (bind _returnvalue (* ActionValue_Y (`self.Vertical Cam Speed`)))
  ;[0.5 0.5 0.5] Basic Movement
  ;;[0.025 0.65 1] Look
  (:`Triggered`
    (`self.AddYawInput` (* ActionValue_X (`self.Horizontal Cam Speed`))) ; Roll on X
    (if (`self.Inverted Cam`)
      (`self.AddPitchInput` _returnvalue) ; Roll on Y
      (else
        (`self.AddPitchInput` (* _returnvalue -1.0)) ; Invert Roll on Y
      ))
    ;;[0.65 0 0.65] Camera Tilt (For Look)
    (if (or (< ActionValue_X (* _tilt_clamp -1.0)) (> ActionValue_X _tilt_clamp))
      (set `self.Tilt` (+ ActionValue_X (* (`self.Tilt`) 1.25)))
      (else
        (set `self.Tilt` 0.0)))))

(fn `UserConstructionScript`)