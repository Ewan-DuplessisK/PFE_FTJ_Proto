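; First-person player character systems: life with invincibility time, dash, kick, weapon pickup and drop, and a grab-escape QTE.
; BeginPlay creates the life, QTE and ammo widgets, caches movement defaults and starts a looping timer that selects an overlapping weapon for pickup.
; Timelines drive the kick placeholder and the dash, which overrides movement, shifts FOV and launches physics props.
; The QTE swaps input mapping contexts, counts presses on one cached enemy, then launches it backward.
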(event `self.ReceiveBeginPlay`
  (bind _playerfeel (`self.PlayerFeel`))
  (bind _charactermovement (`self.CharacterMovement`))
  (bind ((`dashRate` _dashrate) (`dashDistance` _dashdistance)) (break `UPlayerFeel` _playerfeel))
  (`|ExecutionSequence`
    (:`then_0`
      ;[0.025 0.75 0.75] Structure ("S_PlayerFeel")
      (`self.InitializeVarsWithPlayerFeelStruct`)
      ;[0.15 0.15 0.15] Life Init
      (bind _returnvalue (`|CreateWidget` "/Game/UI/W_PlayerLife.W_PlayerLife_C"))
      (bind _output_get (set `self.PlayerLifeWidget` _returnvalue))
      (`UserWidget.AddToViewport` _output_get 0)
      (set `self.PlayerLife Current` (`self.PlayerLife Max`)))
    (:`then_1`
      ;[0.03784 0.15 0.1151 0.5] Add QTE Widget
      (bind _returnvalue_2 (`|CreateWidget` "/Game/UI/W_QTE.W_QTE_C"))
      (bind _output_get_2 (set `self.W_QTE` _returnvalue_2))
      (`UserWidget.AddToViewport` _output_get_2 0)
      (`Widget.SetVisibility` _output_get_2 "Hidden"))
    (:`then_2`
      (bind _returnvalue_3 (`GameplayStatics.GetActorOfClass` "/Game/IA_System/BP_AIManager.BP_AIManager_C"))
      (set `self.AI Manager` _returnvalue_3))
    (:`then_3`
      (`KismetSystemLibrary.K2_SetTimerDelegate` (delegate `EClosestOverlap`) 0.2 true true))
    (:`then_4`
      (`KismetSystemLibrary.Delay` 0.2)
      (set `self.Max Walk Speed` (`CharacterMovementComponent.MaxWalkSpeed` _charactermovement))
      (set `self.Max Acceleration` (`CharacterMovementComponent.MaxAcceleration` _charactermovement))
      (set `self.Rotation Rate` (`CharacterMovementComponent.RotationRate` _charactermovement))
      (`TimelineComponent.SetPlayRate` (`self.Dash_TM`) _dashrate)
      (setmembers `UPlayerFeel` :`StructRef` _playerfeel :`dashSpeed` (* _dashrate _dashdistance)))
    (:`then_5`
      (bind _returnvalue_4 (`GameplayStatics.GetActorOfClass` "/Game/IA_System/01_Coworker_RD/BP_EnemyAI.BP_EnemyAI_C"))
      (set `self.EnemyRef` _returnvalue_4))
    (:`then_6`
      (bind _returnvalue_5 (`|CreateWidget` "/Game/UI/W_Ammo.W_Ammo_C"))
      (bind _output_get_3 (set `self.AmmoWidgetRef` _returnvalue_5))
      (`UserWidget.AddToViewport` _output_get_3 0)
      (`Widget.SetVisibility` _output_get_3 "Hidden"))))

(event `self.KickFeedback`
  (params (Location :type "Vector Structure") (HitEnemy :type "Enemy_Base Object Reference"))
  (bind _returnvalue (`GameplayStatics.GetPlayerController` 0))
  (bind (_returnvalue_roll _returnvalue_pitch) (`KismetMathLibrary.BreakRotator` (`SceneComponent.K2_GetComponentRotation` (`self.FirstPersonCameraComponent`))))
  ; KickAnim
  (`PlayerController.K2_ClientPlayForceFeedback` _returnvalue "/Game/FeedBack/FFB_Kcik.FFB_Kcik" "None" false false false)
  (`PlayerController.ClientStartCameraShake` :`self` _returnvalue :`Shake` "/Game/FeedBack/BP_Camera_Shake.BP_Camera_Shake_C")
  (`/Engine/EditorBlueprintResources/StandardMacros.IsValid` HitEnemy
    (:`Is Valid`
      (`/Game/IA_System/01_Coworker_RD/BP_EnemyAI.Damage_Feedback` (cast `/Game/IA_System/01_Coworker_RD/BP_EnemyAI` HitEnemy :!pure true)))
    (:`Is Not Valid`
      _))
  (`TimelineComponent.SetPlayRate` (`self.KickTime`) (/ 1.0 (`self.KickAnimDuration`)))
  (`KismetSystemLibrary.DelayUntilNextTick`)
  (bind (_direction _kicklengthtransi _kickrotatransi) (`Timeline|KickTime` :!via `PlayFromStart`)
    (:`Update`
      (`SceneComponent.SetRelativeScale3D` (`self.PlaceholderKick`) (`KismetMathLibrary.MakeVector` 1.0 1.0 (`KismetMathLibrary.Lerp` 1.0 (/ (`KismetMathLibrary.Vector_Distance` Location (`self.K2_GetActorLocation`)) 95.0) _kicklengthtransi)))
      (bind _result (`/Engine/EditorBlueprintResources/StandardMacros.NegateFloat` (`KismetMathLibrary.Lerp` 0.0 (+ _returnvalue_pitch 100.0) _kickrotatransi))
        (:`  `
          (`SceneComponent.K2_SetRelativeRotation` (`self.PlaceholderKick`) (`KismetMathLibrary.MakeRotator` _result 0.0 -90.0) false false))))))

(event `EnhancedInput|/Game/_GameManager/Inputs/Actions/IA_QTE`
  (params (ActionValue :type Boolean) (ElapsedSeconds :type "Float (double-precision)") (TriggeredSeconds :type "Float (double-precision)") (InputAction :type "InputAction Object Reference" :default "/Game/_GameManager/Inputs/Actions/IA_QTE.IA_QTE"))
  ;[0 0 1] QTE
  (:`Triggered`
    (`self.QTE_Current`)))

(event `EClosestOverlap`
  (bind _overlaping (`self.Overlaping`))
  (bind _firstpersoncameracomponent (`self.FirstPersonCameraComponent`))
  (bind _returnvalue (+ (`SceneComponent.K2_GetComponentLocation` _firstpersoncameracomponent) (* (`SceneComponent.GetForwardVector` _firstpersoncameracomponent) 50.0)))
  (if (`KismetArrayLibrary.Array_IsNotEmpty` (`self.Overlaping`))
    (set `self.ClosestWeapon` (`|GetArrayItem` _overlaping))
    (for _index (range 1 (`KismetArrayLibrary.Array_Length` _overlaping))
      (bind _output (`|GetArrayItem` (`self.Overlaping`) _index))
      (if (< (`KismetMathLibrary.Vector_Distance` (`self.K2_GetActorLocation` _output) _returnvalue) (`KismetMathLibrary.Vector_Distance` (`self.K2_GetActorLocation`) _returnvalue))
        (set `self.ClosestWeapon` _output)))
    (else
      (set `self.ClosestWeapon` null))))

(event `Check Current Life`
  (bind _hurt (`self.Hurt`))
  ;[0.05925 0.1455 0.15 0.5] Damages & Invincibility Time
  (if (<= (`self.PlayerLife Current`) 40.0) :!label _label
    (set `PostProcessComponent.BlendWeight` 1.0 _hurt)
    (else
      (set `PostProcessComponent.BlendWeight` 0.0 _hurt))))

(event `Damages`
  (params (Damages :type Integer) (`Invincibility Time` :type "Float (double-precision)"))
  ;[0.05925 0.1455 0.15 0.5] Damages & Invincibility Time
  (if (> (`self.Invincibility Time`) 0.0)
    (`KismetSystemLibrary.PrintString` "Player Can't Take Damages" true true (struct :`R` 1.0 :`G` 0.3889 :`A` 1.0))
    (else
      (set `self.PlayerLife Current` (- (`self.PlayerLife Current`) Damages))
      (set `self.Invincibility Time` `Invincibility Time`)
      (goto _label))))

(event `PickupWeapon`
  (bind _ammowidgetref (`self.AmmoWidgetRef`))
  (`self.HeldWeapon`
    (:`then`)
    (:`else`
      (bind _closestweapon (`self.ClosestWeapon`)
        (:`then`
          (`/Game/WeaponsGTP/BP_WeaponBase.OnPickup` _closestweapon)
          (`KismetSystemLibrary.DelayUntilNextTick`)
          (`/Game/UI/W_Ammo.SetCurrentAmmo` _ammowidgetref (`/Game/WeaponsGTP/BP_WeaponBase.Ammo/Durability` (`self.HeldWeapon`)))
          (`/Game/UI/W_Ammo.SetMaxAmmo` _ammowidgetref)
          (`/Game/UI/W_Ammo.SetWeaponCategory` _ammowidgetref)
          (`/Game/UI/W_Ammo.SetName` _ammowidgetref)
          (`Widget.SetVisibility` _ammowidgetref "Visible"))
        (:`else`)))))

(event `self.ReceiveTick`
  (params (DeltaSeconds :type "Float (single-precision)"))
  ;[0.05925 0.1455 0.15 0.5] Damages & Invincibility Time
  (if (> (`self.Invincibility Time`) 0.0)
    (set `self.Invincibility Time` (- (`self.Invincibility Time`) DeltaSeconds))))

(event `Heal`
  (bind _healing (`self.Healing`))
  (set `PostProcessComponent.BlendWeight` 1.0 _healing)
  (`self.Check Current Life`)
  (`KismetSystemLibrary.Delay` 1.0)
  (set `PostProcessComponent.BlendWeight` 0.0 _healing))

(event `DropWeapon`
  (bind _heldweapon (`self.HeldWeapon`)
    (:`then`
      (`/Game/WeaponsGTP/BP_WeaponBase.OnDrop` _heldweapon)
      (`Widget.SetVisibility` (`self.AmmoWidgetRef`) "Hidden"))
    (:`else`)))

(event `self.Capsule.OnComponentBeginOverlap`
  (params (OverlappedComponent :type "PrimitiveComponent Object Reference") (OtherActor :type "Actor Object Reference") (OtherComp :type "PrimitiveComponent Object Reference") (OtherBodyIndex :type Integer) (bFromSweep :type Boolean) (SweepResult :type "HitResult Structure (by ref)"))
  (if (`self.isDashing`)
    (bind _asphysics_props (cast `Physics_Props` OtherActor))
    (`Physics_Props.Launched` _asphysics_props (`self.GetVelocity`))))

(event `PlayerDash`
  (params (`World Direction` :type "Vector Structure"))
  (bind ((`FOVBase` _fovbase) (`FOVTarget` _fovtarget)) (break `UCameraFeel` (`Player_Controller.CameraFeel` (cast `/Game/_GameManager/PC_Systems` (`GameplayStatics.GetPlayerController` 0) :!pure true))))
  ;[1 0 0.5] Dash
  (if (`self.bCanDash`)
    (`self.Set Speed/Accel/Rota` (`.dashSpeed` (break `UPlayerFeel` (`self.PlayerFeel`))) 100000000.0 (struct :`Yaw` 100000000.0))
    (`KismetSystemLibrary.DelayUntilNextTick`)
    (`self.DisableInput` (`GameplayStatics.GetPlayerController` 0))
    (bind (_direction _dash_curve) (`Timeline|Dash_TM` :!via `PlayFromStart`)
      (:`Update`
        (`self.AddMovementInput` `World Direction`)
        (set `self.bCanDash` false)
        (set `self.isDashing` true)
        (`CameraComponent.SetFieldOfView` (`self.FirstPersonCameraComponent`) (`KismetMathLibrary.Lerp` _fovbase _fovtarget _dash_curve)))
      (:`Finished`
        (`self.Set Speed/Accel/Rota` (`self.Max Walk Speed`) (`self.Max Acceleration`) (`self.Rotation Rate`))
        (set `self.isDashing` false)
        (`MovementComponent.StopMovementImmediately` (`self.CharacterMovement`))
        (`self.EnableInput` (`GameplayStatics.GetPlayerController` 0))
        (`KismetSystemLibrary.Delay` (`.delayBetweenTwoDash` (break `UPlayerFeel` (`self.PlayerFeel`))))
        (set `self.bCanDash` true)))))

(fn `QTE End`
  (bind _as_bp_enemy_ai_coworker_rd (`self.As BP Enemy AI Coworker RD`))
  (bind _as_bp_enemy_ai_coworker_rd_2 (`self.As BP Enemy AI Coworker RD`))
  (bind _returnvalue (pcsubsystem `EnhancedInputLocalPlayerSubsystem` (`GameplayStatics.GetPlayerController` 0)))
  (bind (_qte_launchvelocity_x _qte_launchvelocity_y _qte_launchvelocity_z) (`KismetMathLibrary.BreakVector` (`Enemy_Base.QTE_LaunchVelocity` _as_bp_enemy_ai_coworker_rd)))
  (bind (_returnvalue_x _returnvalue_y) (`KismetMathLibrary.BreakVector` (* _qte_launchvelocity_x (* (`self.GetActorForwardVector` (`self.As BP Enemy AI Coworker RD`)) -1.0))))
  (`KismetSystemLibrary.K2_PauseTimerHandle` (`/Game/IA_System/01_Coworker_RD/BP_EnemyAI.QTE Health Timer` _as_bp_enemy_ai_coworker_rd_2))
  (set `/Game/IA_System/01_Coworker_RD/BP_EnemyAI.QTE Current` 0.0 _as_bp_enemy_ai_coworker_rd_2)
  ;[1 1 1 0.5] Change IMC from QTE to Sysem
  (`EnhancedInputSubsystemInterface.RemoveMappingContext` _returnvalue "/Game/_GameManager/Inputs/IMC_QTE.IMC_QTE" (struct))
  (`EnhancedInputSubsystemInterface.AddMappingContext` _returnvalue "/Game/_GameManager/Inputs/IMC_Systems.IMC_Systems" 0 (struct))
  (`Widget.SetVisibility` (`self.W_QTE`) "Hidden")
  (`self.LaunchCharacter` _as_bp_enemy_ai_coworker_rd (`KismetMathLibrary.MakeVector` _returnvalue_x _returnvalue_y _qte_launchvelocity_z) false false) ; Push Player from the enemy who grabbed him
  (`/Engine/EditorBlueprintResources/StandardMacros.IsValid` self
    (:`Is Valid`
      (`/Game/IA_System/01_Coworker_RD/BP_EnemyAI.QTE End` (`self.As BP Enemy AI Coworker RD`)))))

(fn `QTE_Current`
  (bind _as_bp_enemy_ai_coworker_rd (`self.As BP Enemy AI Coworker RD`))
  (`KismetSystemLibrary.PrintString` "QTE Pressed")
  (set `/Game/IA_System/01_Coworker_RD/BP_EnemyAI.QTE Current` (+ (`/Game/IA_System/01_Coworker_RD/BP_EnemyAI.QTE Current` (`self.As BP Enemy AI Coworker RD`)) 1.25) (`self.As BP Enemy AI Coworker RD`))
  (if (>= (`/Game/IA_System/01_Coworker_RD/BP_EnemyAI.QTE Current` _as_bp_enemy_ai_coworker_rd) (`Enemy_Base.QTEInputRequired` _as_bp_enemy_ai_coworker_rd))
    (`self.QTE End`)))

(fn `Raycast Damage`
  (params (Range :type "Float (double-precision)") (Damage :type "Float (double-precision)"))
  (bind (_returnvalue_location _returnvalue_rotation) (`KismetMathLibrary.BreakTransform` (`SceneComponent.K2_GetComponentToWorld` (`self.FirstPersonCameraComponent`))))
  (bind _returnvalue (+ _returnvalue_location (0.0 0.0 -2.0)))
  (bind _outhit (`KismetSystemLibrary.LineTraceSingle` :`Start` _returnvalue :`End` (+ _returnvalue (* (`KismetMathLibrary.GetForwardVector` _returnvalue_rotation) Range)) :`TraceChannel` "TraceTypeQuery2" :`bTraceComplex` true :`DrawDebugType` "ForOneFrame"))
  (cast `Character` (`.HitActor` (`GameplayStatics.BreakHitResult` _outhit)))
  (`GameplayStatics.ApplyDamage` (`.HitActor` (`GameplayStatics.BreakHitResult` _outhit)) Damage)
  (`NiagaraFunctionLibrary.SpawnSystemAtLocation` "/Game/VFX/NS_KickPlaceholder.NS_KickPlaceholder" (`.Location` (`GameplayStatics.BreakHitResult` _outhit))))

(fn `Set Speed/Accel/Rota`
  (params (`Max Walk Speed` :type "Float (double-precision)") (`Max Acceleration` :type "Float (double-precision)") (`Rotation Rate` :type "Rotator Structure"))
  (bind _charactermovement (`self.CharacterMovement`))
  (set `CharacterMovementComponent.MaxWalkSpeed` `Max Walk Speed` _charactermovement)
  (set `CharacterMovementComponent.MaxAcceleration` `Max Acceleration` _charactermovement)
  (set `CharacterMovementComponent.RotationRate` `Rotation Rate` _charactermovement))

(fn `Switch Input Event_`
  (bind _returnvalue (pcsubsystem `EnhancedInputLocalPlayerSubsystem` (`GameplayStatics.GetPlayerController` 0)))
  (bind _asbp_enemy_ai (cast `/Game/IA_System/01_Coworker_RD/BP_EnemyAI` (`self.EnemyRef`)))
  (set `self.As BP Enemy AI Coworker RD` _asbp_enemy_ai)
  (`/Engine/EditorBlueprintResources/StandardMacros.IsValid` _returnvalue
    (:`Is Valid`
      (`/Engine/EditorBlueprintResources/StandardMacros.IsValid` (`self.As BP Enemy AI Coworker RD`)
        (:`Is Valid`
          ; Change IMC from System to QTE
          (`EnhancedInputSubsystemInterface.RemoveMappingContext` _returnvalue "/Game/_GameManager/Inputs/IMC_Systems.IMC_Systems" (struct))
          (`EnhancedInputSubsystemInterface.AddMappingContext` _returnvalue "/Game/_GameManager/Inputs/IMC_QTE.IMC_QTE" 0 (struct)))))))

(fn `UserConstructionScript`)