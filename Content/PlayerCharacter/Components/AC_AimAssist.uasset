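; Aim assist component for the player character; the graph shown here only drives its debug view.
; When AimFeel debug is active, BeginPlay swaps player 0's HUD to the debug HUD and caches it as BPH_AimingSys_Debug, printing status or failure.
; Tick then pushes the current crosshair location to that HUD every frame while debug stays active.
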(event `self.ReceiveBeginPlay`
  (bind _returnvalue (`GameplayStatics.GetPlayerController` 0))
  (bind ((`bIsDebugActive` _bisdebugactive)) (break `UAimAssistFeel` (`self.AimFeel`)))
  (`|ExecutionSequence`
    (:`then_0`
      (if _bisdebugactive
        (`PlayerController.ClientSetHUD` _returnvalue (`self.wAimDebugWidget`))
        (bind _asbph_aiming_sys_debug (cast `/Game/PlayerCharacter/AimAssist_Debug_Hud/BPH_AimingSys_Debug` (`PlayerController.GetHUD` _returnvalue))
          (:`then`
            (set `self.MyAimDebugMenu` _asbph_aiming_sys_debug)
            ;[0.15 1 0.15 0.5] Debug
            (`KismetSystemLibrary.PrintString` "Aim Debug Active" true true (struct :`G` 0.66 :`A` 1.0) 1.0))
          (:`CastFailed`
            (`KismetSystemLibrary.PrintString` "Aim Debug Failed" true true (struct :`R` 1.0 :`A` 1.0) 1.0)))))
    (:`then_1`
      (if _bisdebugactive
        (bind _myaimdebugmenu (`self.MyAimDebugMenu`)
          (:`then`
            (bind _asbph_aiming_sys_debug_2 (cast `/Game/PlayerCharacter/AimAssist_Debug_Hud/BPH_AimingSys_Debug` _myaimdebugmenu)
              (:`then`
                (set `self.BPH Aiming Sys Debug Ref` _asbph_aiming_sys_debug_2))
              (:`CastFailed`
                (`KismetSystemLibrary.PrintString` "Invalid BPH Ref in AC_AimAssist" true true (struct :`R` 1.0 :`A` 1.0) :!label _label))))
          (:`else`
            (goto _label)))))))

(event `self.ReceiveTick`
  (params (DeltaSeconds :type "Float (single-precision)"))
  ;[0 0.75 0.75] Aim Assist
  ;;[0.15 0.15 0.5] Debug View
  (if (`.bIsDebugActive` (break `UAimAssistFeel` (`self.AimFeel`)))
    (bind _returnvalue (`self.GetCrosshairLocation`))
    (set `/Game/PlayerCharacter/AimAssist_Debug_Hud/BPH_AimingSys_Debug.Main Crosshair Location` _returnvalue (`self.BPH Aiming Sys Debug Ref`))))