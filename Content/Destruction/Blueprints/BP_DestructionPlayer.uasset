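; BP_DestructionPlayer is the player pawn for the Destruction feature, handling movement and weapon firing.
; On BeginPlay it spawns a BP_DestructionWeapon and attaches it to itself.
; Enhanced Input move values drive movement along the actor's right and forward vectors.
; Its OnFired event forwards firing to the weapon's EventOnFired.
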(event `self.ReceiveBeginPlay`
  (bind _returnvalue (`|SpawnActorFromClass` "/Game/Destruction/Blueprints/BP_DestructionWeapon.BP_DestructionWeapon_C" (`KismetMathLibrary.MakeTransform` (0.0 0.0 0.0)) "Undefined" "MultiplyWithRoot" null null))
  (bind _output_get (set `self.Weapon` _returnvalue))
  (`self.K2_AttachToActor` _output_get self "None" "KeepRelative" "KeepRelative" "KeepRelative" true))

(event `Event OnFired`
  (`/Game/Destruction/Blueprints/BP_DestructionWeapon.Event OnFired` (`self.Weapon`)))

(event `EnhancedInput|/Game/Destruction/InputActions/IA_DestructionMove`
  (params (ActionValue :type "Vector2D Structure") (ElapsedSeconds :type "Float (double-precision)") (TriggeredSeconds :type "Float (double-precision)") (InputAction :type "InputAction Object Reference" :default "/Game/Destruction/InputActions/IA_DestructionMove.IA_DestructionMove"))
  (:`Triggered`
    (`self.AddMovementInput` (`self.GetActorRightVector`) ActionValue_X)
    (`self.AddMovementInput` (`self.GetActorForwardVector`) ActionValue_Y)))

(fn `UserConstructionScript`)