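; PC_Destruction is the player controller for the destruction mode, handling look and fire input through Enhanced Input.
; On BeginPlay it adds the IMC_Destruction mapping context and caches the controlled pawn as a BP_DestructionPlayer.
; The look action feeds yaw and pitch input on the controller, while the fire action forwards to the pawn's EventOnFired.
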(event `self.ReceiveBeginPlay`
  (`EnhancedInputSubsystemInterface.AddMappingContext` (subsystem `EnhancedInputLocalPlayerSubsystem`) "/Game/Destruction/_manager/IMC_Destruction.IMC_Destruction" 0 (struct))
  (bind _asbp_destruction_player (cast `/Game/Destruction/Blueprints/BP_DestructionPlayer` (`self.K2_GetPawn`)))
  (set `self.Actor` _asbp_destruction_player))

(event `EnhancedInput|/Game/Destruction/InputActions/IA_DestructionLook`
  (params (ActionValue :type "Vector2D Structure") (ElapsedSeconds :type "Float (double-precision)") (TriggeredSeconds :type "Float (double-precision)") (InputAction :type "InputAction Object Reference" :default "/Game/Destruction/InputActions/IA_DestructionLook.IA_DestructionLook"))
  (:`Triggered`
    (`self.AddYawInput` ActionValue_X)
    (`self.AddPitchInput` ActionValue_Y)))

(event `EnhancedInput|/Game/Destruction/InputActions/IA_DestructionFire`
  (params (ActionValue :type Boolean) (ElapsedSeconds :type "Float (double-precision)") (TriggeredSeconds :type "Float (double-precision)") (InputAction :type "InputAction Object Reference" :default "/Game/Destruction/InputActions/IA_DestructionFire.IA_DestructionFire"))
  (:`Triggered`
    (`/Game/Destruction/Blueprints/BP_DestructionPlayer.Event OnFired` (`self.Actor`))))

(fn `UserConstructionScript`)