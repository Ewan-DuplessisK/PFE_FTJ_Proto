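; Player character component that lets the player interact with nearby actors carrying an AC_Interactable.
; Owner overlap events maintain a list of interactables with passive highlights, and Tick actively highlights the one closest to a point just ahead of the owner.
; IA_I_Interact, from a mapping context added on BeginPlay, sends that nearest component an interact message; the follow-up handler only prints a debug string.
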(event `OnActorBeginOverlap_Event`
  (params (OverlappedActor :type "Actor Object Reference") (OtherActor :type "Actor Object Reference"))
  (bind _returnvalue (`Actor.GetComponentByClass` OtherActor "/Game/Usables_System/Interactable/AC_Interactable.AC_Interactable_C"))
  ; Bind Overlapping array to Actor's Overlap begin/end events
  (`/Engine/EditorBlueprintResources/StandardMacros.IsValid` _returnvalue
    (:`Is Valid`
      (if (`/Game/Usables_System/Interactable/AC_Interactable.Interactable?` _returnvalue)
        (`KismetArrayLibrary.Array_AddUnique` (`self.overlappings`) _returnvalue)
        (`/Game/Usables_System/Interactable/AC_Interactable.Highlight` _returnvalue true true)))))

(event `self.ReceiveBeginPlay`
  (bind _returnvalue (`self.GetOwner`))
  ; Add Map Ctx          To be removed, only IMC_Systems should be used, and it already has IA_Interact -Ewan
  ;; char
  (bind _ascharacter (cast `Character` (`self.GetOwner`)))
  (bind _output_get (set `self.сharacter` _ascharacter))
  ;; ctrl
  (bind _asplayer_controller (cast `PlayerController` (`Pawn.GetController` _output_get)))
  (bind _output_get_2 (set `self.playerController` _asplayer_controller))
  (bind _returnvalue_2 (pcsubsystem `EnhancedInputLocalPlayerSubsystem` _output_get_2))
  (`/Engine/EditorBlueprintResources/StandardMacros.IsValid` _returnvalue_2
    (:`Is Valid`
      (`EnhancedInputSubsystemInterface.AddMappingContext` _returnvalue_2 "/Game/Usables_System/Interactable/Inputs/IMC_Interact.IMC_Interact" 1 (struct))
      ; Bind Overlapping array to Actor's Overlap begin/end events
      (`|ExecutionSequence`
        (:`then_0`
          (add `Actor.OnActorBeginOverlap` _returnvalue (delegate `OnActorBeginOverlap_Event`)))
        (:`then_1`
          (add `Actor.OnActorEndOverlap` _returnvalue (delegate `OnActorEndOverlap_Event`)))))))

(event `EnhancedInput|/Game/Usables_System/Interactable/Inputs/IA_I_Interact`
  (params (ActionValue :type Boolean) (ElapsedSeconds :type "Float (double-precision)") (TriggeredSeconds :type "Float (double-precision)") (InputAction :type "InputAction Object Reference" :default "/Game/Usables_System/Interactable/Inputs/IA_I_Interact.IA_I_Interact"))
  ; Keymapping
  (:`Started`
    (`self.Do Interact`)))

(event `OnActorEndOverlap_Event`
  (params (OverlappedActor :type "Actor Object Reference") (OtherActor :type "Actor Object Reference"))
  (bind _returnvalue (`Actor.GetComponentByClass` OtherActor "/Game/Usables_System/Interactable/AC_Interactable.AC_Interactable_C"))
  ; Bind Overlapping array to Actor's Overlap begin/end events
  (`/Engine/EditorBlueprintResources/StandardMacros.IsValid` _returnvalue
    (:`Is Valid`
      (`KismetArrayLibrary.Array_RemoveItem` (`self.overlappings`) _returnvalue)
      (`/Game/Usables_System/Interactable/AC_Interactable.Highlight` _returnvalue false true))))

(event `Do Interact`
  (bind _nearest (`self.nearest`))
  ; Interact w the nearest actor
  (`/Engine/EditorBlueprintResources/StandardMacros.IsValid` _nearest
    (:`Is Valid`
      (message `/Game/Usables_System/Interactable/BPI_Interact.Interact` _nearest (`self.GetOwner`))
      (`self.handle Interact` _nearest))))

(event `handle Interact`
  (params (Interactable :type "/Game/Usables_System/Interactable/AC_Interactable Object Reference"))
  (`KismetSystemLibrary.PrintString` "handle Interactable!" :!enabledstate Disabled))

(event `self.ReceiveTick`
  (params (DeltaSeconds :type "Float (single-precision)"))
  (bind _nearest (`self.nearest`))
  (bind _interactable (`self.Find Closest In Overlappings` (`self.Get Interaction Location`)))
  ; Set nearest and highlight
  (`/Engine/EditorBlueprintResources/StandardMacros.IsValid` _interactable
    (:`Is Valid`
      (`/Game/Usables_System/Interactable/AC_Interactable.Highlight` _interactable true false)
      (`/Engine/EditorBlueprintResources/StandardMacros.IsValid` _nearest
        (:`Is Valid`
          (if (not (== _nearest _interactable))
            (`/Game/Usables_System/Interactable/AC_Interactable.Highlight` _nearest true true)
            (set `self.nearest` _interactable :!label _label)))
        (:`Is Not Valid`
          (goto _label))))
    (:`Is Not Valid`
      (set `self.nearest` null))))

(fn `Find Closest In Overlappings`
  (params (Location :type "Vector Structure"))
  (returns (Interactable :type "/Game/Usables_System/Interactable/AC_Interactable Object Reference"))
  (locals (`Closest Interactable` :type "/Game/Usables_System/Interactable/AC_Interactable Object Reference") (`Closest Dist` :type "Float (double-precision)" :default 9999999.0))
  (bind _overlappings (`self.overlappings`))
  (if (== (`KismetArrayLibrary.Array_Length` _overlappings) 1)
    (return (`|GetArrayItem` _overlappings))
    (else
      (for _array_element (`self.overlappings`)
        (`/Engine/EditorBlueprintResources/StandardMacros.IsValid` _array_element
          (:`Is Valid`
            (bind _returnvalue (- (`Actor.K2_GetActorLocation` (`self.GetOwner` _array_element)) Location))
            (bind _returnvalue_2 (`KismetMathLibrary.Dot_VectorVector` _returnvalue _returnvalue))
            (if (and (`/Game/Usables_System/Interactable/AC_Interactable.Interactable?` _array_element) (< _returnvalue_2 (`local.Closest Dist`)))
              (set `local.Closest Dist` _returnvalue_2)
              (set `local.Closest Interactable` _array_element)))))
      (return (`local.Closest Interactable`)))))

(fn `Get Interaction Location`
  (returns (Location :type "Vector Structure"))
  (bind (_returnvalue_location _returnvalue_rotation) (`KismetMathLibrary.BreakTransform` (`Actor.GetTransform` (`self.GetOwner`))))
  (return (+ _returnvalue_location (`KismetMathLibrary.GreaterGreater_VectorRotator` (100.0 0.0 0.0) _returnvalue_rotation))))