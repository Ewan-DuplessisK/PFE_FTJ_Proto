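; BP_Projectile is a weapon projectile that passes its velocity on to whatever it hits.
; An optional flag disables gravity on its ProjectileMovement at BeginPlay and restores it on a hit, so it flies straight until first impact.
; On hit, Enemy_Base and Physics_Props targets are launched with the projectile's velocity.
; Any other hit goes to BPDestructionAC, which receives the struck component, hit data and velocity as linear input.
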(event `self.ReceiveBeginPlay`
  (if (`self.No Gravity Before 1st Hit`)
    (set `ProjectileMovementComponent.ProjectileGravityScale` 0.0 (`self.ProjectileMovement`))))

(event `self.ReceiveHit`
  (params (MyComp :type "PrimitiveComponent Object Reference") (Other :type "Actor Object Reference") (OtherComp :type "PrimitiveComponent Object Reference") (bSelfMoved :type Boolean) (HitLocation :type "Vector Structure") (HitNormal :type "Vector Structure") (NormalImpulse :type "Vector Structure") (Hit :type "HitResult Structure (by ref)"))
  (bind _returnvalue (* (`self.GetVelocity`) 1.0))
  (if (`self.No Gravity Before 1st Hit`)
    (set `ProjectileMovementComponent.ProjectileGravityScale` 1.0 (`self.ProjectileMovement`)))
  (bind _asenemy_base (cast `Enemy_Base` Other)
    (:`then`
      (`Enemy_Base.Launched` _asenemy_base _returnvalue))
    (:`CastFailed`
      (bind _asphysics_props (cast `Physics_Props` Other)
        (:`then`
          (`Physics_Props.Launched` _asphysics_props _returnvalue))
        (:`CastFailed`
          (`FTJ_ProtoDestructionComponent.Hit` (`self.BP_Destruction_AC`) OtherComp Hit 10.0 0 1.0 1.0 _returnvalue (0.0 0.0 0.0)))))))

(fn `UserConstructionScript`)