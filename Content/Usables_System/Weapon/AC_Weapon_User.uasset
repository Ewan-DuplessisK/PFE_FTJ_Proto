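; Character component that lets the player pick up, attach, attack with, drop and throw weapons via Enhanced Input.
; WeaponData drives cooldown- and ammo-gated attacks, branching into melee or ranged.
; Melee binds weapon overlaps between montage notifies to damage and launch targets, while ranged spawns scattered projectiles aimed by aim assist or camera trace.
; Arm, drop and throw toggle physics and collision, using next-tick delays to avoid collision conflicts.
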(event `self.ReceiveBeginPlay`
  (`parent.ReceiveBeginPlay`)
  ;[1 1 1] Vars
  (set `self.characterMesh` (`Actor.GetComponentByClass` (`self.GetOwner`) "/Script/Engine.SkeletalMeshComponent"))
  (set `self.acAimAssist` (`Actor.GetComponentByClass` (`self.GetOwner`) "/Game/PlayerCharacter/Components/AC_AimAssist.AC_AimAssist_C"))
  ;[1 1 1] DEBUG Input
  (message `EnhancedInputSubsystemInterface.AddMappingContext` (pcsubsystem `EnhancedInputLocalPlayerSubsystem` (`self.playerController`)) "/Game/Usables_System/Weapon/Input/IMC_Weapon2_Test.IMC_Weapon2_Test" 0 (struct))
  (`Actor.EnableInput` (`self.GetOwner`) null))

(event `self.handle Pickup`
  (params (Pickupable :type "/Game/Usables_System/Pickupable/AC_Pickupable Object Reference"))
  (`parent.handle Pickup` Pickupable)
  (bind _asac_weapon (cast `/Game/Usables_System/Weapon/AC_Weapon` Pickupable))
  (`self.Has Weapon?`
    (:`true`
      (`self.Drop Weapon`)
      ; fix collision conflict Arm/Drop
      (`KismetSystemLibrary.DelayUntilNextTick`)
      (`KismetSystemLibrary.DelayUntilNextTick`)
      (`KismetSystemLibrary.DelayUntilNextTick`))
    (:`false`
      _))
  (`self.Arm Weapon` _asac_weapon))

(event `EnhancedInput|/Game/Usables_System/Weapon/Input/IA_W_Attack`
  (params (ActionValue :type Boolean) (ElapsedSeconds :type "Float (double-precision)") (TriggeredSeconds :type "Float (double-precision)") (InputAction :type "InputAction Object Reference" :default "/Game/Usables_System/Weapon/Input/IA_W_Attack.IA_W_Attack"))
  ;[1 1 1] Keymapping
  (:`Triggered`
    (`self.IA_Attack Triggered`))
  (:`Started`
    (`self.IA_Attack Started`)))

(event `EnhancedInput|/Game/Usables_System/Weapon/Input/IA_W_Drop`
  (params (ActionValue :type Boolean) (ElapsedSeconds :type "Float (double-precision)") (TriggeredSeconds :type "Float (double-precision)") (InputAction :type "InputAction Object Reference" :default "/Game/Usables_System/Weapon/Input/IA_W_Drop.IA_W_Drop"))
  ;[1 1 1] Keymapping
  (:`Started`
    (`self.Drop Weapon`)))

(event `Arm Weapon`
  (params (`AC Weapon` :type "/Game/Usables_System/Weapon/AC_Weapon Object Reference"))
  (bind _acweapon (`self.acWeapon`))
  (bind _mesh (`/Game/Usables_System/Interactable/AC_Interactable.mesh` _acweapon))
  ;[0 1 0.1253] Pickup&Arm Weapon
  (`/Game/Usables_System/Interactable/AC_Interactable.Set Interactable` `AC Weapon` false)
  (set `self.acWeapon` `AC Weapon`)
  (set `self.weaponActor` (`self.GetOwner` `AC Weapon`))
  (set `self.weaponData` (`/Game/Usables_System/Weapon/AC_Weapon.Weapon Data` (`self.acWeapon`)))
  (`self.$ Disable Its Physics` _acweapon)
  (set `self.lastMeshProfile` (`PrimitiveComponent.GetCollisionProfileName` _mesh))
  (`PrimitiveComponent.SetCollisionProfileName` _mesh "Melee_Weapon" true)
  ;; fix collision conflict Arm/Drop
  (`KismetSystemLibrary.DelayUntilNextTick`)
  (`self.$ Attach Weapon To Character`))

(event `EnhancedInput|/Game/Usables_System/Weapon/Input/IA_W_Throw`
  (params (ActionValue :type Boolean) (ElapsedSeconds :type "Float (double-precision)") (TriggeredSeconds :type "Float (double-precision)") (InputAction :type "InputAction Object Reference" :default "/Game/Usables_System/Weapon/Input/IA_W_Throw.IA_W_Throw"))
  ;[1 1 1] Keymapping
  (:`Started`
    (`self.Throw Weapon`)))

(event `Drop Weapon`
  ; Drop Weapon
  (`self.Has Weapon?`
    (:`true`
      (`self.$ Detach Weapon`)
      ;; fix collision conflict Arm/Drop
      (`KismetSystemLibrary.DelayUntilNextTick`)
      (`KismetSystemLibrary.DelayUntilNextTick`)
      (`self.$ Respawn Weapon Actor Back`))))

(event `$ Detach Weapon`
  (bind _acweapon (`self.acWeapon`))
  ;[0.1096 0 1] Detach Weapon
  (`self.weaponActor`
    (:`then`
      (`self.$ Restore Its Physics` _acweapon)
      (`PrimitiveComponent.SetCollisionProfileName` (`/Game/Usables_System/Interactable/AC_Interactable.mesh` _acweapon) (`self.lastMeshProfile`) true)
      (`/Game/Usables_System/Interactable/AC_Interactable.Set Interactable` (`self.acWeapon`) true)
      ;; fix collision conflict Arm/Drop
      (`KismetSystemLibrary.DelayUntilNextTick`)
      (`self.$ Detach It` (`self.acWeapon`)))
    (:`else`)))

(event `Throw Weapon`
  (bind _returnvalue (`SceneComponent.GetSocketTransform` (`self.characterMesh`) (`/Game/Usables_System/Weapon/DA_Weapon.Socket Name` (`self.weaponData`)) "RTS_World"))
  (bind _location (.location _returnvalue))
  (bind _dir (`self.Get Aiming Dir` _location))
  ;[0 0.04052 0.15 0.5] Throw Weapon
  (`self.Has Weapon?`
    (:`true`
      (bind _notifyname (`|PlayMontage` (`self.characterMesh`) (`self.Throw Anim`))
        (:`OnNotifyBegin`
          (if (== _notifyname "Throw Weapon")
            (`self.$ Detach Weapon`)
            (`KismetSystemLibrary.DelayUntilNextTick`)
            (`KismetSystemLibrary.DelayUntilNextTick`)
            (`Actor.K2_SetActorTransform` (`self.weaponActor`) _returnvalue false true)
            (`PrimitiveComponent.AddImpulse` (`self.WeaponMesh`) (* _dir (`self.Throw Impulse 1e3`) 10000.0) "None" false)
            (`KismetSystemLibrary.DrawDebugLine` _location (* _dir 1000.0) (struct :`R` 1.0 :`B` 0.035084 :`A` 1.0) 10.0 0.5)
            (set `self.weaponActor` null)
            (set `self.weaponData` null)))))))

(event `IA_Attack Triggered`
  ;[0.15 0.007438 0 0.5] Attack Triggering (Common)
  (`self.Has Weapon?`
    (:`true`
      (if (`/Game/Usables_System/Weapon/DA_Weapon.Automatic` (`self.weaponData`))
        (bind _allowed (`self.$ Attacking _ Process Cooldown` :!label _label))
        (if _allowed
          (bind _allowed_2 (`self.$ Attacking _ Process Ammo`))
          (if _allowed_2
            (`AnimInstance.Montage_Play` (`SkeletalMeshComponent.GetAnimInstance` (`self.characterMesh`)) (`/Game/Usables_System/Weapon/DA_Weapon.Char Anim` (`self.weaponData`)) 1.0 "MontageLength" 0.0 true)
            (switch `/Game/Usables_System/Weapon/E_Weapon_Type` (`/Game/Usables_System/Weapon/DA_Weapon.Type` (`self.weaponData`))
              (:`NewEnumerator0`
                (`self.$ Attacking _ Melee`))
              (:`NewEnumerator1`
                (`self.$ Attacking _ Ranged`)))))))))

(event `IA_Attack Started`
  ;[0.15 0.007438 0 0.5] Attack Triggering (Common)
  (`self.Has Weapon?`
    (:`true`
      (goto _label))))

(event `$ Attacking _ Melee`
  ;[1 0.423 0] MELEE Attack
  (bind _notifyname (`|PlayMontage` (`self.characterMesh`) (`self.Melee Anim`) :!label _label_2)
    (:`OnCompleted`
      (`/Engine/EditorBlueprintResources/StandardMacros.DoOnce` false :!via `Reset`
        (:`Completed`
          (goto _label_2))))
    (:`OnNotifyBegin`
      (switch `name` _notifyname
        (:`Melee Attack Begin`
          (add `PrimitiveComponent.OnComponentBeginOverlap` (`self.WeaponMesh`) (delegate `$ On Weapon Overlap`)))
        (:`Melee Attack End`
          (remove `PrimitiveComponent.OnComponentBeginOverlap` (`self.WeaponMesh`) (delegate `$ On Weapon Overlap`)))))))

(event `$ On Weapon Overlap`
  (params (OverlappedComponent :type "PrimitiveComponent Object Reference") (OtherActor :type "Actor Object Reference") (OtherComp :type "PrimitiveComponent Object Reference") (OtherBodyIndex :type Integer) (bFromSweep :type Boolean) (SweepResult :type "HitResult Structure (by ref)"))
  ;[1 0.423 0] MELEE Attack
  (bind _asenemy_base (cast `Enemy_Base` OtherActor)
    (:`then`
      ;; Damage
      (`GameplayStatics.ApplyDamage` _asenemy_base (`/Game/Usables_System/Weapon/DA_Weapon.Damage` (`self.weaponData`)))
      (bind (_returnvalue_x _returnvalue_y) (`KismetMathLibrary.BreakVector` (* (`KismetMathLibrary.Normal` (- (`Actor.K2_GetActorLocation` _asenemy_base) (`SceneComponent.K2_GetComponentLocation` (`self.WeaponMesh`)))) (`/Game/Usables_System/Weapon/DA_Weapon.Melee Impulse` (`self.weaponData`)))))
      ;; Impulse
      (`Enemy_Base.Launched` _asenemy_base (`KismetMathLibrary.MakeVector` _returnvalue_x _returnvalue_y 50.0)))
    (:`CastFailed`
      (bind _asphysics_props (cast `Physics_Props` OtherActor))
      (bind (_returnvalue_x_2 _returnvalue_y_2) (`KismetMathLibrary.BreakVector` (* (`KismetMathLibrary.Normal` (- (`Actor.K2_GetActorLocation` _asphysics_props) (`Actor.K2_GetActorLocation` (`self.GetOwner`)))) (`/Game/Usables_System/Weapon/DA_Weapon.Melee Impulse` (`self.weaponData`)))))
      (`Physics_Props.Launched` _asphysics_props (`KismetMathLibrary.MakeVector` _returnvalue_x_2 _returnvalue_y_2 50.0)))))

(fn `$ Attach Weapon To Character`
  (bind _scenecomp_to_attach_range_weapon (`self.SceneComp to Attach Range Weapon`))
  (bind _weaponactor (`self.weaponActor`))
  (`Actor.K2_AttachToComponent` _weaponactor (select `bool` (and (`|EnumEquality` (`/Game/Usables_System/Weapon/DA_Weapon.Type` (`self.weaponData`)) "NewEnumerator1") (`KismetSystemLibrary.IsValid` _scenecomp_to_attach_range_weapon)) :`false` (`self.characterMesh`) :`true` _scenecomp_to_attach_range_weapon :!type "SceneComponent Object Reference") (`/Game/Usables_System/Weapon/DA_Weapon.Socket Name` (`self.weaponData`)) "SnapToTarget" "SnapToTarget" "SnapToTarget" false)
  (`SceneComponent.K2_SetRelativeTransform` (`Actor.RootComponent` _weaponactor) (`/Game/Usables_System/Weapon/DA_Weapon.Transform` (`self.weaponData`)) false false)
  (`PrimitiveComponent.SetCollisionEnabled` (`self.WeaponMesh`) "QueryAndPhysics"))

(fn `$ Attacking _ Process Ammo`
  (returns (Allowed :type Boolean))
  (locals (Allow :type Boolean))
  (bind _acweapon (`self.acWeapon`))
  (bind _ammo (`/Game/Usables_System/Weapon/AC_Weapon.Ammo` _acweapon))
  (bind _returnvalue (> _ammo 0.0))
  (`KismetSystemLibrary.PrintString` (`KismetStringLibrary.Concat_StrStr` "Ammo: " (`KismetStringLibrary.Conv_DoubleToString` _ammo :!enabledstate Disabled) " = " (`KismetStringLibrary.Conv_BoolToString` _returnvalue :!enabledstate Disabled) :!enabledstate Disabled) :!enabledstate Disabled)
  (bind _output_get (set `local.Allow` _returnvalue))
  (if _output_get
    (set `/Game/Usables_System/Weapon/AC_Weapon.Ammo` (- _ammo 1.0) _acweapon)
    (elif (`/Game/Usables_System/Weapon/DA_Weapon.Throw Empty` (`self.weaponData`))
      (`self.Throw Weapon`)))
  (return (`local.Allow`)))

(fn `$ Attacking _ Process Cooldown`
  (returns (Allowed :type Boolean))
  (locals (Allow :type Boolean))
  (bind _returnvalue (`KismetSystemLibrary.GetGameTimeInSeconds`))
  (bind _output_get (set `local.Allow` (> (- _returnvalue (`/Game/Usables_System/Weapon/DA_Weapon.Cooldown` (`self.weaponData`))) (`self.lastFireTime`))))
  (if _output_get
    (set `self.lastFireTime` _returnvalue))
  (return _output_get))

(fn `$ Attacking _ Ranged`
  (bind (_assisted _dir _rot) (`self.Get AimAssist Dir`))
  (bind _location (`self.Get Projectile Spawn Loc`))
  (for _ (range (`/Game/Usables_System/Weapon/DA_Weapon.Projectiles Number` (`self.weaponData`)))
    (`|SpawnActorFromClass` (`/Game/Usables_System/Weapon/DA_Weapon.Projectile Class` (`self.weaponData`)) (`KismetMathLibrary.MakeTransform` _location (`self.Scatter Projectile Dir` (`KismetMathLibrary.SelectRotator` _rot (`.Rot` (`self.Get Aiming Dir` (`self.Get Projectile Spawn Loc`))) _assisted))) "AdjustIfPossibleButAlwaysSpawn" "OverrideRootScale" (`self.GetOwner`) (`GameplayStatics.GetPlayerPawn` 0)))
  (`GameplayStatics.PlaySoundAtLocation` (`/Game/Usables_System/Weapon/DA_Weapon.Sound` (`self.weaponData`)) _location (struct) 1.0 1.0 0.0 null null null null))

(fn `$ Pickup Weapon`
  (params (Item :type "/Game/Usables_System/Interactable/AC_Interactable Object Reference (by ref)"))
  (`/Game/Usables_System/Interactable/AC_Interactable.Set Interactable` Item false)
  (`KismetArrayLibrary.Array_RemoveItem` (`self.overlappings`) Item))

(fn `$ Respawn Weapon Actor Back`
  (bind (_returnvalue_location _returnvalue_rotation) (`KismetMathLibrary.BreakTransform` (`Actor.GetTransform` (`self.GetOwner`))))
  (`Actor.K2_SetActorTransform` (`self.weaponActor`) (`KismetMathLibrary.MakeTransform` (+ (* (`KismetMathLibrary.GetForwardVector` _returnvalue_rotation) 100.0) _returnvalue_location) _returnvalue_rotation) false false)
  (set `self.weaponActor` null)
  (set `self.weaponData` null))

(fn `Aiming?`
  (returns (Aiming :type Boolean))
  (return (`KismetSystemLibrary.IsValid` (`self.weaponData`))))

(fn `Get AimAssist Dir`
  (returns (Assisted :type Boolean) (Dir :type "Vector Structure") (Rot :type "Rotator Structure"))
  (bind _pawnhitlocation (`AimComponent_Base.PawnHitLocation` (`self.acAimAssist`)))
  (bind _returnvalue (`KismetMathLibrary.Vector_IsZero` _pawnhitlocation))
  (bind _returnvalue_2 (- _pawnhitlocation (`self.Get Projectile Spawn Loc`)))
  (return (not _returnvalue) (`KismetMathLibrary.Normal` _returnvalue_2) (`KismetMathLibrary.SelectRotator` (struct) (`KismetMathLibrary.MakeRotFromX` _returnvalue_2) _returnvalue)))

(fn `Get Aiming Dir`
  (params (`From Loc` :type "Vector Structure"))
  (returns (Dir :type "Vector Structure") (Rot :type "Rotator Structure"))
  (bind (_returnvalue_location _returnvalue_rotation) (`KismetMathLibrary.BreakTransform` (`Actor.GetTransform` (`GameplayStatics.GetPlayerCameraManager` 0))))
  (bind (_outhit _returnvalue) (`KismetSystemLibrary.LineTraceSingle` _returnvalue_location (* (`KismetMathLibrary.Conv_RotatorToVector` _returnvalue_rotation) 999999.0) "TraceTypeQuery1" true))
  (bind _returnvalue_2 (- (`.Location` (`GameplayStatics.BreakHitResult` _outhit)) `From Loc`))
  (return (`KismetMathLibrary.Normal` _returnvalue_2) (`KismetMathLibrary.SelectRotator` (`KismetMathLibrary.MakeRotFromX` _returnvalue_2) _returnvalue_rotation _returnvalue)))

(fn `Get Projectile Spawn Loc`
  (returns (Location :type "Vector Structure"))
  (bind _returnvalue_location (`KismetMathLibrary.BreakTransform` (`SceneComponent.GetSocketTransform` (`self.WeaponMesh`) "Muzzle" "RTS_World")))
  (return _returnvalue_location))

(fn `Scatter Projectile Dir`
  (params (`In Rot` :type "Rotator Structure"))
  (returns (Rot :type "Rotator Structure"))
  (bind _projectiles_scattering (`/Game/Usables_System/Weapon/DA_Weapon.Projectiles Scattering` (`self.weaponData`)))
  (return (`KismetMathLibrary.SelectRotator` (`KismetMathLibrary.Conv_VectorToRotator` (`KismetMathLibrary.RandomUnitVectorInConeInDegrees` (`KismetMathLibrary.Conv_RotatorToVector` `In Rot`) _projectiles_scattering)) `In Rot` (> _projectiles_scattering 0.0))))

(fn `WeaponMesh`
  (returns (mesh :type "StaticMeshComponent Object Reference"))
  (return (`/Game/Usables_System/Interactable/AC_Interactable.mesh` (`self.acWeapon`))))