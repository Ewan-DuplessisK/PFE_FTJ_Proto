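; Weapon class in the usables system that initializes its ammo and display title from WeaponData.
; On BeginPlay it runs the parent logic, then treats negative Ammo as unset and fills it from the data asset.
; The same branch sets the widget title to the weapon name, so a preset ammo count skips both steps.
; The OnPickup event is an empty stub.
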(event `self.ReceiveBeginPlay`
  (`parent.ReceiveBeginPlay`)
  ; Set default Asset Ammo if this Ammo is -1 (default var)
  (if (< (`self.Ammo`) 0.0)
    (set `self.Ammo` (`/Game/Usables_System/Weapon/DA_Weapon.Ammo` (`self.Weapon Data`)))
    ; Title
    (set `/Game/Usables_System/Interactable/WBP_Interactable.Title` (`KismetTextLibrary.Conv_NameToText` (`/Game/Usables_System/Weapon/DA_Weapon.Name` (`self.Weapon Data`))) (`self.widget`))))

(event `On Pickup`)