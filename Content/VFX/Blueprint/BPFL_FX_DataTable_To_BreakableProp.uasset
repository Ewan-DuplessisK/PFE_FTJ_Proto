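; Blueprint function library that sends breakable prop data from a data table to a Niagara system.
; It gathers each row's position and radius, plus each mesh's full bounds size, then passes them as arrays along with the mesh list and a material.
; All three gathered arrays use AddUnique, so duplicate values collapse and indices can fall out of alignment.
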(fn `SendBreakablePropDataToNiagara`
  (params (DataTable :type "DataTable Object Reference") (NiagaraSystem :type "NiagaraComponent Object Reference") (MeshRenderer :type "Array of NiagaraMeshRendererMeshPropertiesBase Structure") (Material :type "MaterialInterface Object Reference"))
  (locals (Positions :type "Array of Vector Structure") (Radiuses :type "Array of Float (double-precision)") (Bounds :type "Array of Vector Structure"))
  (`/Engine/EditorBlueprintResources/StandardMacros.IsValid` NiagaraSystem
    (:`Is Valid`
      (bind _outrownames (`DataTableFunctionLibrary.GetDataTableRowNames` DataTable))
      (for _array_element _outrownames
        (bind _returnvalue (`|GetDataTableRow` DataTable _array_element)
          (:`then`
            (bind (_position _radius) (break `/Game/VFX/DataTables/S_FX_GetVectorPositionOffsets` _returnvalue))
            (`KismetArrayLibrary.Array_AddUnique` (`local.Positions`) _position)
            (`KismetArrayLibrary.Array_AddUnique` (`local.Radiuses`) _radius))))
      (`|ExecutionSequence`
        (:`then_0`
          (for _array_element_2 MeshRenderer
            (bind (_returnvalue_origin _returnvalue_boxextent) (`KismetMathLibrary.BreakBoxSphereBounds` (`StaticMesh.GetBounds` (`.Mesh` (break `NiagaraMeshRendererMeshPropertiesBase` _array_element_2)))))
            (`KismetArrayLibrary.Array_AddUnique` (`local.Bounds`) (* _returnvalue_boxextent 2.0))))
        (:`then_1`
          (`NiagaraDataInterfaceArrayFunctionLibrary.SetNiagaraArrayPosition` NiagaraSystem "Position_Array" (`local.Positions`))
          (`NiagaraDataInterfaceArrayMesh.SetNiagaraArrayMesh` NiagaraSystem "Mesh Array" MeshRenderer)
          (`NiagaraComponent.SetVariableMaterial` NiagaraSystem "Material Interface" Material)
          (`NiagaraDataInterfaceArrayFunctionLibrary.SetNiagaraArrayFloat` NiagaraSystem "Mesh_Radius" (`local.Radiuses`))
          (`NiagaraDataInterfaceArrayFunctionLibrary.SetNiagaraArrayVector` NiagaraSystem "Mesh_Dimensions" (`local.Bounds`)))))))