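; BP_PropBreak is a VFX actor that plays the NS_Props_Break Niagara effect for a chair prop.
; On BeginPlay it attaches the system inactive and gathers unique positions from every row of the DT_FX_Chair1 data table.
; After a hardcoded delay, it feeds the position array, a mesh array and the chair material into Niagara user parameters, then activates the system.
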(event `self.ReceiveBeginPlay`
  (bind _dt_positions (`self.DT_Positions`))
  (bind _ns (`self.NS`))
  (bind _returnvalue (`NiagaraFunctionLibrary.SpawnSystemAttached` "/Game/VFX/Niagara/Props/NS_Props_Break.NS_Props_Break" (`self.DefaultSceneRoot`) "None" (0.0 0.0 0.0) (struct) "KeepRelativeOffset" false false))
  (set `self.NS` _returnvalue)
  (set `self.DT_Positions` "/Game/VFX/DataTables/DT_FX_Chair1.DT_FX_Chair1")
  (bind _outrownames (`DataTableFunctionLibrary.GetDataTableRowNames` _dt_positions))
  (for _array_element _outrownames
    (bind _returnvalue_2 (`|GetDataTableRow` _dt_positions _array_element)
      (:`then`
        (`KismetArrayLibrary.Array_AddUnique` (`self.Array`) (`.Position_12_299B17A54D3C32752537CC92DAE939E6` (break `/Game/VFX/DataTables/S_FX_GetVectorPositionOffsets` _returnvalue_2))))))
  (`KismetSystemLibrary.Delay` 10.0)
  (`NiagaraDataInterfaceArrayFunctionLibrary.SetNiagaraArrayPosition` _ns "Position_Array" (`self.Array`))
  (`NiagaraDataInterfaceArrayMesh.SetNiagaraArrayMesh` _ns "Mesh Array" (`self.Array Data`))
  (`NiagaraComponent.SetVariableMaterial` _ns "Material Interface" "/Game/Environment/Office/Materials/MI_ChairAB_00.MI_ChairAB_00")
  (`ActorComponent.Activate` _ns false))

(fn `UserConstructionScript`)