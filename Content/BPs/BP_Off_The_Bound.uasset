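; BP_Off_The_Bound is an out-of-bounds trigger that sends the player back to the level's start.
; On BeginPlay it finds a PlayerStart actor and stores it as the spawn reference.
; When the player pawn overlaps its box, it teleports the pawn to that start's location and rotation and also sets the controller's control rotation to match.
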(event `self.ReceiveBeginPlay`
  (bind _returnvalue (`GameplayStatics.GetActorOfClass` "/Script/Engine.PlayerStart"))
  (set `self.Spawn ` _returnvalue))

(event `self.Box.OnComponentBeginOverlap`
  (params (OverlappedComponent :type "PrimitiveComponent Object Reference") (OtherActor :type "Actor Object Reference") (OtherComp :type "PrimitiveComponent Object Reference") (OtherBodyIndex :type Integer) (bFromSweep :type Boolean) (SweepResult :type "HitResult Structure (by ref)"))
  (bind _returnvalue (`GameplayStatics.GetPlayerPawn` 0))
  (bind (_returnvalue_location _returnvalue_rotation) (`KismetMathLibrary.BreakTransform` (`self.GetTransform` (`self.Spawn `))))
  (if (== OtherActor _returnvalue)
    (`self.K2_TeleportTo` _returnvalue _returnvalue_location _returnvalue_rotation)
    (`Controller.SetControlRotation` (`GameplayStatics.GetPlayerController` 0) _returnvalue_rotation)))

(fn `UserConstructionScript`)