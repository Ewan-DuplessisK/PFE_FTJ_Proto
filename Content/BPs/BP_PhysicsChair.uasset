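; Physics chair prop that can be pushed, vacuumed or kicked, with meshes set at construction.
; While kicked, hitting another kickable physics prop breaks it, awards score and swaps it for a spawned chair-bottom actor.
; Hits on other actors send damage, skipping players, and turrets unless kicked.
; Bound feedback events play Wwise sounds and spawn Niagara break debris fed from a data table.
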(event `self.ReceiveTick`
  (params (DeltaSeconds :type "Float (single-precision)")))

(event `StartSimulating`
  (bind (_returnvalue_x _returnvalue_y _returnvalue_z) (`KismetMathLibrary.BreakVector` (`self.K2_GetActorLocation`)))
  (`self.K2_SetActorLocation` (`KismetMathLibrary.MakeVector` _returnvalue_x _returnvalue_y (+ _returnvalue_z 15.0)))
  (`PrimitiveComponent.SetSimulatePhysics` (`self.Bottom_Chair`) true))

(event `self.ReceiveBeginPlay`
  ;[1 0.7316 0 0.5 25] BEGIN PLAY
  (`self.Init Feedback`))

(event `KickedInterface.Kicked`
  (params (KickVector :type "Vector Structure") (PlayerPosition :type "Vector Structure"))
  ;[0 0.4043 1 0.5] What happend when the chair got kicked
  (`PrimitiveComponent.SetSimulatePhysics` (`self.Bottom_Chair`) true)
  (`self.Kicked_Sound_Event`)
  (set `self.IsKicked` true)
  (`KismetArrayLibrary.Array_Add` (`self.Tags`) "Kicked")
  (if (not (`self.IsBroken`))
    (`ActorComponent.Activate` (`self.VFX_Hit`) true)
    (`PrimitiveComponent.AddTorqueInDegrees` (`self.Top_Chair`) (0.0 0.0 50000.0) "None" true)
    (`PrimitiveComponent.AddImpulse` (`self.Bottom_Chair`) (* KickVector (`self.Impulse_Value`)) "None" false)
    (`KismetSystemLibrary.Delay` 1.0)
    (set `self.IsKicked` false)
    (`KismetArrayLibrary.Array_RemoveItem` (`self.Tags`) "Kicked")))

(event `self.ReceiveHit`
  (params (MyComp :type "PrimitiveComponent Object Reference") (Other :type "Actor Object Reference") (OtherComp :type "PrimitiveComponent Object Reference") (bSelfMoved :type Boolean) (HitLocation :type "Vector Structure") (HitNormal :type "Vector Structure") (NormalImpulse :type "Vector Structure") (Hit :type "HitResult Structure (by ref)"))
  (bind _top_chair (`self.Top_Chair`))
  (bind _vfx_hit (`self.VFX_Hit`))
  (bind _chair (`self.Chair`))
  (bind _returnvalue (`self.K2_GetActorLocation` (`.HitActor` (`GameplayStatics.BreakHitResult` Hit))))
  ;[1 0.51 0 0.5] Chair hit "Prop Physics" and what happend
  (`PrimitiveComponent.SetSimulatePhysics` (`self.Bottom_Chair`) true)
  (`/Engine/EditorBlueprintResources/StandardMacros.IsValid` Other
    (:`Is Valid`
      (`/Engine/EditorBlueprintResources/StandardMacros.IsValid` (`self.GetComponentByClass` Other "/Game/CppSystems/Prop/Public/ActorComponent/BP_Prop_PhysicsKickableCompBase_AC.BP_Prop_PhysicsKickableCompBase_AC_C")
        (:`Is Valid`
          (if (`self.IsKicked`)
            (`|ExecutionSequence`
              (:`then_0`
                (`SceneComponent.SetHiddenInGame` _top_chair true false)
                (`PrimitiveComponent.SetCollisionEnabled` _top_chair "NoCollision")
                (`KismetSystemLibrary.Delay` 0.1)
                (`PrimitiveComponent.SetCollisionResponseToChannel` (`self.Bottom_Chair`) "ECC_Pawn" "ECR_Ignore")
                (`PrimitiveComponent.SetSimulatePhysics` (`self.Bottom_Chair`) false)
                (`PrimitiveComponent.SetCollisionEnabled` (`self.Bottom_Chair`) "NoCollision")
                (`ActorComponent.Deactivate` (`self.Hitbox`))
                (set `self.IsBroken` true)
                (set `self.Chair` (`SceneComponent.K2_GetComponentToWorld` (`self.Bottom_Chair`)))
                (bind _bottom_chair (`self.Bottom_Chair`)
                  (:`then`
                    (`ActorComponent.K2_DestroyComponent` _bottom_chair)
                    (`KismetSystemLibrary.DelayUntilNextTick`)
                    (`|SpawnActorFromClass` "/Game/BPs/VacuumProps/BP_ChairBottom_Medium.BP_ChairBottom_Medium_C" (`KismetMathLibrary.MakeTransform` (`KismetMathLibrary.MakeVector` (.x (.location _chair)) (.y (.location _chair)) (+ (.z (.location _chair)) 1.0)) (.rotation _chair) (.scale _chair)) "AdjustIfPossibleButAlwaysSpawn" "MultiplyWithRoot" null null)
                    (`KismetSystemLibrary.DelayUntilNextTick`)
                    (`ActorComponent.K2_DestroyComponent` (`self.Hitbox`))
                    (`KismetSystemLibrary.Delay` 2.0)
                    (`self.K2_DestroyActor`))
                  (:`else`)))
              (:`then_1`
                (`SceneComponent.K2_SetWorldLocation` _vfx_hit _returnvalue false false)
                (`SceneComponent.K2_SetWorldLocation` (`self.VFX_Explosion`) _returnvalue false false)
                (set `self.Hit_Actor_Location` _returnvalue)
                (`self.Explode_Sound_Event`)
                (`ActorComponent.Activate` _vfx_hit true)
                (`self.Break_VFX`)
                ;;[0.15 0.007751 0 0.5] Score
                (`/Engine/EditorBlueprintResources/StandardMacros.DoOnce` false
                  (:`Completed`
                    (`FTJ_ScoringSystem_Score.IncreaseWithText` (subsystem `/Game/CppSystems/ScoringSystem/Public/Blueprint/BP_ScoringSystem_Score`) (`KismetMathLibrary.Conv_IntToDouble` 30) 0.3 false (`|FormatText` "Broke Chair")))))
              (:`then_2`
                (`KismetSystemLibrary.Delay` 0.2)
                (set `self.IsKicked` false)))))
        (:`Is Not Valid`
          (if (or (and (not (`self.ActorHasTag` Other "Player")) (not (`self.ActorHasTag` Other "Turret"))) (and (`self.ActorHasTag` Other "Turret") (`self.IsKicked`)))
            (message `HitInterface.GetHit` Other (`self.Hit_Damage`) 0.0 (0.0 0.0 0.0) 0.0 self)))))))

(event `/Game/BPs/TestProps/BPI_VacuumReaction.ReactToVacuum`
  (params (Force :type "Vector Structure"))
  ;[0 0.9505 1 0.5] Vacuum the chair
  (`PrimitiveComponent.SetSimulatePhysics` (`self.Bottom_Chair`) true)
  (`PrimitiveComponent.AddImpulse` (`self.Bottom_Chair`) (* Force (`self.Vacuum_Effect_Force`)) "None" true))

(event `/Game/BPs/BPI_Push.Push`
  (params (Force :type "Vector Structure"))
  ;[1 0.2344 0.7522 0.5] Player contact with chair make her move
  (`PrimitiveComponent.SetSimulatePhysics` (`self.Bottom_Chair`) true)
  (`PrimitiveComponent.AddImpulse` (`self.Bottom_Chair`) Force "None" true))

(event `Init Feedback`
  (`|ExecutionSequence`
    (:`then_0`
      (add `self.Kicked_Sound` (delegate `Kicked_Sound_Event`)))
    (:`then_1`
      (add `self.Explode_Sound` (delegate `Explode_Sound_Event`)))
    (:`then_3`
      (add `self.Break_VFX` (delegate `Break_VFX_Event`)))))

(event `Kicked_Sound_Event`
  ;[0 1 1 0.5] FB - Sound When Kicked
  (`AkGameObject.PostAkEvent` :`self` (`self.Ak_Chair`) :`AkEvent` "/Game/WwiseAudio/Events/Default_Work_Unit/GPE/GPE_LVL_01/Trolley_Wood_Push.Trolley_Wood_Push"))

(event `Explode_Sound_Event`
  ;[0 1 1 0.5] FB - Sound When Chair Explode
  (`AkGameObject.PostAkEvent` :`self` (`self.Ak_Chair`) :`AkEvent` "/Game/WwiseAudio/Events/Default_Work_Unit/SFX/SFX_GLOBAL/SFX_DESTRUCTION/SFX_Chair_Destruction.SFX_Chair_Destruction"))

(event `Getting_Vaccumed_Event`)

(event `Break_VFX_Event`
  (bind _bottom_chair (`self.Bottom_Chair`))
  (`/Engine/EditorBlueprintResources/StandardMacros.DoOnce` false
    (:`Completed`
      (bind _returnvalue (`NiagaraFunctionLibrary.SpawnSystemAtLocation` (`self.VFX Props Break`) (`SceneComponent.K2_GetComponentLocation` _bottom_chair) (`SceneComponent.K2_GetComponentRotation` _bottom_chair)))
      (bind _output_get (set `self.NS` _returnvalue))
      (`/Game/VFX/Blueprint/BPFL_FX_DataTable_To_BreakableProp.SendBreakablePropDataToNiagara` (`self.DT_Positions`) _output_get (`self.Array Mesh Renderer`) (`self.FX_Material`)))))

(fn `UserConstructionScript`
  (`StaticMeshComponent.SetStaticMesh` (`self.Top_Chair`) (`self.New Mesh Top`))
  (`StaticMeshComponent.SetStaticMesh` (`self.Bottom_Chair`) (`self.New Mesh Bottom`)))