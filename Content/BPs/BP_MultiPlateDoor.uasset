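; Door Blueprint that opens when all of its linked pressure plates are pressed.
; It extends a parent door, storing the linked plate count at BeginPlay and overriding the open and close events.
; Each open request adds pressed and subtracts unpressed plates on a running counter, which resets only at startup and on opening.
; If the counter is below the plate count, open and close requests close an open door through the parent.
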(event `self.ReceiveBeginPlay`
  (set `self.PlateAmount` (`KismetArrayLibrary.Array_Length` (`self.LinkedPlates`)))
  (set `self.PressedCounter` 0)
  (`parent.ReceiveBeginPlay`))

(event `self.Open Door`
  (bind _pressedcounter (`self.PressedCounter`))
  (for _array_element (`self.LinkedPlates`)
    (if (`/Game/BPs/Bp_Pressure_Plate.IsPressed` _array_element)
      (`/Engine/EditorBlueprintResources/StandardMacros.IncrementInt` _pressedcounter)
      (else
        (`/Engine/EditorBlueprintResources/StandardMacros.DecrementInt` _pressedcounter))))
  (if (>= (`self.PressedCounter`) (`self.PlateAmount`))
    (`parent.Open Door`)
    (set `self.PressedCounter` 0)
    (else
      (if (`self.Door Open`) :!label _label
        (`parent.Close Door`)))))

(event `self.Close Door`
  (if (< (`self.PressedCounter`) (`self.PlateAmount`))
    (goto _label)))

(fn `UserConstructionScript`
  (`parent.UserConstructionScript`))