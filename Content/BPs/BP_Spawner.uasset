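; BP_Spawner is an interactive spawner that creates a configurable number of actors when the player walks into its trigger boxes.
; Box and Box2 overlaps raise or lower SpawnNum, and an UpdateSpawn event shows the count on the NombreSpawn text.
; Box1 overlap spawns that many actors at the TargetPoint's location.
; The random-offset nodes are unconnected, so every spawn uses the same point.
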(event `self.ReceiveBeginPlay`
  (`self.Event Update Spawn`))

(event `self.Box1.OnComponentBeginOverlap`
  (params (OverlappedComponent :type "PrimitiveComponent Object Reference") (OtherActor :type "Actor Object Reference") (OtherComp :type "PrimitiveComponent Object Reference") (OtherBodyIndex :type Integer) (bFromSweep :type Boolean) (SweepResult :type "HitResult Structure (by ref)"))
  (bind _returnvalue_location (`KismetMathLibrary.BreakTransform` (`self.GetTransform` (`self.Target Point`))))
  ;[1 0 0.053 0.5] Spawn on Hit
  (if (== OtherActor (`GameplayStatics.GetPlayerCharacter` 0))
    (for _ (range (`self.Spawn Num`))
      (`|SpawnActorFromClass` "/Game/IA_System/01_Coworker_RD/BP_EnemyAI_Coworker_RD.BP_EnemyAI_Coworker_RD_C" (`KismetMathLibrary.MakeTransform` _returnvalue_location (`self.Actor Rotation`)) "Undefined" "MultiplyWithRoot" null null))))

(event `self.Box.OnComponentBeginOverlap`
  (params (OverlappedComponent :type "PrimitiveComponent Object Reference") (OtherActor :type "Actor Object Reference") (OtherComp :type "PrimitiveComponent Object Reference") (OtherBodyIndex :type Integer) (bFromSweep :type Boolean) (SweepResult :type "HitResult Structure (by ref)"))
  ;[0 0.9865 1 0.5] Change Spawn Rate Value
  ;;[0.1771 0.1771 0.1771] Add One Enemy to Spawn
  (if (== OtherActor (`GameplayStatics.GetPlayerCharacter` 0))
    (`/Engine/EditorBlueprintResources/StandardMacros.IncrementInt` (`self.Spawn Num`)
      (:`  `
        (`self.Event Update Spawn`)))))

(event `self.Box2.OnComponentBeginOverlap`
  (params (OverlappedComponent :type "PrimitiveComponent Object Reference") (OtherActor :type "Actor Object Reference") (OtherComp :type "PrimitiveComponent Object Reference") (OtherBodyIndex :type Integer) (bFromSweep :type Boolean) (SweepResult :type "HitResult Structure (by ref)"))
  ;[0 0.9865 1 0.5] Change Spawn Rate Value
  ;;[0.1771 0.1771 0.1771] Remove One Enemy to Spawn
  (if (== OtherActor (`GameplayStatics.GetPlayerCharacter` 0))
    (`/Engine/EditorBlueprintResources/StandardMacros.DecrementInt` (`self.Spawn Num`)
      (:`  `
        (`self.Event Update Spawn`)))))

(event `Event Update Spawn`
  ;[0 0.9865 1 0.5] Change Spawn Rate Value
  ;;[0.1771 0.1771 0.1771] Spawn Rate Value Text
  (`TextRenderComponent.K2_SetText` (`self.Nombre spawn`) (`KismetTextLibrary.Conv_IntToText` (`self.Spawn Num`))))

(fn `UserConstructionScript`)