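; BP_End_Button is a button, triggered by kicks or Light/Medium/Heavy-tagged hits, that either ends the game or spawns cheese, depending on IsChees.
; Both modes post a sound and a one-time Niagara explosion.
; Ending switches input mapping via PC_Systems, turns the view toward the button, and plays a level sequence.
; Cheese mode rains a random batch of suckable cheese above the player until CheeseMaxUse runs out.
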(event `self.ReceiveBeginPlay`
  (set `self.Spawn Count` (`KismetMathLibrary.RandomIntegerInRange` 25 35)))

(event `Event FeedBack`
  (bind (_returnvalue_location _returnvalue_rotation) (`KismetMathLibrary.BreakTransform` (`SceneComponent.K2_GetComponentToWorld` (`self.VFX Spawn`))))
  ;[1 1 1 0.5] FB
  ;[0.15 0 0.07811 0.5] END
  (`AkGameObject.PostAkEvent` :`self` (`self.Ak_Button`) :`AkEvent` "/Game/WwiseAudio/Events/Default_Work_Unit/SFX/SFX_GLOBAL/SFX_Cheese/SFX_ButtonCheese.SFX_ButtonCheese")
  (`/Engine/EditorBlueprintResources/StandardMacros.DoOnce` false
    (:`Completed`
      (bind _returnvalue (`NiagaraFunctionLibrary.SpawnSystemAtLocation` "/Game/VFX/Niagara/Props/NS_Small_Machine_Explosion.NS_Small_Machine_Explosion" _returnvalue_location _returnvalue_rotation))
      (`FXSystemComponent.SetFloatParameter` _returnvalue "SmokeSize" 400.0)
      (`FXSystemComponent.SetFloatParameter` _returnvalue "Sparks_Size" 2.0))))

(event `KickedInterface.Kicked`
  (params (KickVector :type "Vector Structure") (PlayerPosition :type "Vector Structure"))
  ; Get Hit by object or kick
  (if (`self.IsChees`)
    (`self.Trigger Chees`)
    (else
      (`self.Trigger End`))))

(event `HitInterface.GetHit`
  (params (Damage :type "Float (single-precision)") (HitStunDuration :type "Float (single-precision)") (KnockbackVector :type "Vector Structure") (InvincibilityTime :type "Float (single-precision)") (SourceActor :type "Actor Object Reference"))
  ; Get Hit by object or kick
  (if (or (`self.ActorHasTag` SourceActor "Light") (`self.ActorHasTag` SourceActor "Medium") (`self.ActorHasTag` SourceActor "Heavy"))
    (if (`self.IsChees`)
      (`self.Trigger Chees`)
      (else
        (`self.Trigger End`)))))

(event `Trigger End`
  ;[0.15 0 0.07811 0.5] END
  ;;[1 1 1 0.5] Ending Event
  (`self.Event FeedBack`)
  (`/Game/_GameManager/PC_Systems.SwitchIMC` (cast `/Game/_GameManager/PC_Systems` (`GameplayStatics.GetPlayerController` 0) :!pure true) true)
  (`Controller.SetControlRotation` (`GameplayStatics.GetPlayerController` 0) (`KismetMathLibrary.FindLookAtRotation` (`self.K2_GetActorLocation` (`GameplayStatics.GetPlayerPawn` 0)) (`self.K2_GetActorLocation`)))
  (bind (_outactor _returnvalue) (`LevelSequencePlayer.CreateLevelSequencePlayer` (`self.Level Sequence`)))
  (`MovieSceneSequencePlayer.Play` _returnvalue))

(event `Trigger Chees`
  (bind _returnvalue (`KismetMathLibrary.RandomFloatInRange` -50.0 50.0))
  (bind _cheesemaxuse (`self.CheeseMaxUse`))
  (bind _returnvalue_2 (`self.GetTransform` (`GameplayStatics.GetPlayerPawn` 0)))
  (set `self.CheeseMaxUse` (- _cheesemaxuse 1))
  (if (not (<= _cheesemaxuse 0))
    (`self.Event FeedBack`)
    (for _ (range (+ (`self.Spawn Count`) 1))
      (`|SpawnActorFromClass` "/Game/BPs/VacuumProps/BP_Suckable_Cheese.BP_Suckable_Cheese_C" (`KismetMathLibrary.MakeTransform` (`KismetMathLibrary.MakeVector` (+ _returnvalue (.x (.location _returnvalue_2))) (+ (.y (.location _returnvalue_2)) _returnvalue) (+ (.z (.location _returnvalue_2)) 150.0)) (.rotation _returnvalue_2)) "Undefined" "MultiplyWithRoot" null null))))

(fn `UserConstructionScript`)