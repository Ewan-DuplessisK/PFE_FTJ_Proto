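; BP_Duck is a collectible duck that registers with a BP_DucksMan manager, spawning one if none exists.
; Its Type sets the mesh tint and shine Niagara color, applied in the construction script and again at BeginPlay, when a looping Wwise aura also starts.
; DeactivateandStash, behind a DoOnce, turns off the shine, reports collection to the manager, awards score with a message and swaps the loop for pickup sounds.
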(event `self.ReceiveBeginPlay`
  (`parent.ReceiveBeginPlay`)
  (`/Game/BPs/BP_DucksMan.Register Duck` (`self.Get DucksMan`) self)
  (`self.Make`)
  ;[0.7708 0.1766 0.7483 0.5] Aura SFX
  (`AkGameObject.PostAkEvent` :`self` (`self.Ak_Duck`) :`AkEvent` "/Game/WwiseAudio/Events/Default_Work_Unit/SFX/SFX_GLOBAL/SFX_DUCK/SFX_Duck_LP.SFX_Duck_LP")
  (bind _output_get (set `self.BaseHealth` 100))
  (set `self.Health` _output_get))

(event `Make`
  (bind _returnvalue (`KismetMathLibrary.Conv_ColorToLinearColor` (`BlueprintMapLibrary.Map_Find` (`self.Type To Color`) (`self.Type`))))
  (set `self.Color` _returnvalue)
  (`MeshComponent.SetVectorParameterValueOnMaterials` (`self.StaticMeshComp`) "ColorTint" (`KismetMathLibrary.Conv_LinearColorToVector` _returnvalue))
  (`NiagaraComponent.SetVariableLinearColor` (`self.NS_DuckShine`) "Color" _returnvalue))

(event `self.ReceiveTick`
  (params (DeltaSeconds :type "Float (single-precision)")))

(event `self.DeactivateAndStash`
  (params (Location :type "Vector Structure"))
  ; legacy
  (`parent.DeactivateAndStash` Location)
  (`/Engine/EditorBlueprintResources/StandardMacros.DoOnce` false
    (:`Completed`
      (`ActorComponent.Deactivate` (`self.NS_DuckShine`))
      (`/Game/BPs/BP_DucksMan.Set Duck Collected` (`self.Get DucksMan`) self)
      ;; For Scoring if Needed
      (`FTJ_ScoringSystem_Score.IncreaseWithText` (subsystem `/Game/CppSystems/ScoringSystem/Public/Blueprint/BP_ScoringSystem_Score`) (`self.In Score Increase`) (`self.In Gauge Increase`) false (`|FormatText` "Collected Duck N°{x}" _))
      ;;[0.7708 0.1766 0.7483 0.5] Obtained_SFX
      (`GameplayStatics.PlaySound2D` "/Game/_GameManager/Feedbacks/Sounds/A_DuckObtained.A_DuckObtained" 1.0 1.0 0.0 null null)
      (`AkGameplayStatics.PostEvent` "/Game/WwiseAudio/Events/Default_Work_Unit/SFX/SFX_GLOBAL/SFX_DUCK/SFX_Duck.SFX_Duck")
      (`AkGameObject.PostAkEvent` :`self` (`self.Ak_Duck`) :`AkEvent` "/Game/WwiseAudio/Events/Default_Work_Unit/SFX/SFX_GLOBAL/SFX_DUCK/SFX_Stop_Duck_LP.SFX_Stop_Duck_LP"))))

(fn `Get DucksMan`
  (returns (DucksMan :type "/Game/BPs/BP_DucksMan Object Reference"))
  (bind _returnvalue (`GameplayStatics.GetActorOfClass` "/Game/BPs/BP_DucksMan.BP_DucksMan_C"))
  (`/Engine/EditorBlueprintResources/StandardMacros.IsValid` _returnvalue
    (:`Is Valid`
      (return _returnvalue))
    (:`Is Not Valid`
      (bind _returnvalue_2 (`|SpawnActorFromClass` "/Game/BPs/BP_DucksMan.BP_DucksMan_C" (`KismetMathLibrary.MakeTransform` (0.0 0.0 0.0)) "Undefined" "MultiplyWithRoot" null null))
      (return _returnvalue_2))))

(fn `UserConstructionScript`
  (`self.Make`))