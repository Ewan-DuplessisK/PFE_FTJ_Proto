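; Physics door that breaks apart when kicked, shot down or struck by fast heavy objects, other doors, or kicked chairs and carts.
; Damage updates a material "Anim" parameter until zero health routes into Kicked.
; Kicked spawns a BP_Door_Test Geometry Collection, awards score, triggers the fracture with the impulse, then destroys itself.
; Bound feedback events give kick breaks Wwise audio and player-side-oriented Niagara "CRACK" text; shot feedback is empty.
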(event `self.ReceiveBeginPlay`
  ;[1 0.9567 0 0.5 25] BEGIN PLAY
  (`self.Init Feedback`)
  (set `self.CurrentHealth` (`self.MaxHealth`)))

(event `KickedInterface.Kicked`
  (params (KickVector :type "Vector Structure") (PlayerPosition :type "Vector Structure"))
  ;[0 0.4075 1 0.5] What happens when you kick the door
  (bind _staticmesh (`self.StaticMesh`)
    (:`then`
      (bind _returnvalue (`self.Spawn Door Breakable` (`SceneComponent.K2_GetComponentLocation` _staticmesh) (`SceneComponent.K2_GetComponentRotation` _staticmesh)))
      (set `self.Fractured_Door` _returnvalue)
      (set `self.IsKicked` true)
      (set `self.Kick Strength` (* KickVector (`self.Impulse Strength`)))
      (`KismetSystemLibrary.DelayUntilNextTick`)
      (`/Engine/EditorBlueprintResources/StandardMacros.DoOnce` false
        (:`Completed`
          (`FTJ_ScoringSystem_Score.IncreaseWithText` (subsystem `/Game/CppSystems/ScoringSystem/Public/Blueprint/BP_ScoringSystem_Score`) (`KismetMathLibrary.Conv_IntToDouble` 10) 0.1 (`|FormatText` "Broke Door"))
          ;;[0.9716 1 0 0.5] Detect how the door is destroyed for sound play
          (if (`self.Destroyed_By_Shoot`)
            (`self.Destroy_By_Shot`)
            (else
              (`self.Destroy_By_Kick`)))
          (`KismetSystemLibrary.DelayUntilNextTick`)
          ;;[0.588 0.2765 0.599 0.5] Door Despawn after explosion
          (`/Game/BPs/GC_GCBP/test/BP_Door_Test.Trigger` (`self.Fractured_Door`) (`self.Kick Strength`) (`self.Despawn Time`))
          (`self.K2_DestroyActor`))))
    (:`else`)))

(event `self.ReceiveHit`
  (params (MyComp :type "PrimitiveComponent Object Reference") (Other :type "Actor Object Reference") (OtherComp :type "PrimitiveComponent Object Reference") (bSelfMoved :type Boolean) (HitLocation :type "Vector Structure") (HitNormal :type "Vector Structure") (NormalImpulse :type "Vector Structure") (Hit :type "HitResult Structure (by ref)"))
  (bind (_returnvalue_roll _returnvalue_pitch _returnvalue_yaw) (`KismetMathLibrary.BreakRotator` (`self.K2_GetActorRotation`)))
  ;[0.15 0 0 0.5] Event Hit
  (if (> (`KismetMathLibrary.VSize` (`self.GetVelocity` Other)) (`self.Velocity Threshold`))
    (if (or (`self.ActorHasTag` Other "Heavy") (`KismetStringLibrary.Contains` (`KismetSystemLibrary.GetDisplayName` Other) "Door") (and (`self.ActorHasTag` Other "Chair") (`self.ActorHasTag` Other "Kicked")) (and (`self.ActorHasTag` Other "Cart") (`self.ActorHasTag` Other "Kicked")))
      (if (!= _returnvalue_yaw -90.0)
        (`KickedInterface.Kicked` (* HitNormal 250.0))
        (else
          (`KickedInterface.Kicked` (* HitNormal -250.0)))))))

(event `HealthInterface.DamageBreakable`
  (params (Damage :type "Float (single-precision)") (Push :type "Vector Structure"))
  ;[1 1 1 0.5] Door receiving damages
  (bind _output_get (set `self.CurrentHealth` (`KismetMathLibrary.FClamp` (- (`self.CurrentHealth`) Damage) 0.0 (`self.MaxHealth`))))
  (`self.Door Damage Mat`)
  (if (<= _output_get 0.0)
    (`/Engine/EditorBlueprintResources/StandardMacros.DoOnce` false
      (:`Completed`
        (`KismetSystemLibrary.DelayUntilNextTick`)
        (set `self.Destroyed_By_Shoot` true)
        (`KickedInterface.Kicked` (* Push (* (`self.Impulse After 0HP`) -1.0)))))))

(event `Init Feedback`
  (`|ExecutionSequence`
    (:`then_0`
      (add `self.Kicked_Sound` (delegate `Kicked_Sound_Event`)))
    (:`then_1`
      (add `self.Destroy_By_Kick` (delegate `Destroy_By_Kick_Event`)))
    (:`then_2`
      (add `self.Destroy_By_Shot` (delegate `Destroy_By_Shot_Event`)))))

(event `Kicked_Sound_Event`)

(event `Destroy_By_Kick_Event`
  (bind _fx_location (`self.FX_Location`))
  (bind _returnvalue (`SceneComponent.K2_GetComponentLocation` _fx_location))
  (bind _returnvalue_2 (`SceneComponent.K2_GetComponentRotation` _fx_location))
  ;[0 1 1 0.5] FB - Sound when destroyed by kick
  (`AkGameplayStatics.PostEvent` "/Game/WwiseAudio/Events/Default_Work_Unit/MC/MC_KICK_WU/MC_Kick_Door.MC_Kick_Door" (`GameplayStatics.GetPlayerCharacter` 0))
  ;[0.8438 0.8438 0.8438 0.5] FX KRSHH
  (if (< (`KismetMathLibrary.Dot_VectorVector` (`SceneComponent.GetForwardVector` (`self.Arrow`)) (`KismetMathLibrary.Normal` (- (`self.K2_GetActorLocation` (cast `/Game/Characters/Player/Blueprints/BP_Player` (`GameplayStatics.GetPlayerCharacter` 0) :!pure true)) (`self.K2_GetActorLocation`)))) 0.0)
    (`NiagaraFunctionLibrary.SpawnSystemAtLocation` "/Game/VFX/Niagara/Text/NS_Text_CRACK.NS_Text_CRACK" _returnvalue (`KismetMathLibrary.MakeRotator` (.roll _returnvalue_2) (.pitch _returnvalue_2) (+ (.yaw _returnvalue_2) 270.0)))
    (else
      (`NiagaraFunctionLibrary.SpawnSystemAtLocation` "/Game/VFX/Niagara/Text/NS_Text_CRACK.NS_Text_CRACK" _returnvalue (`KismetMathLibrary.MakeRotator` (.roll _returnvalue_2) (.pitch _returnvalue_2) (+ (.yaw _returnvalue_2) 90.0))))))

(event `Destroy_By_Shot_Event`)

(fn `Door Damage Mat`
  (bind _returnvalue (`KismetMathLibrary.FClamp` (/ (`self.CurrentHealth`) (`self.MaxHealth`))))
  (`MeshComponent.SetScalarParameterValueOnMaterials` (`self.StaticMesh`) "Anim" (`KismetMathLibrary.SelectFloat` (/ _returnvalue 10.0) _returnvalue (<= _returnvalue 0.6))))

(fn `Spawn Door Breakable`
  (params (SpawnTransform_Location :type "Vector Structure") (`Spawn Transform Rotation` :type "Rotator Structure"))
  (returns (ReturnValue :type "/Game/BPs/GC_GCBP/test/BP_Door_Test Object Reference"))
  (bind _returnvalue (`|SpawnActorFromClass` "/Game/BPs/GC_GCBP/test/BP_Door_Test.BP_Door_Test_C" (`KismetMathLibrary.MakeTransform` SpawnTransform_Location `Spawn Transform Rotation`) "AlwaysSpawn" "MultiplyWithRoot" null null))
  (`MeshComponent.SetScalarParameterValueOnMaterials` (`/Game/BPs/GC_GCBP/test/BP_Door_Test.GeometryCollection` _returnvalue) "Anim" 0.0)
  (return _returnvalue))

(fn `UserConstructionScript`
  (set `self.CurrentHealth` (`self.MaxHealth`)))