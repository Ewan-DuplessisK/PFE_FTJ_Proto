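; Manager actor that plays prop impact, shooting and RTPC-driven Wwise sounds at requested locations through reusable emitters.
; On BeginPlay it spawns a pool of BP_PropSoundEmitter actors.
; Each request moves the emitter at UseIndex and plays the given event, or one looked up in EnumAk by prop type for impacts.
; UseIndex then advances round-robin, wrapping at EnumAk's length rather than the pool size.
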(event `self.ReceiveBeginPlay`
  (for _ (range 20)
    (bind _returnvalue (`|SpawnActorFromClass` "/Game/BPs/Sounds/BP_PropSoundEmitter.BP_PropSoundEmitter_C" (`self.GetTransform`) "Undefined" "MultiplyWithRoot" null null))
    (`KismetArrayLibrary.Array_AddUnique` (`self.PropsEmitters`) _returnvalue)))

(event `RequestImpactSound`
  (params (Type :type Byte) (Location :type "Vector Structure") (Speed :type "Float (double-precision)"))
  (bind _output (`|GetArrayItem` (`self.PropsEmitters`) (`self.UseIndex`)))
  (`self.K2_SetActorLocation` _output Location false false)
  (`/Game/BPs/Sounds/BP_PropSoundEmitter.PlayImpactSound` _output (`BlueprintMapLibrary.Map_Find` (`self.enum ak`) (cast `/Game/_GameManager/Data_Assets/E_Prop_Sounds` Type)) Speed)
  (set `self.UseIndex` (mod (+ (`self.UseIndex`) 1) (`BlueprintMapLibrary.Map_Length` (`self.enum ak`)))))

(event `RequestShootSound`
  (params (Location :type "Vector Structure") (Event :type "AkAudioEvent Object Reference"))
  (bind _output (`|GetArrayItem` (`self.PropsEmitters`) (`self.UseIndex`)))
  (`self.K2_SetActorLocation` _output Location false false)
  (`/Game/BPs/Sounds/BP_PropSoundEmitter.PlayEvent` _output Event)
  (set `self.UseIndex` (mod (+ (`self.UseIndex`) 1) (`BlueprintMapLibrary.Map_Length` (`self.enum ak`)))))

(event `RequestEventRTPC`
  (params (Event :type "AkAudioEvent Object Reference") (Location :type "Vector Structure") (Speed :type "Float (double-precision)") (RTPC :type "AkRtpc Object Reference"))
  (bind _output (`|GetArrayItem` (`self.PropsEmitters`) (`self.UseIndex`)))
  (`self.K2_SetActorLocation` _output Location false false)
  (`/Game/BPs/Sounds/BP_PropSoundEmitter.PlayEventWithRTPC` _output Event Speed RTPC)
  (set `self.UseIndex` (mod (+ (`self.UseIndex`) 1) (`BlueprintMapLibrary.Map_Length` (`self.enum ak`)))))

(fn `UserConstructionScript`)