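; BP_PropSoundEmitter is a Wwise sound emitter for props that plays events on its Ak component when called.
; PlayImpactSound sets the physics-object volume RTPC from a speed value before posting the event, so impact loudness can follow speed.
; PlayEvent posts a plain event, and PlayEventWithRTPC sets a caller-supplied RTPC from speed first.
; Each call posts only valid events, and the actor does nothing on its own.
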(event `PlayImpactSound`
  (params (Event :type "AkAudioEvent Object Reference") (Speed :type "Float (double-precision)"))
  (`AkGameObject.SetRTPCValue` (`self.Ak`) "/Game/WwiseAudio/Game_Parameters/GPE/RTPC_PhysicsObj_Volume.RTPC_PhysicsObj_Volume" Speed 0 "")
  (`/Engine/EditorBlueprintResources/StandardMacros.IsValid` Event
    (:`Is Valid`
      (`AkGameObject.PostAkEvent` :`self` (`self.Ak`) :`AkEvent` Event))))

(event `PlayEvent`
  (params (Event :type "AkAudioEvent Object Reference"))
  (`/Engine/EditorBlueprintResources/StandardMacros.IsValid` Event
    (:`Is Valid`
      (`AkGameObject.PostAkEvent` :`self` (`self.Ak`) :`AkEvent` Event))))

(event `PlayEventWithRTPC`
  (params (Event :type "AkAudioEvent Object Reference") (Speed :type "Float (double-precision)") (RTPC :type "AkRtpc Object Reference"))
  (`AkGameObject.SetRTPCValue` (`self.Ak`) RTPC Speed 0 "")
  (`/Engine/EditorBlueprintResources/StandardMacros.IsValid` Event
    (:`Is Valid`
      (`AkGameObject.PostAkEvent` :`self` (`self.Ak`) :`AkEvent` Event))))

(fn `UserConstructionScript`)