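; Actor component that makes its owning Character patrol endlessly along a referenced spline, in either direction via a Reverse flag.
; StartPatrol runs a looping timer that finds the closest spline point to the Character and steps ahead by a speed-scaled lookahead, wrapping at the spline's ends.
; The AI controller moves straight to that point without pathfinding, printing Failed or AlreadyAtGoal results; StopPatrol clears the timer.
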(event `self.ReceiveBeginPlay`
  (bind _ascharacter (cast `Character` (`self.GetOwner`))
    (:`then`
      (set `self.Character` _ascharacter))
    (:`CastFailed`
      (`KismetSystemLibrary.PrintString` "[AC_PatrolAlongSpline]: Actor should be Character"))))

(event `self.ReceiveEndPlay`
  (params (EndPlayReason :type "EEndPlayReason Enum" :default "Destroyed"))
  (set `self.Character` null))

(event `Start Patrol`
  (`self.Stop Patrol`)
  (`/Engine/EditorBlueprintResources/StandardMacros.IsValid` (`/Game/Characters/Enemies/Blueprints/BP_PatrolSpline.Spline` (`self.Patrol Spline`))
    (:`Is Valid`
      (bind _returnvalue (`KismetSystemLibrary.K2_SetTimerDelegate` (delegate `$ Patrol`) 0.2 true true))
      (set `self.Patrol Handle` _returnvalue))))

(event `Stop Patrol`
  (`KismetSystemLibrary.K2_ClearAndInvalidateTimerHandle` (`self.Patrol Handle`)))

(event `$ Patrol`
  (bind _character (`self.Character`))
  (bind _returnvalue (`KismetMathLibrary.SelectFloat` -1.0 1.0 (`self.Reverse`)))
  (bind _spline (`/Game/Characters/Enemies/Blueprints/BP_PatrolSpline.Spline` (`self.Patrol Spline`)))
  (bind _returnvalue_2 (`AIController.MoveToLocation` (`AIBlueprintHelperLibrary.GetAIController` (`self.Character`)) (`SplineComponent.GetLocationAtDistanceAlongSpline` _spline (`KismetMathLibrary.FWrap` (+ (`SplineComponent.GetDistanceAlongSplineAtSplineInputKey` _spline (`SplineComponent.FindInputKeyClosestToWorldLocation` _spline (`Actor.K2_GetActorLocation` _character))) (* (/ (`MovementComponent.GetMaxSpeed` (`Character.CharacterMovement` _character)) 5.0) _returnvalue) (* _returnvalue 70.0)) 0.0 (`SplineComponent.GetSplineLength` _spline)) "World") -1.0 true false false false null true))
  (`|ExecutionSequence`
    (:`then_1`
      (switch `EPathFollowingRequestResult` _returnvalue_2
        (:`Failed`
          _)
        (:`AlreadyAtGoal`
          _))
      (`KismetSystemLibrary.PrintString` (`|GetEnumeratorNameAsString` _returnvalue_2) true true (struct :`R` 1.0 :`B` 0.082418 :`A` 1.0)))))