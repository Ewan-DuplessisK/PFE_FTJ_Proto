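; Breakable statue that shatters when kicked or when damage empties its health, awarding score.
; Kicked swaps the mesh for a physics-driven geometry collection with impulse, sound and Niagara debris, then deactivates it after a delay.
; DamageBreakable updates a damage material and at zero health calls Kicked, adding its own score bonus.
; Door-derived leftovers remain: GetHit has no effect, feedback handlers are empty and fractured-door spawning never runs.
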(event `self.ReceiveBeginPlay`
  ;[1 0.9567 0 0.5 25] BEGIN PLAY
  (`self.Init Feedback`)
  (set `self.CurrentHealth` (`self.MaxHealth`)))

(event `self.Kicked`
  (params (KickVector :type "Vector Structure") (PlayerPosition :type "Vector Structure"))
  (bind _returnvalue (`KismetMathLibrary.Normal` KickVector))
  (bind _gc_sm_ceostatue (`self.GC_SM_CEOStatue`))
  (`/Engine/EditorBlueprintResources/StandardMacros.DoOnce` false
    (:`Completed`
      ;[0 0.4075 1 0.5] What happens when you kick the door
      (`FTJ_ScoringSystem_Score.IncreaseWithText` (subsystem `/Game/CppSystems/ScoringSystem/Public/Blueprint/BP_ScoringSystem_Score`) (`KismetMathLibrary.Conv_IntToDouble` 10) 0.1 false (`|FormatText` "Broke Statue (Kicked)"))
      (bind _staticmesh (`self.StaticMesh`)
        (:`then`
          (`AkGameplayStatics.PostEventAtLocation` "/Game/WwiseAudio/Events/Default_Work_Unit/MC/MC_KICK_WU/MC_Kick_Statue.MC_Kick_Statue" (`SceneComponent.K2_GetComponentLocation` (`self.StaticMesh`)))
          (`ActorComponent.K2_DestroyComponent` _staticmesh)
          (`ActorComponent.K2_DestroyComponent` (`self.Box`))
          (`SceneComponent.SetVisibility` _gc_sm_ceostatue true false)
          (`KismetSystemLibrary.DelayUntilNextTick`)
          (`PrimitiveComponent.SetSimulatePhysics` _gc_sm_ceostatue true)
          (`PrimitiveComponent.AddImpulse` _gc_sm_ceostatue (* _returnvalue (`self.Impulse Strength`)) "None" true)
          (bind _returnvalue_2 (`NiagaraFunctionLibrary.SpawnSystemAttached` "/Game/VFX/Niagara/Smoke/NS_Statue_Destruction.NS_Statue_Destruction" _staticmesh "None" (0.0 0.0 0.0) (struct) "KeepRelativeOffset" true))
          (`NiagaraComponent.SetVariableVec3` _returnvalue_2 "Velocity" _returnvalue)
          (`KismetSystemLibrary.Delay` 5.0)
          (`ActorComponent.Deactivate` _gc_sm_ceostatue)
          (`PrimitiveComponent.SetCollisionResponseToChannel` _gc_sm_ceostatue "ECC_PhysicsBody" "ECR_Ignore")
          (`PrimitiveComponent.PutRigidBodyToSleep` _gc_sm_ceostatue "None"))
        (:`else`)))))

(event `self.GetHit`
  (params (Damage :type "Float (single-precision)") (HitStunDuration :type "Float (single-precision)") (KnockbackVector :type "Vector Structure") (InvincibilityTime :type "Float (single-precision)") (SourceActor :type "Actor Object Reference"))
  (bind (_returnvalue_roll _returnvalue_pitch _returnvalue_yaw) (`KismetMathLibrary.BreakRotator` (`self.K2_GetActorRotation`)))
  ;[0.15 0 0 0.5] Event Hit
  (if (> (`KismetMathLibrary.VSize` (`self.GetVelocity` SourceActor)) (`self.Velocity Threshold`))
    (if (or (`self.ActorHasTag` SourceActor "Heavy") (`KismetStringLibrary.Contains` (`KismetSystemLibrary.GetDisplayName` SourceActor) "Door") (and (`self.ActorHasTag` SourceActor "Chair") (`self.ActorHasTag` SourceActor "Kicked")) (and (`self.ActorHasTag` SourceActor "Cart") (`self.ActorHasTag` SourceActor "Kicked")))
      (if (!= _returnvalue_yaw -90.0)
        _))))

(event `self.DamageBreakable`
  (params (Damage :type "Float (single-precision)") (Push :type "Vector Structure"))
  ;[1 1 1 0.5] Door receiving damages
  (bind _output_get (set `self.CurrentHealth` (`KismetMathLibrary.FClamp` (- (`self.CurrentHealth`) Damage) 0.0 (`self.MaxHealth`))))
  (`self.Door Damage Mat`)
  (if (<= _output_get 0.0)
    (`/Engine/EditorBlueprintResources/StandardMacros.DoOnce` false
      (:`Completed`
        (`KismetSystemLibrary.DelayUntilNextTick`)
        (set `self.Destroyed_By_Shoot` true)
        (`KickedInterface.Kicked` (* Push (`self.Impulse After 0HP`)))
        (`FTJ_ScoringSystem_Score.IncreaseWithText` (subsystem `/Game/CppSystems/ScoringSystem/Public/Blueprint/BP_ScoringSystem_Score`) (`KismetMathLibrary.Conv_IntToDouble` 100) 0.5 false (`|FormatText` "Broke Statue"))))))

(event `Init Feedback`
  (`|ExecutionSequence`
    (:`then_0`
      (add `self.Kicked_Sound` (delegate `Kicked_Sound_Event`)))
    (:`then_1`
      (add `self.Destroy_By_Kick` (delegate `Destroy_By_Kick_Event`)))
    (:`then_2`
      (add `self.Destroy_By_Shot` (delegate `Destroy_By_Shot_Event`)))))

(event `Kicked_Sound_Event`)

(event `Destroy_By_Kick_Event`)

(event `Destroy_By_Shot_Event`)

(fn `Door Damage Mat`
  (bind _returnvalue (`KismetMathLibrary.FClamp` (/ (`self.CurrentHealth`) (`self.MaxHealth`))))
  (`MeshComponent.SetScalarParameterValueOnMaterials` (`self.StaticMesh`) "Anim" (`KismetMathLibrary.SelectFloat` (/ _returnvalue 10.0) _returnvalue (<= _returnvalue 0.8))))

(fn `Spawn Door Breakable`
  (params (SpawnTransform_Location :type "Vector Structure") (`Spawn Transform Rotation` :type "Rotator Structure"))
  (returns (ReturnValue :type "/Game/BPs/GC_GCBP/test/BP_Door_Test Object Reference"))
  (bind _returnvalue (`|SpawnActorFromClass` "/Game/BPs/GC_GCBP/test/BP_Door_Test.BP_Door_Test_C" (`KismetMathLibrary.MakeTransform` SpawnTransform_Location `Spawn Transform Rotation`) "AlwaysSpawn" "MultiplyWithRoot" null null))
  (`MeshComponent.SetScalarParameterValueOnMaterials` (`/Game/BPs/GC_GCBP/test/BP_Door_Test.GeometryCollection` _returnvalue) "Anim" 0.0)
  (return _returnvalue))

(fn `UserConstructionScript`
  (set `self.CurrentHealth` (`self.MaxHealth`)))