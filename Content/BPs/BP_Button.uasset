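; BP_Button is an elevator button that is triggered by a kick or by a hit from an actor tagged Light, Medium or Heavy.
; Either trigger messages the Elevator to open and turns the button cube's material green, with the kick also playing a Wwise sound.
; A DoOnce limits the score and gauge reward and the break and spark Niagara effects to the first activation.
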(event `KickedInterface.Kicked`
  (params (KickVector :type "Vector Structure") (PlayerPosition :type "Vector Structure"))
  (`AkGameObject.PostAkEvent` :`self` (`self.AkGameObject`) :`AkEvent` "/Game/WwiseAudio/Events/Default_Work_Unit/MC/MC_Kick.MC_Kick")
  (message `/Game/BPs/TestProps/BPI/BPI_Elevator.Open_Elevator` (`self.Elevator`) :!label _label)
  (`PrimitiveComponent.SetMaterial` (`self.Cube`) 1 "/Game/Materials/Prototyping/Materials/MI_Green.MI_Green")
  (`/Engine/EditorBlueprintResources/StandardMacros.DoOnce` false
    (:`Completed`
      (`FTJ_ScoringSystem_Score.IncreaseWithText` (subsystem `/Game/CppSystems/ScoringSystem/Public/Blueprint/BP_ScoringSystem_Score`) (`KismetMathLibrary.Conv_IntToDouble` 20) 0.1 false (`|FormatText` "Elevator Button Pressed"))
      (`ActorComponent.Activate` (`self.NS_Machine_Break`) true)
      (`ActorComponent.Activate` (`self.NS_Burst_Spark_Loop`) true))))

(event `self.ReceiveHit`
  (params (MyComp :type "PrimitiveComponent Object Reference") (Other :type "Actor Object Reference") (OtherComp :type "PrimitiveComponent Object Reference") (bSelfMoved :type Boolean) (HitLocation :type "Vector Structure") (HitNormal :type "Vector Structure") (NormalImpulse :type "Vector Structure") (Hit :type "HitResult Structure (by ref)"))
  (if (or (`self.ActorHasTag` Other "Light") (`self.ActorHasTag` Other "Medium") (`self.ActorHasTag` Other "Heavy"))
    (goto _label)))

(fn `UserConstructionScript`)