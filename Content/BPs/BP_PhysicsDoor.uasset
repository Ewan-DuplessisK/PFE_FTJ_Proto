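; Kickable physics door that launches when kicked and shatters on impact, swapping its mesh for a spawned BP_Door_Fractured.
; Tag checks on hits decide when it breaks once, with a box overlap flagging when it is grounded.
; Grounded or Heavy hits fracture it with a temporary FS_MasterField, while other impacts pass the kick impulse to the Geometry Collection.
; The debris and actor despawn after a delay.
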(event `KickedInterface.Kicked`
  (params (KickVector :type "Vector Structure") (PlayerPosition :type "Vector Structure") (Damage :type "Float (single-precision)"))
  (bind _staticmesh (`self.StaticMesh`))
  ;[0 0.4075 1 0.5] What happend when you kicked the door
  (`PrimitiveComponent.SetSimulatePhysics` (`self.StaticMesh`) true)
  (set `self.IsKicked` true)
  (bind _output_get (set `self.Kick Strength` (* KickVector (`self.Impulse Strength`))))
  (`PrimitiveComponent.AddImpulse` _staticmesh _output_get "None" true)
  ;;[0 1 1 0.5] FB - Sound When Kicked
  (`GameplayStatics.PlaySoundAtLocation` (`self.Sound_When_Kicked`) (`SceneComponent.K2_GetComponentLocation` _staticmesh) (struct) 1.0 1.0 0.0 null null null null))

(event `self.ReceiveHit`
  (params (MyComp :type "PrimitiveComponent Object Reference") (Other :type "Actor Object Reference") (OtherComp :type "PrimitiveComponent Object Reference") (bSelfMoved :type Boolean) (HitLocation :type "Vector Structure") (HitNormal :type "Vector Structure") (NormalImpulse :type "Vector Structure") (Hit :type "HitResult Structure (by ref)"))
  (bind (_hit_location_x _hit_location_y _hit_location_z) (`KismetMathLibrary.BreakVector` (`self.Hit Location`)))
  (set `self.Hit Location` HitLocation)
  (if (and (not (`self.ActorHasTag` Other "Floor")) (not (`self.ActorHasTag` Other "Small")) (not (`self.ActorHasTag` Other "Medium")) (not (`self.ActorHasTag` Other "Player")))
    (if (not (`self.ActorHasTag` Other "Door"))
      (if (`self.ActorHasTag` Other "Heavy")
        (set `self.OnTheGround` true))
      (`/Engine/EditorBlueprintResources/StandardMacros.DoOnce` false :!label _label
        (:`Completed`
          (bind _returnvalue (`self.Spawn Door Breakable` (`SceneComponent.K2_GetComponentLocation` MyComp) (`SceneComponent.K2_GetComponentRotation` MyComp)))
          (bind _output_get (set `self.Fractured_Door` _returnvalue))
          (`|ExecutionSequence`
            (:`then_0`
              (if (`self.OnTheGround`)
                ;[0.15 0.06016 0.06016 0.5] Breaking System when the door fell to the ground
                (bind _returnvalue_2 (`|SpawnActorFromClass` "/Engine/EditorResources/FieldNodes/FS_MasterField.FS_MasterField_C" (`KismetMathLibrary.MakeTransform` (`KismetMathLibrary.MakeVector` _hit_location_x _hit_location_y (- _hit_location_z 70.0)) (struct) (1.5 1.5 1.5)) "Undefined" "MultiplyWithRoot" null null))
                (set `/Engine/EditorResources/FieldNodes/FS_MasterField.ActivationType` "NewEnumerator4" _returnvalue_2)
                (`/Engine/EditorResources/FieldNodes/FS_MasterField.CE_Trigger` _returnvalue_2)
                (`KismetSystemLibrary.Delay` 0.2)
                (`self.K2_DestroyActor` _returnvalue_2)
                (`ActorComponent.K2_DestroyComponent` (`self.StaticMesh`))
                (`ActorComponent.K2_DestroyComponent` (`self.Box`))
                (else
                  ;[0.561 0 0.6979 0.5] Door Spawn & Explosion when hit something
                  (`PrimitiveComponent.AddImpulse` (`GeometryCollectionActor.GeometryCollectionComponent` _output_get) (/ (`self.Kick Strength`) 1.0) "None" true)
                  (`ActorComponent.K2_DestroyComponent` (`self.StaticMesh`))
                  (`ActorComponent.K2_DestroyComponent` (`self.Box`))
                  ;[0 1 1 0.5] FB - Sound When Break
                  (`GameplayStatics.PlaySoundAtLocation` (`self.Sound_When_Break`) (`self.K2_GetActorLocation` (`self.Fractured_Door`)) (struct) 1.0 1.0 0.0 null null null null))))
            (:`then_1`
              ;[0.588 0.2765 0.599 0.5] Door Despawn after explosion
              (`KismetSystemLibrary.Delay` (`self.Dispawn Time`))
              (`self.K2_DestroyActor` (`self.Fractured_Door`))
              (`self.K2_DestroyActor`))))))
    (elif (`self.OnTheGround`)
      (goto _label))))

(event `self.Box.OnComponentBeginOverlap`
  (params (OverlappedComponent :type "PrimitiveComponent Object Reference") (OtherActor :type "Actor Object Reference") (OtherComp :type "PrimitiveComponent Object Reference") (OtherBodyIndex :type Integer) (bFromSweep :type Boolean) (SweepResult :type "HitResult Structure (by ref)"))
  ;[0.2381 0.4375 0.1442 0.5] Floor Detection
  (if (or (`self.ActorHasTag` OtherActor "Floor") (`self.ActorHasTag` OtherActor "Door"))
    (set `self.OnTheGround` true)))

(fn `Spawn Door Breakable`
  (params (SpawnTransform_Location :type "Vector Structure") (`Spawn Transform Rotation` :type "Rotator Structure"))
  (returns (ReturnValue :type "/Game/BPs/GC_GCBP/Door/BP_Door_Fractured Object Reference"))
  (bind _returnvalue (`|SpawnActorFromClass` "/Game/BPs/GC_GCBP/Door/BP_Door_Fractured.BP_Door_Fractured_C" (`KismetMathLibrary.MakeTransform` SpawnTransform_Location `Spawn Transform Rotation`) "AlwaysSpawn" "MultiplyWithRoot" null null))
  (return _returnvalue))

(fn `UserConstructionScript`)