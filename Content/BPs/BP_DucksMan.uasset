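; Duck collection manager that tracks which duck types in the level have been collected.
; On BeginPlay it finds every BP_Duck and seeds a type-to-collected map with false, and ducks can also register their type.
; Collecting a duck flags its type and shows its color on the scoring widget through PC_Systems.
; It also looks up colors by type and counts collected types.
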(event `self.ReceiveBeginPlay`
  (bind _outactors (`GameplayStatics.GetAllActorsOfClass` "/Game/BPs/BP_Duck.BP_Duck_C"))
  (for _array_element _outactors
    (`BlueprintMapLibrary.Map_Add` (`self.Collected Ducks Types`) (`/Game/BPs/BP_Duck.Type` _array_element))))

(fn `Get Color`
  (params (Type :type "/Game/BPs/E_DuckType Enum" :default "NewEnumerator0"))
  (returns (Color :type "Color Structure"))
  (locals (Blue :type "Color Structure" :default (struct :`B` 255 :`G` 255 :`R` 2 :`A` 255)) (Green :type "Color Structure" :default (struct :`G` 255 :`R` 85 :`A` 255)) (Red :type "Color Structure" :default (struct :`G` 22 :`R` 255 :`A` 255)) (Yellow :type "Color Structure" :default (struct :`G` 231 :`R` 255 :`A` 255)))
  (return (`BlueprintMapLibrary.Map_Find` (`self.Type To Color`) Type)))

(fn `GetDucksCollectedNumber`
  (returns (Num :type Integer))
  (locals (TmpNumber :type Integer))
  (bind (_keypin _valuepin) (`|MapForEach` (`self.Collected Ducks Types`))
    (:`then`
      (if _valuepin
        (`/Engine/EditorBlueprintResources/StandardMacros.IncrementInt` (`local.TmpNumber`))))
    (:`CompletedPin`
      (return (`local.TmpNumber`)))))

(fn `Register Duck`
  (params (Duck :type "/Game/BPs/BP_Duck Object Reference"))
  (bind _collected_ducks_types (`self.Collected Ducks Types`))
  (bind _type (`/Game/BPs/BP_Duck.Type` Duck))
  (if (not (`.ReturnValue` (`BlueprintMapLibrary.Map_Find` _collected_ducks_types _type)))
    (`BlueprintMapLibrary.Map_Add` _collected_ducks_types _type)))

(fn `Set Duck Collected`
  (params (Duck :type "/Game/BPs/BP_Duck Object Reference"))
  (`BlueprintMapLibrary.Map_Add` (`self.Collected Ducks Types`) (`/Game/BPs/BP_Duck.Type` Duck) true)
  (`/Game/UI/Menus/InGameMenu/WBP_Scoring.Show Duck Collected` (`/Game/_GameManager/PC_Systems.WBP Scoring` (cast `/Game/_GameManager/PC_Systems` (`GameplayStatics.GetPlayerController` 0) :!pure true)) (`/Game/BPs/BP_Duck.Color` Duck)))

(fn `UserConstructionScript`)