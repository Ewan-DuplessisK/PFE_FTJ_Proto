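; Pressure plate that opens its linked doors when weighed down by the player or by actors whose display name contains "Chair" or "Heavy".
; Box overlaps maintain an array of occupants, so the plate releases only when the last one leaves.
; A timeline lerps the plate between raised and pressed positions, opening or closing every referenced door when it finishes.
; The construction script sizes the trigger box from the plate's scale and repositions the mesh.
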(event `self.ReceiveBeginPlay`
  (`KismetSystemLibrary.DelayUntilNextTick`)
  (bind _asbp_player (cast `/Game/Characters/Player/Blueprints/BP_Player` (`GameplayStatics.GetPlayerPawn` 0))
    (:`then`
      (set `self.Player Ref` _asbp_player)
      (bind _output_get (set `self.UnPressedLocation` (`SceneComponent.RelativeLocation` (`self.Plate_Mesh`))))
      (set `self.Pressed Location` (- _output_get (`KismetMathLibrary.MakeVector` 0.0 0.0 (`self.Plate Offset`))))
      (if (`KismetArrayLibrary.Array_IsEmpty` (`self.Door Ref`))
        (`KismetSystemLibrary.PrintString` "Missing Door Ref in Pressure Plate" true true (struct :`R` 1.0 :`A` 1.0) 20.0)))
    (:`CastFailed`
      (`KismetSystemLibrary.PrintString` "Invalid Player Ref in Pressure Plate" true true (struct :`R` 1.0 :`A` 1.0) 10.0))))

(event `self.Box.OnComponentBeginOverlap`
  (params (OverlappedComponent :type "PrimitiveComponent Object Reference") (OtherActor :type "Actor Object Reference") (OtherComp :type "PrimitiveComponent Object Reference") (OtherBodyIndex :type Integer) (bFromSweep :type Boolean) (SweepResult :type "HitResult Structure (by ref)"))
  (bind _returnvalue (`KismetSystemLibrary.GetDisplayName` OtherActor))
  (bind _door_ref (`self.Door Ref`))
  (if (or (== OtherActor (`self.Player Ref`)) (`KismetStringLibrary.Contains` _returnvalue "Chair" false true) (`KismetStringLibrary.Contains` _returnvalue "Heavy" false true))
    (`KismetArrayLibrary.Array_AddUnique` (`self.Other Actor`) OtherActor)
    (if (not (`self.IsPressed`))
      (set `self.IsPressed` true)
      (bind (_direction _alpha) (`Timeline|T_PlateMove` :!label _label)
        (:`Update`
          (`SceneComponent.K2_SetRelativeLocation` (`self.Plate_Mesh`) (`KismetMathLibrary.VLerp` (`self.UnPressedLocation`) (`self.Pressed Location`) _alpha) false false))
        (:`Finished`
          (if (`self.IsPressed`)
            (for _array_element _door_ref
              (`/Game/BPs/Arena/BP_Arena_Door.Open Door` _array_element))
            (else
              (for _array_element_2 _door_ref
                (`/Game/BPs/Arena/BP_Arena_Door.Close Door` _array_element_2)))))))))

(event `self.Box.OnComponentEndOverlap`
  (params (OverlappedComponent :type "PrimitiveComponent Object Reference") (OtherActor :type "Actor Object Reference") (OtherComp :type "PrimitiveComponent Object Reference") (OtherBodyIndex :type Integer))
  (bind _other_actor (`self.Other Actor`))
  (if (`KismetArrayLibrary.Array_Contains` _other_actor OtherActor)
    (`KismetArrayLibrary.Array_RemoveItem` _other_actor OtherActor)
    (if (and (`self.IsPressed`) (`KismetArrayLibrary.Array_IsEmpty` _other_actor))
      (set `self.IsPressed` false)
      (goto _label :!via `Reverse`))))

(fn `UserConstructionScript`
  (bind (_boxextent_x _boxextent_y _boxextent_z) (`KismetMathLibrary.BreakVector` (`BoxComponent.BoxExtent` (`self.Box`))))
  (bind (_returnvalue_x _returnvalue_y) (`KismetMathLibrary.BreakVector` (* (40.0 40.0 50.0) (`SceneComponent.RelativeScale3D` (`self.Plate_Mesh`)))))
  (`BoxComponent.SetBoxExtent` (`self.Box`) (`KismetMathLibrary.MakeVector` _returnvalue_x _returnvalue_y 50.0) true)
  (`SceneComponent.K2_SetRelativeLocation` (`self.Plate_Mesh`) (`KismetMathLibrary.MakeVector` 0.0 0.0 (* (- _boxextent_z 2.5) -1.0)) false false))