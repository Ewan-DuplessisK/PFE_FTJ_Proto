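; Breakable plant prop that turns into a trash pile and awards score when destroyed.
; Damage, kicks or box overlaps from actors tagged Heavy, Medium or Light trigger a one-time break that disables collision and swaps the mesh.
; The OnHit dispatcher, bound at BeginPlay, drives feedback: Wwise sound, score and gauge increase, mesh rescale, and Niagara debris fed by a DataTable.
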(event `self.ReceiveBeginPlay`
  (`self.Init Feedback`))

(event `HealthInterface.DamageBreakable`
  (params (Damage :type "Float (single-precision)") (Push :type "Vector Structure"))
  (set `self.Is Broken` true :!label _label)
  (`/Engine/EditorBlueprintResources/StandardMacros.DoOnce` false
    (:`Completed`
      (`self.On Hit`)
      (`PrimitiveComponent.SetCollisionEnabled` (`self.Box`) "NoCollision")
      (`StaticMeshComponent.SetStaticMesh` (`self.StaticMesh`) "/Game/Environment/Office/Meshes/SmallAssets/Plants/SM_PileOfTrash.SM_PileOfTrash"))))

(event `self.Box.OnComponentBeginOverlap`
  (params (OverlappedComponent :type "PrimitiveComponent Object Reference") (OtherActor :type "Actor Object Reference") (OtherComp :type "PrimitiveComponent Object Reference") (OtherBodyIndex :type Integer) (bFromSweep :type Boolean) (SweepResult :type "HitResult Structure (by ref)"))
  (if (or (`self.ActorHasTag` OtherActor "Heavy") (`self.ActorHasTag` OtherActor "Medium") (`self.ActorHasTag` OtherActor "Light"))
    (goto _label)))

(event `KickedInterface.Kicked`
  (params (KickVector :type "Vector Structure") (PlayerPosition :type "Vector Structure"))
  (goto _label))

(event `Init Feedback`
  (`|ExecutionSequence`
    (:`then_0`
      (add `self.On Hit` (delegate `On Hit_Event`)))))

(event `On Hit_Event`
  (bind _staticmesh (`self.StaticMesh`))
  (bind _returnvalue (`SceneComponent.K2_GetComponentLocation` _staticmesh))
  (bind _returnvalue_2 (`SceneComponent.K2_GetComponentRotation` _staticmesh))
  ;[0 1 1 0.5] Sound When Hit
  (`AkGameObject.PostAkEvent` :`self` (`self.Ak_Conditioner`) :`AkEvent` "/Game/WwiseAudio/Events/Default_Work_Unit/SFX/SFX_GLOBAL/SFX_DESTRUCTION/SFX_Pot_Destruction.SFX_Pot_Destruction")
  ;[0 1 1] VFX
  (`NiagaraFunctionLibrary.SpawnSystemAtLocation` (`self.VFX When Hit`) (+ _returnvalue (0.0 -20.0 50.0)) _returnvalue_2)
  (bind _returnvalue_3 (`NiagaraFunctionLibrary.SpawnSystemAtLocation` "/Game/VFX/Niagara/Props/NS_Props_Break.NS_Props_Break" _returnvalue _returnvalue_2))
  (`/Game/VFX/Blueprint/BPFL_FX_DataTable_To_BreakableProp.SendBreakablePropDataToNiagara` (`self.DT_Positions`) _returnvalue_3 (`self.Array Mesh Renderer`) (`self.FX_Material`))
  (`FTJ_ScoringSystem_Score.IncreaseWithText` (subsystem `/Game/CppSystems/ScoringSystem/Public/Blueprint/BP_ScoringSystem_Score`) (`KismetMathLibrary.Conv_IntToDouble` 10) 0.2 false (`|FormatText` "Broke Plant"))
  (`SceneComponent.SetRelativeScale3D` (`self.StaticMesh`) (3.0 3.0 3.0)))

(fn `UserConstructionScript`)