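; Breakable lab screen prop that awards score once when destroyed by damage or a kick.
; Construction script picks one of four mesh and glass variants and configures a dynamic glass material for texture, tint and UVs, with optional material override.
; Unless single-texture, a randomly staggered looping timer cycles textures.
; Non-lethal hits play a glitch timeline on the shader; breaking sets its broken state and spawns an explosion.
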(event `self.ReceiveBeginPlay`
  (set `self.Current_Health` (`self.Max Health`))
  (if (not (`self.One texture ?`))
    (bind _returnvalue (`KismetSystemLibrary.K2_SetTimerDelegate` (delegate `Animation`) 5.0 true true 0.0 2.5))
    (set `self.Animation Handle` _returnvalue)))

(event `Animation`
  (bind _output_get (set `self.Texture Nb` (mod (+ (`self.Texture Nb`) 1) (`KismetArrayLibrary.Array_Length` (`self.3 Textures Switching`)))))
  (`MaterialInstanceDynamic.SetTextureParameterValue` (`self.Dynamic Screen`) "Texture" (`|GetArrayItem` (`self.3 Textures Switching`) _output_get)))

(event `Shader_Anim`
  (bind (_direction _newtrack_0) (`Timeline|Glitch` :!via `PlayFromStart`)
    (:`Update`
      (`MaterialInstanceDynamic.SetScalarParameterValue` (`self.Dynamic Screen`) "Broken State" _newtrack_0))))

(event `KickedInterface.Kicked`
  (params (KickVector :type "Vector Structure") (PlayerPosition :type "Vector Structure"))
  (`/Engine/EditorBlueprintResources/StandardMacros.DoOnce` false :!label _label
    (:`Completed`
      (`MaterialInstanceDynamic.SetScalarParameterValue` (`self.Dynamic Screen`) "Broken State" 1.0)
      (`NiagaraFunctionLibrary.SpawnSystemAtLocation` "/Game/VFX/Niagara/Props/NS_Machine_Explosion.NS_Machine_Explosion" (`self.K2_GetActorLocation`))
      (`/Engine/EditorBlueprintResources/StandardMacros.DoOnce` false
        (:`Completed`
          (`FTJ_ScoringSystem_Score.IncreaseWithText` (subsystem `/Game/CppSystems/ScoringSystem/Public/Blueprint/BP_ScoringSystem_Score`) (`KismetMathLibrary.Conv_IntToDouble` 30) 0.3 false (`|FormatText` "Broke Big Screen")))))))

(event `HealthInterface.DamageBreakable`
  (params (Damage :type "Float (single-precision)") (Push :type "Vector Structure"))
  (`AkGameObject.PostAkEvent` :`self` (`self.Ak_SFX_Tv`) :`AkEvent` "/Game/WwiseAudio/Events/Default_Work_Unit/SFX/SFX_GLOBAL/SFX_DESTRUCTION/SFX_TV_Break.SFX_TV_Break")
  (bind _output_get (set `self.Current_Health` (`KismetMathLibrary.FClamp` (- (`self.Current_Health`) Damage) 0.0 (`self.Max Health`))))
  (if (<= _output_get 0.0)
    (goto _label)
    (else
      (`self.Shader_Anim`)
      (`AkGameObject.PostAkEvent` :`self` (`self.Ak_SFX_Tv`) :`AkEvent` "/Game/WwiseAudio/Events/Default_Work_Unit/SFX/SFX_GLOBAL/SFX_TV/SFX_TV_Hits.SFX_TV_Hits"))))

(fn `UserConstructionScript`
  (locals (NewLocalVar :type "LinearColor Structure"))
  (switch `/Game/BPs/TestProps/Enums/E_Screen_Lab` (`self.Screen Type`)
    (:`NewEnumerator0`
      (`StaticMeshComponent.SetStaticMesh` (`self.Screen Mesh`) (`self.SM_Lab_Bigscreen_01`))
      (`StaticMeshComponent.SetStaticMesh` (`self.Screen Glass`) (`self.SM_Lab_Bigscreen_glass_01`)))
    (:`NewEnumerator1`
      (`StaticMeshComponent.SetStaticMesh` (`self.Screen Mesh`) (`self.SM_Lab_Bigscreen_02`))
      (`StaticMeshComponent.SetStaticMesh` (`self.Screen Glass`) (`self.SM_Lab_Bigscreen_glass_02`)))
    (:`NewEnumerator2`
      (`StaticMeshComponent.SetStaticMesh` (`self.Screen Mesh`) (`self.SM_Lab_Bigscreen_03`))
      (`StaticMeshComponent.SetStaticMesh` (`self.Screen Glass`) (`self.SM_Lab_Bigscreen_glass_03`)))
    (:`NewEnumerator3`
      (`StaticMeshComponent.SetStaticMesh` (`self.Screen Mesh`) (`self.SM_Lab_Bigscreen_04`))
      (`StaticMeshComponent.SetStaticMesh` (`self.Screen Glass`) (`self.SM_Lab_Bigscreen_glass_04`))))
  (bind _returnvalue (`PrimitiveComponent.CreateDynamicMaterialInstance` (`self.Screen Glass`) 0 null "None"))
  (bind _output_get (set `self.Dynamic Screen` _returnvalue))
  (`MaterialInstanceDynamic.SetTextureParameterValue` _output_get "Texture" (`self.Single Texture`))
  (set `self.One texture ?` (`self.One texture ?`))
  (`MaterialInstanceDynamic.SetVectorParameterValue` _output_get "Color_Mult" (`self.Color_Mult`))
  (`MaterialInstanceDynamic.SetVectorParameterValue` _output_get "UV_Tiling_Offset" (make `LinearColor` (`self.Tiling_X`) (`self.Tiling_Y`) (`self.Offset_X`) (`self.Offset_Y`)))
  (if (`self.Change Material?`)
    (`PrimitiveComponent.SetMaterial` (`self.Screen Glass`) 0 (`self.New Mat`))))