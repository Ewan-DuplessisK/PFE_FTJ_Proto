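; BP_HamsterWheel is a hamster wheel prop that plays a sound and spins when kicked.
; The Kicked event posts a Wwise event, then a timeline lerps the wheel mesh's relative pitch through 360 degrees from its current value.
; BeginPlay creates and stores dynamic materials for the wheel and attachment meshes, which this graph never modifies.
; Disconnected projector kick, scoring and camera audio nodes remain in the graph and never run.
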(event `self.ReceiveBeginPlay`
  (bind _returnvalue (`PrimitiveComponent.CreateDynamicMaterialInstance` (`self.SM_HamsterWheel`) 0 null "None"))
  (set `self.Dyn_Mat_01` _returnvalue)
  (bind _returnvalue_2 (`PrimitiveComponent.CreateDynamicMaterialInstance` (`self.SM_HamsterWheel_Attachment`) 0 null "None"))
  (set `self.Dyn_Mat_02` _returnvalue_2))

(event `self.Kicked`
  (params (KickVector :type "Vector Structure") (PlayerPosition :type "Vector Structure"))
  (bind (_relative_rotation_roll _relative_rotation_pitch) (`KismetMathLibrary.BreakRotator` (`self.Relative Rotation`)))
  (`AkGameObject.PostAkEvent` :`self` (`self.Ak_Hamster`) :`AkEvent` "/Game/WwiseAudio/Events/Default_Work_Unit/MC/MC_KICK_WU/MC_Kick_Hamster_Wheel.MC_Kick_Hamster_Wheel")
  (set `self.Relative Rotation` (`SceneComponent.RelativeRotation` (`self.SM_HamsterWheel`)))
  (bind (_direction _newtrack_0) (`Timeline|TL_Rotation` :!via `PlayFromStart`)
    (:`Update`
      (`SceneComponent.K2_SetRelativeRotation` (`self.SM_HamsterWheel`) (`KismetMathLibrary.RLerp` (`KismetMathLibrary.MakeRotator` 0.0 _relative_rotation_pitch) (`KismetMathLibrary.MakeRotator` 0.0 (+ _relative_rotation_pitch 360.0)) _newtrack_0) false false))))

(fn `UserConstructionScript`)