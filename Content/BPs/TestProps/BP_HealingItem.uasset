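; BP_HealingItem is a pickup that heals the player when the player character overlaps its Collision_Sphere.
; On overlap it sends HealingValue to BP_Player through AddHealthMessage, waits a tick, posts the Wwise heal sound on the player and destroys itself.
; A current-versus-max health check is present, but both branches are empty, so pickup happens regardless of health.
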(event `self.Collision_Sphere.OnComponentBeginOverlap`
  (params (OverlappedComponent :type "PrimitiveComponent Object Reference") (OtherActor :type "Actor Object Reference") (OtherComp :type "PrimitiveComponent Object Reference") (OtherBodyIndex :type Integer) (bFromSweep :type Boolean) (SweepResult :type "HitResult Structure (by ref)"))
  (bind _asbp_player (cast `/Game/Characters/Player/Blueprints/BP_Player` (`GameplayStatics.GetPlayerCharacter` 0) :!pure true))
  (if (== OtherActor _asbp_player)
    (if (< (`FTJ_CharaBase.CurrentHealth` _asbp_player) (`FTJ_CharaBase.MaxHealth` _asbp_player))
      _
      (else
        _))
    (message `HealthInterface.AddHealth` _asbp_player (`self.Healing_Value`))
    (`KismetSystemLibrary.DelayUntilNextTick`)
    (`AkGameplayStatics.PostEvent` "/Game/WwiseAudio/Events/Default_Work_Unit/SFX/SFX_GLOBAL/SFX_UI/SFX_UI_Heal.SFX_UI_Heal" (`GameplayStatics.GetPlayerCharacter` 0))
    (`self.K2_DestroyActor`)))

(fn `UserConstructionScript`)