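; Breakable-style divider prop that reacts when hit and awards score, with its mesh picked from three variants in the construction script.
; DamageBreakable, or GetHit from a valid source not tagged Chair, plays a squash-and-stretch timeline and spawns a BONK effect above the prop.
; The timeline drives a scalar on a dynamic material instance rather than the transform.
; A DoOnce limits the score, gauge boost and message to the first hit.
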(event `self.ReceiveBeginPlay`
  (bind _returnvalue (`PrimitiveComponent.CreateDynamicMaterialInstance` (`self.SM_Divider`) 0 null "None"))
  (set `self.DynamicMaterial` _returnvalue))

(event `HealthInterface.DamageBreakable`
  (params (Damage :type "Float (single-precision)") (Push :type "Vector Structure"))
  (bind (_returnvalue_x _returnvalue_y _returnvalue_z) (`KismetMathLibrary.BreakVector` (`self.K2_GetActorLocation`)))
  (`|ExecutionSequence` :!label _label
    (:`then_0`
      (`|ExecutionSequence`
        (:`then_0`
          (bind (_direction _newtrack_0) (`Timeline|Squash And Stretch` :!via `PlayFromStart`)
            (:`Update`
              (`MaterialInstanceDynamic.SetScalarParameterValue` (`self.DynamicMaterial`) "Positions_Boing" _newtrack_0))))
        (:`then_2`
          (`NiagaraFunctionLibrary.SpawnSystemAtLocation` "/Game/VFX/Niagara/Text/NS_Text_BONK.NS_Text_BONK" (`KismetMathLibrary.MakeVector` _returnvalue_x _returnvalue_y (+ _returnvalue_z 100.0))))))
    (:`then_1`
      (`/Engine/EditorBlueprintResources/StandardMacros.DoOnce` false
        (:`Completed`
          (`FTJ_ScoringSystem_Score.IncreaseWithText` (subsystem `/Game/CppSystems/ScoringSystem/Public/Blueprint/BP_ScoringSystem_Score`) (`KismetMathLibrary.Conv_IntToDouble` 5) 0.05 false (`|FormatText` "Dividers Hit")))))))

(event `HitInterface.GetHit`
  (params (Damage :type "Float (single-precision)") (HitStunDuration :type "Float (single-precision)") (KnockbackVector :type "Vector Structure") (InvincibilityTime :type "Float (single-precision)") (SourceActor :type "Actor Object Reference"))
  (`/Engine/EditorBlueprintResources/StandardMacros.IsValid` SourceActor
    (:`Is Valid`
      (if (not (`self.ActorHasTag` SourceActor "Chair"))
        (goto _label)))))

(fn `UserConstructionScript`
  (bind _sm_divider (`self.SM_Divider`))
  (switch `/Game/BPs/TestProps/Enums/E_Dividers` (`self.Select Mesh`)
    (:`NewEnumerator1`
      (`StaticMeshComponent.SetStaticMesh` _sm_divider (`self.Divider_01`)))
    (:`NewEnumerator2`
      (`StaticMeshComponent.SetStaticMesh` _sm_divider (`self.Divider_02`)))
    (:`NewEnumerator3`
      (`StaticMeshComponent.SetStaticMesh` _sm_divider (`self.Divider_03`)))))