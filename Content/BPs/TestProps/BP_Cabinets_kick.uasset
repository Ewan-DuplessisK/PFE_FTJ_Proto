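; BP_Cabinets_kick is a drawer cabinet test prop with a Bounce event that animates a drawer sliding along its Y axis.
; BeginPlay caches the last drawer's relative location as the closed position.
; Bounce restarts a timeline whose curve interpolates the first drawer between that cached position and a fixed Y offset, so the moved drawer differs from the cached one.
; Nothing in this file calls Bounce.
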(event Custom|Event%20Bounce
  (bind _drawer_closed (Variables|Default|GetDrawer_Closed))
  (bind _bounce_01 (Timeline|TL_Bounce PlayFromStart)
    (:Update
      (Transformation|SetRelativeLocation (Variables|Default|GetSM_4DrawerCabinet_FirstDrawer_00) (Math|Vector|Lerp(Vector) _drawer_closed (+ (Math|Vector|MakeVector 0.0 2e+01 0.0) _drawer_closed) _bounce_01) false false))))

(event EventBeginPlay
  (Variables|Default|SetDrawer_Closed (Variables|/Script/Engine.SceneComponent|GetRelativeLocation (Variables|Default|GetSM_4DrawerCabinet_LastDrawer_00))))

(event Collision|EventActorBeginOverlap
  (params (OtherActor :type Actor%20Object%20Reference)))

(event EventTick
  (params (DeltaSeconds :type Float%20%28single-precision%29)))

(event Input|KeyboardEvents|DebugKeyE
  (params (Key :type Key%20Structure :default "None") (ActionValue :type Input%20Action%20Value%20Structure)))

(fn ConstructionScript)