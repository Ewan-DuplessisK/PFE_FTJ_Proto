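; Kickable projector prop that plays an old camera sound and projects a texture through a decal, positioned by the construction script.
; Each kick cycles the decal texture via a dynamic material, plays a kick sound and spawns a BONK Niagara effect.
; A timeline drives the squash-and-stretch material parameter; the light mask is zeroed if already moving and restored when it finishes.
; Only the first kick awards score and gauge.
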(event `self.ReceiveBeginPlay`
  (`AkGameObject.PostAkEvent` :`self` (`self.Ak_Projector`) :`AkEvent` "/Game/WwiseAudio/Events/Default_Work_Unit/AMB/AMB_LVL_OPEN_OFFICE_02/Sp_CameraOld_OFFICE_02.Sp_CameraOld_OFFICE_02")
  (bind _returnvalue (`PrimitiveComponent.CreateDynamicMaterialInstance` (`self.SM_Projector_Light`) 0 null "None"))
  (set `self.Dyn_Light` _returnvalue)
  (bind _returnvalue_2 (`PrimitiveComponent.CreateDynamicMaterialInstance` (`self.SM_Projector`) 0 null "None"))
  (set `self.DynamicMaterial` _returnvalue_2)
  (bind _returnvalue_3 (`DecalComponent.CreateDynamicMaterialInstance` (`self.Decal`)))
  (set `self.DynamicTxtMat` _returnvalue_3)
  (`MaterialInstanceDynamic.SetTextureParameterValue` (`self.DynamicTxtMat`) "Projected_Texture" (`|GetArrayItem` (`self.Textures`))))

(event `KickedInterface.Kicked`
  (params (KickVector :type "Vector Structure") (PlayerPosition :type "Vector Structure"))
  (`|ExecutionSequence`
    (:`then_0`
      (`AkGameObject.PostAkEvent` :`self` (`self.Ak_Projector`) :`AkEvent` "/Game/WwiseAudio/Events/Default_Work_Unit/MC/MC_KICK_WU/MC_Kick_Projector.MC_Kick_Projector")
      (`/Engine/EditorBlueprintResources/StandardMacros.IncrementInt` (`self.Kick_Nb`)
        (:`  `
          (bind _output_get (set `self.Texture_Nb` (mod (+ (`self.Texture_Nb`) 1) (`KismetArrayLibrary.Array_Length` (`self.Textures`)))))
          (`MaterialInstanceDynamic.SetTextureParameterValue` (`self.DynamicTxtMat`) "Projected_Texture" (`|GetArrayItem` (`self.Textures`) _output_get))
          (`|ExecutionSequence`
            (:`then_0`
              (bind (_direction _newtrack_0) (`Timeline|Squash And Stretch` :!via `PlayFromStart`)
                (:`Update`
                  (set `self.Moving` true)
                  (`MaterialInstanceDynamic.SetScalarParameterValue` (`self.DynamicMaterial`) "Positions_Boing" _newtrack_0))
                (:`Finished`
                  (set `self.Moving` false)
                  (`self.Light`))))
            (:`then_1`
              (if (`self.Moving`)
                (`MaterialInstanceDynamic.SetScalarParameterValue` (`self.Dyn_Light`) "Mask_Opacity" 0.0)))
            (:`then_2`
              (`NiagaraFunctionLibrary.SpawnSystemAtLocation` "/Game/VFX/Niagara/Text/NS_Text_BONK.NS_Text_BONK" (`self.K2_GetActorLocation`)))))))
    (:`then_1`
      ;[0.03001 0.7708 0.00126 0.5] Scoring
      (`/Engine/EditorBlueprintResources/StandardMacros.DoOnce` false
        (:`Completed`
          (`FTJ_ScoringSystem_Score.IncreaseWithText` (subsystem `/Game/CppSystems/ScoringSystem/Public/Blueprint/BP_ScoringSystem_Score`) (`KismetMathLibrary.Conv_IntToDouble` 10) 0.2 false (`|FormatText` "Kicked Projector")))))))

(event `Light`
  (if (not (`self.Moving`))
    (`MaterialInstanceDynamic.SetScalarParameterValue` (`self.Dyn_Light`) "Mask_Opacity" 10.0)))

(fn `UserConstructionScript`
  (bind _decal (`self.Decal`))
  (`SceneComponent.K2_SetRelativeLocation` _decal (`self.Projected_Image_Location`) false false)
  (`SceneComponent.SetRelativeScale3D` _decal (`self.New Scale`))
  (`SceneComponent.K2_SetRelativeRotation` _decal (`self.New Rotation`) false false))