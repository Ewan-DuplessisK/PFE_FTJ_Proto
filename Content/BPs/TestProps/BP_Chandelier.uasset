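; Breakable hanging prop (chandelier, labeled as a fan in sound and score feedback) that falls, damages what it hits and awards score.
; A kick or overlap by a weight-tagged actor releases its constraint and enables physics; its first Hit applies damage and destroys it.
; Dispatchers drive Wwise audio and Niagara effects, including debris fed by prop data.
; Vacuum force applies scaled impulses to the mesh.
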(event `self.ReceiveBeginPlay`
  (`self.Init Feedback`))

(event `self.Box.OnComponentBeginOverlap`
  (params (OverlappedComponent :type "PrimitiveComponent Object Reference") (OtherActor :type "Actor Object Reference") (OtherComp :type "PrimitiveComponent Object Reference") (OtherBodyIndex :type Integer) (bFromSweep :type Boolean) (SweepResult :type "HitResult Structure (by ref)"))
  ;[0 0.9505 1 0.5] Detection to destroy
  (`/Engine/EditorBlueprintResources/StandardMacros.DoOnce` false
    (:`Completed`
      (if (or (`self.ActorHasTag` OtherActor "Heavy") (`self.ActorHasTag` OtherActor "Medium") (`self.ActorHasTag` OtherActor "Light"))
        (set `self.Is Broken` true :!label _label)
        (`self.Falling Reset`)
        (`self.On Hit`)
        (`PrimitiveComponent.SetSimulatePhysics` (`self.Chandelier`) true)))))

(event `KickedInterface.Kicked`
  (params (KickVector :type "Vector Structure") (PlayerPosition :type "Vector Structure"))
  ;[0 0.9505 1 0.5] Detection to destroy
  (goto _label))

(event `self.ReceiveHit`
  (params (MyComp :type "PrimitiveComponent Object Reference") (Other :type "Actor Object Reference") (OtherComp :type "PrimitiveComponent Object Reference") (bSelfMoved :type Boolean) (HitLocation :type "Vector Structure") (HitNormal :type "Vector Structure") (NormalImpulse :type "Vector Structure") (Hit :type "HitResult Structure (by ref)"))
  ;[0.15 0.1469 0 0.5] Deal Damage under it when destroyed
  (if (`self.ActorHasTag` Other "Player")
    _
    (else
      _))
  (`/Engine/EditorBlueprintResources/StandardMacros.DoOnce` false
    (:`Completed`
      (`self.Dispawn Hit`)
      (message `HitInterface.GetHit` Other (`self.Break_Damage`) 0.0 (0.0 0.0 0.0) 0.0 null)
      (`KismetSystemLibrary.DelayUntilNextTick`)
      (`self.K2_DestroyActor`))))

(event `self.ReactToVacuum`
  (params (Force :type "Vector Structure"))
  (`PrimitiveComponent.AddImpulse` (`self.Chandelier`) (* Force (`self.Vacuum_Effect_Force`)) "None" true))

(event `Falling Reset`
  (`PrimitiveComponent.SetConstraintMode` (`self.Chandelier`) "None"))

(event `Init Feedback`
  (`|ExecutionSequence`
    (:`then_0`
      (add `self.On Hit` (delegate `On Hit_Event`)))
    (:`then_1`
      (add `self.Dispawn Hit` (delegate `Dispawn Hit_Event`)))))

(event `On Hit_Event`
  (bind _chandelier (`self.Chandelier`))
  ;[0 1 1 0.5] Sound When Hit
  (`AkGameObject.PostAkEvent` :`self` (`self.Ak_Fan`) :`AkEvent` "/Game/WwiseAudio/Events/Default_Work_Unit/SFX/SFX_GLOBAL/SFX_DESTRUCTION/SFX_Metal_Destruction.SFX_Metal_Destruction")
  ;[0 1 1] VFX
  (bind _returnvalue (`NiagaraFunctionLibrary.SpawnSystemAtLocation` "/Game/VFX/Niagara/Props/NS_Small_Machine_Explosion.NS_Small_Machine_Explosion" (- (`SceneComponent.K2_GetComponentLocation` _chandelier) (0.0 0.0 70.0)) (`SceneComponent.K2_GetComponentRotation` _chandelier) (/ (`self.GetActorScale3D`) 5.0)))
  ; VFX Hit
  (set `self.HitVFX` _returnvalue)
  (`|ExecutionSequence`
    (:`then_0`
      (`PrimitiveComponent.SetSimulatePhysics` (`self.Chandelier`) true)
      (`KismetSystemLibrary.Delay` 2.0)
      (`/Engine/EditorBlueprintResources/StandardMacros.IsValid` _returnvalue
        (:`Is Valid`
          (`ActorComponent.K2_DestroyComponent` _returnvalue))))
    (:`then_1`
      (`KismetSystemLibrary.Delay` 1.5)
      (`ActorComponent.K2_DestroyComponent` (`self.HitVFX`)))))

(event `Dispawn Hit_Event`
  (bind _chandelier (`self.Chandelier`))
  (`AkGameplayStatics.PostEventAtLocation` "/Game/WwiseAudio/Events/Default_Work_Unit/SFX/SFX_GLOBAL/SFX_DESTRUCTION/SFX_Fan_Destruction.SFX_Fan_Destruction" (`SceneComponent.K2_GetComponentLocation` (`self.Ak_Fan`)))
  (`SceneComponent.SetVisibility` (`self.Chandelier`) false false)
  (`FTJ_ScoringSystem_Score.IncreaseWithText` (subsystem `/Game/CppSystems/ScoringSystem/Public/Blueprint/BP_ScoringSystem_Score`) (`KismetMathLibrary.Conv_IntToDouble` 10) 0.2 false (`|FormatText` "Broke Fan"))
  (bind _returnvalue (`NiagaraFunctionLibrary.SpawnSystemAtLocation` (`self.VFX When Hit`) (`SceneComponent.K2_GetComponentLocation` _chandelier) (`SceneComponent.K2_GetComponentRotation` _chandelier) (`self.GetActorScale3D`)))
  (bind _output_get (set `self.VFXSpawn` _returnvalue))
  (`NiagaraComponent.SetVariableVec3` _output_get "SmokePositionOffset" (0.0 0.0 -100.0))
  (`NiagaraComponent.SetVariableFloat` _output_get "SmokeLocationSize" 75.0)
  (`/Game/VFX/Blueprint/BPFL_FX_DataTable_To_BreakableProp.SendBreakablePropDataToNiagara` (`self.DT_Positions`) _output_get (`self.Array Mesh Renderer`) (`self.FX_Material`)))

(fn `UserConstructionScript`)