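; BP_Animated_Kick is a kickable prop, apparently a vending machine, that shakes and drops healing items.
; Kicked plays a timeline driving Positions_Boing on two material slots, creating dynamic material instances every update.
; It spawns BP_HealingItem at a randomized offset and yaw near HealingSpawnPoint while stock remains, then calls OnKicked.
; A Feedback graph binds that dispatcher to play smash sounds and electric VFX; the construction script applies NewMesh.
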(event `self.ReceiveBeginPlay`
  (`self.Init Feedback`))

(event `KickedInterface.Kicked`
  (params (KickVector :type "Vector Structure") (PlayerPosition :type "Vector Structure"))
  (`self.Shaking`)
  (`self.Spawn Heal`)
  (`self.On Kicked`))

(event `Shaking`
  (bind _mesh (`self.Mesh`))
  (bind (_direction _newtrack_0) (`Timeline|Shaking_TL` :!via `PlayFromStart`)
    (:`Update`
      (`|ExecutionSequence`
        (:`then_0`
          (bind _returnvalue (`PrimitiveComponent.CreateDynamicMaterialInstance` _mesh 0 (`PrimitiveComponent.GetMaterial` _mesh 0) "None"))
          (`MaterialInstanceDynamic.SetScalarParameterValue` _returnvalue "Positions_Boing" _newtrack_0))
        (:`then_1`
          (bind _returnvalue_2 (`PrimitiveComponent.CreateDynamicMaterialInstance` _mesh 1 (`PrimitiveComponent.GetMaterial` _mesh 1) "None"))
          (`MaterialInstanceDynamic.SetScalarParameterValue` _returnvalue_2 "Positions_Boing" _newtrack_0))))))

(event `Spawn Heal`
  (bind _returnvalue (`KismetMathLibrary.RandomFloatInRange` -50.0 50.0))
  (bind (_returnvalue_x _returnvalue_y _returnvalue_z) (`KismetMathLibrary.BreakVector` (`SceneComponent.K2_GetComponentLocation` (`self.Healing_SpawnPoint`))))
  (if (!= (`self.NumberOfHealAvailable`) 0)
    (`/Engine/EditorBlueprintResources/StandardMacros.DecrementInt` (`self.NumberOfHealAvailable`)
      (:`  `
        (`|SpawnActorFromClass` "/Game/BPs/TestProps/BP_HealingItem.BP_HealingItem_C" (`KismetMathLibrary.MakeTransform` (`KismetMathLibrary.MakeVector` (+ _returnvalue_x _returnvalue) (+ _returnvalue_y _returnvalue) _returnvalue_z) (`KismetMathLibrary.MakeRotator` 0.0 0.0 (`KismetMathLibrary.RandomFloatInRange` -90.0 90.0))) "AdjustIfPossibleButAlwaysSpawn" "MultiplyWithRoot" null 15.0 true null)))))

(event `Init Feedback`
  (`|ExecutionSequence`
    (:`then_0`
      (add `self.On Kicked` (delegate `On Kicked_Event`)))))

(event `On Kicked_Event`
  (bind _returnvalue (`SceneComponent.K2_GetComponentLocation` (`self.Mesh`)))
  ;[0 1 1 0.5] Sound When Kicked
  (`GameplayStatics.SpawnSoundAtLocation` "/Game/_GameManager/Feedbacks/Sounds/A_Vending_Smash.A_Vending_Smash" _returnvalue (struct) 1.0 1.0 0.0 null null)
  (`GameplayStatics.SpawnSoundAtLocation` "/Game/_GameManager/Feedbacks/Sounds/A_Vending_Kicked.A_Vending_Kicked" _returnvalue (struct) 1.0 1.0 0.0 null null)
  ;[0 1 1] Electric VFX
  (`NiagaraFunctionLibrary.SpawnSystemAtLocation` "/Game/VFX/Niagara/Props/NS_VendingMachine_Break.NS_VendingMachine_Break" (`self.K2_GetActorLocation`) (`self.K2_GetActorRotation`)))

(fn `UserConstructionScript`
  (`StaticMeshComponent.SetStaticMesh` (`self.Mesh`) (`self.New Mesh`)))