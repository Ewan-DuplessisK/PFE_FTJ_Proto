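; BP_NeonLight is a neon light prop that can blink by animating the red and green power of its material.
; On BeginPlay it creates a dynamic material instance on the neon mesh, then either starts the blink timeline if IsBlinking is set or zeroes both powers.
; The timeline drives Power_R and Power_G from its Blink and BlinkReverse tracks.
; StopBLINKING stops the timeline and sets both powers to zero.
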(event `Stop BLINKING`
  (bind _dynmatvar (`self.DynMatVar`))
  (`|ExecutionSequence`
    (:`then_0`
      (bind (_direction _blink _blink_reverse) (`Timeline|TL_Blinking` :!via `Stop` :!label _label)
        (:`Update`
          (`|ExecutionSequence`
            (:`then_0`
              (`MaterialInstanceDynamic.SetScalarParameterValue` _dynmatvar "Power_R" _blink))
            (:`then_1`
              (`MaterialInstanceDynamic.SetScalarParameterValue` _dynmatvar "Power_G" _blink_reverse))))))
    (:`then_1`
      (`MaterialInstanceDynamic.SetScalarParameterValue` (`self.DynMatVar`) "Power_R" 0.0 :!label _label_2)
      (`MaterialInstanceDynamic.SetScalarParameterValue` (`self.DynMatVar`) "Power_G" 0.0))))

(event `self.ReceiveBeginPlay`
  (bind _returnvalue (`PrimitiveComponent.CreateDynamicMaterialInstance` (`self.SM_Neonlight`) 0 null "None"))
  (set `self.DynMatVar` _returnvalue)
  (if (`self.Is Blinking`)
    (goto _label :!via `PlayFromStart`)
    (else
      (goto _label_2))))

(fn `UserConstructionScript`)