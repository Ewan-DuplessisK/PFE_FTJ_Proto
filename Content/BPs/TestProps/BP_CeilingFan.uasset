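; BP_CeilingFan is a breakable ceiling fan prop that spins at FanSpeed until a tagged object hits it.
; Overlaps from Heavy, Medium or Light actors flag it broken, fire the OnHit dispatcher, disable the box collision and stop rotation.
; The bound feedback handler plays sound and Niagara effects, hides the fan mesh, and awards score and multiplier through the player's scoring component.
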(event `self.ReceiveBeginPlay`
  (`self.Init Feedback`)
  (set `RotatingMovementComponent.RotationRate` (`KismetMathLibrary.MakeRotator` 0.0 0.0 (`self.Fan_Speed`)) (`self.RotatingMovement`)))

(event `self.Box.OnComponentBeginOverlap`
  (params (OverlappedComponent :type "PrimitiveComponent Object Reference") (OtherActor :type "Actor Object Reference") (OtherComp :type "PrimitiveComponent Object Reference") (OtherBodyIndex :type Integer) (bFromSweep :type Boolean) (SweepResult :type "HitResult Structure (by ref)"))
  (if (or (`self.ActorHasTag` OtherActor "Heavy") (`self.ActorHasTag` OtherActor "Medium") (`self.ActorHasTag` OtherActor "Light"))
    (set `self.Is Broken` true)
    (`self.On Hit`)
    (`PrimitiveComponent.SetCollisionEnabled` (`self.Box`) "NoCollision")
    (set `RotatingMovementComponent.RotationRate` (struct) (`self.RotatingMovement`))))

(event `Init Feedback`
  (`|ExecutionSequence`
    (:`then_0`
      (add `self.On Hit` (delegate `On Hit_Event`)))))

(event `On Hit_Event`
  (bind _fan (`self.Fan`))
  (bind _returnvalue (`SceneComponent.K2_GetComponentRotation` _fan))
  (bind _returnvalue_2 (/ (`self.GetActorScale3D`) 5.0))
  (bind _returnvalue_3 (- (`SceneComponent.K2_GetComponentLocation` _fan) (0.0 0.0 100.0)))
  ;[0 1 1 0.5] Sound When Hit
  (`GameplayStatics.SpawnSoundAtLocation` (`self.Sound When Hit`) (0.0 0.0 0.0) (struct) 1.0 1.0 0.0 null null)
  ;[0 1 1] VFX
  (`NiagaraFunctionLibrary.SpawnSystemAtLocation` (`self.VFX When Hit`) _returnvalue_3 _returnvalue _returnvalue_2)
  (`NiagaraFunctionLibrary.SpawnSystemAtLocation` "/Game/VFX/Niagara/Props/NS_VendingMachine_Break.NS_VendingMachine_Break" _returnvalue_3 _returnvalue _returnvalue_2)
  (`SceneComponent.SetVisibility` (`self.Fan`) false false)
  (`FTJ_ScoringSystem_Score.IncreaseWithText` (`self.GetComponentByClass` (`GameplayStatics.GetPlayerCharacter` 0) "/Game/ScoringSystem/Public/ActorComponent/BP_ScoringSystem_Score_AC.BP_ScoringSystem_Score_AC_C") 10 1 (`|FormatText` "Broke Fan")))

(fn `UserConstructionScript`)