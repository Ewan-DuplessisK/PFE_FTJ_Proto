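; Breakable robotic arm prop that tracks and snatches at a nearby player, built from static meshes chained by sockets in the construction script.
; A looping timer checks player range, while Tick blends interpolated look-at rotations with a grabbing timeline to animate joints and claws procedurally.
; Kicks or depleted health stop tracking and trigger timeline-driven recoil and collapse, with sound, explosion, temporary sparks and a one-time score reward.
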(event `Death Event`
  (bind _returnvalue (`SceneComponent.K2_GetComponentLocation` (`self.Zap Location`)))
  (`AkGameObject.PostAkEvent` :`self` (`self.Ak_SFX_RobotArm`) :`AkEvent` "/Game/WwiseAudio/Events/Default_Work_Unit/SFX/SFX_GLOBAL/SFX_ARMROBOT/SFX_ArmRobot_Dead.SFX_ArmRobot_Dead")
  (if (> (`self.NbKicks`) 1)
    ; Death
    (bind (_direction _ease_out _rebound) (`Timeline|Timeline_0` :!via `PlayFromStart` :!label _label)
      (:`Update`
        (`SceneComponent.K2_SetRelativeRotation` (`self.SM_RoboArm_01`) (`KismetMathLibrary.MakeRotator` 0.0 (* _ease_out -90.0)) false false)
        (`SceneComponent.K2_SetRelativeRotation` (`self.SM_RoboArm_02`) (`KismetMathLibrary.MakeRotator` 0.0 (* _ease_out -20.0)) false false)
        (`SceneComponent.K2_SetRelativeRotation` (`self.SM_RoboArm_03`) (`KismetMathLibrary.MakeRotator` 0.0 (* _rebound 20.0)) false false)
        (`SceneComponent.K2_SetRelativeRotation` (`self.SM_Claw_00`) (`KismetMathLibrary.MakeRotator` 0.0 (* _ease_out -120.0)) false false)
        (`SceneComponent.K2_SetRelativeRotation` (`self.SM_Claw_01`) (`KismetMathLibrary.MakeRotator` 0.0 (* _ease_out -110.0)) false false)
        (`SceneComponent.K2_SetRelativeRotation` (`self.SM_Claw_02`) (`KismetMathLibrary.MakeRotator` 0.0 (* _ease_out -90.0)) false false)
        (`SceneComponent.K2_SetRelativeRotation` (`self.SM_Claw_03`) (`KismetMathLibrary.MakeRotator` 0.0 (* _ease_out -115.0)) false false)))
    (else
      (`|ExecutionSequence`
        (:`then_0`
          (bind (_direction_2 _quick _quick_v2) (`Timeline|Timeline` :!via `PlayFromStart`)
            (:`Update`
              (set `self.PlayerIsInRange` false)
              (`SceneComponent.K2_SetRelativeRotation` (`self.SM_RoboRotating`) (`KismetMathLibrary.Conv_VectorToRotator` (stale `KickedInterface.Kicked` KickVector)) false false)
              (`SceneComponent.K2_SetRelativeRotation` (`self.SM_RoboArm_01`) (`KismetMathLibrary.MakeRotator` 0.0 (* _quick 20.0)) false false)
              (`SceneComponent.K2_SetRelativeRotation` (`self.SM_RoboArm_02`) (`KismetMathLibrary.MakeRotator` 0.0 (* _quick_v2 50.0)) false false)
              (`SceneComponent.K2_SetRelativeRotation` (`self.SM_RoboArm_03`) (`KismetMathLibrary.MakeRotator` 0.0 (* _quick 40.0)) false false)
              (set `self.Is_Dead` true))
            (:`Finished`
              (goto _label :!via `PlayFromStart`))))
        (:`then_1`
          (`NiagaraFunctionLibrary.SpawnSystemAtLocation` "/Game/VFX/Niagara/Props/NS_Machine_Explosion.NS_Machine_Explosion" _returnvalue)
          (bind _returnvalue_2 (`NiagaraFunctionLibrary.SpawnSystemAtLocation` "/Game/VFX/Niagara/Sparks/NS_ContinuousSparks.NS_ContinuousSparks" _returnvalue))
          (`KismetSystemLibrary.Delay` 5.0)
          (`ActorComponent.K2_DestroyComponent` _returnvalue_2))
        (:`then_2`
          (`/Engine/EditorBlueprintResources/StandardMacros.DoOnce` false
            (:`Completed`
              (`FTJ_ScoringSystem_Score.IncreaseWithText` (subsystem `/Game/CppSystems/ScoringSystem/Public/Blueprint/BP_ScoringSystem_Score`) (`KismetMathLibrary.Conv_IntToDouble` 30) 0.3 false (`|FormatText` "Broke RoboticArm")))))))))

(event `KickedInterface.Kicked`
  (params (KickVector :type "Vector Structure") (PlayerPosition :type "Vector Structure"))
  (`/Engine/EditorBlueprintResources/StandardMacros.IncrementInt` (`self.NbKicks`)
    (:`  `
      (set `self.Is Kicked` true)
      (`self.Death Event`))))

(event `HealthInterface.DamageBreakable`
  (params (Damage :type "Float (single-precision)") (Push :type "Vector Structure"))
  (bind _output_get (set `self.Current Health` (`KismetMathLibrary.FClamp` (- (`self.Current Health`) Damage) 0.0 (`self.Max Health`))))
  (if (<= _output_get 0.0)
    (set `self.Is Kicked` true)
    (`self.Death Event`)))

(event `self.ReceiveBeginPlay`
  (`KismetSystemLibrary.K2_SetTimerDelegate` (delegate `Refresh`) 0.05 true true))

(event `Refresh`
  (if (`self.Is Kicked`)
    _
    (elif (< (`KismetMathLibrary.VSize` (- (`self.K2_GetActorLocation` (`GameplayStatics.GetPlayerCharacter` 0)) (`self.K2_GetActorLocation`))) 700.0)
      (if (not (`self.PlayerIsInRange`))
        (set `self.PlayerIsInRange` true)
        (bind (_direction _quick _quick_v2 _slow _slow_v2 _quickv3) (`Timeline|TL_Grabbing` :!via `PlayFromStart` :!label _label_2)))
      (elif (`self.PlayerIsInRange`)
        (set `self.PlayerIsInRange` false)
        (goto _label_2 :!via `Stop`)))))

(event `self.ReceiveTick`
  (params (DeltaSeconds :type "Float (single-precision)"))
  (bind _returnvalue (`GameplayStatics.GetWorldDeltaSeconds`))
  (bind (_relativerotation_roll _relativerotation_pitch) (`KismetMathLibrary.BreakRotator` (`SceneComponent.RelativeRotation` (`self.SM_RoboArm_03`))))
  (bind (_relativerotation_roll_2 _relativerotation_pitch_2 _relativerotation_yaw) (`KismetMathLibrary.BreakRotator` (`SceneComponent.RelativeRotation` (`self.SM_RoboRotating`))))
  (bind (_relativerotation_roll_3 _relativerotation_pitch_3) (`KismetMathLibrary.BreakRotator` (`SceneComponent.RelativeRotation` (`self.SM_RoboArm_01`))))
  (bind (_relativerotation_roll_4 _relativerotation_pitch_4) (`KismetMathLibrary.BreakRotator` (`SceneComponent.RelativeRotation` (`self.SM_RoboArm_02`))))
  (bind (_returnvalue_roll _returnvalue_pitch _returnvalue_yaw) (`KismetMathLibrary.BreakRotator` (`KismetMathLibrary.FindLookAtRotation` (0.0 0.0 0.0) (`KismetMathLibrary.InverseTransformLocation` (`SceneComponent.K2_GetComponentToWorld` (`self.DefaultSceneRoot`)) (`self.K2_GetActorLocation` (`GameplayStatics.GetPlayerCharacter` 0))))))
  (bind (_returnvalue_roll_2 _returnvalue_pitch_2 _returnvalue_yaw_2) (`KismetMathLibrary.BreakRotator` (`KismetMathLibrary.RInterpTo` (`KismetMathLibrary.MakeRotator` 0.0 0.0 _relativerotation_yaw) (`KismetMathLibrary.MakeRotator` 0.0 0.0 _returnvalue_yaw) _returnvalue 5.0)))
  (if (`self.Is Kicked`)
    _
    (elif (`self.PlayerIsInRange`)
      (`SceneComponent.K2_SetRelativeRotation` (`self.SM_RoboRotating`) (`KismetMathLibrary.MakeRotator` 0.0 0.0 _returnvalue_yaw_2) false false)
      (`SceneComponent.K2_SetRelativeRotation` (`self.SM_RoboArm_01`) (`KismetMathLibrary.MakeRotator` 0.0 (+ (* (stale `Refresh` _slow) -10.0) (`KismetMathLibrary.FInterpTo` _relativerotation_pitch_3 (+ _returnvalue_pitch -100.0) _returnvalue 5.0))) false false)
      (`SceneComponent.K2_SetRelativeRotation` (`self.SM_RoboArm_02`) (`KismetMathLibrary.MakeRotator` 0.0 (+ (stale `Refresh` _quick_v2) (`KismetMathLibrary.FInterpTo` _relativerotation_pitch_4 _returnvalue_pitch _returnvalue 5.0))) false false)
      (`SceneComponent.K2_SetRelativeRotation` (`self.SM_RoboArm_03`) (`KismetMathLibrary.MakeRotator` 0.0 (+ (* (stale `Refresh` _quick) 5.0) (`KismetMathLibrary.FInterpTo` _relativerotation_pitch (+ _returnvalue_pitch 50.0) _returnvalue 5.0))) false false)
      (bind _returnvalue_2 (* (stale `Refresh` _quickv3) -100.0))
      (`SceneComponent.K2_SetRelativeRotation` (`self.SM_Claw_00`) (`KismetMathLibrary.MakeRotator` 0.0 _returnvalue_2) false false)
      (bind _returnvalue_3 (* (stale `Refresh` _quick) -85.0))
      (`SceneComponent.K2_SetRelativeRotation` (`self.SM_Claw_01`) (`KismetMathLibrary.MakeRotator` 0.0 _returnvalue_3) false false)
      (`SceneComponent.K2_SetRelativeRotation` (`self.SM_Claw_02`) (`KismetMathLibrary.MakeRotator` 0.0 _returnvalue_2) false false)
      (`SceneComponent.K2_SetRelativeRotation` (`self.SM_Claw_03`) (`KismetMathLibrary.MakeRotator` 0.0 _returnvalue_3) false false))))

(fn `UserConstructionScript`
  (set `StaticMeshSocket.RelativeRotation` (`self.Rotating Part Rota`) (`StaticMesh.FindSocket` (`StaticMeshComponent.StaticMesh` (`self.SM_RoboBase`)) "RotatingPart"))
  (`SceneComponent.K2_AttachToComponent` (`self.SM_RoboRotating`) (`self.SM_RoboBase`) "RotatingPart" "KeepRelative" "SnapToTarget" "KeepRelative" true)
  (`SceneComponent.K2_AttachToComponent` (`self.SM_RoboArm_01`) (`self.SM_RoboRotating`) "Arm_01" "KeepRelative" "SnapToTarget" "KeepRelative" true)
  (`SceneComponent.K2_AttachToComponent` (`self.SM_RoboArm_02`) (`self.SM_RoboArm_01`) "Arm_02" "KeepRelative" "SnapToTarget" "KeepRelative" true)
  (`SceneComponent.K2_AttachToComponent` (`self.SM_RoboArm_03`) (`self.SM_RoboArm_02`) "Arm_03" "KeepRelative" "SnapToTarget" "KeepRelative" true)
  (`SceneComponent.K2_AttachToComponent` (`self.SM_Claw_00`) (`self.SM_RoboArm_03`) "Claw_00" "KeepRelative" "SnapToTarget" "KeepRelative" true)
  (`SceneComponent.K2_AttachToComponent` (`self.SM_Claw_01`) (`self.SM_RoboArm_03`) "Claw_01" "KeepRelative" "SnapToTarget" "KeepRelative" true)
  (`SceneComponent.K2_AttachToComponent` (`self.SM_Claw_02`) (`self.SM_RoboArm_03`) "Claw_02" "KeepRelative" "SnapToTarget" "KeepRelative" true)
  (`SceneComponent.K2_AttachToComponent` (`self.SM_Claw_03`) (`self.SM_RoboArm_03`) "Claw_03" "KeepRelative" "SnapToTarget" "KeepRelative" true))