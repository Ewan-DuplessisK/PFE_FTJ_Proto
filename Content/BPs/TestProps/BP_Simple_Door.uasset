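; BP_Simple_Door is a test prop door that reacts to being kicked with a physics push on its static mesh.
; Kicked passes the kick vector to GetKicked, which stores it and sets a pushed flag for one second before clearing both.
; While the flag is set, Tick adds a scaled velocity-change impulse to the mesh every frame, so the push is sustained and frame-rate dependent.
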(event `self.ReceiveTick`
  (params (DeltaSeconds :type "Float (single-precision)"))
  (if (`self.IsPushed`)
    (`PrimitiveComponent.AddImpulse` (`self.StaticMesh`) (* (`self.ForceVector`) 20.0) "None" true)))

(event `GetKicked`
  (params (Vector :type "Vector Structure"))
  (set `self.ForceVector` Vector)
  (set `self.IsPushed` true)
  (`KismetSystemLibrary.Delay` 1.0)
  (set `self.ForceVector` (0.0 0.0 0.0))
  (set `self.IsPushed` false))

(event `KickedInterface.Kicked`
  (params (KickVector :type "Vector Structure") (PlayerPosition :type "Vector Structure"))
  (`self.GetKicked` KickVector))

(fn `UserConstructionScript`)