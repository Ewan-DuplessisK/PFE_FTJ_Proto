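; BP_LedLight is a breakable LED light prop that rewards the player with score when smashed.
; An object tagged Heavy, Medium or Light overlapping its box triggers a one-time break that fires OnHit, disables box collision and swaps in the broken mesh.
; The OnHit handler, bound at BeginPlay, plays destruction sound and VFX, activates looping sparks and increases score and gauge with a "Broke AirCo" message.
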(event `self.ReceiveBeginPlay`
  (`self.Init Feedback`))

(event `self.Box.OnComponentBeginOverlap`
  (params (OverlappedComponent :type "PrimitiveComponent Object Reference") (OtherActor :type "Actor Object Reference") (OtherComp :type "PrimitiveComponent Object Reference") (OtherBodyIndex :type Integer) (bFromSweep :type Boolean) (SweepResult :type "HitResult Structure (by ref)"))
  (if (or (`self.ActorHasTag` OtherActor "Heavy") (`self.ActorHasTag` OtherActor "Medium") (`self.ActorHasTag` OtherActor "Light"))
    (set `self.Is Broken` true)
    (`/Engine/EditorBlueprintResources/StandardMacros.DoOnce` false
      (:`Completed`
        (`self.On Hit`)
        (`PrimitiveComponent.SetCollisionEnabled` (`self.Box`) "NoCollision")
        (`StaticMeshComponent.SetStaticMesh` (`self.StaticMesh`) "/Game/Environment/Office/Meshes/Lights/SM_LedLight_01_Broken.SM_LedLight_01_Broken")))))

(event `self.GetHit`
  (params (Damage :type "Float (single-precision)") (HitStunDuration :type "Float (single-precision)") (KnockbackVector :type "Vector Structure") (InvincibilityTime :type "Float (single-precision)") (SourceActor :type "Actor Object Reference")))

(event `Init Feedback`
  (`|ExecutionSequence`
    (:`then_0`
      (add `self.On Hit` (delegate `On Hit_Event`)))))

(event `On Hit_Event`
  (bind _staticmesh (`self.StaticMesh`))
  ;[0 1 1 0.5] Sound When Hit
  (`AkGameObject.PostAkEvent` :`self` (`self.Ak_Conditioner`) :`AkEvent` "/Game/WwiseAudio/Events/Default_Work_Unit/SFX/SFX_GLOBAL/SFX_DESTRUCTION/SFX_Metal_Destruction.SFX_Metal_Destruction")
  ;[0 1 1] VFX
  (`NiagaraFunctionLibrary.SpawnSystemAtLocation` (`self.VFX When Hit`) (+ (`SceneComponent.K2_GetComponentLocation` _staticmesh) (0.0 -20.0 -40.0)) (`SceneComponent.K2_GetComponentRotation` _staticmesh) (/ (`self.GetActorScale3D`) 5.0))
  (`ActorComponent.Activate` (`self.NS_Burst_Spark_Loop`) false)
  (`ActorComponent.Activate` (`self.NS_Burst_Spark_Loop1`) false)
  (`FTJ_ScoringSystem_Score.IncreaseWithText` (subsystem `/Game/CppSystems/ScoringSystem/Public/Blueprint/BP_ScoringSystem_Score`) (`KismetMathLibrary.Conv_IntToDouble` 10) 0.2 (`|FormatText` "Broke AirCo")))

(fn `UserConstructionScript`)