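; Kickable physics fire extinguisher prop that flies away, leaks foam and explodes.
; A kick applies an impulse, then after a delay Tick adds thrust and random torque before an explosion with timeline-driven material deformation.
; Hitting another kickable prop while kicked swaps it for a chair-bottom actor with VFX; other non-player hits send damage.
; Event bindings trigger kick and break sounds; the vacuum handler is empty.
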(event `self.ReceiveBeginPlay`
  (`self.Init Feedback`))

(event `self.ReactToVacuum`
  (params (Force :type "Vector Structure"))
  ;[1 0 0.8709 0.5] VACCUM CHAIR
  (`self.Getting_Vaccumed_Event`))

(event `self.Kicked`
  (params (KickVector :type "Vector Structure") (PlayerPosition :type "Vector Structure"))
  (`self.Kicked_Sound_Event`)
  (set `self.IsKicked` true)
  (`KismetArrayLibrary.Array_Add` (`self.Tags`) "Kicked")
  (`PrimitiveComponent.AddImpulse` (`self.SM_Extinguisher_00`) (* KickVector (`self.Impulse_Value`)) "None" true)
  (`KismetSystemLibrary.Delay` 1.0)
  (set `self.IsKicked` false)
  (`KismetArrayLibrary.Array_RemoveItem` (`self.Tags`) "Kicked")
  (set `self.IsLeaking` true)
  (`KismetArrayLibrary.Array_Add` (`self.Tags`) "Leaking"))

(event `self.ReceiveTick`
  (params (DeltaSeconds :type "Float (single-precision)"))
  (if (`self.IsLeaking`)
    (`|ExecutionSequence`
      (:`then_0`
        (`PrimitiveComponent.AddForce` (`self.SM_Extinguisher_00`) (* (* (`SceneComponent.GetUpVector` (`self.SM_Extinguisher_00`)) (`KismetMathLibrary.Conv_DoubleToVector` -1.0)) (`self.Leaking_Speed`)) "None" true)
        (`PrimitiveComponent.AddTorqueInDegrees` (`self.SM_Extinguisher_00`) (* (`KismetMathLibrary.RandomUnitVector`) (`KismetMathLibrary.Conv_DoubleToVector` 2000.0)) "None" true)
        (`KismetSystemLibrary.Delay` 2.0)
        (set `self.IsLeaking` false)
        (set `self.IsExploding` true)
        (`self.Event Explode`))
      (:`then_1`
        (`ActorComponent.Activate` (`self.NS_Extinguisher_Foam`) false)))))

(event `Event Explode`
  (if (`self.IsExploding`)
    (`|ExecutionSequence`
      (:`then_0`
        (`KismetSystemLibrary.Delay` 2.5)
        (`ActorComponent.K2_DestroyComponent` (`self.SM_Extinguisher_00`))
        (`ActorComponent.Activate` (`self.NS_Explosion_Extinguisher`) false))
      (:`then_1`
        (bind _returnvalue (`PrimitiveComponent.CreateDynamicMaterialInstance` (`self.SM_Extinguisher_00`) 0 null "None"))
        (set `self.DynMatRef` _returnvalue)
        (bind (_direction _explosion) (`Timeline|TL_Explosion`)
          (:`Update`
            (`/Engine/EditorBlueprintResources/StandardMacros.IsValid` (`self.SM_Extinguisher_00`)
              (:`Is Valid`
                (`MaterialInstanceDynamic.SetScalarParameterValue` (`self.DynMatRef`) "Positions_Boing" _explosion)))))))))

(event `self.ReceiveHit`
  (params (MyComp :type "PrimitiveComponent Object Reference") (Other :type "Actor Object Reference") (OtherComp :type "PrimitiveComponent Object Reference") (bSelfMoved :type Boolean) (HitLocation :type "Vector Structure") (HitNormal :type "Vector Structure") (NormalImpulse :type "Vector Structure") (Hit :type "HitResult Structure (by ref)"))
  (bind _vfx_hit (`self.VFX_Hit`))
  (bind _chair (`self.Chair`))
  (bind _sm_extinguisher_00 (`self.SM_Extinguisher_00`))
  (bind _sm_extinguisher_00_2 (`self.SM_Extinguisher_00`))
  (bind _returnvalue (`self.K2_GetActorLocation` (`.HitActor` (`GameplayStatics.BreakHitResult` Hit))))
  ;[1 0.51 0 0.5] Chair hit "Prop Physics" and what happend
  (`/Engine/EditorBlueprintResources/StandardMacros.IsValid` (`self.GetComponentByClass` Other "/Game/CppSystems/Prop/Public/ActorComponent/BP_Prop_PhysicsKickableCompBase_AC.BP_Prop_PhysicsKickableCompBase_AC_C")
    (:`Is Valid`
      (if (`self.IsKicked`)
        (`|ExecutionSequence`
          (:`then_0`
            (`SceneComponent.SetHiddenInGame` _sm_extinguisher_00 true false)
            (`PrimitiveComponent.SetCollisionEnabled` _sm_extinguisher_00 "NoCollision")
            (`KismetSystemLibrary.Delay` 0.1)
            (`PrimitiveComponent.SetCollisionResponseToChannel` _sm_extinguisher_00 "ECC_Pawn" "ECR_Ignore")
            (`PrimitiveComponent.SetSimulatePhysics` _sm_extinguisher_00 false)
            (`PrimitiveComponent.SetCollisionEnabled` _sm_extinguisher_00 "NoCollision")
            (`ActorComponent.Deactivate` (`self.Hitbox`))
            (set `self.IsBroken` true)
            (set `self.Chair` (`SceneComponent.K2_GetComponentToWorld` _sm_extinguisher_00_2))
            (`ActorComponent.K2_DestroyComponent` _sm_extinguisher_00_2)
            (`KismetSystemLibrary.DelayUntilNextTick`)
            (bind _returnvalue_2 (`|SpawnActorFromClass` "/Game/BPs/VacuumProps/BP_ChairBottom_Medium.BP_ChairBottom_Medium_C" (`KismetMathLibrary.MakeTransform` (`KismetMathLibrary.MakeVector` (.x (.location _chair)) (.y (.location _chair)) (+ (.z (.location _chair)) 5.0)) (.rotation _chair) (.scale _chair)) "AlwaysSpawn" "MultiplyWithRoot" null null))
            (`KismetSystemLibrary.Delay` 0.15)
            (`PrimitiveComponent.SetSimulatePhysics` (`SuckablePropParent.StaticMeshComp` _returnvalue_2) true))
          (:`then_1`
            (`SceneComponent.K2_SetWorldLocation` _vfx_hit _returnvalue false false)
            (set `self.Hit_Actor_Location` _returnvalue)
            (`self.Explode_Sound_Event`)
            (`ActorComponent.Activate` _vfx_hit true)
            (`ActorComponent.Activate` null true)
            (`/Engine/EditorBlueprintResources/StandardMacros.DoOnce` false))
          (:`then_2`
            (`KismetSystemLibrary.Delay` 0.2)
            (set `self.IsKicked` false)))))
    (:`Is Not Valid`
      (if (not (`self.ActorHasTag` Other "Player"))
        (message `HitInterface.GetHit` Other (`self.Hit_Damage`) 0.0 (0.0 0.0 0.0) 0.0 self)))))

(event `Init Feedback`
  (`|ExecutionSequence`
    (:`then_0`
      (add `self.Kicked_Sound` (delegate `Kicked_Sound_Event`)))
    (:`then_1`
      (add `self.Explode_Sound` (delegate `Explode_Sound_Event`)))
    (:`then_2`
      (add `self.Getting_Vaccumed` (delegate `Getting_Vaccumed_Event`)))))

(event `Kicked_Sound_Event`
  ;[0 1 1 0.5] FB - Sound When Kicked
  (`GameplayStatics.SpawnSoundAtLocation` (`self.Sound_Chair_Kicked`) (`SceneComponent.K2_GetComponentLocation` (`self.SM_Extinguisher_00`)) (struct) 1.0 1.0 0.0 null null))

(event `Explode_Sound_Event`
  ;[0 1 1 0.5] FB - Sound When Chair Explode
  (`GameplayStatics.SpawnSoundAtLocation` (`self.Sound_Chair_Explode`) (`self.Hit_Actor_Location`) (struct) 1.0 1.0 0.0 null null))

(event `Getting_Vaccumed_Event`)

(fn `UserConstructionScript`)