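; Physics cart prop that can be kicked, pushed or vacuumed through impulses, and sends damage to non-player pawns it hits.
; The construction script uses CartStyle to set one of four body meshes, lay out wheels and size the hitbox.
; Tick yaws the wheels toward the velocity while moving, like casters.
; Kicks add a temporary "Kicked" tag, VFX and sound; BeginPlay binds that sound and gives a small upward impulse.
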(event `self.ReceiveTick`
  (params (DeltaSeconds :type "Float (single-precision)"))
  (bind _returnvalue (`self.GetVelocity`))
  ;[1 0.3033 0.2134] Wheel Change direction when moved
  (if (> (`KismetMathLibrary.VSize` _returnvalue) 10.0)
    (`SceneComponent.K2_SetRelativeRotation` (`self.Wheel_1`) (`KismetMathLibrary.MakeRotator` 0.0 0.0 (+ (.yaw (`KismetMathLibrary.MakeRotFromX` (`KismetMathLibrary.Normal` _returnvalue))) 90.0)) false false)
    (`SceneComponent.K2_SetRelativeRotation` (`self.Wheel_2`) (`KismetMathLibrary.MakeRotator` 0.0 0.0 (+ (.yaw (`KismetMathLibrary.MakeRotFromX` (`KismetMathLibrary.Normal` _returnvalue))) 90.0)) false false)
    (`SceneComponent.K2_SetRelativeRotation` (`self.Wheel_3`) (`KismetMathLibrary.MakeRotator` 0.0 0.0 (+ (.yaw (`KismetMathLibrary.MakeRotFromX` (`KismetMathLibrary.Normal` _returnvalue))) 90.0)) false false)
    (`SceneComponent.K2_SetRelativeRotation` (`self.Wheel_4`) (`KismetMathLibrary.MakeRotator` 0.0 0.0 (+ (.yaw (`KismetMathLibrary.MakeRotFromX` (`KismetMathLibrary.Normal` _returnvalue))) 90.0)) false false)))

(event `self.ReceiveBeginPlay`
  ;[0.7448 0.159 0.6313 0.5] Enable the whole system
  (`self.Init Feedback`)
  (`PrimitiveComponent.AddImpulse` (`self.Mesh`) (0.0 0.0 2.0) "None" true))

(event `self.Kicked`
  (params (KickVector :type "Vector Structure") (PlayerPosition :type "Vector Structure"))
  ;[0 0.4043 1 0.5] What happend when the chair got kicked
  (`self.Kicked_Sound_Event`)
  (set `self.IsKicked` true)
  (`KismetArrayLibrary.Array_Add` (`self.Tags`) "Kicked")
  (`ActorComponent.Activate` (`self.VFX_Hit`) true)
  (`PrimitiveComponent.AddImpulse` (`self.Mesh`) (* KickVector (`self.Impulse_Value`)) "None" false)
  (`KismetSystemLibrary.Delay` 1.0)
  (set `self.IsKicked` false)
  (`KismetArrayLibrary.Array_RemoveItem` (`self.Tags`) "Kicked"))

(event `self.ReceiveHit`
  (params (MyComp :type "PrimitiveComponent Object Reference") (Other :type "Actor Object Reference") (OtherComp :type "PrimitiveComponent Object Reference") (bSelfMoved :type Boolean) (HitLocation :type "Vector Structure") (HitNormal :type "Vector Structure") (NormalImpulse :type "Vector Structure") (Hit :type "HitResult Structure (by ref)"))
  ;[1 0.51 0 0.5] Cart hit "Prop Physics" and what happend
  (if (not (`self.ActorHasTag` Other "Player"))
    (bind _aspawn (cast `Pawn` Other))
    (message `HitInterface.GetHit` _aspawn (`self.Damage`) 0.0 (0.0 0.0 0.0) (`self.Invincibility Time`) null)))

(event `self.Push`
  (params (Force :type "Vector Structure"))
  ;[0.15 0.03563 0.1418 0.5] Reaction when pushed & vacuumed
  (`PrimitiveComponent.AddImpulse` (`self.Mesh`) Force "None" true))

(event `self.ReactToVacuum`
  (params (Force :type "Vector Structure"))
  ;[0.15 0.03563 0.1418 0.5] Reaction when pushed & vacuumed
  (`PrimitiveComponent.AddImpulse` (`self.Mesh`) (* Force (`self.Vacuum_Effect_Force`)) "None" true))

(event `Init Feedback`
  (`|ExecutionSequence`
    (:`then_0`
      (add `self.Kicked_Sound` (delegate `Kicked_Sound_Event`)))))

(event `Kicked_Sound_Event`
  ;[0 1 1 0.5] FB - Sound When Kicked
  (`GameplayStatics.SpawnSoundAtLocation` (`self.Sound_Chair_Kicked`) (`SceneComponent.K2_GetComponentLocation` (`self.Mesh`)) (struct) 1.0 1.0 0.0 null null))

(fn `Transform Custom`
  (params (`CollisionBox Ref` :type "BoxComponent Object Reference") (`Box Vector` :type "Vector Structure") (`Relative Location` :type "Vector Structure") (`Relative Scale` :type "Vector Structure") (`CustomWheel?` :type Boolean) (`Custom Wheel Mesh` :type "StaticMesh Object Reference"))
  (`BoxComponent.SetBoxExtent` `CollisionBox Ref` `Box Vector` true)
  (`SceneComponent.K2_SetRelativeLocation` `CollisionBox Ref` `Relative Location` false false)
  (`SceneComponent.SetRelativeScale3D` `CollisionBox Ref` `Relative Scale`)
  (if `CustomWheel?`
    (`self.Wheel Custom Mesh` `Custom Wheel Mesh`)
    (return)))

(fn `UserConstructionScript`
  (switch `/Game/BPs/Enums/E_Cart` (`self.Cart Style`)
    (:`NewEnumerator0`
      (`StaticMeshComponent.SetStaticMesh` (`self.Mesh`) "/Game/Environment/Office/Meshes/Furniture/Carts/FoodCart/SM_FoodCart_01.SM_FoodCart_01")
      ; Food Cart
      (`self.Wheel Position` (28.0 23.0 18.0) (-29.0 23.0 18.0) (-33.0 -23.0 18.0) (33.0 -23.0 18.0))
      (`self.Transform Custom` (`self.Hitbox`) (45.0 45.0 50.0) (0.0 0.0 59.0) (1.0 1.0 1.0)))
    (:`NewEnumerator1`
      (`StaticMeshComponent.SetStaticMesh` (`self.Mesh`) "/Game/Environment/Office/Meshes/Furniture/Carts/PlatterCart/SM_PlatterCart_01.SM_PlatterCart_01")
      ; Platter Cart
      (`self.Wheel Position` (48.0 22.0 9.0) (-20.0 22.0 9.0) (-20.0 -31.0 9.0) (48.0 -31.0 9.0))
      (`self.Transform Custom` (`self.Hitbox`) (40.0 40.0 95.0) (14.0 -2.0 93.0) (1.0 1.0 1.0)))
    (:`NewEnumerator2`
      (`StaticMeshComponent.SetStaticMesh` (`self.Mesh`) "/Game/Environment/Office/Meshes/SmallAssets/SM_JanitorCart_02.SM_JanitorCart_02")
      ; Janitor Cart
      (`self.Wheel Position` (18.0 43.0 12.5) (-18.0 43.0 12.5) (22.0 -32.0 12.5) (-22.0 -32.0 12.5) false false true true)
      (`self.Transform Custom` (`self.Hitbox`) (40.0 80.0 60.0) (0.0 -10.0 75.0) (1.0 0.7075 1.0) true "/Game/Environment/Office/Meshes/SmallAssets/SM_JanitorCartWheel_02.SM_JanitorCartWheel_02"))
    (:`NewEnumerator3`
      (`StaticMeshComponent.SetStaticMesh` (`self.Mesh`) "/Game/Environment/Office/Meshes/Furniture/Carts/SM_CartFile_A_01.SM_CartFile_A_01")
      ; Cart File
      (`self.Wheel Position` (63.0 -31.0 1.0) (63.0 31.0 1.0) (-60.0 -31.0 1.0) (-60.0 31.0 1.0) false false false false true (struct :`Yaw` 90.0))
      (`self.Transform Custom` (`self.Hitbox`) (80.0 40.0 50.0) (0.0 0.0 52.0) (1.0 0.7075 1.0) true "/Game/Environment/Office/Meshes/Furniture/Carts/SM_CartFile_B_01.SM_CartFile_B_01"))))

(fn `Wheel Custom Mesh`
  (params (`Wheel Mesh` :type "StaticMesh Object Reference"))
  (`|ExecutionSequence`
    (:`then_0`
      (`StaticMeshComponent.SetStaticMesh` (`self.Wheel_1`) `Wheel Mesh`))
    (:`then_1`
      (`StaticMeshComponent.SetStaticMesh` (`self.Wheel_2`) `Wheel Mesh`))
    (:`then_2`
      (`StaticMeshComponent.SetStaticMesh` (`self.Wheel_3`) `Wheel Mesh`))
    (:`then_3`
      (`StaticMeshComponent.SetStaticMesh` (`self.Wheel_4`) `Wheel Mesh`))))

(fn `Wheel Position`
  (params (`Wheel 1` :type "Vector Structure") (`Wheel 2` :type "Vector Structure") (`Wheel 3` :type "Vector Structure") (`Wheel 4` :type "Vector Structure") (`Hide Wheel 1` :type Boolean) (`Hide Wheel 2` :type Boolean) (`Hide Wheel 3` :type Boolean) (`Hide Wheel 4` :type Boolean) (`Custom Rotation?` :type Boolean) (`Custom Wheel Rotation` :type "Rotator Structure"))
  (`|ExecutionSequence`
    (:`then_0`
      (`SceneComponent.K2_SetRelativeLocation` (`self.Wheel_1`) `Wheel 1` false false)
      (if `Hide Wheel 1`
        (`SceneComponent.SetVisibility` (`self.Wheel_1`) false false)))
    (:`then_1`
      (`SceneComponent.K2_SetRelativeLocation` (`self.Wheel_2`) `Wheel 2` false false)
      (if `Hide Wheel 2`
        (`SceneComponent.SetVisibility` (`self.Wheel_2`) false false)))
    (:`then_2`
      (`SceneComponent.K2_SetRelativeLocation` (`self.Wheel_3`) `Wheel 3` false false)
      (if `Hide Wheel 3`
        (`SceneComponent.SetVisibility` (`self.Wheel_3`) false false)))
    (:`then_3`
      (`SceneComponent.K2_SetRelativeLocation` (`self.Wheel_4`) `Wheel 4` false false)
      (if `Hide Wheel 4`
        (`SceneComponent.SetVisibility` (`self.Wheel_4`) false false)))
    (:`then_4`
      (if `Custom Rotation?`
        (`SceneComponent.K2_SetRelativeRotation` (`self.Wheel_1`) `Custom Wheel Rotation` false false)
        (`SceneComponent.K2_SetRelativeRotation` (`self.Wheel_2`) `Custom Wheel Rotation` false false)
        (`SceneComponent.K2_SetRelativeRotation` (`self.Wheel_3`) `Custom Wheel Rotation` false false)
        (`SceneComponent.K2_SetRelativeRotation` (`self.Wheel_4`) `Custom Wheel Rotation` false false)))))