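; BP_Chair is a chair prop the player can kick or bump, sending it spinning along the player's forward direction.
; Hitbox overlaps branch on component tags, with timelines driving ProjectileMovement velocity and random RotatingMovement spin for kicks, pushes and furniture collisions.
; Furniture hits temporarily arm an unkicked chair as kicked.
; Walls, doors, hurtboxes, or furniture when kicked trigger Niagara effects and hide it, delaying collision shutoff to catch nearby enemies.
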(event `self.ReceiveBeginPlay`
  (`MovementComponent.SetUpdatedComponent` (`self.RotatingMovement`) (`self.Chair`)))

(event `self.Hitbox.OnComponentBeginOverlap`
  (params (OverlappedComponent :type "PrimitiveComponent Object Reference") (OtherActor :type "Actor Object Reference") (OtherComp :type "PrimitiveComponent Object Reference") (OtherBodyIndex :type Integer) (bFromSweep :type Boolean) (SweepResult :type "HitResult Structure (by ref)"))
  (bind (_bblockinghit _binitialoverlap _time _distance _location _impactpoint _normal _impactnormal _physmat _hitactor) (`GameplayStatics.BreakHitResult` SweepResult))
  (bind _projectilemovement (`self.ProjectileMovement`))
  (bind _projectilemovement_2 (`self.ProjectileMovement`))
  (if (`ActorComponent.ComponentHasTag` OtherComp "Kick")
    (set `self.AlreadyKicked?` true)
    (`ActorComponent.Activate` (`self.NS_Sample_BONK`) true)
    (`ActorComponent.Activate` _projectilemovement_2 false)
    (bind (_direction _distancemultiplier _chairpower) (`Timeline|Timeline` :!via `PlayFromStart`)
      (:`Update`
        (bind (_returnvalue_x _returnvalue_y) (`KismetMathLibrary.BreakVector` (* (`self.GetActorForwardVector` (`GameplayStatics.GetPlayerPawn` 0)) (* _distancemultiplier (`self.Hit Back Distance`)))))
        (set `MovementComponent.Velocity` (`KismetMathLibrary.MakeVector` _returnvalue_x _returnvalue_y) _projectilemovement_2)
        (set `RotatingMovementComponent.RotationRate` (`KismetMathLibrary.MakeRotator` 0.0 0.0 (* _chairpower (`KismetMathLibrary.RandomFloatInRange` 500.0 2000.0))) (`self.RotatingMovement`))))
    (elif (`self.AlreadyKicked?`)
      (if (or (`ActorComponent.ComponentHasTag` OtherComp "Chair") (`ActorComponent.ComponentHasTag` OtherComp "Table"))
        (`|ExecutionSequence`
          (:`then_0`
            (`SceneComponent.K2_SetWorldLocation` (`self.NS_FinisherHit`) (`self.K2_GetActorLocation` _hitactor) false false)
            (`SceneComponent.K2_SetWorldLocation` (`self.NS_Sample_BONK`) (`self.K2_GetActorLocation` _hitactor) false false)
            (`ActorComponent.Activate` (`self.NS_Sample_BONK`) true)
            (`ActorComponent.Activate` (`self.NS_FinisherHit`) true))
          (:`then_1`
            (`SceneComponent.SetHiddenInGame` (`self.Chair`) true false)
            (`KismetSystemLibrary.Delay` 0.1)
            (`self.SetActorEnableCollision` false)))
        (elif (or (`ActorComponent.ComponentHasTag` OtherComp "Wall") (`ActorComponent.ComponentHasTag` OtherComp "Hurtbox") (`ActorComponent.ComponentHasTag` OtherComp "Door"))
          (`|ExecutionSequence`
            (:`then_0`
              (`SceneComponent.K2_SetWorldLocation` (`self.NS_FinisherHit`) (`self.K2_GetActorLocation` _hitactor) false false)
              (`SceneComponent.K2_SetWorldLocation` (`self.NS_Sample_BONK`) (`self.K2_GetActorLocation` _hitactor) false false)
              (`ActorComponent.Activate` (`self.NS_Sample_BONK`) true)
              (`ActorComponent.Activate` (`self.NS_FinisherHit`) true))
            (:`then_1`
              (`SceneComponent.SetHiddenInGame` (`self.Chair`) true false)
              (`KismetSystemLibrary.Delay` 0.1) ; Let the game hit other enemies really close to the 1st one hit
              (`self.SetActorEnableCollision` false)))))
      (elif (or (`ActorComponent.ComponentHasTag` OtherComp "Player") (`ActorComponent.ComponentHasTag` OtherComp "Weapon"))
        (`ActorComponent.Activate` (`self.ProjectileMovement`) false)
        (bind (_direction_2 _distancemultiplier_2 _chairpower_2) (`Timeline|Timeline_1` :!via `PlayFromStart`)
          (:`Update`
            (bind (_returnvalue_x_2 _returnvalue_y_2) (`KismetMathLibrary.BreakVector` (* (`self.GetActorForwardVector` (`GameplayStatics.GetPlayerPawn` 0)) (* _distancemultiplier_2 (`self.Table Push`)))))
            (set `MovementComponent.Velocity` (`KismetMathLibrary.MakeVector` _returnvalue_x_2 _returnvalue_y_2) (`self.ProjectileMovement`))
            (set `RotatingMovementComponent.RotationRate` (`KismetMathLibrary.MakeRotator` 0.0 0.0 (* _chairpower_2 (`KismetMathLibrary.RandomFloatInRange` 1.0 100.0))) (`self.RotatingMovement`))))
        (elif (or (`ActorComponent.ComponentHasTag` OtherComp "Wall") (`ActorComponent.ComponentHasTag` OtherComp "Hurtbox") (`ActorComponent.ComponentHasTag` OtherComp "Door"))
          (`|ExecutionSequence`
            (:`then_0`
              (`SceneComponent.K2_SetWorldLocation` (`self.NS_FinisherHit`) (`self.K2_GetActorLocation` (`.HitActor` (`GameplayStatics.BreakHitResult` SweepResult))) false false)
              (`SceneComponent.K2_SetWorldLocation` (`self.NS_Sample_BONK`) (`self.K2_GetActorLocation` (`.HitActor` (`GameplayStatics.BreakHitResult` SweepResult))) false false)
              (`ActorComponent.Activate` (`self.NS_Sample_BONK`) true)
              (`ActorComponent.Activate` (`self.NS_FinisherHit`) true))
            (:`then_1`
              (`SceneComponent.SetHiddenInGame` (`self.Chair`) true false)
              (`KismetSystemLibrary.Delay` 0.1) ; Let the game hit other enemies really close to the 1st one hit
              (`self.SetActorEnableCollision` false)))
          (elif (or (`ActorComponent.ComponentHasTag` OtherComp "Chair") (`ActorComponent.ComponentHasTag` OtherComp "Table"))
            (`|ExecutionSequence`
              (:`then_0`
                (`ActorComponent.Activate` (`self.NS_Sample_BONK`) true)
                (`ActorComponent.Activate` _projectilemovement false)
                (bind (_direction_3 _distancemultiplier_3 _chairpower_3) (`Timeline|Timeline_0` :!via `PlayFromStart`)
                  (:`Update`
                    (bind (_returnvalue_x_3 _returnvalue_y_3) (`KismetMathLibrary.BreakVector` (* (`self.GetActorForwardVector` (`GameplayStatics.GetPlayerPawn` 0)) (* _distancemultiplier_3 (`self.Hit Back Distance No Kick`)))))
                    (set `MovementComponent.Velocity` (`KismetMathLibrary.MakeVector` _returnvalue_x_3 _returnvalue_y_3) _projectilemovement)
                    (set `RotatingMovementComponent.RotationRate` (`KismetMathLibrary.MakeRotator` 0.0 0.0 (* _chairpower_3 (`KismetMathLibrary.RandomFloatInRange` 500.0 1500.0))) (`self.RotatingMovement`)))
                  (:`Finished`
                    (set `self.AlreadyKicked?` false))))
              (:`then_1`
                (`KismetSystemLibrary.Delay` 0.1)
                (set `self.AlreadyKicked?` true)))))))))

(fn `UserConstructionScript`)