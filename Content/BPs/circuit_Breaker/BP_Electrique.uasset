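; Breakable electrical box that loses life from kicks and Light, Medium or Heavy tagged hits, with break VFX and sound.
; At zero life it swaps mesh, plays destruction audio, awards score, then plays an optional cutscene or runs Feedback.
; Feedback opens linked doors, moves sparks along a spline and animates the box mesh through chained rotation timelines.
; An explosion VFX branch is unwired and flagged for fixing.
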(event `KickedInterface.Kicked`
  (params (KickVector :type "Vector Structure") (PlayerPosition :type "Vector Structure"))
  ;[1 0.7787 0] Hit Behavior
  (set `self.Life Point` (- (`self.Life Point`) 10))
  (`self.Update Life`))

(event `self.ReceiveHit`
  (params (MyComp :type "PrimitiveComponent Object Reference") (Other :type "Actor Object Reference") (OtherComp :type "PrimitiveComponent Object Reference") (bSelfMoved :type Boolean) (HitLocation :type "Vector Structure") (HitNormal :type "Vector Structure") (NormalImpulse :type "Vector Structure") (Hit :type "HitResult Structure (by ref)"))
  ;[1 0.7787 0] Hit Behavior
  (if (`self.ActorHasTag` Other "Light")
    (set `self.Life Point` (- (`self.Life Point`) 1))
    (`self.Update Life`)
    (elif (`self.ActorHasTag` Other "Medium")
      (set `self.Life Point` (- (`self.Life Point`) 2))
      (`self.Update Life`)
      (elif (`self.ActorHasTag` Other "Heavy")
        (set `self.Life Point` (- (`self.Life Point`) 3))
        (`self.Update Life`)))))

(event `Update Life`
  (bind _sm_electricalbox_b_01 (`self.SM_ElectricalBox_B_01`))
  (if (<= (`self.Life Point`) 0)
    (`/Engine/EditorBlueprintResources/StandardMacros.DoOnce` false
      (:`Completed`
        (`StaticMeshComponent.SetStaticMesh` _sm_electricalbox_b_01 "/Game/Environment/GPE/SM_ElectricalBox_C_01.SM_ElectricalBox_C_01")
        (`SceneComponent.K2_SetRelativeLocationAndRotation` _sm_electricalbox_b_01 (-67.0 32.0 6.0) (struct :`Yaw` -360.0) false false)
        (`AkGameObject.PostAkEvent` :`self` (`self.Ak_Electrique`) :`AkEvent` "/Game/WwiseAudio/Events/Default_Work_Unit/SFX/SFX_GLOBAL/SFX_DESTRUCTION/SFX_Metal_Destruction.SFX_Metal_Destruction")
        (`FTJ_ScoringSystem_Score.IncreaseWithText` (subsystem `/Game/CppSystems/ScoringSystem/Public/Blueprint/BP_ScoringSystem_Score`) (`KismetMathLibrary.Conv_IntToDouble` 50) 0.2 (`|FormatText` "Broke Electrical"))
        (if (`KismetSystemLibrary.IsValid` (`self.Cinematique Ref`))
          ; For Cutscene
          (`KismetSystemLibrary.Delay` 0.75)
          (bind _cinematique_ref (`self.Cinematique Ref`)
            (:`then`
              (bind (_outactor _returnvalue) (`LevelSequencePlayer.CreateLevelSequencePlayer` _cinematique_ref))
              (`/Game/BPs/Other/FL_Common.Play Cinematique` _returnvalue))
            (:`else`))
          (else
            (`self.Feedback`)))))
    (else
      (bind _returnvalue_2 (`NiagaraFunctionLibrary.SpawnSystemAtLocation` "/Game/VFX/Niagara/Props/NS_Machine_Break.NS_Machine_Break" (`SceneComponent.K2_GetComponentLocation` (`self.hurtbox`))))
      (`NiagaraComponent.SetVariableVec3` _returnvalue_2 "LocationSize" (50.0 50.0 50.0))
      (`NiagaraComponent.SetVariableVec3` _returnvalue_2 "LocationMidPoint" (0.5 0.5 0.5))
      (`AkGameObject.PostAkEvent` :`self` (`self.Ak_Electrique`) :`AkEvent` "/Game/WwiseAudio/Events/Default_Work_Unit/SFX/SFX_GLOBAL/SFX_DESTRUCTION/SFX_Fan_Destruction.SFX_Fan_Destruction"))))

(event `Feedback`
  (bind _spline (`self.Spline`))
  (bind _spark (`self.Spark`))
  ;[0 1 1] Feedback
  (`self.Anim Open Door Event`)
  (for _array_element (`self.Door to Open`)
    (`/Game/BPs/Arena/BP_Arena_Door.Open Door` _array_element)
    (bind _returnvalue (`NiagaraFunctionLibrary.SpawnSystemAtLocation` "/Game/VFX/Niagara/Sparks/NS_ContinuousSparks.NS_ContinuousSparks"))
    (set `self.Spark` _returnvalue)
    (bind (_direction _newtrack_0) (`Timeline|Anim` :`NewTime` (`self.Spark Speed`))
      (:`Update`
        (`SceneComponent.K2_SetWorldLocation` _spark (`SplineComponent.GetLocationAtTime` _spline _newtrack_0 "World" true) false false)
        (`SceneComponent.K2_SetWorldRotation` _spark (`SplineComponent.GetRotationAtTime` _spline _newtrack_0 "World" true) false false))
      (:`Finished`
        (`ActorComponent.K2_DestroyComponent` (`self.Spark`))))))

(event `Anim Open Door Event`
  ;[0 1 1] Feedback
  (bind (_direction _alpha) (`Timeline|Anim Open Door` :!via `PlayFromStart`)
    (:`Update`
      (`SceneComponent.K2_SetRelativeRotation` (`self.SM_ElectricalBox_B_01`) (`KismetMathLibrary.RLerp` (struct :`Yaw` -360.0) (struct :`Yaw` -205.0) _alpha) false false))
    (:`Finished`
      (`self.Anim Break Door Event`))))

(event `Anim Break Door Event`
  ;[0 1 1] Feedback
  (`KismetSystemLibrary.Delay` 0.2)
  (bind (_direction _alpha) (`Timeline|Anim Break Door`)
    (:`Update`
      (`SceneComponent.K2_SetRelativeRotation` (`self.SM_ElectricalBox_B_01`) (`KismetMathLibrary.RLerp` (struct :`Yaw` -205.0) (struct :`Pitch` -22.0 :`Yaw` -365.0 :`Roll` 165.0) _alpha) false false))
    (:`Finished`
      (`self.Anim Break Door Loop Event`))))

(event `Anim Break Door Loop Event`
  ;[0 1 1] Feedback
  (`/Engine/EditorBlueprintResources/StandardMacros.FlipFlop`
    (:`A`
      (bind (_direction _alpha) (`Timeline|Anim Break Door Loop` :!label _label)
        (:`Update`
          (`SceneComponent.K2_SetRelativeRotation` (`self.SM_ElectricalBox_B_01`) (`KismetMathLibrary.RLerp` (struct :`Pitch` -22.0 :`Yaw` -365.0 :`Roll` 165.0) (struct :`Pitch` -60.0 :`Yaw` -365.0 :`Roll` 165.0) _alpha) false false))
        (:`Finished`
          (`self.Anim Break Door Loop Event`))))
    (:`B`
      (goto _label :!via `Reverse`))))

(fn `UserConstructionScript`)