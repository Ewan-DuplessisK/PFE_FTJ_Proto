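; Level manager that tracks streamed sublevels and handles checkpoint respawns.
; On BeginPlay it spawns a BP_LvlMan_Volume proxy per LevelStreamingVolume, maps them by level name and volume, and relays load/unload events.
; Respawn pauses the game, then either restarts the level or moves the player, reloads the checkpoint's sublevel and applies checkpoint data once loaded.
; It also records walked-through volumes and includes a test reload event for LVL_01.
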(event `self.ReceiveBeginPlay`
  (`|ExecutionSequence`
    (:`then_0`
      (bind _returnvalue (`GameplayStatics.GetActorOfClass` "/Game/Characters/Player/Blueprints/BP_Player.BP_Player_C"))
      (set `self.Player` _returnvalue))
    (:`then_1`
      (bind _outactors (`GameplayStatics.GetAllActorsOfClass` "/Script/Engine.LevelStreamingVolume"))
      (if (`KismetArrayLibrary.Array_IsNotEmpty` _outactors)
        (bind _output_get (set `self.LevelVolumes` _outactors))
        (for _array_element _output_get
          (bind (_returnvalue_location _returnvalue_rotation) (`KismetMathLibrary.BreakTransform` (`self.GetTransform` _array_element)))
          ; spawn proxy volumes
          (bind _returnvalue_2 (`|SpawnActorFromClass` "/Game/BPs/LvlManager/BP_LvlMan_Volume.BP_LvlMan_Volume_C" (`KismetMathLibrary.MakeTransform` _returnvalue_location _returnvalue_rotation) "Undefined" "MultiplyWithRoot" null null))
          (`/Game/BPs/LvlManager/BP_LvlMan_Volume.Set Volume` _returnvalue_2 _array_element)
          (`|ExecutionSequence`
            (:`then_0`
              (bind _output (`|GetArrayItem` (`LevelStreamingVolume.StreamingLevelNames` (`/Game/BPs/LvlManager/BP_LvlMan_Volume.Volume` _returnvalue_2))))
              ; set index maps
              (`BlueprintMapLibrary.Map_Add` (`self.LvlManVolume By LevelName`) (`KismetStringLibrary.Conv_StringToName` (`.RightS` (`KismetStringLibrary.Split` (`KismetStringLibrary.Conv_NameToString` _output) "_0_" "IgnoreCase" "FromEnd"))) _returnvalue_2)
              (`BlueprintMapLibrary.Map_Add` (`self.LvlManVolume By LevelVolume`) _array_element _returnvalue_2))
            (:`then_2`
              ; bind load/unload
              (`|ExecutionSequence`
                (:`then_0`
                  (bind _returnvalue_3 (`GameplayStatics.GetStreamingLevel` _output))
                  (add `LevelStreaming.OnLevelLoaded` _returnvalue_3 (delegate `OnLevelLoaded_Event`)))
                (:`then_1`
                  (add `LevelStreaming.OnLevelUnloaded` _returnvalue_3 (delegate `OnLevelUnloaded_Event`)))))))
        (else
          (`KismetSystemLibrary.Delay` 2.0)
          (`self.On SubLevel Loaded` "NO_SUBLVLS"))))))

(event `OnLevelLoaded_Event`
  ; bind load/unload
  (bind _output (`|GetArrayItem` (`LevelStreamingVolume.StreamingLevelNames` (`/Game/BPs/LvlManager/BP_LvlMan_Volume.Volume` (stale `self.ReceiveBeginPlay` _returnvalue_2)))))
  (`KismetSystemLibrary.PrintText` (`|FormatText` "LVL LOADED: {i} " _output))
  (`self.On SubLevel Loaded` _output))

(event `OnLevelUnloaded_Event`
  ; bind load/unload
  (bind _output (`|GetArrayItem` (`LevelStreamingVolume.StreamingLevelNames` (`/Game/BPs/LvlManager/BP_LvlMan_Volume.Volume` (stale `self.ReceiveBeginPlay` _returnvalue_2)))))
  (`KismetSystemLibrary.PrintText` (`|FormatText` "LVL UNLOADED: {i} " _output))
  (`self.On SubLevel Unloaded` _output))

(event `Respawn from Current Checkpoint`
  (bind _current_checkpoint (`self.Current Checkpoint`))
  (bind _value (`BlueprintMapLibrary.Map_Find` (`self.LvlManVolume By LevelVolume`) (`/Game/BPs/LvlManager/BP_LvlMan_Checkpoint.Level Volume` (`self.Current Checkpoint`))))
  (`/Game/Characters/Player/Blueprints/BP_Player.Show Loading` (`self.Player`))
  (`GameplayStatics.SetGamePaused` true)
  (`/Engine/EditorBlueprintResources/StandardMacros.IsValid` _current_checkpoint
    (:`Is Valid`
      (if (`KismetSystemLibrary.IsValidSoftObjectReference` (`/Game/BPs/LvlManager/BP_LvlMan_Checkpoint.Full Reload Level` _current_checkpoint))
        (`/Game/Developers/vladislavpavlov/LevelManager/GI_Systems_Base.Restart Level` (`/Game/Characters/Player/Blueprints/WeaponSystem/Interactable/FL_Common.Get GI Systems`) :!label _label)
        (else
          (`/Game/Characters/Player/Blueprints/BP_Player.Set Transform` (`self.Player`) (`self.GetTransform` (`self.Current Checkpoint`)))
          (`/Game/BPs/LvlManager/BP_LvlMan_Volume.Reload Level` _value)
          (add `LevelStreaming.OnLevelLoaded` (`.Level` (`/Game/BPs/LvlManager/BP_LvlMan_Volume.Get Streaming Level` _value)) (delegate `OnLevelLoaded_Event_0`)))))
    (:`Is Not Valid`
      (goto _label))))

(event `OnLevelLoaded_Event_0`
  (remove `LevelStreaming.OnLevelLoaded` (`.Level` (`/Game/BPs/LvlManager/BP_LvlMan_Volume.Get Streaming Level` (`BlueprintMapLibrary.Map_Find` (`self.LvlManVolume By LevelVolume`) (`/Game/BPs/LvlManager/BP_LvlMan_Checkpoint.Level Volume` (`self.Current Checkpoint`))))) (delegate `OnLevelLoaded_Event_0`))
  (`/Game/BPs/LvlManager/BP_LvlMan_Checkpoint.Apply Checkpoint Data` (`self.Current Checkpoint`))
  (`/Game/Characters/Player/Blueprints/BP_Player.Enable Playing` (`self.Player`))
  (`GameplayStatics.SetGamePaused` false))

(event `Set Volume WalkedThrough`
  (params (NewItem :type "/Game/BPs/LvlManager/BP_LvlMan_Volume Object Reference (by ref)"))
  (bind _returnvalue (`KismetArrayLibrary.Array_AddUnique` (`self.WalkedThrough`) NewItem)))

(event `TEST Reaload 01`
  (bind (_value _returnvalue) (`BlueprintMapLibrary.Map_Find` (`self.LvlManVolume By LevelName`) "LVL_01"))
  ; TEST reload
  (bind _outactors (`GameplayStatics.GetAllActorsOfClass` "/Script/Engine.PlayerStart"))
  (`self.K2_SetActorTransform` (`GameplayStatics.GetPlayerPawn` 0) (`self.GetTransform` (`|GetArrayItem` _outactors)) false true)
  (if _returnvalue
    (`/Game/BPs/LvlManager/BP_LvlMan_Volume.Unload Level` _value)
    (`KismetSystemLibrary.Delay` 1.0)
    (`/Game/BPs/LvlManager/BP_LvlMan_Volume.Load Level` _value)
    (else
      (`KismetSystemLibrary.PrintString` "[LevelManager]: Level not found"))))

(fn `Set Current Checkpoint`
  (params (`Current Checkpoint` :type "/Game/BPs/LvlManager/BP_LvlMan_Checkpoint Object Reference"))
  (returns (Changed :type Boolean))
  (locals (_Changed :type Boolean))
  (bind _output_get (set `local._Changed` (!= (`self.Current Checkpoint`) `Current Checkpoint`)))
  (if _output_get
    (set `self.Current Checkpoint` `Current Checkpoint`))
  (return _output_get))

(fn `UserConstructionScript`)