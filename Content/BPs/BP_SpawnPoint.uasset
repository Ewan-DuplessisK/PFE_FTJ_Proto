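; BP_SpawnPoint is a spawn point that creates an actor of a given class at its own transform, apparently for enemies.
; Spawn only acts when the tracked CurrentActor is invalid or being destroyed, so the point holds one live actor at a time.
; Each spawn plays a Niagara burst slightly below the point, then stores the new actor and the game time of the spawn.
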(fn `Spawn`
  (params (Class :type "Actor Class Reference"))
  (bind _returnvalue (`self.K2_GetActorRotation`))
  (bind _returnvalue_2 (`self.K2_GetActorLocation`))
  (bind _current_actor_ (`self.Current Actor `)
    (:`then`
      (if (`self.IsActorBeingDestroyed` _current_actor_)
        (bind _returnvalue_3 (`|SpawnActorFromClass` Class (`KismetMathLibrary.MakeTransform` _returnvalue_2 _returnvalue) "Undefined" "MultiplyWithRoot" null null :!label _label))
        (`NiagaraFunctionLibrary.SpawnSystemAtLocation` "/Game/VFX/Niagara/Bursts/NS_Burst_Enemy_Spawn.NS_Burst_Enemy_Spawn" (- _returnvalue_2 (0.0 0.0 30.0)) _returnvalue)
        (set `self.Current Actor ` _returnvalue_3)
        (set `self.Spawn Time` (`KismetSystemLibrary.GetGameTimeInSeconds`))))
    (:`else`
      (goto _label))))

(fn `UserConstructionScript`)