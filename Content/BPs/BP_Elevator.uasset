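; BP_Elevator is the level's elevator exit, which ends the game when the player enters it after it opens.
; OpenElevator hides both door meshes, disables their collision and sets IsOpen.
; While IsOpen is set, player pawn overlap with the Inside trigger calls StopGame on the GI_Systems game instance.
; Disconnected leftover logic holds a DT_Ranks score-to-rank lookup for ForceEnd and an elevator-unlocked dialogue call.
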(event `self.ReceiveBeginPlay`
  (bind _asgi_systems (cast `/Game/_GameManager/GI_Systems` (`GameplayStatics.GetGameInstance`)))
  (set `self.As GI Systems` _asgi_systems))

(event `/Game/BPs/TestProps/BPI/BPI_Elevator.Open_Elevator`
  (`SceneComponent.SetHiddenInGame` (`self.SM_ElevatorRightDoor_00`) true true)
  (`SceneComponent.SetHiddenInGame` (`self.SM_ElevatorLeftDoor_00`) true true)
  (`PrimitiveComponent.SetCollisionEnabled` (`self.SM_ElevatorLeftDoor_00`) "NoCollision")
  (`PrimitiveComponent.SetCollisionEnabled` (`self.SM_ElevatorRightDoor_00`) "NoCollision")
  (set `self.Is Open` true))

(event `self.Inside.OnComponentBeginOverlap`
  (params (OverlappedComponent :type "PrimitiveComponent Object Reference") (OtherActor :type "Actor Object Reference") (OtherComp :type "PrimitiveComponent Object Reference") (OtherBodyIndex :type Integer) (bFromSweep :type Boolean) (SweepResult :type "HitResult Structure (by ref)"))
  (if (and (`self.Is Open`) (== OtherActor (`GameplayStatics.GetPlayerPawn` 0)))
    (bind _asgi_systems (cast `/Game/_GameManager/GI_Systems` (`GameplayStatics.GetGameInstance`)))
    (`/Game/_GameManager/GI_Systems.StopGame` _asgi_systems)))

(fn `UserConstructionScript`)