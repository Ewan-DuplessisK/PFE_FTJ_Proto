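; Breakable physics window that loses health through damage and shatters at zero or when struck by fast Heavy or Medium actors or kicked chairs and carts.
; Damage drives the mesh's "Anim" material parameter, with optional debug health bars.
; Breaking spawns BP_Window_Fractured, impulses its Geometry Collection, removes the intact mesh and despawns both actors after a delay.
; Event-bound feedback plays kick and break sounds plus a "KRSSHH" Niagara text oriented by player side.
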(event `self.ReceiveTick`
  (params (DeltaSeconds :type "Float (single-precision)"))
  (if (`self.Debug_Health_Show`)
    (bind _aswbp_health_destruction (cast `/Game/UI/WBP_HealthDestruction` (`WidgetComponent.GetWidget` (`self.HealthBar Widget`))))
    (`ProgressBar.SetPercent` (`/Game/UI/WBP_HealthDestruction.Health_Bar` _aswbp_health_destruction) (/ (`self.CurrentHealth`) (`self.MaxHealth`)))
    (`ProgressBar.SetPercent` (`/Game/UI/WBP_HealthDestruction.Health_Bar` (cast `/Game/UI/WBP_HealthDestruction` (`WidgetComponent.GetWidget` (`self.HealthBar Widget1`)) :!pure true)) (/ (`self.CurrentHealth`) (`self.MaxHealth`)))))

(event `self.ReceiveBeginPlay`
  (bind _healthbar_widget (`self.HealthBar Widget`))
  (`self.Init Feedback`)
  (set `self.CurrentHealth` (`self.MaxHealth`))
  (if (`self.Debug_Health_Show`)
    (`SceneComponent.SetVisibility` _healthbar_widget true false)
    (`SceneComponent.SetVisibility` (`self.HealthBar Widget1`) true false)
    (else
      (`SceneComponent.SetVisibility` _healthbar_widget false false)
      (`SceneComponent.SetVisibility` (`self.HealthBar Widget1`) false false))))

(event `KickedInterface.Kicked`
  (params (KickVector :type "Vector Structure") (PlayerPosition :type "Vector Structure"))
  (bind _staticmesh (`self.StaticMesh`))
  ;[0 0.4075 1 0.5] What happend when you kicked the door
  (`SceneComponent.SetVisibility` (`self.HealthBar Widget`) false false)
  (`SceneComponent.SetVisibility` (`self.HealthBar Widget1`) false false)
  (bind _returnvalue (`self.Spawn Window Breakable` (`SceneComponent.K2_GetComponentLocation` _staticmesh) (`SceneComponent.K2_GetComponentRotation` _staticmesh)))
  (set `self.Fractured_Window` _returnvalue)
  (`PrimitiveComponent.SetSimulatePhysics` (`self.StaticMesh`) true)
  (set `self.IsKicked` true)
  (bind _output_get (set `self.Kick Strength` (* KickVector (`self.Impulse Strength`))))
  (`PrimitiveComponent.AddImpulse` (`self.StaticMesh`) _output_get "None" true)
  (`self.Kicked_Sound_Event`)
  (`/Engine/EditorBlueprintResources/StandardMacros.DoOnce` false
    (:`Completed`
      (`|ExecutionSequence`
        (:`then_0`
          ;;[0.561 0 0.6979 0.5] Door Spawn & Explosion when hit something
          (`PrimitiveComponent.AddImpulse` (`/Game/BPs/GC_GCBP/Window/BP_Window_Fractured.GeometryCollection` (`self.Fractured_Window`)) (/ (`self.Kick Strength`) 1.0) "None" true)
          (`ActorComponent.K2_DestroyComponent` (`self.StaticMesh`))
          (`ActorComponent.K2_DestroyComponent` (`self.Box`))
          (`self.Break_Sound_Event`))
        (:`then_1`
          ;;[0.588 0.2765 0.599 0.5] Door Despawn after explosion
          (`KismetSystemLibrary.Delay` (`self.Despawn Time`))
          (`self.K2_DestroyActor` (`self.Fractured_Window`))
          (`self.K2_DestroyActor`))))))

(event `self.ReceiveHit`
  (params (MyComp :type "PrimitiveComponent Object Reference") (Other :type "Actor Object Reference") (OtherComp :type "PrimitiveComponent Object Reference") (bSelfMoved :type Boolean) (HitLocation :type "Vector Structure") (HitNormal :type "Vector Structure") (NormalImpulse :type "Vector Structure") (Hit :type "HitResult Structure (by ref)"))
  ;[0.15 0 0 0.5] Event Hit
  (if (> (`KismetMathLibrary.VSize` (`self.GetVelocity` Other)) (`self.Velocity Threshold`))
    (if (or (`self.ActorHasTag` Other "Heavy") (`self.ActorHasTag` Other "Medium") (and (`self.ActorHasTag` Other "Chair") (`self.ActorHasTag` Other "Kicked")) (and (`self.ActorHasTag` Other "Cart") (`self.ActorHasTag` Other "Kicked")))
      (`KickedInterface.Kicked` (`self.Kick Strength`)))))

(event `HealthInterface.DamageBreakable`
  (params (Damage :type "Float (single-precision)") (Push :type "Vector Structure"))
  (bind _output_get (set `self.CurrentHealth` (`KismetMathLibrary.FClamp` (- (`self.CurrentHealth`) Damage) 0.0 (`self.MaxHealth`))))
  (`self.Window Damage Mat`)
  (if (<= _output_get 0.0)
    (`/Engine/EditorBlueprintResources/StandardMacros.DoOnce` false
      (:`Completed`
        (`KickedInterface.Kicked` (* Push 50.0))))))

(event `Init Feedback`
  (`|ExecutionSequence`
    (:`then_0`
      (add `self.Kicked_Sound` (delegate `Kicked_Sound_Event`)))
    (:`then_1`
      (add `self.Break_Sound` (delegate `Break_Sound_Event`)))))

(event `Kicked_Sound_Event`
  ;[0 1 1 0.5] FB - Sound When Kicked
  (`GameplayStatics.PlaySoundAtLocation` (`self.Sound_When_Kicked`) (`SceneComponent.K2_GetComponentLocation` (`self.StaticMesh`)) (struct) 1.0 1.0 0.0 null null null null))

(event `Break_Sound_Event`
  (bind _box (`self.Box`))
  ;[0 1 1 0.5] FB - Sound When Break
  (`GameplayStatics.PlaySoundAtLocation` (`self.Sound_When_Break`) (`self.K2_GetActorLocation` (`self.Fractured_Window`)) (struct) 1.0 1.0 0.0 null null null null)
  (if (< (`KismetMathLibrary.Dot_VectorVector` (`self.GetActorForwardVector`) (`KismetMathLibrary.Normal` (- (`self.K2_GetActorLocation` (cast `/Game/Characters/Player/Blueprints/BP_Player` (`GameplayStatics.GetPlayerCharacter` 0) :!pure true)) (`self.K2_GetActorLocation`)))) 0.0)
    (`NiagaraFunctionLibrary.SpawnSystemAttached` "/Game/VFX/Niagara/Text/NS_Text_KRSSHH.NS_Text_KRSSHH" _box "None" (0.0 0.0 0.0) (struct :`Yaw` 270.0) "KeepRelativeOffset" true)
    (else
      (`NiagaraFunctionLibrary.SpawnSystemAttached` "/Game/VFX/Niagara/Text/NS_Text_KRSSHH.NS_Text_KRSSHH" _box "None" (0.0 0.0 0.0) (struct :`Yaw` 90.0) "KeepRelativeOffset" true))))

(fn `Spawn Window Breakable`
  (params (SpawnTransform_Location :type "Vector Structure") (`Spawn Transform Rotation` :type "Rotator Structure"))
  (returns (ReturnValue :type "/Game/BPs/GC_GCBP/Window/BP_Window_Fractured Object Reference"))
  (bind _returnvalue (`|SpawnActorFromClass` "/Game/BPs/GC_GCBP/Window/BP_Window_Fractured.BP_Window_Fractured_C" (`KismetMathLibrary.MakeTransform` SpawnTransform_Location `Spawn Transform Rotation`) "AlwaysSpawn" "MultiplyWithRoot" null null))
  (`MeshComponent.SetScalarParameterValueOnMaterials` (`/Game/BPs/GC_GCBP/Window/BP_Window_Fractured.GeometryCollection` _returnvalue) "Anim" 0.0)
  (return _returnvalue))

(fn `UserConstructionScript`
  (bind _healthbar_widget (`self.HealthBar Widget`))
  (set `self.CurrentHealth` (`self.MaxHealth`))
  (if (`self.Debug_Health_Show`)
    (`SceneComponent.SetVisibility` _healthbar_widget true false)
    (`SceneComponent.SetVisibility` (`self.HealthBar Widget1`) true false)
    (else
      (`SceneComponent.SetVisibility` _healthbar_widget false false)
      (`SceneComponent.SetVisibility` (`self.HealthBar Widget1`) false false))))

(fn `Window Damage Mat`
  (bind _returnvalue (`KismetMathLibrary.FClamp` (/ (`self.CurrentHealth`) (`self.MaxHealth`))))
  (`MeshComponent.SetScalarParameterValueOnMaterials` (`self.StaticMesh`) "Anim" (`KismetMathLibrary.SelectFloat` (/ _returnvalue 10.0) _returnvalue (<= _returnvalue 0.6))))