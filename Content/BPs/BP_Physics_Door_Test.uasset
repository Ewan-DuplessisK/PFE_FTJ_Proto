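; Physics door prop that launches and shatters when kicked or struck by a fast Heavy- or Chair-tagged actor or another door.
; Hit converts the striker's velocity into a kick along the door's right vector, flipping sign by yaw.
; Kicked applies an impulse, then once swaps the mesh for a spawned BP_Door_Test geometry collection carrying that impulse.
; Kick and break sounds play through bound events; despawn logic is disconnected.
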(event `KickedInterface.Kicked`
  (params (KickVector :type "Vector Structure") (PlayerPosition :type "Vector Structure"))
  (bind _staticmesh (`self.StaticMesh`))
  ;[0 0.4075 1 0.5] What happens when you kick the door
  (`PrimitiveComponent.SetSimulatePhysics` (`self.StaticMesh`) true)
  (set `self.IsKicked` true)
  (bind _output_get (set `self.Kick Strength` (* KickVector (`self.Impulse Strength`))))
  (`PrimitiveComponent.AddImpulse` (`self.StaticMesh`) _output_get "None" true)
  (`self.Kicked_Sound_Event`)
  ;[0.15 0 0 0.5] Event Hit
  (`/Engine/EditorBlueprintResources/StandardMacros.DoOnce` false
    (:`Completed`
      (bind _returnvalue (`self.Spawn Window Breakable` (`SceneComponent.K2_GetComponentLocation` _staticmesh) (`SceneComponent.K2_GetComponentRotation` _staticmesh)))
      (bind _output_get_2 (set `self.Fractured_Door` _returnvalue))
      (`|ExecutionSequence`
        (:`then_0`
          ;;[0.561 0 0.6979 0.5] Door Spawn & Explosion when hit something
          (`PrimitiveComponent.AddImpulse` (`/Game/BPs/GC_GCBP/test/BP_Door_Test.GeometryCollection` _output_get_2) (/ (`self.Kick Strength`) 1.0) "None" true)
          (`ActorComponent.K2_DestroyComponent` (`self.StaticMesh`))
          (`ActorComponent.K2_DestroyComponent` (`self.Box`))
          (`self.Break_Sound_Event`))
        (:`then_1`)))))

(event `self.ReceiveHit`
  (params (MyComp :type "PrimitiveComponent Object Reference") (Other :type "Actor Object Reference") (OtherComp :type "PrimitiveComponent Object Reference") (bSelfMoved :type Boolean) (HitLocation :type "Vector Structure") (HitNormal :type "Vector Structure") (NormalImpulse :type "Vector Structure") (Hit :type "HitResult Structure (by ref)"))
  (bind (_returnvalue_roll _returnvalue_pitch _returnvalue_yaw) (`KismetMathLibrary.BreakRotator` (`self.K2_GetActorRotation`)))
  (bind _returnvalue (* (`self.GetVelocity` Other) (`self.GetActorRightVector`)))
  ;[0.15 0 0 0.5] Event Hit
  (if (> (`KismetMathLibrary.VSize` (`self.GetVelocity` Other)) (`self.Velocity Threshold`))
    (if (or (`self.ActorHasTag` Other "Heavy") (`self.ActorHasTag` Other "Chair") (`KismetStringLibrary.Contains` (`KismetSystemLibrary.GetDisplayName` Other) "Door"))
      (if (!= _returnvalue_yaw -90.0)
        (`KickedInterface.Kicked` (* _returnvalue 10.0))
        (else
          (`KickedInterface.Kicked` (* _returnvalue -10.0)))))))

(event `Init Feedback`
  (`|ExecutionSequence`
    (:`then_0`
      (add `self.Kicked_Sound` (delegate `Kicked_Sound_Event`)))
    (:`then_1`
      (add `self.Break_Sound` (delegate `Break_Sound_Event`)))))

(event `Kicked_Sound_Event`
  (`GameplayStatics.PlaySoundAtLocation` (`self.Sound_When_Kicked`) (`SceneComponent.K2_GetComponentLocation` (`self.StaticMesh`)) (struct) 1.0 1.0 0.0 null null null null))

(event `Break_Sound_Event`
  ;[0 1 1 0.5] FB - Sound When Break
  (`GameplayStatics.PlaySoundAtLocation` (`self.Sound_When_Break`) (`self.K2_GetActorLocation` (`self.Fractured_Door`)) (struct) 1.0 1.0 0.0 null null null null))

(fn `Spawn Window Breakable`
  (params (SpawnTransform_Location :type "Vector Structure") (`Spawn Transform Rotation` :type "Rotator Structure"))
  (returns (ReturnValue :type "/Game/BPs/GC_GCBP/test/BP_Door_Test Object Reference"))
  (bind _returnvalue (`|SpawnActorFromClass` "/Game/BPs/GC_GCBP/test/BP_Door_Test.BP_Door_Test_C" (`KismetMathLibrary.MakeTransform` SpawnTransform_Location `Spawn Transform Rotation`) "AlwaysSpawn" "MultiplyWithRoot" null null))
  (return _returnvalue))

(fn `UserConstructionScript`)