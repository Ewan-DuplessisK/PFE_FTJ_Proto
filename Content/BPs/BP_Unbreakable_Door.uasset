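; BP_Unbreakable_Door is a kickable door that reacts to a kick with sound and a material wobble.
; Kicked posts Wwise audio, then a timeline drives the Positions_Boing parameter on a dynamic material instance created each update.
; Functions for spawning a breakable BP_Door_Test and showing health-based damage through the Anim parameter exist but are not called here.
; The Feedback graph's kick and break sound bindings never run, as nothing calls InitFeedback.
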(event `self.ReceiveBeginPlay`)

(event `self.Kicked`
  (params (KickVector :type "Vector Structure") (PlayerPosition :type "Vector Structure"))
  ;[0 0.4075 1 0.5] What happens when you kick the door
  (`AkGameplayStatics.PostEvent` "/Game/WwiseAudio/Events/Default_Work_Unit/MC/MC_KICK_WU/MC_Kick_Door.MC_Kick_Door" (`GameplayStatics.GetPlayerCharacter` 0))
  (`AkGameObject.PostAssociatedAkEvent` :`self` (`self.Audio`))
  (bind (_direction _newtrack_0) (`Timeline|Timeline` :!via `PlayFromStart`)
    (:`Update`
      (bind _returnvalue (`PrimitiveComponent.CreateDynamicMaterialInstance` (`self.StaticMesh`) 0 null "None"))
      (`MaterialInstanceDynamic.SetScalarParameterValue` _returnvalue "Positions_Boing" _newtrack_0))))

(event `Init Feedback`
  (`|ExecutionSequence`
    (:`then_0`
      (add `self.Kicked_Sound` (delegate `Kicked_Sound_Event`)))
    (:`then_1`
      (add `self.Break_Sound` (delegate `Break_Sound_Event`)))))

(event `Kicked_Sound_Event`
  (`GameplayStatics.PlaySoundAtLocation` (`self.Sound_When_Kicked`) (`SceneComponent.K2_GetComponentLocation` (`self.StaticMesh`)) (struct) 1.0 1.0 0.0 null null null null))

(event `Break_Sound_Event`
  ;[0 1 1 0.5] FB - Sound When Break
  (`GameplayStatics.PlaySoundAtLocation` (`self.Sound_When_Break`) (`self.K2_GetActorLocation`) (struct) 1.0 1.0 0.0 null null null null))

(fn `Door Damage Mat`
  (bind _returnvalue (`KismetMathLibrary.FClamp` (/ (`self.CurrentHealth`) (`self.MaxHealth`))))
  (`MeshComponent.SetScalarParameterValueOnMaterials` (`self.StaticMesh`) "Anim" (`KismetMathLibrary.SelectFloat` (/ _returnvalue 10.0) _returnvalue (<= _returnvalue 0.6))))

(fn `Spawn Door Breakable`
  (params (SpawnTransform_Location :type "Vector Structure") (`Spawn Transform Rotation` :type "Rotator Structure"))
  (returns (ReturnValue :type "/Game/BPs/GC_GCBP/test/BP_Door_Test Object Reference"))
  (bind _returnvalue (`|SpawnActorFromClass` "/Game/BPs/GC_GCBP/test/BP_Door_Test.BP_Door_Test_C" (`KismetMathLibrary.MakeTransform` SpawnTransform_Location `Spawn Transform Rotation`) "AlwaysSpawn" "MultiplyWithRoot" null null))
  (`MeshComponent.SetScalarParameterValueOnMaterials` (`/Game/BPs/GC_GCBP/test/BP_Door_Test.GeometryCollection` _returnvalue) "Anim" 0.0)
  (return _returnvalue))

(fn `UserConstructionScript`)