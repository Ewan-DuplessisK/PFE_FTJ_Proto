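; BP_Enemy is an AI enemy character that chases the player and dies when shot.
; It spawns its default controller on BeginPlay, and PawnSensing triggers an AI MoveTo toward player 0 on sight.
; A capsule hit from an actor tagged "Player Shoot" enables capsule physics, disables HitCollision and destroys the enemy after a short delay.
; QTEBegin and QTEEnd freeze and restore its walk speed around quick-time events.
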(event `self.ReceiveBeginPlay`
  (`self.SpawnDefaultController`))

(event `self.CapsuleComponent.OnComponentHit`
  (params (HitComponent :type "PrimitiveComponent Object Reference") (OtherActor :type "Actor Object Reference") (OtherComp :type "PrimitiveComponent Object Reference") (NormalImpulse :type "Vector Structure") (Hit :type "HitResult Structure (by ref)"))
  ;[0.5729 0.02466 0 0.5] Die From Hit
  (if (`self.ActorHasTag` OtherActor "Player Shoot")
    (`PrimitiveComponent.SetSimulatePhysics` (`self.CapsuleComponent`) true)
    (`PrimitiveComponent.SetCollisionEnabled` (`self.Hit Collision`) "NoCollision")
    ;;[1 1 1 0.5] Delay Death
    (`KismetSystemLibrary.Delay` 0.5)
    (`self.K2_DestroyActor`)))

(event `self.PawnSensing.OnSeePawn`
  (params (Pawn :type "Pawn Object Reference"))
  (bind _returnvalue (`GameplayStatics.GetPlayerCharacter` 0))
  ;[0.04145 0.4948 0 0.5] AI Behavior
  (`|AIMoveTo` self (`self.K2_GetActorLocation` _returnvalue) _returnvalue (`self.Acceptance Radius`)))

(event `QTE End`
  (bind _charactermovement (`self.CharacterMovement`))
  ;[0 0.4964 1 0.5] QTE Enemy Speed
  (`/Engine/EditorBlueprintResources/StandardMacros.IsValid` _charactermovement
    (:`Is Valid`
      (set `CharacterMovementComponent.MaxWalkSpeed` 600.0 _charactermovement) ; Change Back enemy walk speed to normal after QTE
    )))

(event `QTE Begin`
  (bind _charactermovement (`self.CharacterMovement`))
  ;[0 0.4964 1 0.5] QTE Enemy Speed
  (`/Engine/EditorBlueprintResources/StandardMacros.IsValid` _charactermovement
    (:`Is Valid`
      (set `CharacterMovementComponent.MaxWalkSpeed` 0.0 _charactermovement) ; Stop enemy to walk when in QTE
    )))

(fn `UserConstructionScript`)