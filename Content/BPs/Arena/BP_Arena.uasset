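; BP_Arena is a one-time combat encounter that locks the player in until every spawned enemy is gone.
; Player overlap with the resizable box shuts the linked doors or plays an intro cinematic, then after a delay spawns enemies at referenced spawners.
; Tick prunes dead enemies, then reopens doors or plays an outro sequence once none remain.
; Destroying the arena or ending play also destroys its enemies.
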(event `self.ReceiveTick`
  (params (DeltaSeconds :type "Float (single-precision)"))
  ;[1 0.15 0.15] Remove Enemies upon Death
  (if (`self.Arena Open`)
    _
    (elif (not (`KismetArrayLibrary.Array_IsEmpty` (`self.Spawned Enemies`)))
      (for (_array_element _array_index) (`self.Spawned Enemies`)
        (`/Engine/EditorBlueprintResources/StandardMacros.IsValid` _array_element
          (:`Is Not Valid`
            (`KismetArrayLibrary.Array_Remove` (`self.Spawned Enemies`) _array_index)
            (break))))
      (if (`KismetArrayLibrary.Array_IsEmpty` (`self.Spawned Enemies`))
        (`/Engine/EditorBlueprintResources/StandardMacros.DoOnce` false
          (:`Completed`
            ;;[0.03579 0.15 0 0.5] Add no Collision fot play test becaus we can vac or kick object after arena
            (`PrimitiveComponent.SetCollisionEnabled` (`self.Box`) "NoCollision")
            (if (`self.Need Cut Scene`)
              (`self.Cut Scene End`) ; New Event for Cut Scene
              (else
                (for _array_element_2 (`self.Door Ref`)
                  (`/Game/BPs/Arena/BP_Arena_Door.Open Door` _array_element_2))))
            (set `self.Arena Open` true)))))))

(event `self.ReceiveDestroyed`
  (bind _spawned_enemies (`self.Spawned Enemies`))
  (for _array_element _spawned_enemies :!label _label
    (`self.K2_DestroyActor` _array_element))
  (`KismetArrayLibrary.Array_Clear` _spawned_enemies))

(event `self.ReceiveEndPlay`
  (params (EndPlayReason :type "EEndPlayReason Enum" :default "Destroyed"))
  (goto _label))

(event `self.ReceiveBeginPlay`
  (bind _door_ref (`self.Door Ref`))
  (`KismetSystemLibrary.DelayUntilNextTick`)
  (bind _asbp_player (cast `/Game/Characters/Player/Blueprints/BP_Player` (`GameplayStatics.GetPlayerPawn` 0))
    (:`then`
      (set `self.Player Ref` _asbp_player)
      (if (`KismetArrayLibrary.Array_IsEmpty` _door_ref)
        (`KismetSystemLibrary.PrintString` "Door Ref in Arena NOT SET" true true (struct :`R` 1.0 :`A` 1.0) 10.0)
        (else
          (for _array_element _door_ref
            (`/Game/BPs/Arena/BP_Arena_Door.Open Door` _array_element))
          (if (`KismetArrayLibrary.Array_IsEmpty` (`self.Spawner Refs`))
            (`KismetSystemLibrary.PrintString` "Spawner Ref in Arena NOT SET" true true (struct :`R` 1.0 :`A` 1.0) 10.0)))))
    (:`CastFailed`
      (`KismetSystemLibrary.PrintString` "Invalid Player Ref in Arena" true true (struct :`R` 1.0 :`A` 1.0) 10.0))))

(event `self.Box.OnComponentBeginOverlap`
  (params (OverlappedComponent :type "PrimitiveComponent Object Reference") (OtherActor :type "Actor Object Reference") (OtherComp :type "PrimitiveComponent Object Reference") (OtherBodyIndex :type Integer) (bFromSweep :type Boolean) (SweepResult :type "HitResult Structure (by ref)"))
  ;[0.15 1 0.15] Spawn Enemies when player enters arena
  (if (== OtherActor (`self.Player Ref`))
    (`/Engine/EditorBlueprintResources/StandardMacros.DoOnce` false
      (:`Completed`
        (if (not (`self.Need Cut Scene`))
          (for _array_element (`self.Door Ref`)
            (`/Game/BPs/Arena/BP_Arena_Door.Close Door` _array_element)))
        (`PrimitiveComponent.SetCollisionEnabled` (`self.Box`) "NoCollision")
        (set `self.Arena Open` false)
        (`self.Cut Scene Start`)
        (`KismetSystemLibrary.Delay` 2.45) ; Need Delet
        (bind _succes (`self.Spawn Enemies`))
        (if (not _succes)
          (`KismetSystemLibrary.PrintString` "Arena Spawn Failed" true true (struct :`R` 1.0 :`A` 1.0) 10.0))))))

(event `self.Box.OnComponentEndOverlap`
  (params (OverlappedComponent :type "PrimitiveComponent Object Reference") (OtherActor :type "Actor Object Reference") (OtherComp :type "PrimitiveComponent Object Reference") (OtherBodyIndex :type Integer))
  ;[0.15 0.15 1] Close Doors when player leaves arena
  (`PrimitiveComponent.SetCollisionEnabled` (`self.Box`) "NoCollision")
  (if (and (== OtherActor (`self.Player Ref`)) (`self.Close Doors after player leaves ?`) (`self.Arena Open`))
    (for _array_element (`self.Door Ref`)
      (`/Game/BPs/Arena/BP_Arena_Door.Close Door` _array_element))))

(event `Cut Scene End`
  (if (`self.Need Cut Scene`)
    (bind (_outactor _returnvalue) (`LevelSequencePlayer.CreateLevelSequencePlayer` (`self.Level Sequence End`)))
    (`/Game/Characters/Player/Blueprints/WeaponSystem/Interactable/FL_Common.Play Cinematique` _returnvalue)))

(event `Cut Scene Start`
  (if (`self.Need Cut Scene`)
    (bind (_outactor _returnvalue) (`LevelSequencePlayer.CreateLevelSequencePlayer` (`self.Level Sequence Start`)))
    (`/Game/Characters/Player/Blueprints/WeaponSystem/Interactable/FL_Common.Play Cinematique` _returnvalue)))

(fn `Spawn Enemies`
  (returns (Succes :type Boolean))
  (bind _spawner_refs (`self.Spawner Refs`))
  (bind _actor_to_spawn (`self.Actor to Spawn`))
  (if (`KismetArrayLibrary.Array_IsNotEmpty` _spawner_refs)
    (for _array_element _spawner_refs
      ;[0 0.75 0.75] Enemy Spawn Logic
      (if (`KismetSystemLibrary.IsValidClass` _actor_to_spawn)
        (bind (_returnvalue_location _returnvalue_rotation) (`KismetMathLibrary.BreakTransform` (`SceneComponent.K2_GetComponentToWorld` (`/Game/BPs/BP_Spawner.DefaultSceneRoot` _array_element))))
        (bind _returnvalue (`|SpawnActorFromClass` _actor_to_spawn (`KismetMathLibrary.MakeTransform` (+ _returnvalue_location (`KismetMathLibrary.MakeVector` 0.0 0.0 (`self.Spawn Height Offset`))) _returnvalue_rotation (`self.Spawn Actor Scale`)) "AdjustIfPossibleButAlwaysSpawn" "MultiplyWithRoot" null null))
        (`KismetArrayLibrary.Array_AddUnique` (`self.Spawned Enemies`) _returnvalue)
        (else
          (`KismetSystemLibrary.PrintString` "Invalid Class to spawn in BP_Spawn")
          (return false))))
    (return true)
    (else
      (`KismetSystemLibrary.PrintString` "No Spawner Detected in Arena" true true (struct :`R` 1.0 :`A` 1.0) 10.0)
      (return false))))

(fn `UserConstructionScript`
  (bind (_box_size_x _box_size_y) (`KismetMathLibrary.BreakVector2D` (`self.Box Size`)))
  (bind _box (`self.Box`))
  (bind (_returnvalue_x _returnvalue_y _returnvalue_z) (`KismetMathLibrary.BreakVector` (`BoxComponent.GetUnscaledBoxExtent` _box)))
  (`BoxComponent.SetBoxExtent` _box (`KismetMathLibrary.MakeVector` _box_size_x _box_size_y _returnvalue_z) true))