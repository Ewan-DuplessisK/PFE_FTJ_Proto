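; Debug component that visualizes where the player's camera is aiming.
; TraceForward sphere-traces on the Camera channel from the player pawn's location along the camera's forward vector, ignoring that pawn.
; While Visible is set, Tick draws a one-frame debug sphere at the returned hit location, without checking whether the trace hit anything.
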(event `self.ReceiveTick`
  (params (DeltaSeconds :type "Float (single-precision)"))
  (if (`self.visible`)
    (`KismetSystemLibrary.DrawDebugSphere` (`.Location` (`GameplayStatics.BreakHitResult` (`self.Trace Forward`))) 50.0 12 (struct :`R` 1.0 :`B` 0.86413 :`A` 1.0) DeltaSeconds 1.0)))

(fn `Trace Forward`
  (returns (OutHit :type "HitResult Structure") (Bool :type Boolean))
  (bind _returnvalue (`GameplayStatics.GetPlayerPawn` 0))
  (bind _returnvalue_2 (`Actor.K2_GetActorLocation` _returnvalue))
  (bind (_outhit _returnvalue_3) (`KismetSystemLibrary.SphereTraceSingle` _returnvalue_2 (+ _returnvalue_2 (* (`KismetMathLibrary.GetForwardVector` (`PlayerCameraManager.GetCameraRotation` (`/Game/BPs/Other/FL_Common.Actor's Camera` _returnvalue))) 10000.0)) 25.0 "TraceTypeQuery2" false (`|MakeArray` (`GameplayStatics.GetPlayerPawn` 0) :!type "Actor Object Reference") "None" true (struct :`R` 1.0 :`A` 1.0) (struct :`G` 1.0 :`A` 1.0) 1.0))
  (return _outhit _returnvalue_3))