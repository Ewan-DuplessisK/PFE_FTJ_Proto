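; Debug controller that creates the WBP_Dbg overlay, toggled with Alt+D, and saves its visibility and options to a save slot.
; While visible, Tick feeds it player and vacuum values, with Score and actor Z editable.
; Hotkeys spawn or kill enemies and spawn suckables via a forward trace, kill the player, teleport, skip cinematics and end levels.
; A polling loop waits for level instances to load, then calls the player's SkipLoading.
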(event Custom|Toggle
  ;[0.15 0.15 0.15 0.5] OPEN WIDGET
  (CallFunction|SetVisibility (not (Variables|Default|GetVisible))))

(event Custom|Handle%20Level%20Loading%20_%20Loop%20Delay
  (Utilities|FlowControl|Delay 0.2)
  (CallFunction|HandleLevelLoading))

(event Custom|Delete%20SaveData
  (bind _returnvalue (SaveGame|DeleteGameinSlot "cu"))
  (Development|PrintString (Utilities|String|ToString(Text) (Utilities|Text|FormatText "Dbg: saved data deleted = {b}" (Utilities|String|ToString(Boolean) _returnvalue)))))

(event Custom|Set%20Visibility
  (params (Visible :type Boolean))
  (bind _returnvalue (Game|GetPlayerController 0))
  (bind _wbp_dbg (Variables|Default|GetWBP_Dbg))
  (bind _output_get (Variables|Default|SetVisible Visible))
  (Utilities|FlowControl|Delay 0.1)
  (if _output_get
    (Input|SetInputModeGameandUI _returnvalue _wbp_dbg "DoNotLock" false false)
    (Widget|SetVisibility _wbp_dbg "Visible")
    (else
      (Input|SetInputModeGameOnly _returnvalue false)
      (Widget|SetVisibility _wbp_dbg "Hidden"))))

(event Custom|Teleport%20Forward
  (bind _player (Variables|Default|GetPlayer))
  (bind _camera_man (CallFunction|Actor'sCamera _player))
  (bind _returnvalue (Camera|GetCameraRotation _camera_man))
  (bind _returnvalue_2 (Math|Vector|GetForwardVector _returnvalue))
  (Variables|Default|Setactor%20loc (Transformation|GetActorLocation _player))
  (bind (_outhit _returnvalue_3) (Collision|SphereTraceByChannel (+ (Variables|Default|Getactor%20loc) "0.000000,0.000000,50.000000" (* _returnvalue_2 1.2e+02)) (+ (+ (Variables|Default|Getactor%20loc) "0.000000,0.000000,50.000000" (* _returnvalue_2 1.2e+02)) (* _returnvalue_2 1e+04)) 25.0 "TraceTypeQuery2" false (Utilities|Array|MakeArray (Game|Player|GetPlayerPawn 0)) "None" true "(R=1.000000,G=0.000000,B=0.000000,A=1.000000)" "(R=0.000000,G=1.000000,B=0.000000,A=1.000000)" 1.0))
  (if _returnvalue_3
    (if (> (Math|Vector|Distance(Vector) (- (.Location (Collision|BreakHitResult _outhit)) (* _returnvalue_2 1.2e+02)) (Variables|Default|Getactor%20loc)) 2e+02)
      (bind _newtrack_0 (Timeline|Timeline PlayFromStart)
        (:Update
          (Transformation|SetActorLocation (Variables|Default|GetPlayer) (Math|Vector|Lerp(Vector) (Variables|Default|Getactor%20loc) (- (.Location (Collision|BreakHitResult _outhit)) (* _returnvalue_2 1.2e+02)) _newtrack_0) false false))
        (:Finished
          ;[0.15 0.15 0.15 0.5] restore control since on a ground
          (Utilities|FlowControl|Delay 0.1 :!label _label)
          (Default|EnablePlaying (Variables|Default|GetPlayer))
          (if (not (.bwalkablefloor (Variables|/Script/Engine.CharacterMovementComponent|GetCurrentFloor (Variables|/Script/Engine.Character|GetCharacterMovement (Variables|Default|GetPlayer)))))
            (goto _label)))))))

(event Custom|Save@
  (CallFunction|SaveSaveData))

(event EventBeginPlay
  (bind _returnvalue (Game|GetPlayerController 0))
  (Utilities|FlowControl|Sequence
    (:then_0
      (bind _asgi_systems (Utilities|Casting|CastToGI_Systems (Game|GetGameInstance)))
      (Variables|Default|SetGI%20Systems _asgi_systems)
      ;[0.15 0.15 0.15 0.5] Add Widget
      (bind _returnvalue_2 (AddComponent|AddWidgetComponent (HUD|GetHUD _returnvalue) false))
      (bind _returnvalue_3 (UserInterface|CreateWidget "/Game/BPs/Dbg/UI/WBP_Dbg.WBP_Dbg_C" _returnvalue))
      (UserInterface|SetWidget _returnvalue_2 _returnvalue_3)
      (Variables|Default|SetWBP_Dbg _returnvalue_3)
      (Class|WidgetComponent|SetWidgetSpace _returnvalue_2 "Screen")
      (Widget|SetVisibility _returnvalue_3 "Collapsed")
      (UserInterface|Viewport|AddtoViewport _returnvalue_3 0))
    (:then_1
      (bind _saved_data (CallFunction|LoadSaveData))
      (Utilities|FlowControl|Delay 0.1)
      (CallFunction|SetVisibility (and (Variables|/Game/BPs/Dbg/BP_Dbg_Save.BP_Dbg_Save_C|GetDbg%20Visible _saved_data) (Variables|Default|GetVisible%20Here))))
    (:then_2
      (bind _returnvalue_4 (Actor|GetActorOfClass "/Game/Characters/Player/Blueprints/BP_Vacuum.BP_Vacuum_C"))
      (Variables|Default|SetVacuum _returnvalue_4))
    (:then_3
      (bind _asbp_player (Utilities|Casting|CastToBP_Player (Game|Player|GetPlayerPawn 0)))
      (Variables|Default|SetPlayer _asbp_player))
    (:then_4)))

(event EventEndPlay
  (params (EndPlayReason :type EEndPlayReason%20Enum :default "Destroyed"))
  (Development|PrintString "Hello")
  (CallFunction|SaveSaveData))

(event EventDestroyed
  (Development|PrintString "Hello")
  (CallFunction|SaveSaveData))

(event EventTick
  (params (DeltaSeconds :type Float%20%28single-precision%29))
  (bind _returnvalue (Game|Player|GetPlayerPawn 0))
  (bind _returnvalue_2 (Subsystems|GetBPScoringSystemScore))
  (bind _vacuum (Variables|Default|GetVacuum))
  (bind _wbp_dbg (Variables|Default|GetWBP_Dbg))
  (bind _returnvalue_3 (Transformation|GetActorLocation _returnvalue))
  (Utilities|FlowControl|Sequence
    (:then_1
      (if (Variables|Default|GetVisible)
        (Utilities|FlowControl|Sequence
          (:then_0
            ;[0.15 0.15 0.15 0.5] Player
            ;;[0.15 0.15 0.15 0.5] Score
            (Utilities|IsValid (Variables|Default|GetPlayer)
              (:Is%20Valid
                (Default|AddHeader (Variables|Default|GetWBP_Dbg) "Character")
                (bind (_is_changed _last_changed) (Default|AddFloatEntry (Variables|Default|GetWBP_Dbg) "Score" (Variables|/Script/FThisJob.FTJ_ScoringSystem_ScoreBase|GetScore _returnvalue_2)))
                (if _is_changed
                  (Variables|/Script/FThisJob.FTJ_ScoringSystem_ScoreBase|SetScore _returnvalue_2 _last_changed))
                ;;[0.15 0.15 0.15 0.5] HP
                (Default|AddFloatEntry (Variables|Default|GetWBP_Dbg) "HP" (Variables|/Script/FThisJob.FTJ_CharaBase|GetCurrentHealth (Variables|Default|GetPlayer)))
                ;;[0.15 0.15 0.15 0.5] HP
                (Default|AddFloatEntry (Variables|Default|GetWBP_Dbg) "Timer" (Variables|/Game/BPs/LvlMan/GI_Systems_Base.GI_Systems_Base_C|GetTimer%20Time (Variables|Default|GetGI%20Systems)))
                ;;[0.15 0.15 0.15 0.5] Walk Speed
                (Default|AddFloatEntry (Variables|Default|GetWBP_Dbg) "Walk Speed" (Variables|/Script/Engine.CharacterMovementComponent|GetMaxWalkSpeed (Variables|/Script/Engine.Character|GetCharacterMovement (Variables|Default|GetPlayer))))
                ;;[0.15 0.15 0.15 0.5] Kick Cooldown
                (Default|AddFloatEntry (Variables|Default|GetWBP_Dbg) "Kick Cooldown" (Variables|/Game/_GameManager/Data_Assets/Data_3C/PDA_Player.PDA_Player_C|GetKickCooldown (Variables|/Game/Characters/Player/Blueprints/BP_Player.BP_Player_C|GetData_Asset_Player (Variables|Default|GetPlayer))))
                ;;[0.15 0.15 0.15 0.5] Actor Z
                (bind (_is_changed_2 _last_changed_2) (Default|AddFloatEntry (Variables|Default|GetWBP_Dbg) "Actor Z" (.z _returnvalue_3)))
                (Transformation|SetActorLocation _returnvalue (Math|Vector|MakeVector (.x _returnvalue_3) (.y _returnvalue_3) (Math|Float|SelectFloat _last_changed_2 (.z _returnvalue_3) _is_changed_2)) false false))))
          (:then_1
            ;[0.15 0.15 0.15 0.5] Vacuum
            (Utilities|IsValid _vacuum
              (:Is%20Valid
                (Default|AddHeader _wbp_dbg "Vaccum")
                (Default|AddFloatEntry _wbp_dbg "Blow Light" (Variables|/Game/Characters/Player/Blueprints/BP_Vacuum.BP_Vacuum_C|GetBlowForceLight _vacuum))
                (Default|AddFloatEntry _wbp_dbg "Blow Medium" (Variables|/Game/Characters/Player/Blueprints/BP_Vacuum.BP_Vacuum_C|GetBlowForceMedium _vacuum))
                (Default|AddFloatEntry _wbp_dbg "Blow Heavy" (Variables|/Game/Characters/Player/Blueprints/BP_Vacuum.BP_Vacuum_C|GetBlowForceHeavy _vacuum))
                (Default|AddFloatEntry _wbp_dbg "Shoot Delay" (Variables|/Game/Characters/Player/Blueprints/BP_Vacuum.BP_Vacuum_C|GetShootDelay _vacuum))))))))))

(event Input|KeyboardEvents|DebugKeyN
  (params (Key :type Key%20Structure :default "None") (ActionValue :type Input%20Action%20Value%20Structure)))

(event Input|KeyboardEvents|DebugKeyU
  (params (Key :type Key%20Structure :default "None") (ActionValue :type Input%20Action%20Value%20Structure)))

(event Input|KeyboardEvents|DebugKeyK
  (params (Key :type Key%20Structure :default "None") (ActionValue :type Input%20Action%20Value%20Structure)))

(event Input|KeyboardEvents|K
  (params (Key :type Key%20Structure :default "None"))
  (bind _ac_dbg_tracevisualizer (Variables|Default|GetAC_Dbg_TraceVisualizer))
  (bind (_outhit _bool) (Default|TraceForward _ac_dbg_tracevisualizer))
  (bind _hitactor (Collision|BreakHitResult _outhit))
  (:Pressed
    (Variables|/Game/BPs/Dbg/AC_Dbg_TraceVisualizer.AC_Dbg_TraceVisualizer_C|Setvisible _ac_dbg_tracevisualizer true))
  (:Released
    (Variables|/Game/BPs/Dbg/AC_Dbg_TraceVisualizer.AC_Dbg_TraceVisualizer_C|Setvisible _ac_dbg_tracevisualizer false)
    (if _bool
      (Utilities|IsValid _hitactor
        (:Is%20Valid
          (if (Utilities|Set|Contains (Variables|/Game/BPs/Dbg/UI/WBP_Dbg_SpawnClass2.WBP_Dbg_SpawnClass2_C|GetClasses (Variables|/Game/BPs/Dbg/UI/WBP_Dbg.WBP_Dbg_C|GetWBP_Dbg_SpawnEnemy (Variables|Default|GetWBP_Dbg))) (Utilities|GetClass _hitactor))
            (bind _ascharacter (Utilities|Casting|CastToCharacter _hitactor))
            (Class|HealthInterface|RemoveHealth(Message) _ascharacter 1e+03)))))))

(event Input|KeyboardEvents|AltD
  (params (Key :type Key%20Structure :default "None"))
  ;[0.15 0.15 0.15 0.5] OPEN WIDGET
  (:Pressed
    (CallFunction|SetVisibility (not (Variables|Default|GetVisible)))))

(event Input|KeyboardEvents|N
  (params (Key :type Key%20Structure :default "None"))
  (bind _ac_dbg_tracevisualizer (Variables|Default|GetAC_Dbg_TraceVisualizer))
  (bind (_outhit _bool) (Default|TraceForward _ac_dbg_tracevisualizer))
  (:Pressed
    (Variables|/Game/BPs/Dbg/AC_Dbg_TraceVisualizer.AC_Dbg_TraceVisualizer_C|Setvisible _ac_dbg_tracevisualizer true))
  (:Released
    (Variables|/Game/BPs/Dbg/AC_Dbg_TraceVisualizer.AC_Dbg_TraceVisualizer_C|Setvisible _ac_dbg_tracevisualizer false)
    (if _bool
      (Game|SpawnActorfromClass (Default|GetSpawnClassValue (Variables|/Game/BPs/Dbg/UI/WBP_Dbg.WBP_Dbg_C|GetWBP_Dbg_SpawnEnemy (Variables|Default|GetWBP_Dbg))) (Math|Transform|MakeTransform (.Location (Collision|BreakHitResult _outhit)) "0, 0, 0" "1.000000,1.000000,1.000000") "Undefined" "MultiplyWithRoot" 0 0))))

(event Input|KeyboardEvents|L
  (params (Key :type Key%20Structure :default "None"))
  (:Pressed
    (Class|HealthInterface|RemoveHealth(Message) (Game|Player|GetPlayerPawn 0) 1e+03)))

(event Input|KeyboardEvents|M
  (params (Key :type Key%20Structure :default "None"))
  (:Pressed
    (Default|EndLevel (CallFunction|GetGISystems))))

(event Input|MouseEvents|MiddleMouseButton
  (params (Key :type Key%20Structure :default "None"))
  (bind _player (Variables|Default|GetPlayer))
  (bind _camera_man (CallFunction|Actor'sCamera _player))
  (bind _returnvalue (Camera|GetCameraRotation _camera_man))
  (bind _returnvalue_2 (Math|Vector|GetForwardVector _returnvalue))
  (:Pressed
    (Variables|Default|Setactor%20loc (Transformation|GetActorLocation _player))
    (bind (_outhit _returnvalue_3) (Collision|SphereTraceByChannel (+ (Variables|Default|Getactor%20loc) "0.000000,0.000000,50.000000" (* _returnvalue_2 1.2e+02)) (+ (+ (Variables|Default|Getactor%20loc) "0.000000,0.000000,50.000000" (* _returnvalue_2 1.2e+02)) (* _returnvalue_2 1e+04)) 25.0 "TraceTypeQuery2" false (Utilities|Array|MakeArray (Game|Player|GetPlayerPawn 0)) "None" true "(R=1.000000,G=0.000000,B=0.000000,A=1.000000)" "(R=0.000000,G=1.000000,B=0.000000,A=1.000000)" 1.0))
    (if _returnvalue_3
      (if (> (Math|Vector|Distance(Vector) (- (.Location (Collision|BreakHitResult _outhit)) (* _returnvalue_2 1.2e+02)) (Variables|Default|Getactor%20loc)) 2e+02)
        (bind _newtrack_0 (Timeline|Timeline PlayFromStart)
          (:Update
            (Transformation|SetActorLocation (Variables|Default|GetPlayer) (Math|Vector|Lerp(Vector) (Variables|Default|Getactor%20loc) (- (.Location (Collision|BreakHitResult _outhit)) (* _returnvalue_2 1.2e+02)) _newtrack_0) false false))
          (:Finished
            ;[0.15 0.15 0.15 0.5] restore control since on a ground
            (Utilities|FlowControl|Delay 0.1 :!label _label)
            (Default|EnablePlaying (Variables|Default|GetPlayer))
            (if (not (.bwalkablefloor (Variables|/Script/Engine.CharacterMovementComponent|GetCurrentFloor (Variables|/Script/Engine.Character|GetCharacterMovement (Variables|Default|GetPlayer)))))
              (goto _label))))))))

(event Input|KeyboardEvents|U
  (params (Key :type Key%20Structure :default "None"))
  (bind _ac_dbg_tracevisualizer (Variables|Default|GetAC_Dbg_TraceVisualizer))
  (bind (_outhit _bool) (Default|TraceForward _ac_dbg_tracevisualizer))
  (:Pressed
    (Variables|/Game/BPs/Dbg/AC_Dbg_TraceVisualizer.AC_Dbg_TraceVisualizer_C|Setvisible _ac_dbg_tracevisualizer true))
  (:Released
    (Variables|/Game/BPs/Dbg/AC_Dbg_TraceVisualizer.AC_Dbg_TraceVisualizer_C|Setvisible _ac_dbg_tracevisualizer false)
    (if _bool
      (bind _returnvalue (Game|SpawnActorfromClass (Default|GetSpawnClassValue (Variables|/Game/BPs/Dbg/UI/WBP_Dbg.WBP_Dbg_C|GetWBP_Dbg_SpawnSuckables (Variables|Default|GetWBP_Dbg))) (Math|Transform|MakeTransform (.Location (Collision|BreakHitResult _outhit)) "0, 0, 0" "1.000000,1.000000,1.000000") "Undefined" "MultiplyWithRoot" 0 0))
      (bind _assuckable_prop_parent (Utilities|Casting|CastToSuckablePropParent _returnvalue))
      (Utilities|FlowControl|Delay 0.1)
      (Default|WakeUp _assuckable_prop_parent))))

(event Input|KeyboardEvents|Add
  (params (Key :type Key%20Structure :default "None"))
  (:Pressed
    (Default|SkipCinematique (CallFunction|GetGISystems))))

(fn ConstructionScript)

(fn LoadSaveData
  (bind _returnvalue (SaveGame|LoadGamefromSlot "Dbg"))
  (bind _asbp_dbg_save (Utilities|Casting|CastToBP_Dbg_Save _returnvalue)
    (:then
      (bind _output_get (Variables|Default|SetLast%20SaveData _asbp_dbg_save))
      (Default|CallOnSaveLoaded _output_get)
      (return _output_get))
    (:CastFailed
      (bind _returnvalue_2 (SaveGame|CreateSaveGameObject "/Game/BPs/Dbg/BP_Dbg_Save.BP_Dbg_Save_C"))
      (SaveGame|SaveGametoSlot _returnvalue_2 "Dbg")
      (CallFunction|LoadSaveData))))

(fn SaveSaveData
  (bind _wbp_dbg (Variables|Default|GetWBP_Dbg))
  (bind _returnvalue (SaveGame|CreateSaveGameObject "/Game/BPs/Dbg/BP_Dbg_Save.BP_Dbg_Save_C"))
  (Variables|/Game/BPs/Dbg/BP_Dbg_Save.BP_Dbg_Save_C|SetDbg%20Visible _returnvalue (Variables|Default|GetVisible))
  (Variables|/Game/BPs/Dbg/BP_Dbg_Save.BP_Dbg_Save_C|SetShow%20Collisions _returnvalue (Variables|/Game/BPs/Dbg/UI/WBP_Dbg_Bool.WBP_Dbg_Bool_C|GetValue (Variables|/Game/BPs/Dbg/UI/WBP_Dbg.WBP_Dbg_C|GetHitboxes _wbp_dbg)))
  (Variables|/Game/BPs/Dbg/BP_Dbg_Save.BP_Dbg_Save_C|SetPlayer%20Invincible _returnvalue (Variables|/Game/BPs/Dbg/UI/WBP_Dbg_Bool.WBP_Dbg_Bool_C|GetValue (Variables|/Game/BPs/Dbg/UI/WBP_Dbg.WBP_Dbg_C|GetWBP_Dbg_Invicible _wbp_dbg)))
  (Variables|/Game/BPs/Dbg/BP_Dbg_Save.BP_Dbg_Save_C|SetSkip%20Loading _returnvalue (Variables|/Game/BPs/Dbg/UI/WBP_Dbg_Bool.WBP_Dbg_Bool_C|GetValue (Variables|/Game/BPs/Dbg/UI/WBP_Dbg.WBP_Dbg_C|GetSkipLoading _wbp_dbg)))
  (SaveGame|SaveGametoSlot _returnvalue "Dbg")
  (return _returnvalue))

(fn HandleLevelLoading
  (bind _outactors (Actor|GetAllActorsOfClass "/Script/Engine.LevelInstance"))
  (if (Math|Conversions|ToBoolean(Integer) (Utilities|Array|Length _outactors))
    (Variables|Default|Setnow%20loaded 0)
    (for _array_element _outactors
      (Development|PrintText (Utilities|Text|FormatText "{name} = {loaded} {hidden} {assets}" (Utilities|GetDisplayName _array_element) (Class|LevelInstanceInterface|IsLoaded _array_element)) true true "(R=0.000000,G=0.660000,B=1.000000,A=1.000000)" 5.0)
      (if (or (Class|KismetStringLibrary|MatchesWildcard (Utilities|GetDisplayName _array_element) "*blockout*" "IgnoreCase") (Class|LevelInstanceInterface|IsLoaded _array_element))
        (Math|Integer|IncrementInt (Variables|Default|Getnow%20loaded))))
    (Development|PrintText (Utilities|Text|FormatText "Loading Level Instances: {a} / {b}" (Variables|Default|Getnow%20loaded) (Utilities|Array|Length _outactors)) true true "(R=0.000000,G=0.660000,B=1.000000,A=1.000000)" 2.0 "LOADING_LEVEL")
    (if (and (== (Variables|Default|Getlast%20levels%20num) (Utilities|Array|Length _outactors)) (== (Utilities|Array|Length _outactors) (Variables|Default|Getnow%20loaded)))
      (Development|PrintString "LOADED" true true "(R=1.000000,G=0.000000,B=0.875273,A=1.000000)" 5.0)
      (bind _asbp_player (Utilities|Casting|CastToBP_Player (Game|Player|GetPlayerPawn 0)))
      (Default|SkipLoading _asbp_player)
      (else
        (Variables|Default|Setlast%20levels%20num (Utilities|Array|Length _outactors))
        (CallFunction|HandleLevelLoadingLoopDelay :!label _label)))
    (else
      (Development|PrintString "No Instances to wait :(")
      (goto _label))))