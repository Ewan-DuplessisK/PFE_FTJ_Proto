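; Medium variant of a vacuum-suckable physics prop that can be thrown to damage actors and breakables, pulling its stats from a data asset.
; Hits wake sleeping props, request speed-based impact sounds through a throttle, and apply armed damage once, sparing the player unless it is an enemy attack.
; Damaging hits wear down durability; at zero it spawns destruction VFX, awards score and multiplier, then returns to its pool.
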(event `self.ReceiveBeginPlay`
  (bind _da (`self.DA`))
  (`parent.ReceiveBeginPlay`)
  (set `self.BaseHealth` (`/Game/BPs/VacuumProps/PDA_Props.BaseHealth_Med` _da))
  (set `self.DestructionVFX` (`/Game/BPs/VacuumProps/PDA_Props.DestructionVFX_Med` _da))
  (set `self.ScoreOnDestruction` (`/Game/BPs/VacuumProps/PDA_Props.ScoreOnDestruction_Med` _da))
  (set `self.MultiplierOnDestruction` (`/Game/BPs/VacuumProps/PDA_Props.MultiplierOnDestruction_Med` _da))
  (set `self.MessageOnDestruction` (`/Game/BPs/VacuumProps/PDA_Props.MessageOnDestruction_Med` _da))
  (set `self.Damage` (`/Game/BPs/VacuumProps/PDA_Props.Damage_Med` _da))
  (set `self.DamageToBreakable` (`/Game/BPs/VacuumProps/PDA_Props.DamageToBreakable_Med` _da))
  (`KismetSystemLibrary.Delay` 0.2)
  (bind _returnvalue (`GameplayStatics.GetActorOfClass` "/Game/BPs/Sounds/BP_SoundEmitterManager.BP_SoundEmitterManager_C"))
  (set `self.SoundEmitter` _returnvalue))

(event `self.LooseDurability`
  (bind _result (`/Engine/EditorBlueprintResources/StandardMacros.DecrementInt` (`self.Health`))
    (:`  `
      (if (<= _result 0)
        (bind _destructionvfx (`self.DestructionVFX`)
          (:`then`
            (`NiagaraFunctionLibrary.SpawnSystemAtLocation` _destructionvfx (`self.K2_GetActorLocation`)))
          (:`else`
            _))
        (`FTJ_ScoringSystem_Score.IncreaseWithText` (subsystem `/Game/CppSystems/ScoringSystem/Public/Blueprint/BP_ScoringSystem_Score`) (`KismetMathLibrary.Conv_IntToDouble` (`self.ScoreOnDestruction`)) (`self.MultiplierOnDestruction`) false (`self.MessageOnDestruction`))
        (`KismetSystemLibrary.Delay` 0.3)
        (`PooledActor_Component.SetInUse` (`self.PooledActor_Component`) false)))))

(event `self.ReceiveHit`
  (params (MyComp :type "PrimitiveComponent Object Reference") (Other :type "Actor Object Reference") (OtherComp :type "PrimitiveComponent Object Reference") (bSelfMoved :type Boolean) (HitLocation :type "Vector Structure") (HitNormal :type "Vector Structure") (NormalImpulse :type "Vector Structure") (Hit :type "HitResult Structure (by ref)"))
  (if (!= (`self.HoldingActor`) Other)
    (`|ExecutionSequence`
      (:`then_0`
        (if (`self.Asleep`)
          (cast `SuckablePropParent` Other
            (:`then`
              (if (> (`KismetMathLibrary.VSize` (`SceneComponent.GetComponentVelocity` (`self.StaticMeshComp`))) (`self.SleepVelocity`))
                (`self.WakeUp` :!label _label)))
            (:`CastFailed`
              (goto _label)))))
      (:`then_1`
        (`self.SoundOnFloorHit`))
      (:`then_2`
        (`/Engine/EditorBlueprintResources/StandardMacros.IsValid` Other
          (:`Is Valid`
            (if (and (`self.DamageEnabled`) (or (not (`self.ActorHasTag` Other "Player")) (`self.EnemyAttack`)))
              (if (`self.bCanHitOnce`)
                (set `self.bCanHitOnce` false)
                (message `HitInterface.GetHit` Other (`self.Damage`) 0.0 HitNormal 0.0 self)
                (message `HealthInterface.DamageBreakable` Other (`self.DamageToBreakable`) HitNormal)
                (`|ExecutionSequence` :!label _label_2
                  (:`then_0`
                    (`KismetSystemLibrary.Delay` 0.1)
                    (set `self.DamageEnabled` false)
                    (set `self.EnemyAttack` false)
                    (set `self.HoldingActor` null)
                    (`PrimitiveComponent.SetCollisionObjectType` (`self.StaticMeshComp`) "ECC_GameTraceChannel7"))
                  (:`then_1`
                    (`self.LooseDurability`))))))
          (:`Is Not Valid`
            (goto _label_2)))))))

(event `self.ActivateTrail`
  (bind _trailcomp (`self.TrailComp`))
  (`ActorComponent.Activate` _trailcomp true)
  (`KismetSystemLibrary.Delay` 3.0)
  (`ActorComponent.Deactivate` _trailcomp))

(event `/Game/BPs/BPI_Push.Push`
  (params (Force :type "Vector Structure"))
  (`self.WakeUp`)
  (`PrimitiveComponent.AddImpulse` (`self.StaticMeshComp`) Force "None" true))

(event `SoundOnFloorHit`
  (bind _returnvalue (`KismetMathLibrary.VSize` (`self.GetVelocity`)))
  (if (> _returnvalue 200.0)
    (`/Engine/EditorBlueprintResources/StandardMacros.DoOnce` false :!label _label_3
      (:`Completed`
        (`/Game/BPs/Sounds/BP_SoundEmitterManager.RequestImpactSound` (`self.SoundEmitter`) (`self.SoundType`) (`self.K2_GetActorLocation`) _returnvalue)
        (`KismetSystemLibrary.Delay` 0.2)
        (goto _label_3 :!via `Reset`)))))

(fn `UserConstructionScript`
  (`parent.UserConstructionScript`)
  (`StaticMeshComponent.SetStaticMesh` (`self.StaticMeshComp`) (`self.Mesh`)))