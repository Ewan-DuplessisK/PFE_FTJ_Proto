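; Suckable fire extinguisher prop that, when active and hitting something other than the player, turns into an erratic rocket and then explodes.
; On BeginPlay it leaves a wall-mount mesh behind and loads tuning from its data asset.
; A looping timer applies thrust and random torque until the fuse ends.
; A material swell timeline precedes Niagara debris and sphere traces that damage pawns, push props and hit breakables.
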(event `self.ReceiveBeginPlay`
  (bind _da (`self.DA`))
  (`parent.ReceiveBeginPlay`)
  (bind _returnvalue (`|SpawnActorFromClass` "/Script/Engine.StaticMeshActor" (`SceneComponent.K2_GetComponentToWorld` (`self.Wall_Attach`)) "Undefined" "MultiplyWithRoot" null null))
  (bind _staticmeshcomponent (`StaticMeshActor.StaticMeshComponent` _returnvalue))
  (`StaticMeshComponent.SetStaticMesh` _staticmeshcomponent "/Game/Hero_Props/Extinguisher/Meshes/SM_ExtinguisherExtras_00.SM_ExtinguisherExtras_00")
  (`PrimitiveComponent.SetCollisionEnabled` _staticmeshcomponent "NoCollision")
  (`ActorComponent.K2_DestroyComponent` (`self.Wall_Attach`))
  (set `self.BaseHealth` (`/Game/BPs/VacuumProps/PDA_Props.BaseHealth_Ext` _da))
  (set `self.DestructionVFX` (`/Game/BPs/VacuumProps/PDA_Props.DestructionVFX_Ext` _da))
  (set `self.ScoreOnDestruction` (`/Game/BPs/VacuumProps/PDA_Props.ScoreOnDestruction_Ext` _da))
  (set `self.MultiplierOnDestruction` (`/Game/BPs/VacuumProps/PDA_Props.MultiplierOnDestruction_Ext` _da))
  (set `self.MessageOnDestruction` (`/Game/BPs/VacuumProps/PDA_Props.MessageOnDestruction_Ext` _da))
  (set `self.Damage` (`/Game/BPs/VacuumProps/PDA_Props.Damage_Ext` _da))
  (set `self.DamageToBreakable` (`/Game/BPs/VacuumProps/PDA_Props.DamageToBreakable_Ext` _da))
  (set `self.AOE_Radius` (`/Game/BPs/VacuumProps/PDA_Props.AOE_Radius_Ext` _da))
  (set `self.PushForceEnemies` (`/Game/BPs/VacuumProps/PDA_Props.PushForceEnemies_Ext` _da))
  (set `self.PushForceProps` (`/Game/BPs/VacuumProps/PDA_Props.PushForceProps_Ext` _da))
  (set `self.Leaking_Speed` (`/Game/BPs/VacuumProps/PDA_Props.LeakingSpeed` _da))
  (set `self.RandomDirectionForce` (`/Game/BPs/VacuumProps/PDA_Props.RandomDirectionForce` _da))
  (set `self.FlightDuration` (`/Game/BPs/VacuumProps/PDA_Props.FlightDuration` _da))
  (set `self.DamageWhenFlying` (`/Game/BPs/VacuumProps/PDA_Props.FlyingDamage` _da))
  (set `self.ExplosionGrowthTime` (`/Game/BPs/VacuumProps/PDA_Props.ExplosionGrowthTime` _da))
  (`ActorComponent.Deactivate` (`self.Ak_Extinguisher`)))

(event `self.ReceiveTick`
  (params (DeltaSeconds :type "Float (single-precision)")))

(event `self.ReceiveHit`
  (params (MyComp :type "PrimitiveComponent Object Reference") (Other :type "Actor Object Reference") (OtherComp :type "PrimitiveComponent Object Reference") (bSelfMoved :type Boolean) (HitLocation :type "Vector Structure") (HitNormal :type "Vector Structure") (NormalImpulse :type "Vector Structure") (Hit :type "HitResult Structure (by ref)"))
  (bind _returnvalue (`KismetMathLibrary.VSize` (`self.GetVelocity`)))
  (if (`self.IsActive`)
    (`|ExecutionSequence`
      (:`then_0`
        (if (not (`self.ActorHasTag` Other "Player"))
          (message `HitInterface.GetHit` Other (`self.DamageWhenFlying`) 0.0 (0.0 0.0 0.0) 0.0 null)
          (`/Engine/EditorBlueprintResources/StandardMacros.DoOnce` false
            (:`Completed`
              (bind _returnvalue_2 (`KismetSystemLibrary.K2_SetTimerDelegate` (delegate `ExtinguisherFly`) 0.033333 true true))
              (set `self.FlightTimeHandle` _returnvalue_2)))))
      (:`then_1`
        ;[0.5555 0.04653 0.724 0.5] SFX Extinguisher Impact Velocity
        (if (> _returnvalue 50.0)
          (`|ExecutionSequence`
            (:`then_0`
              (`/Engine/EditorBlueprintResources/StandardMacros.DoOnce` false :!label _label
                (:`Completed`
                  (`/Game/BPs/Sounds/BP_SoundEmitterManager.RequestEventRTPC` (`self.SoundEmitter`) "/Game/WwiseAudio/Events/Default_Work_Unit/GPE/GPE_LVL_01/Extinguisher_ImpactFloor.Extinguisher_ImpactFloor" (`self.K2_GetActorLocation`) _returnvalue "/Game/WwiseAudio/Game_Parameters/GPE/RTPC_Extinguisher_Volume.RTPC_Extinguisher_Volume")
                  (`KismetSystemLibrary.Delay` 0.2)
                  (goto _label :!via `Reset`))))
            (:`then_1`
              (`/Engine/EditorBlueprintResources/StandardMacros.DoOnce` false
                (:`Completed`
                  (`ActorComponent.Activate` (`self.Ak_Extinguisher`) false)
                  (`AkGameObject.PostAkEvent` :`self` (`self.Ak_Extinguisher`) :`AkEvent` "/Game/WwiseAudio/Events/Default_Work_Unit/GPE/GPE_LVL_01/Extinguisher_Steam.Extinguisher_Steam"))))))))))

(event `ExtinguisherFly`
  (`ActorComponent.Activate` (`self.TrailComp`) true)
  (`PrimitiveComponent.AddForce` (`self.StaticMeshComp`) (* (* (`SceneComponent.GetUpVector` (`self.StaticMeshComp`)) (`KismetMathLibrary.Conv_DoubleToVector` -1.0)) (`self.Leaking_Speed`)) "None" true)
  (`PrimitiveComponent.AddTorqueInDegrees` (`self.StaticMeshComp`) (* (`KismetMathLibrary.RandomUnitVector`) (`self.RandomDirectionForce`)) "None" true)
  (`/Engine/EditorBlueprintResources/StandardMacros.DoOnce` false
    (:`Completed`
      (bind _returnvalue (`KismetSystemLibrary.K2_SetTimerDelegate` (delegate `Explode`) 0.03 false false (`self.FlightDuration`)))
      (set `self.ExplosionTimeHandle` _returnvalue))))

(event `Explode`
  (bind _returnvalue (`self.K2_GetActorLocation`))
  (bind _returnvalue_2 (`self.K2_GetActorLocation`))
  (bind _returnvalue_3 (`self.K2_GetActorLocation`))
  (bind _staticmeshcomp (`self.StaticMeshComp`))
  (bind _staticmeshcomp_2 (`self.StaticMeshComp`))
  (`ActorComponent.Deactivate` (`self.Ak_Extinguisher`))
  (`KismetSystemLibrary.K2_ClearAndInvalidateTimerHandle` (`self.FlightTimeHandle`))
  (`KismetSystemLibrary.DelayUntilNextTick`)
  (`TimelineComponent.SetPlayRate` (`self.Timeline`) (/ 1.0 (`self.ExplosionGrowthTime`)))
  (bind _returnvalue_4 (`PrimitiveComponent.CreateDynamicMaterialInstance` (`self.StaticMeshComp`) 0 null "None"))
  (set `self.DynMatRef` _returnvalue_4)
  (bind (_direction _explosion) (`Timeline|Timeline` :!via `PlayFromStart`)
    (:`Update`
      (`/Engine/EditorBlueprintResources/StandardMacros.IsValid` (`self.StaticMeshComp`)
        (:`Is Valid`
          (`MaterialInstanceDynamic.SetScalarParameterValue` (`self.DynMatRef`) "Positions_Boing" _explosion))))
    (:`Finished`
      (`PrimitiveComponent.SetSimulatePhysics` _staticmeshcomp_2 false)
      (`PrimitiveComponent.SetCollisionEnabled` _staticmeshcomp_2 "NoCollision")
      (`SceneComponent.SetHiddenInGame` (`self.StaticMeshComp`) false false)
      ;[0.03659 0.6519 0.7708 0.5] VFX
      (bind _returnvalue_5 (`NiagaraFunctionLibrary.SpawnSystemAtLocation` (`self.NS_PropsBreak`) (+ (`SceneComponent.K2_GetComponentLocation` _staticmeshcomp) (0.0 0.0 15.0)) (`SceneComponent.K2_GetComponentRotation` _staticmeshcomp)))
      (`NiagaraComponent.SetVariableFloat` _returnvalue_5 "Velocity" 2500.0)
      (`NiagaraComponent.SetVariableFloat` _returnvalue_5 "Velocity_ConeAngle" 360.0)
      (`NiagaraComponent.SetVariableInt` _returnvalue_5 "SmokeCount" 0)
      (`/Game/VFX/Blueprint/BPFL_FX_DataTable_To_BreakableProp.SendBreakablePropDataToNiagara` (`self.Data Table`) _returnvalue_5 (`self.Mesh Renderer`) (`self.FX_Material`))
      (`NiagaraFunctionLibrary.SpawnSystemAtLocation` (`self.NS_Smoke`) _returnvalue_3)
      (bind _outhits (`KismetSystemLibrary.SphereTraceMultiForObjects` _returnvalue_3 _returnvalue_3 (`self.AOE_Radius`) (`|MakeArray` "ObjectTypeQuery3" "ObjectTypeQuery19" :!type "EObjectTypeQuery Enum")))
      (for _array_element _outhits
        (bind (_bblockinghit _binitialoverlap _time _distance _location _impactpoint _normal _impactnormal _physmat _hitactor) (`GameplayStatics.BreakHitResult` _array_element))
        (message `HitInterface.GetHit` _hitactor (`self.Damage`) 0.0 (* (- (`self.K2_GetActorLocation` _hitactor) (`self.K2_GetActorLocation`)) (`self.PushForceEnemies`)) 0.0 null))
      (bind _outhits_2 (`KismetSystemLibrary.SphereTraceMultiForObjects` _returnvalue_2 _returnvalue_2 (`self.AOE_Radius`) (`|MakeArray` "ObjectTypeQuery13" "ObjectTypeQuery23" :!type "EObjectTypeQuery Enum")))
      (for _array_element_2 _outhits_2
        (bind _assuckable_prop_parent (cast `SuckablePropParent` (`.HitActor` (`GameplayStatics.BreakHitResult` _array_element_2))))
        (set `self.currprop` _assuckable_prop_parent)
        (message `/Game/BPs/BPI_Push.Push` (`self.currprop`) (* (- (`self.K2_GetActorLocation` (`self.currprop`)) (`self.K2_GetActorLocation`)) (`self.PushForceProps`))))
      (bind _outhits_3 (`KismetSystemLibrary.SphereTraceMultiForObjects` _returnvalue _returnvalue (`self.AOE_Radius`) (`|MakeArray` "ObjectTypeQuery4" "ObjectTypeQuery2" "ObjectTypeQuery12" :!type "EObjectTypeQuery Enum")))
      (for _array_element_3 _outhits_3
        (message `HealthInterface.DamageBreakable` (`.HitActor` (`GameplayStatics.BreakHitResult` _array_element_3)) (`self.DamageToBreakable`) (`KismetMathLibrary.Normal` (- (`self.K2_GetActorLocation`) (`self.K2_GetActorLocation`)))))
      (`/Engine/EditorBlueprintResources/StandardMacros.DoOnce` false
        (:`Completed`
          (`AkGameplayStatics.PostEvent` "/Game/WwiseAudio/Events/Default_Work_Unit/GPE/GPE_LVL_01/Extinguisher_ImpactExplosion.Extinguisher_ImpactExplosion")
          (`KismetSystemLibrary.Delay` 0.2)
          (`self.K2_DestroyActor`))))))

(fn `UserConstructionScript`
  (`parent.UserConstructionScript`))