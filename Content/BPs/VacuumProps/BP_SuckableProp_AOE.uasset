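; Explosive variant of a suckable prop that, once ready to shoot, detonates on its first hit against anything other than its holder or another suckable prop.
; BeginPlay copies AOE tuning from a data asset, and detonation runs three sphere traces to damage and knock back pawns, push non-AOE props and damage breakables.
; It plays sounds through BP_SoundEmitterManager, shows explosion VFX, hides, then awards score and destroys itself after a delay.
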(event `self.ReceiveBeginPlay`
  (bind _da (`self.DA`))
  (set `self.BaseHealth` (`/Game/BPs/VacuumProps/PDA_Props.BaseHealth_AOE` _da))
  (set `self.DestructionVFX` (`/Game/BPs/VacuumProps/PDA_Props.DestructionVFX_AOE` _da))
  (set `self.ScoreOnDestruction` (`/Game/BPs/VacuumProps/PDA_Props.ScoreOnDestruction_AOE` _da))
  (set `self.MultiplierOnDestruction` (`/Game/BPs/VacuumProps/PDA_Props.MultiplierOnDestruction_AOE` _da))
  (set `self.MessageOnDestruction` (`/Game/BPs/VacuumProps/PDA_Props.MessageOnDestruction_AOE` _da))
  (set `self.Damage` (`/Game/BPs/VacuumProps/PDA_Props.Damage_AOE` _da))
  (set `self.DamageToBreakable` (`/Game/BPs/VacuumProps/PDA_Props.DamageToBreakable_AOE` _da))
  (set `self.AOE_Radius` (`/Game/BPs/VacuumProps/PDA_Props.AOE_Radius` _da))
  (set `self.PushForceEnemies` (`/Game/BPs/VacuumProps/PDA_Props.PushForceEnemies` _da))
  (set `self.PushForceProps` (`/Game/BPs/VacuumProps/PDA_Props.PushForceProps` _da))
  (`KismetSystemLibrary.Delay` 0.2)
  (bind _returnvalue (`GameplayStatics.GetActorOfClass` "/Game/BPs/Sounds/BP_SoundEmitterManager.BP_SoundEmitterManager_C"))
  (bind _output_get (set `self.SoundEmitter` _returnvalue))
  (`/Engine/EditorBlueprintResources/StandardMacros.IsValid` _output_get
    (:`Is Not Valid`
      (`KismetSystemLibrary.PrintString` "Heavy emitter not valid"))))

(event `self.OnSetReadyToShoot`
  (`parent.OnSetReadyToShoot`)
  (set `self.IsActive` true))

(event `self.ReceiveHit`
  (params (MyComp :type "PrimitiveComponent Object Reference") (Other :type "Actor Object Reference") (OtherComp :type "PrimitiveComponent Object Reference") (bSelfMoved :type Boolean) (HitLocation :type "Vector Structure") (HitNormal :type "Vector Structure") (NormalImpulse :type "Vector Structure") (Hit :type "HitResult Structure (by ref)"))
  (bind _returnvalue (`self.K2_GetActorLocation`))
  (bind _returnvalue_2 (`self.K2_GetActorLocation`))
  (bind _returnvalue_3 (`self.K2_GetActorLocation`))
  (bind _staticmeshcomp (`self.StaticMeshComp`))
  (bind _array (`|MakeArray` (`GameplayStatics.GetPlayerPawn` 0) :!type "Actor Object Reference"))
  (if (!= (`self.HoldingActor`) Other)
    (if (`self.IsActive`)
      (cast `SuckablePropParent` Other
        (:`CastFailed`
          (`/Engine/EditorBlueprintResources/StandardMacros.DoOnce` false
            (:`Completed`
              (bind _outhits (`KismetSystemLibrary.SphereTraceMultiForObjects` _returnvalue_2 _returnvalue_2 (`self.AOE_Radius`) (`|MakeArray` "ObjectTypeQuery3" "ObjectTypeQuery19" :!type "EObjectTypeQuery Enum")))
              (for _array_element _outhits
                (bind (_bblockinghit _binitialoverlap _time _distance _location _impactpoint _normal _impactnormal _physmat _hitactor) (`GameplayStatics.BreakHitResult` _array_element))
                (message `HitInterface.GetHit` _hitactor (`self.Damage`) 0.0 (* (- (`self.K2_GetActorLocation` _hitactor) (`self.K2_GetActorLocation`)) (`self.PushForceEnemies`)) 0.0 self))
              (bind _outhits_2 (`KismetSystemLibrary.SphereTraceMultiForObjects` _returnvalue _returnvalue (`self.AOE_Radius`) (`|MakeArray` "ObjectTypeQuery13" "ObjectTypeQuery23" :!type "EObjectTypeQuery Enum") false _array))
              (for _array_element_2 _outhits_2
                (bind (_bblockinghit_2 _binitialoverlap_2 _time_2 _distance_2 _location_2 _impactpoint_2 _normal_2 _impactnormal_2 _physmat_2 _hitactor_2) (`GameplayStatics.BreakHitResult` _array_element_2))
                (cast `/Game/BPs/VacuumProps/BP_SuckableProp_AOE` _hitactor_2
                  (:`CastFailed`
                    (bind _assuckable_prop_parent (cast `SuckablePropParent` _hitactor_2))
                    (set `self.currprop` _assuckable_prop_parent)
                    (message `/Game/BPs/BPI_Push.Push` (`self.currprop`) (* (- (`self.K2_GetActorLocation` (`self.currprop`)) (`self.K2_GetActorLocation`)) (`self.PushForceProps`)))
                    (`self.IsWater`
                      (:`then`
                        (`/Game/BPs/Sounds/BP_SoundEmitterManager.RequestShootSound` (`self.SoundEmitter`) (`self.K2_GetActorLocation`) "/Game/WwiseAudio/Events/Default_Work_Unit/SFX/SFX_LVL_01/Water_Launch.Water_Launch"))
                      (:`else`
                        (`/Game/BPs/Sounds/BP_SoundEmitterManager.RequestShootSound` (`self.SoundEmitter`) (`self.K2_GetActorLocation`) "/Game/WwiseAudio/Events/Default_Work_Unit/SFX/SFX_LVL_01/Water_Launch.Water_Launch"))))))
              (bind _outhits_3 (`KismetSystemLibrary.SphereTraceMultiForObjects` _returnvalue_3 _returnvalue_3 (`self.AOE_Radius`) (`|MakeArray` "ObjectTypeQuery4" "ObjectTypeQuery2" :!type "EObjectTypeQuery Enum") false _array))
              (for _array_element_3 _outhits_3
                (bind (_bblockinghit_3 _binitialoverlap_3 _time_3 _distance_3 _location_3 _impactpoint_3 _normal_3 _impactnormal_3 _physmat_3 _hitactor_3) (`GameplayStatics.BreakHitResult` _array_element_3))
                (message `HealthInterface.DamageBreakable` _hitactor_3 (`self.DamageToBreakable`) (`KismetMathLibrary.Normal` (- (`self.K2_GetActorLocation` _hitactor_3) (`self.K2_GetActorLocation`))))
                (`self.IsWater`
                  (:`then`
                    (`/Engine/EditorBlueprintResources/StandardMacros.DoOnce` false
                      (:`Completed`
                        (`/Game/BPs/Sounds/BP_SoundEmitterManager.RequestShootSound` (`self.SoundEmitter`) (`self.K2_GetActorLocation`) "/Game/WwiseAudio/Events/Default_Work_Unit/SFX/SFX_LVL_01/Water_Impact.Water_Impact"))))
                  (:`else`
                    (`/Engine/EditorBlueprintResources/StandardMacros.DoOnce` false
                      (:`Completed`
                        (`/Game/BPs/Sounds/BP_SoundEmitterManager.RequestShootSound` (`self.SoundEmitter`) (`self.K2_GetActorLocation`) "/Game/WwiseAudio/Events/Default_Work_Unit/SFX/SFX_LVL_02/Water_ExplosionElec.Water_ExplosionElec"))))))
              (`/Engine/EditorBlueprintResources/StandardMacros.DoOnce` false
                (:`Completed`
                  (`ActorComponent.Activate` (`self.NS_Explosion`) false)
                  (`ActorComponent.Deactivate` (`self.TrailComp`))
                  (`SceneComponent.SetHiddenInGame` _staticmeshcomp true false)
                  (`PrimitiveComponent.SetCollisionEnabled` _staticmeshcomp "NoCollision")
                  (`KismetSystemLibrary.Delay` 5.0)
                  (`self.DestroyShield`))))))))))

(event `self.DestroyShield`
  (set `self.Health` 1)
  (`self.LooseDurability`))

(event `self.LooseDurability`
  (bind _result (`/Engine/EditorBlueprintResources/StandardMacros.DecrementInt` (`self.Health`))
    (:`  `
      (if (<= _result 0)
        (bind _destructionvfx (`self.DestructionVFX`)
          (:`then`
            (`NiagaraFunctionLibrary.SpawnSystemAtLocation` _destructionvfx (`self.K2_GetActorLocation`)))
          (:`else`
            _))
        (`FTJ_ScoringSystem_Score.IncreaseWithText` (subsystem `/Game/CppSystems/ScoringSystem/Public/Blueprint/BP_ScoringSystem_Score`) (`KismetMathLibrary.Conv_IntToDouble` (`self.ScoreOnDestruction`)) (`self.MultiplierOnDestruction`) false (`self.MessageOnDestruction`))
        (`KismetSystemLibrary.DelayUntilNextTick`)
        (`self.K2_DestroyActor`)))))

(fn `UserConstructionScript`
  (`parent.UserConstructionScript`))