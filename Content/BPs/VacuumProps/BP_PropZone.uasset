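; Prop zone for the vacuum game that switches HISM instances inside its box to pooled suckable props and back.
; Overlapped HISMs go to parent-class populate and switch functions, with initial population spread across frames by a spawn cutoff.
; Player triggers bump the Zone to refire overlaps, a trick also used on the triggers at restart and reload.
; When the player leaves, sleeping, unheld props become HISM instances again and are released to the pool.
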(event `ActivateAgain`
  (`KismetArrayLibrary.Array_Clear` (`self.Props`))
  (for _array_element (`PrimitiveComponent.GetOverlappingComponents` (`self.Zone`))
    (bind _ashierarchical_instanced_static_mesh_component (cast `HierarchicalInstancedStaticMeshComponent` _array_element))
    (`KismetArrayLibrary.Array_AddUnique` (`self.Props`) _ashierarchical_instanced_static_mesh_component))
  (`self.PopulateZone`))

(event `RestartZone`
  (bind _trigger2 (`self.Trigger2`))
  (bind _trigger1 (`self.Trigger1`))
  (bind _trigger2_2 (`self.Trigger2`))
  (bind _trigger1_2 (`self.Trigger1`))
  (bind (_relativelocation_x _relativelocation_y _relativelocation_z) (`KismetMathLibrary.BreakVector` (`SceneComponent.RelativeLocation` _trigger2_2)))
  (bind (_relativelocation_x_2 _relativelocation_y_2 _relativelocation_z_2) (`KismetMathLibrary.BreakVector` (`SceneComponent.RelativeLocation` _trigger1_2)))
  (bind (_relativelocation_x_3 _relativelocation_y_3 _relativelocation_z_3) (`KismetMathLibrary.BreakVector` (`SceneComponent.RelativeLocation` _trigger1)))
  (bind (_relativelocation_x_4 _relativelocation_y_4 _relativelocation_z_4) (`KismetMathLibrary.BreakVector` (`SceneComponent.RelativeLocation` _trigger2)))
  (set `self.Init` true)
  (bind _asbp_player (cast `/Game/Characters/Player/Blueprints/BP_Player` (`GameplayStatics.GetPlayerPawn` 0) :!label _label))
  (set `self.As BP Player` _asbp_player)
  (set `self.Pool_Parent` (`/Game/Characters/Player/Blueprints/BP_Player.ObjectPool_Comp` _asbp_player))
  (set `self.PropClasses` (`|MakeArray` "/Game/BPs/VacuumProps/BP_SuckableProp.BP_SuckableProp_C" "/Game/BPs/VacuumProps/BP_SuckableProp_Medium.BP_SuckableProp_Medium_C" "/Game/BPs/VacuumProps/BP_SuckableProp_Heavy.BP_SuckableProp_Heavy_C" :!type "SuckablePropParent Class Reference"))
  (bind (_keypin _valuepin) (`|MapForEach` (`self.mesh sounds`))
    (:`then`
      (`BlueprintMapLibrary.Map_Add` (`self.Sounds`) _keypin _valuepin))
    (:`CompletedPin`
      (`SceneComponent.K2_SetRelativeLocation` _trigger1_2 (`KismetMathLibrary.MakeVector` _relativelocation_x_2 _relativelocation_y_2 (+ _relativelocation_z_2 1000.0)) false false)
      (`SceneComponent.K2_SetRelativeLocation` _trigger2_2 (`KismetMathLibrary.MakeVector` _relativelocation_x _relativelocation_y (+ _relativelocation_z 1000.0)) false false)
      (`KismetSystemLibrary.Delay` 0.2)
      (`SceneComponent.K2_SetRelativeLocation` _trigger1 (`KismetMathLibrary.MakeVector` _relativelocation_x_3 _relativelocation_y_3 (+ _relativelocation_z_3 -1000.0)) true false)
      (`SceneComponent.K2_SetRelativeLocation` _trigger2 (`KismetMathLibrary.MakeVector` _relativelocation_x_4 _relativelocation_y_4 (+ _relativelocation_z_4 -1000.0)) true false))))

(event `self.ReceiveBeginPlay`
  (`KismetSystemLibrary.Delay` 2.5)
  (goto _label))

(event `self.Zone.OnComponentBeginOverlap`
  (params (OverlappedComponent :type "PrimitiveComponent Object Reference") (OtherActor :type "Actor Object Reference") (OtherComp :type "PrimitiveComponent Object Reference") (OtherBodyIndex :type Integer) (bFromSweep :type Boolean) (SweepResult :type "HitResult Structure (by ref)"))
  (bind _zone (`self.Zone`))
  (bind _ashierarchical_instanced_static_mesh_component (cast `HierarchicalInstancedStaticMeshComponent` OtherComp))
  (if (`self.Init`)
    (`KismetArrayLibrary.Array_AddUnique` (`self.Props`) _ashierarchical_instanced_static_mesh_component)
    (`KismetSystemLibrary.RetriggerableDelay` 0.1)
    (`KismetSystemLibrary.PrintString` "PopulateZone")
    (`self.PopulateZone`)
    (else
      (bind _output_get (set `self.HISM` _ashierarchical_instanced_static_mesh_component))
      (`self.SwitchPropIn_Parent` OtherBodyIndex (`StaticMeshComponent.StaticMesh` _output_get) false (`SceneComponent.K2_GetComponentToWorld` _zone) (`BoxComponent.GetScaledBoxExtent` _zone)))))

(event `PopulateZone`
  (bind _currentframeprops (`self.CurrentFrameProps`))
  (bind _zone (`self.Zone`))
  (set `self.LoopIndex` 0)
  (`self.PopulateZone_Parent` (`|GetArrayItem` (`self.Props`) (`self.LoopIndex`)) (`SceneComponent.K2_GetComponentToWorld` _zone) (`BoxComponent.GetScaledBoxExtent` _zone) :!label _label_2)
  (if (< (`self.LoopIndex`) (- (`KismetArrayLibrary.Array_Length` (`self.Props`)) 1))
    (`/Engine/EditorBlueprintResources/StandardMacros.IncrementInt` (`self.LoopIndex`)
      (:`  `
        (if (<= _currentframeprops (`self.PerFrameCutoff`))
          (set `self.CurrentFrameProps` (+ _currentframeprops (`KismetArrayLibrary.Array_Length` (`self.CurrSpawnedInstances_Parent`))))
          (goto _label_2)
          (else
            (`KismetSystemLibrary.DelayUntilNextTick`)
            (set `self.CurrentFrameProps` 0)
            (goto _label_2)))))
    (else
      (set `self.Init` false)
      (`KismetSystemLibrary.PrintString` "Init done"))))

(event `Reset Triggers`
  (bind _zone (`self.Zone`))
  (bind _zone_2 (`self.Zone`))
  (bind (_relativelocation_x _relativelocation_y _relativelocation_z) (`KismetMathLibrary.BreakVector` (`SceneComponent.RelativeLocation` _zone)))
  (bind (_relativelocation_x_2 _relativelocation_y_2 _relativelocation_z_2) (`KismetMathLibrary.BreakVector` (`SceneComponent.RelativeLocation` _zone_2)))
  (goto _label_3 :!via `Reset`))

(event `self.Trigger1.OnComponentBeginOverlap`
  (params (OverlappedComponent :type "PrimitiveComponent Object Reference") (OtherActor :type "Actor Object Reference") (OtherComp :type "PrimitiveComponent Object Reference") (OtherBodyIndex :type Integer) (bFromSweep :type Boolean) (SweepResult :type "HitResult Structure (by ref)"))
  (bind _zone (`self.Zone`))
  (bind _zone_2 (`self.Zone`))
  (bind (_relativelocation_x _relativelocation_y _relativelocation_z) (`KismetMathLibrary.BreakVector` (`SceneComponent.RelativeLocation` _zone)))
  (bind (_relativelocation_x_2 _relativelocation_y_2 _relativelocation_z_2) (`KismetMathLibrary.BreakVector` (`SceneComponent.RelativeLocation` _zone_2)))
  (if (`self.ActorHasTag` OtherActor "Player")
    (`/Engine/EditorBlueprintResources/StandardMacros.DoOnce` false :!label _label_3
      (:`Completed`
        (set `self.CanEndOverlap` false)
        (`SceneComponent.K2_SetRelativeLocation` _zone (`KismetMathLibrary.MakeVector` _relativelocation_x _relativelocation_y (+ _relativelocation_z 500.0)) false false)
        (`KismetSystemLibrary.Delay` 0.2)
        (`SceneComponent.K2_SetRelativeLocation` _zone_2 (`KismetMathLibrary.MakeVector` _relativelocation_x_2 _relativelocation_y_2 (+ _relativelocation_z_2 -500.0)) true false)
        (set `self.CanEndOverlap` true)
        (`KismetSystemLibrary.PrintString` "Zone Extend")))))

(event `self.Trigger2.OnComponentBeginOverlap`
  (params (OverlappedComponent :type "PrimitiveComponent Object Reference") (OtherActor :type "Actor Object Reference") (OtherComp :type "PrimitiveComponent Object Reference") (OtherBodyIndex :type Integer) (bFromSweep :type Boolean) (SweepResult :type "HitResult Structure (by ref)"))
  (if (`self.ActorHasTag` OtherActor "Player")
    (goto _label_3)))

(event `self.Trigger3.OnComponentBeginOverlap`
  (params (OverlappedComponent :type "PrimitiveComponent Object Reference") (OtherActor :type "Actor Object Reference") (OtherComp :type "PrimitiveComponent Object Reference") (OtherBodyIndex :type Integer) (bFromSweep :type Boolean) (SweepResult :type "HitResult Structure (by ref)"))
  (if (`self.ActorHasTag` OtherActor "Player")
    (goto _label_3)))

(event `EndZone`
  (bind _currreturnprop (`self.CurrReturnProp`))
  (bind _returnvalue (`self.FindComponentByTag` (`/Game/BPs/VacuumProps/BP_SuckableProp.Origin` _currreturnprop) "/Script/Engine.HierarchicalInstancedStaticMeshComponent" (`KismetStringLibrary.Conv_StringToName` (`KismetSystemLibrary.GetObjectName` (`StaticMeshComponent.StaticMesh` (`SuckablePropParent.StaticMeshComp` _currreturnprop))))))
  (`|ExecutionSequence` :!label _label_4
    (:`then_0`
      (bind _asgi_systems (cast `/Game/_GameManager/GI_Systems` (`GameplayStatics.GetGameInstance`)))
      (set `self.As GI Systems` _asgi_systems)
      (bind _output_get (set `self.Overlapping Actors` (`PrimitiveComponent.GetOverlappingActors` (`self.Zone`) "/Script/FThisJob.SuckablePropParent")))
      (for _array_element _output_get
        (set `self.Other Actor` _array_element)
        (bind _assuckable_prop_parent (cast `SuckablePropParent` (`self.Other Actor`)))
        (bind _output_get_2 (set `self.As BP Suckable Prop` _assuckable_prop_parent))
        (`/Engine/EditorBlueprintResources/StandardMacros.IsValid` (`SuckablePropParent.HoldingActor` _output_get_2)
          (:`Is Not Valid`
            (if (`/Game/BPs/VacuumProps/BP_SuckableProp.Asleep` _output_get_2)
              (bind _as_bp_suckable_prop (`self.As BP Suckable Prop`)
                (:`then`
                  (bind _output_get_3 (set `self.CurrReturnProp` _as_bp_suckable_prop))
                  (`PrimitiveComponent.SetSimulatePhysics` (`SuckablePropParent.StaticMeshComp` _output_get_3) false)
                  (bind _currreturnprop_2 (`self.CurrReturnProp`)
                    (:`then`
                      (`SuckablePropParent.Origin` _currreturnprop_2
                        (:`then`
                          _)
                        (:`else`
                          (bind _currentdefaulthism (`/Game/_GameManager/GI_Systems.CurrentDefaultHISM` (`self.As GI Systems`))
                            (:`then`
                              (set `/Game/BPs/VacuumProps/BP_SuckableProp.Origin` _currentdefaulthism (`self.CurrReturnProp`)))
                            (:`else`))))
                      (set `self.CurrTransform` (`self.GetTransform` (`self.CurrReturnProp`)))
                      (`/Engine/EditorBlueprintResources/StandardMacros.IsValid` _returnvalue
                        (:`Is Valid`
                          (`InstancedStaticMeshComponent.AddInstance` _returnvalue (`self.CurrTransform`) true)
                          (`PooledActor_Component.SetInUse` (`SuckablePropParent.PooledActor_Component` (`self.CurrReturnProp`)) false))))
                    (:`else`)))
                (:`else`))))))
      (`KismetSystemLibrary.PrintString` "Zone end done"))
    (:`then_1`
      (goto _label_3 :!via `Reset`))))

(event `self.Zone.OnComponentEndOverlap`
  (params (OverlappedComponent :type "PrimitiveComponent Object Reference") (OtherActor :type "Actor Object Reference") (OtherComp :type "PrimitiveComponent Object Reference") (OtherBodyIndex :type Integer))
  (if (`self.CanEndOverlap`)
    (if (`self.ActorHasTag` OtherActor "Player")
      (goto _label_4))))

(event `Move Triggers`
  (bind _trigger1 (`self.Trigger1`))
  ;[1 1 1] Trigger move for reloads
  (`self.Reset Triggers`)
  (`KismetSystemLibrary.Delay` 0.2)
  (set `self.Temp Loc` (`SceneComponent.K2_GetComponentLocation` _trigger1))
  (`SceneComponent.K2_SetWorldLocation` _trigger1 (`self.K2_GetActorLocation` (`self.As BP Player`)) true false)
  (`KismetSystemLibrary.Delay` 0.2)
  (`SceneComponent.K2_SetWorldLocation` _trigger1 (`self.Temp Loc`) false false))

(fn `UserConstructionScript`)