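; BP_AutoSpawner periodically spawns batches of BP_Dummy actors around itself, with constant chase enabled.
; BeginPlay starts a looping timer with a random interval, picked once.
; Each tick of that timer counts existing dummies through the last loop index and spawns SpawnNum more only while under 30, so a batch can overshoot.
; Spawn points use random unit-vector offsets scaled by XLocation and YLocation, at ZLocation height relative to the spawner.
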(event `self.ReceiveBeginPlay`
  (`KismetSystemLibrary.K2_SetTimerDelegate` (delegate `SpawnRate`) (`KismetMathLibrary.RandomFloatInRange` 1.0 5.0) true))

(event `SpawnRate`
  (bind (_returnvalue_x _returnvalue_y) (`KismetMathLibrary.BreakVector` (`KismetMathLibrary.RandomUnitVector`)))
  (bind _outactors (`GameplayStatics.GetAllActorsOfClass` "/Game/Systems_Integration/BP_Dummy.BP_Dummy_C"))
  (for (_ _array_index) _outactors
    _)
  (if (< _array_index (- 30 1))
    ;[1 0 0.053 0.5] Spawn
    (for _ (range (`self.Spawn Num`))
      (`|SpawnActorFromClass` "/Game/Systems_Integration/BP_Dummy.BP_Dummy_C" (`KismetMathLibrary.MakeTransform` (`KismetMathLibrary.TransformLocation` (`self.GetTransform`) (`KismetMathLibrary.MakeVector` (* (`self.X (Location)`) _returnvalue_x) (* (`self.Y (Location)`) _returnvalue_y) (`self.Z (Location)`))) (`self.Actor Rotation`)) "Undefined" "MultiplyWithRoot" null true null))))

(fn `UserConstructionScript`)