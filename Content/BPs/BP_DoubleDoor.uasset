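; BP_DoubleDoor is a kickable double door that swings both leaves open in opposite directions.
; Kicked passes a DoOnce gate, which can start closed until Unlock resets it, then disables box collision and lerps relative yaw on the Opening timeline, calling OnOpened when finished.
; Close reverses the timeline without restoring collision.
; A KickedSound dispatcher, bound at BeginPlay, posts the Wwise kick sound on the player character.
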(event `self.ReceiveTick`
  (params (DeltaSeconds :type "Float (single-precision)"))
  ;[1 0.9567 0 0.5 25] BEGIN PLAY & EVENT TICK
)

(event `self.ReceiveBeginPlay`
  ;[1 0.9567 0 0.5 25] BEGIN PLAY & EVENT TICK
  (`self.Init Feedback`))

(event `KickedInterface.Kicked`
  (params (KickVector :type "Vector Structure") (PlayerPosition :type "Vector Structure"))
  ;[0 0.4075 1 0.5] What happens when you kick the door
  (`/Engine/EditorBlueprintResources/StandardMacros.DoOnce` (`self.Start Closed`) :!label _label
    (:`Completed`
      (`self.Kicked_Sound`)
      (`PrimitiveComponent.SetCollisionEnabled` (`self.Box`) "NoCollision")
      (set `self.StartRot_Right` (`SceneComponent.RelativeRotation` (`self.Right`)))
      (set `self.StartRot_Left` (`SceneComponent.RelativeRotation` (`self.Left`)))
      (set `self.TargetRot_Right` (`KismetMathLibrary.ComposeRotators` (`self.StartRot_Right`) (`KismetMathLibrary.MakeRotator` 0.0 0.0 (`self.OpenAngle`))))
      (set `self.TargetRot_Left` (`KismetMathLibrary.ComposeRotators` (`self.StartRot_Left`) (`KismetMathLibrary.MakeRotator` 0.0 0.0 (* (`self.OpenAngle`) -1.0))))
      (bind (_direction _openingspeed) (`Timeline|Opening` :!via `PlayFromStart` :!label _label_2)
        (:`Update`
          (`SceneComponent.K2_SetRelativeRotation` (`self.Right`) (`KismetMathLibrary.RLerp` (`self.StartRot_Right`) (`self.TargetRot_Right`) _openingspeed) false false)
          (`SceneComponent.K2_SetRelativeRotation` (`self.Left`) (`KismetMathLibrary.RLerp` (`self.StartRot_Left`) (`self.TargetRot_Left`) _openingspeed) false false))
        (:`Finished`
          (`self.On Opened`))))))

(event `Unlock`
  ;[0 0.4075 1 0.5] What happens when you kick the door
  (goto _label :!via `Reset`))

(event `Close`
  ;[0 0.4075 1 0.5] What happens when you kick the door
  (goto _label_2 :!via `ReverseFromEnd`))

(event `Init Feedback`
  (`|ExecutionSequence`
    (:`then_0`
      (add `self.Kicked_Sound` (delegate `Kicked_Sound_Event`)))))

(event `Kicked_Sound_Event`
  ;[0 1 1 0.5] FB - Sound When Kicked
  (`AkGameplayStatics.PostEvent` "/Game/WwiseAudio/Events/Default_Work_Unit/MC/MC_KICK_WU/MC_Kick_DoorBoss.MC_Kick_DoorBoss" (`GameplayStatics.GetPlayerCharacter` 0)))

(fn `UserConstructionScript`)