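; Boss arena controller that runs the boss fight from intro cinematic to victory sequence.
; A player-tagged overlap plays the intro; StartFight closes doors, starts the boss, switches Wwise music and spawns turrets, with optional drones via SpawnLoop.
; SpawnPropTrigger, on a cooldown, shakes the camera and wakes random suckable props from the player's object pool.
; Boss EndPlay kills spawned enemies, unlocks doors and plays the ending cinematic, dialogue and electric effects.
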(event `Spawn Props`
  (bind _returnvalue (`PlayerCameraManager.StartCameraShake` :`self` (`GameplayStatics.GetPlayerCameraManager` 0) :`ShakeClass` "/Game/VFX/Blueprint/BP_FX_Earthquake.BP_FX_Earthquake_C"))
  (`KismetSystemLibrary.K2_SetTimerDelegate` (delegate `StopShaking`) 1.0)
  (for _ (range 1 (+ (`KismetMathLibrary.RandomIntegerInRange` (`self.Min Spawn`) (`self.Max Spawn`)) 1))
    (bind _returnvalue_2 (`ObjectPool_Component.SpawnFromPool` (`self.As Prop Pool`) (`KismetMathLibrary.MakeTransform` (`/Game/BPs/BP_Extent.Get Random Location` (`self.PropsSpawnExtent`)) (`KismetMathLibrary.MakeRotator` 0.0 0.0 (`KismetMathLibrary.RandomFloatInRange` 0.0 360.0))) (`KismetArrayLibrary.Array_Random` (`self.Suckable Classes`))))
    (`SuckablePropParent.WakeUp` (cast `SuckablePropParent` _returnvalue_2 :!pure true))))

(event `StopShaking`
  (`PlayerCameraManager.StopCameraShake` (`GameplayStatics.GetPlayerCameraManager` 0) (stale `Spawn Props` _returnvalue) false))

(event `self.ReceiveBeginPlay`
  (`|ExecutionSequence`
    (:`then_0`
      (if (`KismetArrayLibrary.Array_IsEmpty` (`self.DroneSpawnPoints`))
        (bind _outactors (`GameplayStatics.GetAllActorsOfClassWithTag` "/Game/BPs/BP_SpawnPoint.BP_SpawnPoint_C" "DRONE_SPAWN"))
        (set `self.DroneSpawnPoints` _outactors)))
    (:`then_1`
      (if (`KismetArrayLibrary.Array_IsEmpty` (`self.TurretsSpawnPoints`))
        (bind _outactors_2 (`GameplayStatics.GetAllActorsOfClassWithTag` "/Game/BPs/BP_SpawnPoint.BP_SpawnPoint_C" "TURRET_SPAWN"))
        (set `self.TurretsSpawnPoints` _outactors_2)))
    (:`then_2`
      (`KismetSystemLibrary.Delay` 2.0)
      (bind _asbp_player (cast `/Game/Characters/Player/Blueprints/BP_Player` (`GameplayStatics.GetPlayerCharacter` 0)))
      (set `self.As Prop Pool` (`/Game/Characters/Player/Blueprints/BP_Player.ObjectPool_Comp` _asbp_player)))))

(event `self.start.OnComponentBeginOverlap`
  (params (OverlappedComponent :type "PrimitiveComponent Object Reference") (OtherActor :type "Actor Object Reference") (OtherComp :type "PrimitiveComponent Object Reference") (OtherBodyIndex :type Integer) (bFromSweep :type Boolean) (SweepResult :type "HitResult Structure (by ref)"))
  ; Start Trigger
  (if (`self.ActorHasTag` OtherActor "Player")
    (`/Engine/EditorBlueprintResources/StandardMacros.DoOnce` false
      (:`Completed`
        (bind (_outactor _returnvalue) (`LevelSequencePlayer.CreateLevelSequencePlayer` (`self.Start Level Sequence`)))
        (`/Game/BPs/Other/FL_Common.Play Cinematique` _returnvalue)))))

(event `self.Boss.OnEndPlay`
  (params (Actor :type "Actor Object Reference") (EndPlayReason :type "EEndPlayReason Enum" :default "Destroyed"))
  ; End Trigger
  (`self.Stop Fight`))

(event `Start Fight`
  (`/Game/Characters/Enemies/Blueprints/BP_ChargerEnemy.StartFight` (`self.Boss`))
  (`/Engine/EditorBlueprintResources/StandardMacros.DoOnce` false
    (:`Completed`
      (`|ExecutionSequence`
        (:`then_0`
          (bind _outactors (`GameplayStatics.GetAllActorsOfClass` "/Game/BPs/BP_DoubleDoor.BP_DoubleDoor_C"))
          (for _array_element _outactors
            (`/Game/BPs/BP_DoubleDoor.Close` _array_element))
          (`self.Spawn Loop` false))
        (:`then_1`
          (`AkGameplayStatics.SetState` "/Game/WwiseAudio/States/MUSIC/STG_MUSIC_MASTER/STG_MUSIC_MASTER-ST_InLevel.STG_MUSIC_MASTER-ST_InLevel")
          (`AkGameplayStatics.SetState` "/Game/WwiseAudio/States/MUSIC/STG_MUSIC_LEVEL_ID/STG_MUSIC_LEVEL_ID-ST_LEVEL_Boss.STG_MUSIC_LEVEL_ID-ST_LEVEL_Boss")
          (`AkGameplayStatics.PostEvent` "/Game/WwiseAudio/Events/Default_Work_Unit/MUSIC/MusicMaster.MusicMaster"))))))

(event `SpawnPropTrigger`
  (`/Engine/EditorBlueprintResources/StandardMacros.DoOnce` false :!label _label
    (:`Completed`
      (`self.Spawn Props`)
      (`KismetSystemLibrary.Delay` 5.0)
      (goto _label :!via `Reset`))))

(event `Spawn Loop`
  (params (Drones :type Boolean))
  (`|ExecutionSequence`
    (:`then_0`
      (for _array_element (`self.TurretsSpawnPoints`)
        (`/Game/BPs/BP_SpawnPoint.Spawn` _array_element "/Game/Turret/Actor/BP_Turret_Turret.BP_Turret_Turret_C")))
    (:`then_1`
      (if Drones
        (for _array_element_2 (`self.DroneSpawnPoints`)
          (`/Game/BPs/BP_SpawnPoint.Spawn` _array_element_2 "/Game/Characters/Enemies/Blueprints/BP_Drone.BP_Drone_C"))))
    (:`then_2`
      (`KismetSystemLibrary.Delay` 1.0)
      (set `/Game/Characters/Enemies/Blueprints/BP_ChargerEnemy.IsSpawning` false (`self.Boss`)))))

(event `Stop Fight`
  (bind _turretsspawnpoints (`self.TurretsSpawnPoints`))
  (`/Engine/EditorBlueprintResources/StandardMacros.DoOnce` false
    (:`Completed`
      (`|ExecutionSequence`
        (:`then_0`
          (`KismetSystemLibrary.K2_ClearAndInvalidateTimerHandle` (`self.SpawnTimer`))
          (`KismetArrayLibrary.Array_Append` _turretsspawnpoints (`self.DroneSpawnPoints`))
          (for _array_element _turretsspawnpoints
            (`/Engine/EditorBlueprintResources/StandardMacros.IsValid` _array_element
              (:`Is Valid`
                (if (not (`self.IsActorBeingDestroyed` _array_element))
                  (bind _current_actor_ (`/Game/BPs/BP_SpawnPoint.Current Actor ` _array_element)
                    (:`then`
                      (message `HealthInterface.RemoveHealth` _current_actor_ 9999.0 null))
                    (:`else`))))))
          (bind _outactors (`GameplayStatics.GetAllActorsOfClass` "/Game/BPs/BP_DoubleDoor.BP_DoubleDoor_C"))
          (for _array_element_2 _outactors
            (`/Game/BPs/BP_DoubleDoor.Unlock` _array_element_2))
          (`self.K2_DestroyActor` (`self.Rope`))
          (`ActorComponent.K2_DestroyComponent` (`self.Box`))
          (bind (_outactor _returnvalue) (`LevelSequencePlayer.CreateLevelSequencePlayer` (`self.End Level Sequence`)))
          (`/Game/BPs/Other/FL_Common.Play Cinematique` _returnvalue)
          (bind _aspc_systems (cast `/Game/_GameManager/PC_Systems` (`GameplayStatics.GetPlayerController` 0)))
          (`Widget.SetVisibility` (`/Game/_GameManager/PC_Systems.WBP Boss Life Bar` _aspc_systems) "Collapsed"))
        (:`then_1`
          (`AkGameplayStatics.PostEvent` "/Game/WwiseAudio/Events/Default_Work_Unit/MUSIC/Stop_MusicMaster.Stop_MusicMaster")
          (`AkGameplayStatics.SetState` "/Game/WwiseAudio/States/MC/MC_CriticalHealth/MC_CriticalHealth-OFF.MC_CriticalHealth-OFF")
          (`AkGameplayStatics.PostEvent` "/Game/WwiseAudio/Events/Default_Work_Unit/MC/MC_Stop_CriticalHealth.MC_Stop_CriticalHealth")
          (`/Game/Progress/Blueprint/BP_Progress_Progress.Dialogue` (subsystem `/Game/Progress/Blueprint/BP_Progress_Progress`) (cast `/Game/_GameManager/PC_Systems` (`GameplayStatics.GetPlayerController` 0) :!pure true) "C_CEO_End" false))
        (:`then_2`
          (for _array_element_3 (`self.BP_Electric`)
            (if (`KismetSystemLibrary.IsValidSoftObjectReference` _array_element_3)
              (`/Game/Audio/BP_Electric.PlayElectric` (`|ConvertAsset` _array_element_3)))))))))

(fn `UserConstructionScript`)