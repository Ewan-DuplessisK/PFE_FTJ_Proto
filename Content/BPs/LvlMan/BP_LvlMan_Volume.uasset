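; Level-manager helper actor that tracks a level streaming volume and records when the player first walks through it.
; SetVolume fits its Box to the volume's bounds; a player overlap, also checked shortly after BeginPlay, scales the volume to MAXV3 and notifies BP_LvlMan once.
; It also exposes blocking load and unload of the volume's first streaming level, with reload chained through the level's unloaded delegate.
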(event `self.ReceiveBeginPlay`
  (`KismetSystemLibrary.Delay` 2.0)
  (`|ExecutionSequence`
    (:`then_1`
      (if (`PrimitiveComponent.IsOverlappingActor` (`self.Box`) (`GameplayStatics.GetPlayerPawn` 0))
        (if (not (`self.Walked`)) :!label _label
          (`KismetSystemLibrary.Delay` 0.1)
          (`self.SetActorScale3D` (`self.Volume`) (`self.MAX_V3`))
          (set `self.Walked` true)
          (`/Game/BPs/LvlMan/BP_LvlMan.Set Volume WalkedThrough` (`self.Get LvlMan`) self))))))

(event `self.ReceiveActorBeginOverlap`
  (params (OtherActor :type "Actor Object Reference"))
  (`self.Is Player` OtherActor
    (:`true`
      (goto _label))))

(event `self.Box.OnComponentBeginOverlap`
  (params (OverlappedComponent :type "PrimitiveComponent Object Reference") (OtherActor :type "Actor Object Reference") (OtherComp :type "PrimitiveComponent Object Reference") (OtherBodyIndex :type Integer) (bFromSweep :type Boolean) (SweepResult :type "HitResult Structure (by ref)"))
  (`self.Is Player` OverlappedComponent
    (:`true`
      (goto _label))))

(event `Set Volume`
  (params (Volume :type "LevelStreamingVolume Object Reference"))
  (bind _box (`self.Box`))
  (bind (_origin _boxextent) (`KismetSystemLibrary.GetComponentBounds` (`Brush.BrushComponent` (`self.Volume`))))
  (set `self.Volume` Volume)
  (`BoxComponent.SetBoxExtent` _box _boxextent true)
  (`SceneComponent.K2_SetWorldLocation` _box _origin false true))

(event `Unload Level`
  (`GameplayStatics.UnloadStreamLevel` (`|GetArrayItem` (`LevelStreamingVolume.StreamingLevelNames` (`self.Volume`))) true)
  (`GameplayStatics.FlushLevelStreaming`))

(event `Load Level`
  (`GameplayStatics.LoadStreamLevel` (`|GetArrayItem` (`LevelStreamingVolume.StreamingLevelNames` (`self.Volume`))) true true)
  (`GameplayStatics.FlushLevelStreaming`))

(event `Reload Level`
  (`self.Unload Level`)
  (add `LevelStreaming.OnLevelUnloaded` (`.Level` (`self.Get Streaming Level`)) (delegate `OnLevelUnloaded_Event`)))

(event `OnLevelUnloaded_Event`
  (remove `LevelStreaming.OnLevelUnloaded` (`.Level` (`self.Get Streaming Level`)) (delegate `OnLevelUnloaded_Event`))
  (`self.Load Level`))

(fn `Get LvlMan`
  (returns (ReturnValue :type "/Game/BPs/LvlMan/BP_LvlMan Object Reference"))
  (bind _returnvalue (`GameplayStatics.GetActorOfClass` "/Game/BPs/LvlMan/BP_LvlMan.BP_LvlMan_C"))
  (return _returnvalue))

(fn `Get Streaming Level`
  (returns (Name :type "Name (by ref)") (Level :type "LevelStreaming Object Reference"))
  (bind _output (`|GetArrayItem` (`LevelStreamingVolume.StreamingLevelNames` (`self.Volume`))))
  (return _output (`GameplayStatics.GetStreamingLevel` _output)))

(fn `UserConstructionScript`)