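; Level checkpoint actor that becomes current when the player first overlaps its listed Triggers, or its own collision if none are set.
; Once the level manager from GI_Systems accepts it, it snapshots player health, vacuum inventory and music state, storing score as zero.
; Applying the checkpoint restores score, music and inventory, calls RestoreHealth without the saved value, and resets the linked PropZone and Arena.
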(event `Bind Trigger`
  (`|ExecutionSequence`
    (:`then_1`
      (add `self.OnActorBeginOverlap` (stale `self.ReceiveBeginPlay` _array_element) (delegate `OnActorBeginOverlap_Event`) :!label _label))))

(event `OnActorBeginOverlap_Event` :!signature `self.OnActorBeginOverlap`
  (params (OverlappedActor :type "Actor Object Reference") (OtherActor :type "Actor Object Reference"))
  (`self.on Overlap` OtherActor))

(event `self.ReceiveBeginPlay`
  (bind _returnvalue (`GameplayStatics.GetPlayerPawn` 0))
  (bind _triggers (`self.Triggers`))
  (if (`KismetArrayLibrary.Array_IsNotEmpty` _triggers)
    (for _array_element _triggers
      (goto _label))
    (else
      (add `PrimitiveComponent.OnComponentBeginOverlap` (`self.CollisionComponent`) (delegate `OnComponentBeginOverlap_Event`))
      (`KismetSystemLibrary.Delay` 0.5)
      (if (`PrimitiveComponent.IsOverlappingActor` (`self.CollisionComponent`) _returnvalue)
        (`self.on Overlap` _returnvalue)))))

(event `OnComponentBeginOverlap_Event`
  (params (OverlappedComponent :type "PrimitiveComponent Object Reference") (OtherActor :type "Actor Object Reference") (OtherComp :type "PrimitiveComponent Object Reference") (OtherBodyIndex :type Integer) (bFromSweep :type Boolean) (SweepResult :type "HitResult Structure (by ref)"))
  (`self.on Overlap` OtherActor))

(event `Set as Current`
  (if (not (`self.Walked`))
    (set `self.Walked` true)
    (bind _changed (`/Game/BPs/LvlMan/BP_LvlMan.Set Current Checkpoint` (`self.Get LvlMan`) self))
    (if _changed
      (`self.Save Checkpoint Data`))))

(fn `Apply Checkpoint Data`
  (bind (_saved_scores _saved_health _saved_vacuuminventory _saved_musicstate) (break `/Game/BPs/LvlMan/F_LvlMan_Checkpoint_Save` (`self.Saved`)))
  (bind _returnvalue (`GameplayStatics.GetActorOfClass` "/Game/Characters/Player/Blueprints/BP_Player.BP_Player_C"))
  (set `FTJ_ScoringSystem_ScoreBase.Score` _saved_scores (subsystem `/Game/CppSystems/ScoringSystem/Public/Blueprint/BP_ScoringSystem_Score`))
  (`AkGameplayStatics.SetState` _saved_musicstate)
  (`AkGameplayStatics.SetState` "/Game/WwiseAudio/States/MUSIC/STG_MUSIC_MASTER/STG_MUSIC_MASTER-ST_InLevel.STG_MUSIC_MASTER-ST_InLevel")
  (`/Game/Characters/Player/Blueprints/BP_Player.Restore Health` _returnvalue)
  (bind _returnvalue_2 (`GameplayStatics.GetActorOfClass` "/Game/Characters/Player/Blueprints/BP_Vacuum.BP_Vacuum_C"))
  (`/Game/Characters/Player/Blueprints/BP_Vacuum.Set Inventory Serialized` _returnvalue_2 _saved_vacuuminventory)
  (bind _propzone (`self.PropZone`)
    (:`then`
      (`/Game/BPs/VacuumProps/BP_PropZone.RestartZone` _propzone))
    (:`else`
      _))
  (bind _arena (`self.Arena`)
    (:`then`
      (`/Game/BPs/Arena/BP_Arena.Reset Arena` _arena))
    (:`else`
      _))
  (`KismetSystemLibrary.PrintText` (`|FormatText` "[LvlMan_Checkpoint]: Save HP={hp}, Score={score}" _saved_health (`KismetMathLibrary.FTrunc` 0.0))))

(fn `Get LvlMan`
  (returns (ReturnValue :type "/Game/BPs/LvlMan/BP_LvlMan Object Reference"))
  (bind _asgi_systems (cast `/Game/_GameManager/GI_Systems` (`GameplayStatics.GetGameInstance`)))
  (bind _lvlman (`/Game/BPs/LvlMan/GI_Systems_Base.Get LvlMan` _asgi_systems))
  (return _lvlman))

(fn `on Overlap`
  (params (A :type "Object Object Reference"))
  (if (== A (`GameplayStatics.GetPlayerPawn` 0))
    (`self.Set as Current`)))

(fn `Save Checkpoint Data`
  (bind _returnvalue (`GameplayStatics.GetActorOfClass` "/Game/Characters/Player/Blueprints/BP_Player.BP_Player_C"))
  (bind _returnvalue_2 (`GameplayStatics.GetActorOfClass` "/Game/Characters/Player/Blueprints/BP_Vacuum.BP_Vacuum_C"))
  (bind _inventoryclasses (`/Game/Characters/Player/Blueprints/BP_Vacuum.Get Inventory Serialized` _returnvalue_2))
  (bind _currenthealth (`FTJ_CharaBase.CurrentHealth` _returnvalue))
  (set `self.Saved` (make `/Game/BPs/LvlMan/F_LvlMan_Checkpoint_Save` 0.0 _currenthealth _inventoryclasses (`self.MusicState`)))
  (`KismetSystemLibrary.PrintText` (`|FormatText` "[LvlMan_Checkpoint]: Save HP={hp}, Score={score}" _currenthealth (`FTJ_ScoringSystem_ScoreBase.Score` (subsystem `/Game/CppSystems/ScoringSystem/Public/Blueprint/BP_ScoringSystem_Score`)))))

(fn `UserConstructionScript`)