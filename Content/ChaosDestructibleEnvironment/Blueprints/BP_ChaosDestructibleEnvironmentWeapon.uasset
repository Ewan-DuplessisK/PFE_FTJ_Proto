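; Weapon actor for a Chaos destruction test that fires projectiles at a destructible geometry collection.
; On BeginPlay it spawns a GeometryCollectionActor at a fixed location, assigns the GC_ChaosDestructibleEnvironment rest collection with asset defaults and turns on bone colors.
; OnFired spawns a BP_ChaosDestructibleEnvironmentProjectile just ahead of the actor, oriented along its rotation.
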(event `self.ReceiveBeginPlay`
  (bind _returnvalue (`|SpawnActorFromClass` "/Script/GeometryCollectionEngine.GeometryCollectionActor" (`KismetMathLibrary.MakeTransform` (0.0 -150.0 50.0)) "Undefined" "MultiplyWithRoot" null null))
  (bind _geometrycollectioncomponent (`GeometryCollectionActor.GeometryCollectionComponent` _returnvalue))
  (`GeometryCollectionComponent.SetRestCollection` _geometrycollectioncomponent "/Game/ChaosDestructibleEnvironment/_manager/GC_ChaosDestructibleEnvironment.GC_ChaosDestructibleEnvironment" true)
  (set `GeometryCollectionComponent.bShowBoneColors` true _geometrycollectioncomponent))

(event `Event OnFired`
  (`|SpawnActorFromClass` "/Game/ChaosDestructibleEnvironment/Blueprints/BP_ChaosDestructibleEnvironmentProjectile.BP_ChaosDestructibleEnvironmentProjectile_C" (`KismetMathLibrary.MakeTransform` (+ (`self.K2_GetActorLocation`) (* (`self.GetActorForwardVector`) 50.0)) (`self.K2_GetActorRotation`)) "Undefined" "MultiplyWithRoot" null null))

(fn `UserConstructionScript`)