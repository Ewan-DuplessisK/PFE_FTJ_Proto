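; Player controller for the Chaos destructible environment map that handles Enhanced Input for looking and firing.
; On BeginPlay it adds the map's input mapping context and caches the controlled pawn as a BP_ChaosDestructibleEnvironmentPlayer.
; Look input drives yaw and pitch, and Fire calls EventOnFired on the cached pawn.
; The Move input event is present but does nothing.
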(event `self.ReceiveBeginPlay`
  (`EnhancedInputSubsystemInterface.AddMappingContext` (subsystem `EnhancedInputLocalPlayerSubsystem`) "/Game/ChaosDestructibleEnvironment/_manager/IMC_ChaosDestructibleEnvironment.IMC_ChaosDestructibleEnvironment" 0 (struct))
  (bind _asbp_chaos_destructible_environment_player (cast `/Game/ChaosDestructibleEnvironment/Blueprints/BP_ChaosDestructibleEnvironmentPlayer` (`self.K2_GetPawn`)))
  (set `self.Actor` _asbp_chaos_destructible_environment_player))

(event `EnhancedInput|/Game/ChaosDestructibleEnvironment/InputActions/IA_ChaosDestructibleEnvironmentMove`
  (params (ActionValue :type "Vector2D Structure") (ElapsedSeconds :type "Float (double-precision)") (TriggeredSeconds :type "Float (double-precision)") (InputAction :type "InputAction Object Reference" :default "/Game/ChaosDestructibleEnvironment/InputActions/IA_ChaosDestructibleEnvironmentMove.IA_ChaosDestructibleEnvironmentMove")))

(event `EnhancedInput|/Game/ChaosDestructibleEnvironment/InputActions/IA_ChaosDestructibleEnvironmentLook`
  (params (ActionValue :type "Vector2D Structure") (ElapsedSeconds :type "Float (double-precision)") (TriggeredSeconds :type "Float (double-precision)") (InputAction :type "InputAction Object Reference" :default "/Game/ChaosDestructibleEnvironment/InputActions/IA_ChaosDestructibleEnvironmentLook.IA_ChaosDestructibleEnvironmentLook"))
  (:`Triggered`
    (`self.AddYawInput` ActionValue_X)
    (`self.AddPitchInput` ActionValue_Y)))

(event `EnhancedInput|/Game/ChaosDestructibleEnvironment/InputActions/IA_ChaosDestructibleEnvironmentFire`
  (params (ActionValue :type Boolean) (ElapsedSeconds :type "Float (double-precision)") (TriggeredSeconds :type "Float (double-precision)") (InputAction :type "InputAction Object Reference" :default "/Game/ChaosDestructibleEnvironment/InputActions/IA_ChaosDestructibleEnvironmentFire.IA_ChaosDestructibleEnvironmentFire"))
  (:`Triggered`
    (`/Game/ChaosDestructibleEnvironment/Blueprints/BP_ChaosDestructibleEnvironmentPlayer.Event OnFired` (`self.Actor`))))

(fn `UserConstructionScript`)