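; BP_MusicGate is a trigger gate that switches the gameplay music state between Calm and Fight as the player passes through it.
; Overlapping BoxIn sets the Fight state, and overlapping BoxOut sets Calm, both only for BP_Player.
; The IsFighting flag tracks the current side, so each box calls SetState only when the state needs to change.
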(event `self.BoxOut.OnComponentBeginOverlap`
  (params (OverlappedComponent :type "PrimitiveComponent Object Reference") (OtherActor :type "Actor Object Reference") (OtherComp :type "PrimitiveComponent Object Reference") (OtherBodyIndex :type Integer) (bFromSweep :type Boolean) (SweepResult :type "HitResult Structure (by ref)"))
  (cast `/Game/Characters/Player/Blueprints/BP_Player` OtherActor)
  (if (`self.IsFighting`)
    (`AkGameplayStatics.SetState` "/Game/WwiseAudio/States/MUSIC/STG_MUSIC_GAMEPLAY/STG_MUSIC_GAMEPLAY-ST_Calm.STG_MUSIC_GAMEPLAY-ST_Calm")
    (set `self.IsFighting` false)))

(event `self.BoxIn.OnComponentBeginOverlap`
  (params (OverlappedComponent :type "PrimitiveComponent Object Reference") (OtherActor :type "Actor Object Reference") (OtherComp :type "PrimitiveComponent Object Reference") (OtherBodyIndex :type Integer) (bFromSweep :type Boolean) (SweepResult :type "HitResult Structure (by ref)"))
  (cast `/Game/Characters/Player/Blueprints/BP_Player` OtherActor)
  (if (not (`self.IsFighting`))
    (`AkGameplayStatics.SetState` "/Game/WwiseAudio/States/MUSIC/STG_MUSIC_GAMEPLAY/STG_MUSIC_GAMEPLAY-ST_Fight.STG_MUSIC_GAMEPLAY-ST_Fight")
    (set `self.IsFighting` true)))

(fn `UserConstructionScript`)