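; Audio component for the vacuum tool that wraps its Wwise calls in custom events.
; Activate, deactivate, suck and shoot events each post their matching vacuum event on a passed-in Ak component.
; An inventory event, and the shoot event as well, write the current inventory count to the vacuum ammo RTPC with no interpolation.
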(event `AudioSetRtpcInventory`
  (params (AKComponent :type "AkComponent Object Reference") (CurrentInventory :type Integer))
  (`AkGameObject.SetRTPCValue` AKComponent "/Game/WwiseAudio/Game_Parameters/MC/RTPC_Vaccum_Ammo.RTPC_Vaccum_Ammo" (`KismetMathLibrary.Conv_IntToDouble` CurrentInventory) 0 ""))

(event `AudioDeactivate`
  (params (AkComponent :type "AkComponent Object Reference"))
  (`AkGameObject.PostAkEvent` :`self` AkComponent :`AkEvent` "/Game/WwiseAudio/Events/Default_Work_Unit/MC/MC_Vacuum_Deactivate.MC_Vacuum_Deactivate"))

(event `AudioActivate`
  (params (AkComponent :type "AkComponent Object Reference"))
  (`AkGameObject.PostAkEvent` :`self` AkComponent :`AkEvent` "/Game/WwiseAudio/Events/Default_Work_Unit/MC/MC_Vacuum_Activate.MC_Vacuum_Activate"))

(event `AudioSuck`
  (params (AkComponent :type "AkComponent Object Reference"))
  (`AkGameObject.PostAkEvent` :`self` AkComponent :`AkEvent` "/Game/WwiseAudio/Events/Default_Work_Unit/MC/MC_Vacuum_Suck.MC_Vacuum_Suck"))

(event `AudioShoot`
  (params (`Ak Component` :type "AkComponent Object Reference") (CurrentInventory :type Integer))
  (`AkGameObject.PostAkEvent` :`self` `Ak Component` :`AkEvent` "/Game/WwiseAudio/Events/Default_Work_Unit/MC/MC_Vacuum_Shoot.MC_Vacuum_Shoot")
  (`AkGameObject.SetRTPCValue` `Ak Component` "/Game/WwiseAudio/Game_Parameters/MC/RTPC_Vaccum_Ammo.RTPC_Vaccum_Ammo" (`KismetMathLibrary.Conv_IntToDouble` CurrentInventory) 0 ""))