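; Audio component for BP_Animated_Kick that plays Wwise sounds for vending machine and printer moments.
; On BeginPlay it caches two Ak components from its owner, one standard and one with no refresh interval.
; Named events post can drop with jingle, error and printer jam on the validity-checked no-refresh component.
; Explosion and the machine-on loop post to the standard component without a validity check.
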(event `self.ReceiveBeginPlay`
  (bind _asbp_animated_kick (cast `/Game/BPs/TestProps/BP_Animated_Kick` (`self.GetOwner`)))
  (set `self.Ak Animated Kick No Refresh` (`/Game/BPs/TestProps/BP_Animated_Kick.Ak_Animated_Kick_NoRefreshInterval` _asbp_animated_kick))
  (set `self.Ak Animated Kick` (`/Game/BPs/TestProps/BP_Animated_Kick.Ak_Animated_Kick` _asbp_animated_kick)))

(event `AudioVendingMachineCanDrop`
  (bind _ak_animated_kick_no_refresh (`self.Ak Animated Kick No Refresh`)
    (:`then`
      (`AkGameObject.PostAkEvent` :`self` _ak_animated_kick_no_refresh :`AkEvent` "/Game/WwiseAudio/Events/Default_Work_Unit/SFX/SFX_LVL_01/Vending_Machine_Can_Drop.Vending_Machine_Can_Drop")
      (`AkGameObject.PostAkEvent` :`self` _ak_animated_kick_no_refresh :`AkEvent` "/Game/WwiseAudio/Events/Default_Work_Unit/SFX/SFX_LVL_01/Vending_Machine_Jingle.Vending_Machine_Jingle"))
    (:`else`)))

(event `AudioError`
  (bind _ak_animated_kick_no_refresh (`self.Ak Animated Kick No Refresh`)
    (:`then`
      (`AkGameObject.PostAkEvent` :`self` _ak_animated_kick_no_refresh :`AkEvent` "/Game/WwiseAudio/Events/Default_Work_Unit/SFX/SFX_LVL_01/Vending_Machine_Error.Vending_Machine_Error"))
    (:`else`)))

(event `AudioExplosion`
  (`AkGameObject.PostAkEvent` :`self` (`self.Ak Animated Kick`) :`AkEvent` "/Game/WwiseAudio/Events/Default_Work_Unit/SFX/SFX_LVL_01/Vending_Machine_Explosion.Vending_Machine_Explosion"))

(event `AudioOn`
  (`AkGameObject.PostAkEvent` :`self` (`self.Ak Animated Kick`) :`AkEvent` "/Game/WwiseAudio/Events/Default_Work_Unit/SFX/SFX_LVL_01/Vending_Machine_On_LP.Vending_Machine_On_LP"))

(event `AudioPrinterJam`
  (bind _ak_animated_kick_no_refresh (`self.Ak Animated Kick No Refresh`)
    (:`then`
      (`AkGameObject.PostAkEvent` :`self` _ak_animated_kick_no_refresh :`AkEvent` "/Game/WwiseAudio/Events/Default_Work_Unit/SFX/SFX_LVL_01/Printer_Jam.Printer_Jam"))
    (:`else`)))