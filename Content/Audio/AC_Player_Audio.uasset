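; Player audio component that drives Wwise footstep sounds and posts a kick foley event.
; Play_SFX_Footsteps sets the volume RTPC from pawn speed and starts one looping timer while horizontal movement occurs without vertical velocity.
; Each timer tick sphere-traces below the mesh, maps the physical surface to a ground-material switch and posts the footstep event.
; Stopping, vertical motion or ResetFootstepsDelays clears the timer and re-arms it.
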(event `PlayFootsteps`
  (bind _returnvalue (`SceneComponent.K2_GetComponentLocation` (stale `Play_SFX_Footsteps` Mesh)))
  (bind (_outhit _returnvalue_2) (`KismetSystemLibrary.SphereTraceSingle` _returnvalue (- _returnvalue (0.0 0.0 150.0)) 5.0 "TraceTypeQuery1"))
  (if _returnvalue_2
    (`AkComponent.SetSwitch` (stale `Play_SFX_Footsteps` AkComponent) (select `EPhysicalSurface` (`PhysicalMaterial.SurfaceType` (`.PhysMat` (`GameplayStatics.BreakHitResult` _outhit))) :`SurfaceType_Default` "/Game/WwiseAudio/Switches/MC/MC_GroundMaterials/MC_GroundMaterials-Concrete.MC_GroundMaterials-Concrete" :`SurfaceType1` "/Game/WwiseAudio/Switches/MC/MC_GroundMaterials/MC_GroundMaterials-Carpet.MC_GroundMaterials-Carpet" :`SurfaceType2` "/Game/WwiseAudio/Switches/MC/MC_GroundMaterials/MC_GroundMaterials-Concrete.MC_GroundMaterials-Concrete" :`SurfaceType3` "/Game/WwiseAudio/Switches/MC/MC_GroundMaterials/MC_GroundMaterials-Metal.MC_GroundMaterials-Metal" :`SurfaceType4` "/Game/WwiseAudio/Switches/MC/MC_GroundMaterials/MC_GroundMaterials-Paper.MC_GroundMaterials-Paper" :`SurfaceType5` "/Game/WwiseAudio/Switches/MC/MC_GroundMaterials/MC_GroundMaterials-Tiles.MC_GroundMaterials-Tiles" :`SurfaceType6` "/Game/WwiseAudio/Switches/MC/MC_GroundMaterials/MC_GroundMaterials-Wood.MC_GroundMaterials-Wood" :!type "AkSwitchValue Object Reference"))
    (`AkGameObject.PostAkEvent` :`self` (stale `Play_SFX_Footsteps` AkComponent) :`AkEvent` "/Game/WwiseAudio/Events/Default_Work_Unit/MC/MC_FTS.MC_FTS")))

(event `Play_SFX_Footsteps`
  (params (Mesh :type "SkeletalMeshComponent Object Reference") (AkComponent :type "AkComponent Object Reference"))
  (bind _returnvalue (`GameplayStatics.GetPlayerPawn` 0))
  (bind (_returnvalue_x _returnvalue_y _returnvalue_z) (`KismetMathLibrary.BreakVector` (`Actor.GetVelocity` _returnvalue)))
  (`AkGameObject.SetRTPCValue` AkComponent "/Game/WwiseAudio/Game_Parameters/MC/RTPC_MC_FT_Volume.RTPC_MC_FT_Volume" (`KismetMathLibrary.VSize` (`Actor.GetVelocity` _returnvalue)) 0 "")
  (if (and (or (<= _returnvalue_x -2.0) (>= _returnvalue_x 2.0) (>= _returnvalue_y 2.0) (<= _returnvalue_y -2.0)) (== _returnvalue_z 0.0))
    (`/Engine/EditorBlueprintResources/StandardMacros.DoOnce` false :!label _label
      (:`Completed`
        (bind _returnvalue_2 (`KismetSystemLibrary.K2_SetTimerDelegate` (delegate `PlayFootsteps`) (`self.DelayFootsteps`) true))
        (set `self.FootstepsTimers` _returnvalue_2)))
    (else
      (`KismetSystemLibrary.K2_ClearAndInvalidateTimerHandle` (`self.FootstepsTimers`) :!label _label_2)
      (goto _label :!via `Reset`))))

(event `ResetFootstepsDelays`
  (goto _label_2))

(event `Play_Fol_Kick`
  (`AkGameplayStatics.PostEvent` "/Game/WwiseAudio/Events/Default_Work_Unit/MC/MC_FOL_Kick.MC_FOL_Kick"))