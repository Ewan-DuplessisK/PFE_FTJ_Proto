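; Actor component that plays Wwise sounds for BP_Turret_Turret, covering shooting, charging, getting hit and destruction.
; On BeginPlay it caches the owning turret and its Ak component, and binds an any-damage handler that is empty.
; Custom events post the Ak events: hit and charge on the cached component, shoot and death on a component passed in by the caller.
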(event `self.ReceiveBeginPlay`
  (bind _asbp_turret_turret (cast `/Game/Turret/Actor/BP_Turret_Turret` (`self.GetOwner`)))
  (bind _output_get (set `self.BPTurretTurret` _asbp_turret_turret))
  (set `self.Ak Turret` (`/Game/Turret/Actor/BP_Turret_Turret.Ak_Turret` _output_get))
  (add `Actor.OnTakeAnyDamage` (`self.BPTurretTurret`) (delegate `OnTakeAnyDamage_Event`)))

(event `OnTakeAnyDamage_Event`
  (params (DamagedActor :type "Actor Object Reference") (Damage :type "Float (single-precision)") (DamageType :type "DamageType Object Reference") (InstigatedBy :type "Controller Object Reference") (DamageCauser :type "Actor Object Reference")))

(event `AudioDestroyed`
  (params (`Ak Component` :type "AkComponent Object Reference"))
  (`AkGameObject.PostAkEvent` :`self` `Ak Component` :`AkEvent` "/Game/WwiseAudio/Events/Default_Work_Unit/ENEMIES/TURRET/Turret_Death.Turret_Death"))

(event `AudioShoot`
  (params (`Ak Component` :type "AkComponent Object Reference"))
  (`AkGameObject.PostAkEvent` :`self` `Ak Component` :`AkEvent` "/Game/WwiseAudio/Events/Default_Work_Unit/ENEMIES/TURRET/Turret_Shoot.Turret_Shoot"))

(event `AudioTakeDamage`
  (`AkGameObject.PostAkEvent` :`self` (`self.Ak Turret`) :`AkEvent` "/Game/WwiseAudio/Events/Default_Work_Unit/ENEMIES/TURRET/Turret_Hit.Turret_Hit"))

(event `AudioCharge`
  (`AkGameObject.PostAkEvent` :`self` (`self.Ak Turret`) :`AkEvent` "/Game/WwiseAudio/Events/Default_Work_Unit/ENEMIES/TURRET/Turret_Charge.Turret_Charge"))