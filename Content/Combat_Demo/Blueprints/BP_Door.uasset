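; BP_Door is a combat-demo door that gets launched when struck by tagged furniture, kicks or hurtboxes.
; Front and back hitboxes each trigger a one-time push, activating projectile movement with timeline-scaled horizontal velocity along that side's arrow.
; Once pushed, contact with a wall or hurtbox hides the door, disables collision and destroys it after a short delay.
; Wall contact also destroys an unpushed door.
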(event `self.FrontHitbox.OnComponentBeginOverlap`
  (params (OverlappedComponent :type "PrimitiveComponent Object Reference") (OtherActor :type "Actor Object Reference") (OtherComp :type "PrimitiveComponent Object Reference") (OtherBodyIndex :type Integer) (bFromSweep :type Boolean) (SweepResult :type "HitResult Structure (by ref)"))
  ;[1 0.3028 0 0.5] FrontHitbox
  (if (`self.Door Already Pushed`)
    (if (or (`ActorComponent.ComponentHasTag` OtherComp "Wall") (`ActorComponent.ComponentHasTag` OtherComp "Hurtbox")) :!label _label
      (`SceneComponent.SetHiddenInGame` (`self.Door`) true false)
      (`self.SetActorEnableCollision` false)
      (`KismetSystemLibrary.Delay` 0.5)
      (`self.K2_DestroyActor`))
    (elif (or (`ActorComponent.ComponentHasTag` OtherComp "Table") (`ActorComponent.ComponentHasTag` OtherComp "Chair") (`ActorComponent.ComponentHasTag` OtherComp "Kick") (`ActorComponent.ComponentHasTag` OtherComp "Hurtbox"))
      (set `self.Door Already Pushed` true)
      (`ActorComponent.Activate` (`self.ProjectileMovement`) false)
      (bind (_direction _distancemultiplier) (`Timeline|Timeline` :!via `PlayFromStart`)
        (:`Update`
          (bind (_returnvalue_x _returnvalue_y) (`KismetMathLibrary.BreakVector` (* (`SceneComponent.GetForwardVector` (`self.FrontArrow`)) (* _distancemultiplier (`self.Door Push`)))))
          (set `MovementComponent.Velocity` (`KismetMathLibrary.MakeVector` _returnvalue_x _returnvalue_y) (`self.ProjectileMovement`))))
      (else
        (goto _label)))))

(event `self.BackHitbox.OnComponentBeginOverlap`
  (params (OverlappedComponent :type "PrimitiveComponent Object Reference") (OtherActor :type "Actor Object Reference") (OtherComp :type "PrimitiveComponent Object Reference") (OtherBodyIndex :type Integer) (bFromSweep :type Boolean) (SweepResult :type "HitResult Structure (by ref)"))
  ;[0.000419 0.8871 1 0.5] BackHitbox
  (if (`self.Door Already Pushed`)
    (if (or (`ActorComponent.ComponentHasTag` OtherComp "Wall") (`ActorComponent.ComponentHasTag` OtherComp "Hurtbox")) :!label _label_2
      (`SceneComponent.SetHiddenInGame` (`self.Door`) true false)
      (`self.SetActorEnableCollision` false)
      (`KismetSystemLibrary.Delay` 0.5)
      (`self.K2_DestroyActor`))
    (elif (or (`ActorComponent.ComponentHasTag` OtherComp "Table") (`ActorComponent.ComponentHasTag` OtherComp "Chair") (`ActorComponent.ComponentHasTag` OtherComp "Kick") (`ActorComponent.ComponentHasTag` OtherComp "Hurtbox"))
      (set `self.Door Already Pushed` true)
      (`ActorComponent.Activate` (`self.ProjectileMovement`) false)
      (bind (_direction _distancemultiplier) (`Timeline|Timeline_0` :!via `PlayFromStart`)
        (:`Update`
          (bind (_returnvalue_x _returnvalue_y) (`KismetMathLibrary.BreakVector` (* (`SceneComponent.GetForwardVector` (`self.BackArrow`)) (* _distancemultiplier (`self.Door Push`)))))
          (set `MovementComponent.Velocity` (`KismetMathLibrary.MakeVector` _returnvalue_x _returnvalue_y) (`self.ProjectileMovement`))))
      (else
        (goto _label_2)))))

(fn `UserConstructionScript`)