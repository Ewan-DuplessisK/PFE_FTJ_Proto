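; BP_Table is a combat prop table that the player kicks into things, breaking it on impact.
; Kick overlaps start a timeline driving projectile velocity along player forward; chair or table bumps use a separate distance and set AlreadyKicked shortly after.
; Hits on walls, hurtboxes, doors, or furniture while kicked play Niagara effects, hide the mesh, briefly keep collision for nearby enemies, then destroy the actor.
; DestoryAuto also breaks it when the kick ends.
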(event `self.Table.OnComponentBeginOverlap`
  (params (OverlappedComponent :type "PrimitiveComponent Object Reference") (OtherActor :type "Actor Object Reference") (OtherComp :type "PrimitiveComponent Object Reference") (OtherBodyIndex :type Integer) (bFromSweep :type Boolean) (SweepResult :type "HitResult Structure (by ref)"))
  (bind (_bblockinghit _binitialoverlap _time _distance _location _impactpoint _normal _impactnormal _physmat _hitactor) (`GameplayStatics.BreakHitResult` SweepResult))
  (bind _projectilemovement (`self.ProjectileMovement`))
  (bind _projectilemovement_2 (`self.ProjectileMovement`))
  (if (`ActorComponent.ComponentHasTag` OtherComp "Kick")
    (set `self.AlreadyKicked?` true)
    (`ActorComponent.Activate` (`self.NS_Sample_BONK`) true)
    (`ActorComponent.Activate` _projectilemovement_2 false)
    (bind (_direction _distancemultiplier) (`Timeline|Timeline_1` :!via `PlayFromStart`)
      (:`Update`
        (bind (_returnvalue_x _returnvalue_y) (`KismetMathLibrary.BreakVector` (* (`self.GetActorForwardVector` (`GameplayStatics.GetPlayerPawn` 0)) (* _distancemultiplier (`self.Hit Back Distance`)))))
        (set `MovementComponent.Velocity` (`KismetMathLibrary.MakeVector` _returnvalue_x _returnvalue_y) _projectilemovement_2))
      (:`Finished`
        (set `self.AlreadyKicked?` false)
        (if (`self.Destory Auto`)
          (`self.Auto Destroyed`))))
    (elif (`self.AlreadyKicked?`)
      (if (or (`ActorComponent.ComponentHasTag` OtherComp "Chair") (`ActorComponent.ComponentHasTag` OtherComp "Table"))
        (`|ExecutionSequence`
          (:`then_0`
            (`SceneComponent.K2_SetWorldLocation` (`self.NS_FinisherHit`) (`self.K2_GetActorLocation` _hitactor) false false)
            (`SceneComponent.K2_SetWorldLocation` (`self.NS_Sample_BONK`) (`self.K2_GetActorLocation` _hitactor) false false)
            (`ActorComponent.Activate` (`self.NS_Sample_BONK`) true)
            (`ActorComponent.Activate` (`self.NS_FinisherHit`) true))
          (:`then_1`
            (`SceneComponent.SetHiddenInGame` (`self.Table`) true false)
            (`KismetSystemLibrary.Delay` 0.1)
            (`self.SetActorEnableCollision` false)
            (`KismetSystemLibrary.Delay` 2.0)
            (`self.K2_DestroyActor`)))
        (elif (or (`ActorComponent.ComponentHasTag` OtherComp "Wall") (`ActorComponent.ComponentHasTag` OtherComp "Hurtbox") (`ActorComponent.ComponentHasTag` OtherComp "Door"))
          (`|ExecutionSequence`
            (:`then_0`
              (`SceneComponent.K2_SetWorldLocation` (`self.NS_FinisherHit`) (`self.K2_GetActorLocation` _hitactor) false false)
              (`SceneComponent.K2_SetWorldLocation` (`self.NS_Sample_BONK`) (`self.K2_GetActorLocation` _hitactor) false false)
              (`ActorComponent.Activate` (`self.NS_Sample_BONK`) true)
              (`ActorComponent.Activate` (`self.NS_FinisherHit`) true))
            (:`then_1`
              (`SceneComponent.SetHiddenInGame` (`self.Table`) true false)
              (`KismetSystemLibrary.Delay` 0.1) ; Let the game hit other enemies really close to the 1st one hit
              (`self.SetActorEnableCollision` false)
              (`KismetSystemLibrary.Delay` 2.0)
              (`self.K2_DestroyActor`)))))
      (elif (or (`ActorComponent.ComponentHasTag` OtherComp "Wall") (`ActorComponent.ComponentHasTag` OtherComp "Hurtbox") (`ActorComponent.ComponentHasTag` OtherComp "Door"))
        (`|ExecutionSequence`
          (:`then_0`
            (`SceneComponent.K2_SetWorldLocation` (`self.NS_FinisherHit`) (`self.K2_GetActorLocation` (`.HitActor` (`GameplayStatics.BreakHitResult` SweepResult))) false false)
            (`SceneComponent.K2_SetWorldLocation` (`self.NS_Sample_BONK`) (`self.K2_GetActorLocation` (`.HitActor` (`GameplayStatics.BreakHitResult` SweepResult))) false false)
            (`ActorComponent.Activate` (`self.NS_Sample_BONK`) true)
            (`ActorComponent.Activate` (`self.NS_FinisherHit`) true))
          (:`then_1`
            (`SceneComponent.SetHiddenInGame` (`self.Table`) true false :!label _label)
            (`KismetSystemLibrary.Delay` 0.1) ; Let the game hit other enemies really close to the 1st one hit
            (`self.SetActorEnableCollision` false)
            (`KismetSystemLibrary.Delay` 2.0)
            (`self.K2_DestroyActor`)))
        (elif (or (`ActorComponent.ComponentHasTag` OtherComp "Chair") (`ActorComponent.ComponentHasTag` OtherComp "Table"))
          (`|ExecutionSequence`
            (:`then_0`
              (`ActorComponent.Activate` (`self.NS_Sample_BONK`) true)
              (`ActorComponent.Activate` _projectilemovement false)
              (bind (_direction_2 _distancemultiplier_2) (`Timeline|Timeline` :!via `PlayFromStart`)
                (:`Update`
                  (bind (_returnvalue_x_2 _returnvalue_y_2) (`KismetMathLibrary.BreakVector` (* (`self.GetActorForwardVector` (`GameplayStatics.GetPlayerPawn` 0)) (* _distancemultiplier_2 (`self.Hit Back Distance No Kick`)))))
                  (set `MovementComponent.Velocity` (`KismetMathLibrary.MakeVector` _returnvalue_x_2 _returnvalue_y_2) _projectilemovement))
                (:`Finished`
                  (set `self.AlreadyKicked?` false))))
            (:`then_1`
              (`KismetSystemLibrary.Delay` 0.1)
              (set `self.AlreadyKicked?` true))))))))

(event `Auto Destroyed`
  (goto _label))

(fn `UserConstructionScript`)