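; Anim notify state that controls whether the player character can move during a window of an animation and passes it an attack distance.
; On begin it sends player character 0 the CanMove and AttackDistance messages, and on end it sends CanMove again with a separate end value.
; It always targets player 0 rather than the owner of the animated mesh, which serves only as world context.
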(fn `Received_NotifyBegin`
  (params (MeshComp :type "SkeletalMeshComponent Object Reference") (Animation :type "AnimSequenceBase Object Reference") (TotalDuration :type "Float (single-precision)") (EventReference :type "AnimNotifyEventReference Structure (by ref)"))
  (returns (ReturnValue :type Boolean))
  (bind _returnvalue (`GameplayStatics.GetPlayerCharacter` MeshComp))
  (message `/Game/Combat_Demo/Player/Blueprints/BPI_Player.CanMove` _returnvalue (`self.Block Movement? (BEGIN)`))
  (message `/Game/Combat_Demo/Player/Blueprints/BPI_Player.AttackDistance` _returnvalue (`self.Attack Distance`))
  (return false))

(fn `Received_NotifyEnd`
  (params (MeshComp :type "SkeletalMeshComponent Object Reference") (Animation :type "AnimSequenceBase Object Reference") (EventReference :type "AnimNotifyEventReference Structure (by ref)"))
  (returns (ReturnValue :type Boolean))
  (message `/Game/Combat_Demo/Player/Blueprints/BPI_Player.CanMove` (`GameplayStatics.GetPlayerCharacter` MeshComp) (`self.Block Movement? (END)`))
  (return false))