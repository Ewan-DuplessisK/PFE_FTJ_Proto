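; BP_NotifyHitbox is an animation notify state that toggles sword hitbox collision during combat animations.
; On begin, it gets the hitboxes from player character 0 through SwordHitboxActivationMessage and applies CollisionBEGIN to the one selected by HitboxToUse.
; On end, it applies CollisionEND to the whole returned set.
; A sphere trace along the greatsword sockets remains as disconnected, unused logic.
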(fn `Received_NotifyBegin`
  (params (MeshComp :type "SkeletalMeshComponent Object Reference") (Animation :type "AnimSequenceBase Object Reference") (TotalDuration :type "Float (single-precision)") (EventReference :type "AnimNotifyEventReference Structure (by ref)"))
  (returns (ReturnValue :type Boolean))
  (bind _box_collision (message `/Game/Combat_Demo/Player/Blueprints/BPI_Player.Sword Hitbox Activation` (`GameplayStatics.GetPlayerCharacter` MeshComp)))
  (`PrimitiveComponent.SetCollisionEnabled` (`|GetArrayItem` _box_collision (`self.Hitbox to Use`)) (`self.Collision (BEGIN)`))
  (return false))

(fn `Received_NotifyEnd`
  (params (MeshComp :type "SkeletalMeshComponent Object Reference") (Animation :type "AnimSequenceBase Object Reference") (EventReference :type "AnimNotifyEventReference Structure (by ref)"))
  (returns (ReturnValue :type Boolean))
  (bind _box_collision (message `/Game/Combat_Demo/Player/Blueprints/BPI_Player.Sword Hitbox Activation` (`GameplayStatics.GetPlayerCharacter` MeshComp)))
  (`PrimitiveComponent.SetCollisionEnabled` _box_collision (`self.Collision (END)`))
  (return false))