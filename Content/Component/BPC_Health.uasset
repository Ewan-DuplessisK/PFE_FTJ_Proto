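; BPC_Health is a health component that applies damage and healing, clamped between zero and max health.
; HealthRemove reports death for non-players; for the player it shakes the camera, scaled only for non-enemy hits.
; Enemy hits on the player also notify WBP_InGameMenu and BP_Player before reporting death.
; HealthAdd always triggers the healing effect on player character zero, whichever actor owns the component.
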(fn `Health_Add`
  (params (Amount :type "Float (double-precision)"))
  (set `self.Health_Current` (`KismetMathLibrary.FClamp` (+ (`self.Health_Current`) Amount) 0.0 (`self.Health_Max`)))
  (`/Game/Characters/Player/Blueprints/BP_Player.Healing_Effect` (cast `/Game/Characters/Player/Blueprints/BP_Player` (`GameplayStatics.GetPlayerCharacter` 0) :!pure true)))

(fn `Health_Remove`
  (params (Amount :type "Float (double-precision)") (IsPlayer :type Boolean) (`Not Enemy Hit` :type Boolean) (Scale :type "Float (double-precision)") (`Enemy Ref` :type "Actor Object Reference"))
  (returns (Dead :type Boolean))
  (bind _output_get (set `self.Health_Current` (`KismetMathLibrary.FClamp` (- (`self.Health_Current`) Amount) 0.0 (`self.Health_Max`))))
  (if IsPlayer
    (`PlayerController.ClientStartCameraShake` :`self` (`GameplayStatics.GetPlayerController` 0) :`Shake` (select `bool` `Not Enemy Hit` :`false` "/Game/Camera_Shake/CS_OnHit.CS_OnHit_C" :`true` "/Game/Camera_Shake/CS_OnHit.CS_OnHit_C" :!type "CameraShakeBase Class Reference") :`Scale` (`KismetMathLibrary.SelectFloat` Scale 1.0 `Not Enemy Hit`))
    (if (not `Not Enemy Hit`)
      (bind _foundwidgets (`WidgetBlueprintLibrary.GetAllWidgetsOfClass` "/Game/UI/Menus/InGameMenu/WBP_InGameMenu.WBP_InGameMenu_C"))
      (`/Game/UI/Menus/InGameMenu/WBP_InGameMenu.On Hit` (`|GetArrayItem` _foundwidgets) `Enemy Ref`)
      (bind _asbp_player (cast `/Game/Characters/Player/Blueprints/BP_Player` (`GameplayStatics.GetPlayerCharacter` 0)))
      (bind _returnvalue (<= _output_get 0.0))
      (`/Game/Characters/Player/Blueprints/BP_Player.After Taking Damage` _asbp_player _returnvalue)
      (return _returnvalue))
    (else
      (return _returnvalue))))