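; BP_Dummy is an enemy character that chases the player, either on a looping timer or when PawnSensing spots them.
; Damage or a launch throws it with a ragdoll profile, then physics takes over on landing.
; While launched, its physics overlap passes reduced velocity to other dummies and kickable doors, chaining launches.
; QTE events freeze and restore walk speed, and hits from "Player Shoot" actors destroy it after a short delay.
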(event `self.ReceiveBeginPlay`
  (if (`self.ConstantChase`)
    (`KismetSystemLibrary.K2_SetTimerDelegate` (delegate `Chase`) 0.033333 true true)))

(event `Chase`
  (`|AIMoveTo` self (0.0 0.0 0.0) (`GameplayStatics.GetPlayerPawn` 0) (`self.Acceptance Radius`)))

(event `Launched`
  (params (Force :type "Vector Structure"))
  (`PrimitiveComponent.SetCollisionProfileName` (`self.Mesh`) "Ragdoll" true)
  (set `self.isLaunched` true)
  (`KismetArrayLibrary.Array_Add` (`self.Tags`) "Dead")
  (`self.LaunchCharacter` Force true))

(event `self.OnLanded`
  (params (Hit :type "HitResult Structure (by ref)"))
  (if (`self.isLaunched`)
    (`PrimitiveComponent.SetSimulatePhysics` (`self.Mesh`) true)
    (set `self.isLaunched` false)
    (`PrimitiveComponent.SetCollisionEnabled` (`self.CapsuleComponent`) "NoCollision")))

(event `self.OverlapPhysics.OnComponentBeginOverlap`
  (params (OverlappedComponent :type "PrimitiveComponent Object Reference") (OtherActor :type "Actor Object Reference") (OtherComp :type "PrimitiveComponent Object Reference") (OtherBodyIndex :type Integer) (bFromSweep :type Boolean) (SweepResult :type "HitResult Structure (by ref)"))
  (bind _returnvalue (`self.GetVelocity`))
  (bind _returnvalue_2 (* _returnvalue 0.8))
  ; Physics enabled objects collisions
  ; If the object is moving and not detecting itself
  (if (`self.isLaunched`)
    (if (!= OtherActor self)
      ; Colliding with an enemy
      (bind _asbp_dummy (cast `/Game/FullBPProto/GPEs/BP_Dummy` OtherActor)
        (:`then`
          (if (not (`/Game/FullBPProto/GPEs/BP_Dummy.isLaunched` _asbp_dummy))
            (`self.Launched` _asbp_dummy _returnvalue_2)
            ; Reduce actor speed after transmitting force
            (`PrimitiveComponent.SetAllPhysicsLinearVelocity` (`self.CapsuleComponent`) (* _returnvalue 0.5) false :!label _label)))
        (:`CastFailed`
          ; Colliding with a door
          (bind _asbp_kickable_door (cast `/Game/FullBPProto/GPEs/BP_KickableDoor` OtherActor))
          (if (not (`/Game/FullBPProto/GPEs/BP_KickableDoor.isLaunched` _asbp_kickable_door))
            (`/Game/FullBPProto/GPEs/BP_KickableDoor.Launched` _asbp_kickable_door _returnvalue_2)
            (goto _label)))))))

(event `self.ReceiveAnyDamage`
  (params (Damage :type "Float (single-precision)") (DamageType :type "DamageType Object Reference") (InstigatedBy :type "Controller Object Reference") (DamageCauser :type "Actor Object Reference"))
  (`KismetSystemLibrary.PrintString` (`KismetStringLibrary.Concat_StrStr` "I've got a damage: " (`KismetStringLibrary.Conv_DoubleToString` Damage)))
  (`self.Launched` (-150.0 0.0 150.0)))

(event `QTE End`
  (bind _charactermovement (`self.CharacterMovement`))
  ;[0 0.4964 1 0.5] QTE Enemy Speed
  (`/Engine/EditorBlueprintResources/StandardMacros.IsValid` _charactermovement
    (:`Is Valid`
      (set `CharacterMovementComponent.MaxWalkSpeed` 400.0 _charactermovement) ; Change Back enemy walk speed to normal after QTE
      (`KismetSystemLibrary.PrintString` "Reset speed"))))

(event `QTE Begin`
  (bind _charactermovement (`self.CharacterMovement`))
  ;[0 0.4964 1 0.5] QTE Enemy Speed
  (`/Engine/EditorBlueprintResources/StandardMacros.IsValid` _charactermovement
    (:`Is Valid`
      (set `CharacterMovementComponent.MaxWalkSpeed` 0.0 _charactermovement) ; Stop enemy to walk when in QTE
    )))

(event `self.CapsuleComponent.OnComponentHit`
  (params (HitComponent :type "PrimitiveComponent Object Reference") (OtherActor :type "Actor Object Reference") (OtherComp :type "PrimitiveComponent Object Reference") (NormalImpulse :type "Vector Structure") (Hit :type "HitResult Structure (by ref)"))
  ;[0.5729 0.02466 0 0.5] Die From Hit
  (if (`self.ActorHasTag` OtherActor "Player Shoot")
    (`PrimitiveComponent.SetSimulatePhysics` (`self.CapsuleComponent`) true)
    (`PrimitiveComponent.SetCollisionEnabled` (`self.OverlapPhysics`) "NoCollision")
    ;;[1 1 1 0.5] Delay Death
    (`KismetSystemLibrary.Delay` 0.5)
    (`self.K2_DestroyActor`)))

(event `self.PawnSensing.OnSeePawn`
  (params (Pawn :type "Pawn Object Reference"))
  ;[0.04145 0.4948 0 0.5] AI Behavior
  (if (not (`self.ConstantChase`))
    (bind _asbp_chara_systems (cast `/Game/FullBPProto/BP_CharaSystems` Pawn))
    (`|AIMoveTo` self (`self.K2_GetActorLocation` _asbp_chara_systems) null (`self.Acceptance Radius`))))

(fn `UserConstructionScript`)