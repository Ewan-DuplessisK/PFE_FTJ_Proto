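; AC_AimAssist is an aim assist component whose event graph currently contains only debug-view setup on BeginPlay.
; When the AimFeel debug flag is active, it sets the player's HUD to the aim debug class and caches it as BPH_AimingSys_Debug.
; It then passes the crosshair screen location to that HUD once, printing a message if the reference is invalid.
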(event `self.ReceiveBeginPlay`
  (bind _returnvalue (`GameplayStatics.GetPlayerController` 0))
  ;[0.15 1 0.15 0.5] Debug
  (`KismetSystemLibrary.PrintString` "Aim Sys Active" true true (struct :`R` 0.012392 :`G` 0.139398 :`B` 1.0 :`A` 1.0) 1.0)
  (`|ExecutionSequence`
    (:`then_0`
      (if (`.bIsDebugActive` (break `UAimAssistFeel` (`self.AimFeel`)))
        (`PlayerController.ClientSetHUD` _returnvalue (`self.wAimDebugWidget`))
        (set `self.MyAimDebugMenu` (cast `/Game/FullBPProto/AimAssist_Debug_Hud/BPH_AimingSys_Debug` (`PlayerController.GetHUD` _returnvalue) :!pure true))
        ;[0.15 1 0.15 0.5] Comment
        (`KismetSystemLibrary.PrintString` "Debug Active" true true (struct :`G` 0.66 :`A` 1.0) 1.0)))
    (:`then_1`
      ;[0 0.75 0.75] Aim Assist
      ;;[0.15 0.15 0.5] Debug View
      (if (`.bIsDebugActive` (break `UAimAssistFeel` (`self.AimFeel`)))
        (bind _asbph_aiming_sys_debug (cast `/Game/FullBPProto/AimAssist_Debug_Hud/BPH_AimingSys_Debug` (`self.MyAimDebugMenu`))
          (:`then`
            (set `/Game/FullBPProto/AimAssist_Debug_Hud/BPH_AimingSys_Debug.Main Crosshair Location` (`self.CrosshairScreenLocation`) _asbph_aiming_sys_debug))
          (:`CastFailed`
            (`KismetSystemLibrary.PrintString` "Invalid Ref in AC_AimAssist")))))))