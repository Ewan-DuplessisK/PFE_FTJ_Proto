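; First-person player character systems for life and QTE widgets, enemy alerting and a grab-escape QTE.
; While PlayerAction is true, a temporary Tick loop flags every coworker enemy's blackboard.
; SwitchInputEvent swaps mapping contexts for button mashing against the first enemy found; success launches the player, then releases that enemy after a delay.
; RaycastDamage provides camera-line hits; the sphere-trace kick for enemies and doors is unwired.
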(event `Key|Four`
  (params (Key :type "Key Structure"))
  (bind _returnvalue (`GameplayStatics.GetPlayerController` 0))
  (:`Pressed`
    (`/Engine/EditorBlueprintResources/StandardMacros.FlipFlop`
      (:`A`
        (set `PlayerController.bShowMouseCursor` true _returnvalue))
      (:`B`
        (set `PlayerController.bShowMouseCursor` false _returnvalue)))))

(event `self.ReceiveTick`
  (params (DeltaSeconds :type "Float (single-precision)"))
  ;[1 0 0] Need to be move / TEMPORARY
  (if (`self.PlayerAction`)
    (bind _outactors (`GameplayStatics.GetAllActorsOfClass` "/Game/IA_System/01_Coworker_RD/BP_EnemyAI_Coworker_RD.BP_EnemyAI_Coworker_RD_C"))
    (for _array_element _outactors
      (bind _asbp_enemy_ai_coworker_rd (cast `/Game/IA_System/01_Coworker_RD/BP_EnemyAI_Coworker_RD` _array_element))
      (`/Game/IA_System/01_Coworker_RD/BP_EnemyAI_Coworker_RD.Activate PlayerInRangeBox` _asbp_enemy_ai_coworker_rd)
      (`BlackboardComponent.SetValueAsBool` (`AIBlueprintHelperLibrary.GetBlackboard` (`AIBlueprintHelperLibrary.GetAIController` _array_element)) "playerAction?" true))))

(event `self.ReceiveBeginPlay`
  (`|ExecutionSequence`
    (:`then_0`
      ;[0.025 0.75 0.75] Structure ("S_PlayerFeel")
      (`self.InitializeVarsWithPlayerFeelStruct`)
      ;[0.15 0.15 0.15] Life Init
      (bind _returnvalue (`|CreateWidget` "/Game/UI/W_PlayerLife.W_PlayerLife_C"))
      (bind _output_get (set `self.PlayerLifeWidget` _returnvalue))
      (`UserWidget.AddToViewport` _output_get 0)
      (set `self.PlayerLife Current` (`self.PlayerLife Max`)))
    (:`then_1`
      ;[0.03784 0.15 0.1151 0.5] Add QTE Widget
      (bind _returnvalue_2 (`|CreateWidget` "/Game/UI/W_QTE.W_QTE_C"))
      (bind _output_get_2 (set `self.W_QTE` _returnvalue_2))
      (`UserWidget.AddToViewport` _output_get_2 0)
      (`Widget.SetVisibility` _output_get_2 "Hidden"))
    (:`then_2`
      (bind _returnvalue_3 (`|CreateWidget` "/Game/IA_System/Viewport/WBP_EnemyAITestMap.WBP_EnemyAITestMap_C"))
      (`UserWidget.AddToViewport` _returnvalue_3 0))
    (:`then_3`
      (if (not (`PlayerController.bShowMouseCursor` (`GameplayStatics.GetPlayerController` 0)))
        (`/Engine/EditorBlueprintResources/StandardMacros.DoOnce` false
          (:`Completed`
            (`Widget.SetVisibility` _returnvalue_3 "Hidden")))))))

(event `Switch Input Event`
  (bind _returnvalue (pcsubsystem `EnhancedInputLocalPlayerSubsystem` (`GameplayStatics.GetPlayerController` 0)))
  ;[0 0 1] QTE
  (bind _returnvalue_2 (`GameplayStatics.GetActorOfClass` "/Game/IA_System/01_Coworker_RD/BP_EnemyAI_Coworker_RD.BP_EnemyAI_Coworker_RD_C"))
  (`/Engine/EditorBlueprintResources/StandardMacros.IsValid` _returnvalue
    (:`Is Valid`
      (`/Engine/EditorBlueprintResources/StandardMacros.IsValid` _returnvalue_2
        (:`Is Valid`
          (if (`/Game/IA_System/01_Coworker_RD/BP_EnemyAI_Coworker_RD.isPlayerInAttackRange?` _returnvalue_2)
            ;; Change IMC from System to QTE
            (`EnhancedInputSubsystemInterface.RemoveMappingContext` _returnvalue "/Game/FullBPProto/Inputs/IMC_Systems.IMC_Systems" (struct))
            (`EnhancedInputSubsystemInterface.AddMappingContext` _returnvalue "/Game/FirstPerson/Input/IMC_QTE.IMC_QTE" 0 (struct))))))))

(event `EnhancedInput|/Game/FullBPProto/Inputs/Actions/IA_QTE`
  (params (ActionValue :type Boolean) (ElapsedSeconds :type "Float (double-precision)") (TriggeredSeconds :type "Float (double-precision)") (InputAction :type "InputAction Object Reference" :default "/Game/FullBPProto/Inputs/Actions/IA_QTE.IA_QTE"))
  ;[0 0 1] QTE
  (:`Triggered`
    (`KismetSystemLibrary.PrintString` "QTE Pressed")
    (set `/Game/IA_System/01_Coworker_RD/BP_EnemyAI_Coworker_RD.QTE Current` (+ (`/Game/IA_System/01_Coworker_RD/BP_EnemyAI_Coworker_RD.QTE Current` (stale `Switch Input Event` _returnvalue_2)) 1.25) (stale `Switch Input Event` _returnvalue_2))
    (if (>= (`/Game/IA_System/01_Coworker_RD/BP_EnemyAI_Coworker_RD.QTE Current` (stale `Switch Input Event` _returnvalue_2)) (`Enemy_Base.QTEInputRequired` (stale `Switch Input Event` _returnvalue_2)))
      (`self.QTE End Event`))))

(event `QTE End Event`
  (bind _returnvalue (pcsubsystem `EnhancedInputLocalPlayerSubsystem` (`GameplayStatics.GetPlayerController` 0)))
  ;[0 0 1] QTE
  (`KismetSystemLibrary.K2_PauseTimerHandle` (`/Game/IA_System/01_Coworker_RD/BP_EnemyAI_Coworker_RD.QTE Health Timer` (stale `Switch Input Event` _returnvalue_2)))
  (set `/Game/IA_System/01_Coworker_RD/BP_EnemyAI_Coworker_RD.QTE Current` 0.0 (stale `Switch Input Event` _returnvalue_2))
  ;;[1 1 1 0.5] Change IMC from QTE to Sysem
  (`EnhancedInputSubsystemInterface.RemoveMappingContext` _returnvalue "/Game/FirstPerson/Input/IMC_QTE.IMC_QTE" (struct))
  (`EnhancedInputSubsystemInterface.AddMappingContext` _returnvalue "/Game/FullBPProto/Inputs/IMC_Systems.IMC_Systems" 0 (struct))
  (`Widget.SetVisibility` (stale `self.ReceiveBeginPlay` _returnvalue_2) "Hidden")
  (`self.LaunchCharacter` (`Enemy_Base.LaunchVelocity` (stale `Switch Input Event` _returnvalue_2))) ; Push Player from the enemy who grabbed him
  (`KismetSystemLibrary.Delay` (`Enemy_Base.TimeAFKAfterQTE` (stale `Switch Input Event` _returnvalue_2))) ; Time before enemy reactivate
  (`/Engine/EditorBlueprintResources/StandardMacros.IsValid` self
    (:`Is Valid`
      (`/Game/IA_System/01_Coworker_RD/BP_EnemyAI_Coworker_RD.QTE End` (stale `Switch Input Event` _returnvalue_2))
      (set `/Game/IA_System/01_Coworker_RD/BP_EnemyAI_Coworker_RD.isPlayerInAttackRange?` false (stale `Switch Input Event` _returnvalue_2)))))

(fn `Raycast Damage`
  (params (Range :type "Float (double-precision)") (Damage :type "Float (double-precision)"))
  (bind (_returnvalue_location _returnvalue_rotation) (`KismetMathLibrary.BreakTransform` (`SceneComponent.K2_GetComponentToWorld` (`self.FirstPersonCameraComponent`))))
  (bind _returnvalue (+ _returnvalue_location (0.0 0.0 -2.0)))
  (bind _outhit (`KismetSystemLibrary.LineTraceSingle` :`Start` _returnvalue :`End` (+ _returnvalue (* (`KismetMathLibrary.GetForwardVector` _returnvalue_rotation) Range)) :`TraceChannel` "TraceTypeQuery2" :`bTraceComplex` true :`DrawDebugType` "ForOneFrame"))
  (cast `Character` (`.HitActor` (`GameplayStatics.BreakHitResult` _outhit)))
  (`GameplayStatics.ApplyDamage` (`.HitActor` (`GameplayStatics.BreakHitResult` _outhit)) Damage)
  (`NiagaraFunctionLibrary.SpawnSystemAtLocation` "/Game/VFX/NS_KickPlaceholder.NS_KickPlaceholder" (`.Location` (`GameplayStatics.BreakHitResult` _outhit))))

(fn `UserConstructionScript`)