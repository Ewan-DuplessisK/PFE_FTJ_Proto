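; Player controller that drives the run timer, routes player input and provides a quick 180-degree turn.
; It starts and ticks the timer in GI_Systems, pauses it on Y, and creates timer and hidden camera debug widgets.
; Fire, throw, kick and interact inputs forward to the BP_CharaSystems pawn or its weapon-user component.
; The turn stops movement and timeline-lerps control rotation; mapping-context and debug-toggle logic are unwired.
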(event `self.ReceiveTick`
  (params (DeltaSeconds :type "Float (single-precision)"))
  (bind _as_gi_systems (`self.As GI Systems`)
    (:`then`
      (`/Game/FullBPProto/GI_Systems.RunTimer` _as_gi_systems DeltaSeconds))
    (:`else`)))

(event `self.ReceiveBeginPlay`
  ;[0.5 0.5 1] Add IMC
  (`|ExecutionSequence`
    (:`then_0`
      (bind _asgi_systems (cast `/Game/FullBPProto/GI_Systems` (`GameplayStatics.GetGameInstance`)))
      (set `self.As GI Systems` _asgi_systems)
      (`/Game/FullBPProto/GI_Systems.StartTimer` (`self.As GI Systems`))
      (bind _returnvalue (`|CreateWidget` "/Game/UI/WBP_Timer.WBP_Timer_C"))
      (set `self.TimerWidget` _returnvalue)
      (`UserWidget.AddToViewport` (`self.TimerWidget`) 0))
    (:`then_2`
      (bind _returnvalue_2 (`|CreateWidget` "/Game/FullBPProto/AimAssist_Debug_Hud/WBP_Camera_Debug.WBP_Camera_Debug_C"))
      (bind _output_get (set `self.Debug Widget Ref` _returnvalue_2))
      (`UserWidget.AddToViewport` _output_get 0)
      (`Widget.SetVisibility` _output_get "Collapsed"))))

(event `Key|P` :paused true
  (params (Key :type "Key Structure"))
  ;[1 0 1] Debug
)

(event `EnhancedInput|/Game/FullBPProto/Inputs/Actions/IA_180Turn`
  (params (ActionValue :type Boolean) (ElapsedSeconds :type "Float (double-precision)") (TriggeredSeconds :type "Float (double-precision)") (InputAction :type "InputAction Object Reference" :default "/Game/FullBPProto/Inputs/Actions/IA_180Turn.IA_180Turn"))
  (bind (_returnvalue_roll _returnvalue_pitch _returnvalue_yaw) (`KismetMathLibrary.BreakRotator` (`self.GetControlRotation`)))
  (bind _180_rotation (`self.180_Rotation`))
  (bind _yaw (.yaw (select `bool` (< _returnvalue_yaw 0.0) :`false` (`KismetMathLibrary.MakeRotator` _returnvalue_roll _returnvalue_pitch (+ _returnvalue_yaw _180_rotation)) :`true` (`KismetMathLibrary.MakeRotator` _returnvalue_roll _returnvalue_pitch (+ _returnvalue_yaw (* _180_rotation -1.0))))))
  ;[0.2 1 0.2] 180 Rotation
  (:`Triggered`
    (if (`self.bCan180Rota`)
      (set `self.bCan180Rota` false)
      (`MovementComponent.StopMovementImmediately` (`Character.CharacterMovement` (`self.Player Ref`)))
      (bind _output_get (set `self.Temp Rota` (`KismetMathLibrary.MakeRotator` (.roll (select `bool` (< _returnvalue_yaw 0.0) :`false` (`KismetMathLibrary.MakeRotator` _returnvalue_roll _returnvalue_pitch (+ _returnvalue_yaw _180_rotation)) :`true` (`KismetMathLibrary.MakeRotator` _returnvalue_roll _returnvalue_pitch (+ _returnvalue_yaw (* _180_rotation -1.0))))) (.pitch (select `bool` (< _returnvalue_yaw 0.0) :`false` (`KismetMathLibrary.MakeRotator` _returnvalue_roll _returnvalue_pitch (+ _returnvalue_yaw _180_rotation)) :`true` (`KismetMathLibrary.MakeRotator` _returnvalue_roll _returnvalue_pitch (+ _returnvalue_yaw (* _180_rotation -1.0))))) (select `bool` (>= _yaw 360.0) :`false` (select `bool` (<= _yaw 0.0) :`false` _yaw :`true` (+ _yaw 360.0) :!type "Float (single-precision)") :`true` (- _yaw 360.0) :!type "Float (single-precision)"))))
      (bind (_direction _rota_speed) (`Timeline|Timeline` :!via `PlayFromStart`)
        (:`Update`
          (`self.SetControlRotation` (`KismetMathLibrary.RLerp` (`self.GetControlRotation`) _output_get _rota_speed)))
        (:`Finished`
          (set `self.bCan180Rota` true))))))

(event `EnhancedInput|/Game/FullBPProto/Inputs/Actions/IA_Fire`
  (params (ActionValue :type Boolean) (ElapsedSeconds :type "Float (double-precision)") (TriggeredSeconds :type "Float (double-precision)") (InputAction :type "InputAction Object Reference" :default "/Game/FullBPProto/Inputs/Actions/IA_Fire.IA_Fire"))
  (bind _returnvalue (`self.K2_GetPawn`))
  (:`Triggered`
    (bind _asbp_chara_systems (cast `/Game/FullBPProto/BP_CharaSystems` _returnvalue))
    (`/Game/Developers/ISh/Weapon2/AC_Weapon_User.IA_Attack Triggered` (`/Game/FullBPProto/BP_CharaSystems.AC_Weapon_User` _asbp_chara_systems)))
  (:`Started`
    (bind _asbp_chara_systems_2 (cast `/Game/FullBPProto/BP_CharaSystems` _returnvalue))
    (`/Game/Developers/ISh/Weapon2/AC_Weapon_User.IA_Attack Started` (`/Game/FullBPProto/BP_CharaSystems.AC_Weapon_User` _asbp_chara_systems_2))))

(event `EnhancedInput|/Game/FullBPProto/Inputs/Actions/IA_Throw`
  (params (ActionValue :type Boolean) (ElapsedSeconds :type "Float (double-precision)") (TriggeredSeconds :type "Float (double-precision)") (InputAction :type "InputAction Object Reference" :default "/Game/FullBPProto/Inputs/Actions/IA_Throw.IA_Throw"))
  (:`Triggered`
    (bind _asbp_chara_systems (cast `/Game/FullBPProto/BP_CharaSystems` (`self.K2_GetPawn`)))
    (`/Game/Developers/ISh/Weapon2/AC_Weapon_User.Throw Weapon` (`/Game/FullBPProto/BP_CharaSystems.AC_Weapon_User` _asbp_chara_systems))))

(event `EnhancedInput|/Game/FullBPProto/Inputs/Actions/IA_Kick`
  (params (ActionValue :type Boolean) (ElapsedSeconds :type "Float (double-precision)") (TriggeredSeconds :type "Float (double-precision)") (InputAction :type "InputAction Object Reference" :default "/Game/FullBPProto/Inputs/Actions/IA_Kick.IA_Kick"))
  (:`Triggered`
    (bind _asbp_chara_systems (cast `/Game/FullBPProto/BP_CharaSystems` (`self.K2_GetPawn`)))
    (`/Game/FullBPProto/BP_CharaSystems.Kick` _asbp_chara_systems)))

(event `EnhancedInput|/Game/FullBPProto/Inputs/Actions/IA_Interact`
  (params (ActionValue :type Boolean) (ElapsedSeconds :type "Float (double-precision)") (TriggeredSeconds :type "Float (double-precision)") (InputAction :type "InputAction Object Reference" :default "/Game/FullBPProto/Inputs/Actions/IA_Interact.IA_Interact"))
  (:`Triggered`
    (`/Game/Developers/ISh/Interactable/AC_Interact_User.Do Interact` (`/Game/FullBPProto/BP_CharaSystems.AC_Weapon_User` (cast `/Game/FullBPProto/BP_CharaSystems` (`self.K2_GetPawn`) :!pure true)))))

(event `Key|Gamepad_DPad_Down`
  (params (Key :type "Key Structure")))

(event `Key|Y`
  (params (Key :type "Key Structure"))
  (:`Released`
    (`/Game/FullBPProto/GI_Systems.PauseTimer` (`self.As GI Systems`))))

(fn `UserConstructionScript`)