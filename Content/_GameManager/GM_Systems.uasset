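; GM_Systems is a game manager Blueprint that handles player death and the level restart.
; It caches the player's BP_CharaSystems on BeginPlay and polls its current life every Tick.
; When life reaches zero, a DoOnce shows the PC_Systems lose widget, plays a death sound and pauses the GI_Systems timer.
; The current level reloads by name after a short delay.
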(event `self.ReceiveBeginPlay`
  (bind _asbp_chara_systems (cast `/Game/PlayerCharacter/BP_CharaSystems` (`GameplayStatics.GetPlayerPawn` 0)))
  (set `self.Player` _asbp_chara_systems))

(event `self.ReceiveTick`
  (params (DeltaSeconds :type "Float (single-precision)"))
  (if (<= (`/Game/PlayerCharacter/BP_CharaSystems.PlayerLife Current` (`self.Player`)) 0.0)
    (`/Engine/EditorBlueprintResources/StandardMacros.DoOnce` false
      (:`Completed`
        (bind _aspc_systems (cast `/Game/_GameManager/PC_Systems` (`GameplayStatics.GetPlayerController` 0)))
        (`Widget.SetVisibility` (`/Game/_GameManager/PC_Systems.LoseWidget` _aspc_systems) "Visible")
        (`GameplayStatics.PlaySound2D` "/Game/Sound/DS_Death.DS_Death" 1.0 1.0 0.0 null null)
        (`|ExecutionSequence`
          (:`then_0`
            (`KismetSystemLibrary.Delay` 5.5)
            (bind _returnvalue (`GameplayStatics.GetCurrentLevelName` true))
            (`GameplayStatics.OpenLevel` (`KismetStringLibrary.Conv_StringToName` _returnvalue)))
          (:`then_1`
            (bind _asgi_systems (cast `/Game/_GameManager/GI_Systems` (`GameplayStatics.GetGameInstance`)))
            (`/Game/_GameManager/GI_Systems.PauseTimer` _asgi_systems)))))))

(fn `UserConstructionScript`)