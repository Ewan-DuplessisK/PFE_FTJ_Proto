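; Player controller that wires gameplay input, the pause menu with its settings, the run timer and debug tools.
; Enhanced Input events route attack, throw and interact to the pawn's weapon component, and handle dash and a timeline-lerped 180 turn directly.
; BeginPlay spawns timer and debug widgets; Tick advances the GI_Systems timer and feeds sticks and triggers to the controller input visualizer.
; Debug keys toggle the debug menu, flip camera inversion and reload the level.
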(event Custom|PlayButtonEvent
  ;[0.15 0.15 0.15 0.5] Menu related thingies
  (bind _as_gi_systems (Variables|Ref|GetAs%20GI%20Systems)
    (:then
      (Default|PauseTimer _as_gi_systems)
      (Game|SetGamePaused false)
      (Variables|/Script/UMG.Widget|SetVisibility (Variables|/Game/UI/HUD_InGame.HUD_InGame_C|GetRef%20PauseMenu (Variables|Ref|GetRef%20HUD%20InGame)) "Hidden")
      (Input|SetInputModeGameOnly self false))
    (:else)))

(event Custom|OpenSettingsButtonEvent
  (bind _ref_hud_ingame (Variables|Ref|GetRef%20HUD%20InGame))
  (bind _ref_pausemenu (Variables|/Game/UI/HUD_InGame.HUD_InGame_C|GetRef%20PauseMenu _ref_hud_ingame))
  ;[0.15 0.15 0.15 0.5] Menu related thingies
  ;;[0.2206 0.5625 0 0.5] Settings
  (Variables|/Script/UMG.Widget|SetVisibility (Variables|/Game/UI/PauseMenu/WBP_PauseMenu.WBP_PauseMenu_C|GetSettingsPanel _ref_pausemenu) "Visible")
  (Widget|SetIsEnabled (Variables|/Game/UI/PauseMenu/WBP_PauseMenu.WBP_PauseMenu_C|GetGridPanelMainMenu _ref_pausemenu) false)
  (Widget|SetFocus (Variables|/Game/UI/MainMenu/WBP_SettingsContent.WBP_SettingsContent_C|GetSoundLess_Btn (Variables|/Game/UI/PauseMenu/WBP_PauseMenu.WBP_PauseMenu_C|GetWBP_SettingsContent _ref_pausemenu))))

(event Custom|SendControllerVisualizerData
  (bind _returnvalue (PlayerController|LocalPlayerSubsystems|GetEnhancedInputLocalPlayerSubsystem))
  ;[0 0 0 0.33 50] ControllerVisualizer Debug
  ;;[0.08067 0.6955 1 0.33] Stick Movement & Trigger Axes
  (Utilities|IsValid _returnvalue
    (:Is%20Valid
      (if (.ReturnValue (Class|EnhancedInputSubsystemInterface|HasMappingContext _returnvalue "/Game/ControllerInputVisualizer/Inputs/IMC_ControllerVisualizer.IMC_ControllerVisualizer"))
        (bind _controller_input_visualizer (Variables|DebugMenu|GetController%20Input%20Visualizer)
          (:then
            (Default|ReceiveInputVisualizationDataStick _controller_input_visualizer (Input|EnhancedActionValues|GetIA_Visu_StickLeft_Movement) true)
            (Default|ReceiveInputVisualizationDataStick (Variables|DebugMenu|GetController%20Input%20Visualizer) (Input|EnhancedActionValues|GetIA_Visu_StickRight_Movement) false)
            (Default|ReceiveInputVisualizationDataAxis (Variables|DebugMenu|GetController%20Input%20Visualizer) (Input|EnhancedActionValues|GetIA_Visu_Trigger_Left) true)
            (Default|ReceiveInputVisualizationDataAxis (Variables|DebugMenu|GetController%20Input%20Visualizer) (Input|EnhancedActionValues|GetIA_Visu_Trigger_Right) false))
          (:else))))))

(event Custom|CloseSettingsButtonEvent
  (bind _ref_hud_ingame (Variables|Ref|GetRef%20HUD%20InGame))
  (bind _ref_pausemenu (Variables|/Game/UI/HUD_InGame.HUD_InGame_C|GetRef%20PauseMenu _ref_hud_ingame))
  ;[0.15 0.15 0.15 0.5] Menu related thingies
  ;;[0.2206 0.5625 0 0.5] Settings
  (Variables|/Script/UMG.Widget|SetVisibility (Variables|/Game/UI/PauseMenu/WBP_PauseMenu.WBP_PauseMenu_C|GetSettingsPanel _ref_pausemenu) "Hidden")
  (Widget|SetIsEnabled (Variables|/Game/UI/PauseMenu/WBP_PauseMenu.WBP_PauseMenu_C|GetGridPanelMainMenu _ref_pausemenu) true)
  (Widget|SetFocus (Variables|/Game/UI/PauseMenu/WBP_PauseMenu.WBP_PauseMenu_C|GetSettingsBtn _ref_pausemenu)))

(event Custom|CustomEvent
  (params (Visibility :type Boolean))
  ;[0 0 0 0.33 50] ControllerVisualizer Debug
  (Default|SetUIVisibility (Variables|DebugMenu|GetController%20Input%20Visualizer) Visibility))

(event Input|EnhancedActionEvents|EnhancedInputActionIA_Interact
  (params (ActionValue :type Boolean) (ElapsedSeconds :type Float%20%28double-precision%29) (TriggeredSeconds :type Float%20%28double-precision%29) (InputAction :type Input%20Action%20Object%20Reference :default "/Game/_GameManager/Inputs/Actions/IA_Interact.IA_Interact"))
  ;[0.15 0.15 0.15 0.5] Weapon Input Actions
  (Default|DoInteract (Variables|/Game/PlayerCharacter/BP_CharaSystems.BP_CharaSystems_C|GetAC_Weapon_User (.AsBP%20Chara%20Systems (Utilities|Casting|CastToBP_CharaSystems (Pawn|GetControlledPawn))))))

(event Input|EnhancedActionEvents|EnhancedInputActionIA_Pause
  (params (ActionValue :type Boolean) (ElapsedSeconds :type Float%20%28double-precision%29) (TriggeredSeconds :type Float%20%28double-precision%29) (InputAction :type Input%20Action%20Object%20Reference :default "/Game/_GameManager/Inputs/Actions/IA_Pause.IA_Pause"))
  (bind _ref_hud_ingame (Variables|Ref|GetRef%20HUD%20InGame))
  (bind _ref_pausemenu (Variables|/Game/UI/HUD_InGame.HUD_InGame_C|GetRef%20PauseMenu _ref_hud_ingame))
  ;[0.15 0.15 0.15 0.5] Menu related thingies
  (Variables|Ref|GetRef%20HUD%20InGame
    (:then
      (if (not (Game|IsGamePaused))
        (Game|SetGamePaused true)
        (Variables|/Script/UMG.Widget|SetVisibility _ref_pausemenu "Visible")
        (Input|SetInputModeUIOnly self _ref_pausemenu "DoNotLock" false)
        (Widget|SetFocus (Variables|/Game/UI/PauseMenu/WBP_PauseMenu.WBP_PauseMenu_C|GetPlayBtn _ref_pausemenu))
        (bind _as_gi_systems (Variables|Ref|GetAs%20GI%20Systems)
          (:then
            (Default|PauseTimer _as_gi_systems))
          (:else))))
    (:else
      (Development|PrintString "HUD_InGame invalid 
Desactive HUD Debug"))))

(event Input|EnhancedActionEvents|EnhancedInputActionIA_Visu_FaceButton_Top
  (params (ActionValue :type Boolean) (ElapsedSeconds :type Float%20%28double-precision%29) (TriggeredSeconds :type Float%20%28double-precision%29) (InputAction :type Input%20Action%20Object%20Reference :default "/Game/ControllerInputVisualizer/Inputs/IA_Visu_FaceButton_Top.IA_Visu_FaceButton_Top"))
  ;[0 0 0 0.33 50] ControllerVisualizer Debug
  ;;[1 0.5477 0.8376 0.33] Face Button
  (:Started
    (Default|ReceiveInputVisualizationDataButton (Variables|DebugMenu|GetController%20Input%20Visualizer) true "NewEnumerator7"))
  (:Completed
    (Default|ReceiveInputVisualizationDataButton (Variables|DebugMenu|GetController%20Input%20Visualizer) false "NewEnumerator7")))

(event Input|EnhancedActionEvents|EnhancedInputActionIA_Visu_FaceButton_Left
  (params (ActionValue :type Boolean) (ElapsedSeconds :type Float%20%28double-precision%29) (TriggeredSeconds :type Float%20%28double-precision%29) (InputAction :type Input%20Action%20Object%20Reference :default "/Game/ControllerInputVisualizer/Inputs/IA_Visu_FaceButton_Left.IA_Visu_FaceButton_Left"))
  ;[0 0 0 0.33 50] ControllerVisualizer Debug
  ;;[1 0.5477 0.8376 0.33] Face Button
  (:Started
    (Default|ReceiveInputVisualizationDataButton (Variables|DebugMenu|GetController%20Input%20Visualizer) true "NewEnumerator5"))
  (:Completed
    (Default|ReceiveInputVisualizationDataButton (Variables|DebugMenu|GetController%20Input%20Visualizer) false "NewEnumerator5")))

(event Input|EnhancedActionEvents|EnhancedInputActionIA_Visu_FaceButton_Right
  (params (ActionValue :type Boolean) (ElapsedSeconds :type Float%20%28double-precision%29) (TriggeredSeconds :type Float%20%28double-precision%29) (InputAction :type Input%20Action%20Object%20Reference :default "/Game/ControllerInputVisualizer/Inputs/IA_Visu_FaceButton_Right.IA_Visu_FaceButton_Right"))
  ;[0 0 0 0.33 50] ControllerVisualizer Debug
  ;;[1 0.5477 0.8376 0.33] Face Button
  (:Started
    (Default|ReceiveInputVisualizationDataButton (Variables|DebugMenu|GetController%20Input%20Visualizer) true "NewEnumerator6"))
  (:Completed
    (Default|ReceiveInputVisualizationDataButton (Variables|DebugMenu|GetController%20Input%20Visualizer) false "NewEnumerator6")))

(event Input|EnhancedActionEvents|EnhancedInputActionIA_Visu_DPad_Bottom
  (params (ActionValue :type Boolean) (ElapsedSeconds :type Float%20%28double-precision%29) (TriggeredSeconds :type Float%20%28double-precision%29) (InputAction :type Input%20Action%20Object%20Reference :default "/Game/ControllerInputVisualizer/Inputs/IA_Visu_DPad_Bottom.IA_Visu_DPad_Bottom"))
  ;[0 0 0 0.33 50] ControllerVisualizer Debug
  ;;[0.3557 1 0.4036 0.33] DPad
  (:Started
    (Default|ReceiveInputVisualizationDataButton (Variables|DebugMenu|GetController%20Input%20Visualizer) true "NewEnumerator0"))
  (:Completed
    (Default|ReceiveInputVisualizationDataButton (Variables|DebugMenu|GetController%20Input%20Visualizer) false "NewEnumerator0")))

(event Input|EnhancedActionEvents|EnhancedInputActionIA_Visu_DPad_Left
  (params (ActionValue :type Boolean) (ElapsedSeconds :type Float%20%28double-precision%29) (TriggeredSeconds :type Float%20%28double-precision%29) (InputAction :type Input%20Action%20Object%20Reference :default "/Game/ControllerInputVisualizer/Inputs/IA_Visu_DPad_Left.IA_Visu_DPad_Left"))
  ;[0 0 0 0.33 50] ControllerVisualizer Debug
  ;;[0.3557 1 0.4036 0.33] DPad
  (:Started
    (Default|ReceiveInputVisualizationDataButton (Variables|DebugMenu|GetController%20Input%20Visualizer) true "NewEnumerator1"))
  (:Completed
    (Default|ReceiveInputVisualizationDataButton (Variables|DebugMenu|GetController%20Input%20Visualizer) false "NewEnumerator1")))

(event Input|EnhancedActionEvents|EnhancedInputActionIA_Visu_Special_Left
  (params (ActionValue :type Boolean) (ElapsedSeconds :type Float%20%28double-precision%29) (TriggeredSeconds :type Float%20%28double-precision%29) (InputAction :type Input%20Action%20Object%20Reference :default "/Game/ControllerInputVisualizer/Inputs/IA_Visu_Special_Left.IA_Visu_Special_Left"))
  ;[0 0 0 0.33 50] ControllerVisualizer Debug
  ;;[0.6146 0.6146 0.6146 0.33] Special Buttons
  (:Started
    (Default|ReceiveInputVisualizationDataButton (Variables|DebugMenu|GetController%20Input%20Visualizer) true "NewEnumerator10"))
  (:Completed
    (Default|ReceiveInputVisualizationDataButton (Variables|DebugMenu|GetController%20Input%20Visualizer) false "NewEnumerator10")))

(event Input|EnhancedActionEvents|EnhancedInputActionIA_Fire
  (params (ActionValue :type Boolean) (ElapsedSeconds :type Float%20%28double-precision%29) (TriggeredSeconds :type Float%20%28double-precision%29) (InputAction :type Input%20Action%20Object%20Reference :default "/Game/_GameManager/Inputs/Actions/IA_Fire.IA_Fire"))
  (bind _returnvalue (Pawn|GetControlledPawn))
  ;[0.15 0.15 0.15 0.5] Weapon Input Actions
  (:Triggered
    (bind _asbp_chara_systems (Utilities|Casting|CastToBP_CharaSystems _returnvalue))
    (Default|IAAttackTriggered (Variables|/Game/PlayerCharacter/BP_CharaSystems.BP_CharaSystems_C|GetAC_Weapon_User _asbp_chara_systems)))
  (:Started
    (bind _asbp_chara_systems_2 (Utilities|Casting|CastToBP_CharaSystems _returnvalue))
    (Default|IAAttackStarted (Variables|/Game/PlayerCharacter/BP_CharaSystems.BP_CharaSystems_C|GetAC_Weapon_User _asbp_chara_systems_2))))

(event Input|EnhancedActionEvents|EnhancedInputActionIA_Visu_Special_Right
  (params (ActionValue :type Boolean) (ElapsedSeconds :type Float%20%28double-precision%29) (TriggeredSeconds :type Float%20%28double-precision%29) (InputAction :type Input%20Action%20Object%20Reference :default "/Game/ControllerInputVisualizer/Inputs/IA_Visu_Special_Right.IA_Visu_Special_Right"))
  ;[0 0 0 0.33 50] ControllerVisualizer Debug
  ;;[0.6146 0.6146 0.6146 0.33] Special Buttons
  (:Started
    (Default|ReceiveInputVisualizationDataButton (Variables|DebugMenu|GetController%20Input%20Visualizer) true "NewEnumerator11"))
  (:Completed
    (Default|ReceiveInputVisualizationDataButton (Variables|DebugMenu|GetController%20Input%20Visualizer) false "NewEnumerator11")))

(event Input|EnhancedActionEvents|EnhancedInputActionIA_Visu_Shoulder_Left
  (params (ActionValue :type Boolean) (ElapsedSeconds :type Float%20%28double-precision%29) (TriggeredSeconds :type Float%20%28double-precision%29) (InputAction :type Input%20Action%20Object%20Reference :default "/Game/ControllerInputVisualizer/Inputs/IA_Visu_Shoulder_Left.IA_Visu_Shoulder_Left"))
  ;[0 0 0 0.33 50] ControllerVisualizer Debug
  ;;[0.9995 1 0.2907 0.33] Shoulder Buttons
  (:Started
    (Default|ReceiveInputVisualizationDataButton (Variables|DebugMenu|GetController%20Input%20Visualizer) true "NewEnumerator8"))
  (:Completed
    (Default|ReceiveInputVisualizationDataButton (Variables|DebugMenu|GetController%20Input%20Visualizer) false "NewEnumerator8")))

(event Input|EnhancedActionEvents|EnhancedInputActionIA_Visu_Shoulder_Right
  (params (ActionValue :type Boolean) (ElapsedSeconds :type Float%20%28double-precision%29) (TriggeredSeconds :type Float%20%28double-precision%29) (InputAction :type Input%20Action%20Object%20Reference :default "/Game/ControllerInputVisualizer/Inputs/IA_Visu_Shoulder_Right.IA_Visu_Shoulder_Right"))
  ;[0 0 0 0.33 50] ControllerVisualizer Debug
  ;;[0.9995 1 0.2907 0.33] Shoulder Buttons
  (:Started
    (Default|ReceiveInputVisualizationDataButton (Variables|DebugMenu|GetController%20Input%20Visualizer) true "NewEnumerator9"))
  (:Completed
    (Default|ReceiveInputVisualizationDataButton (Variables|DebugMenu|GetController%20Input%20Visualizer) false "NewEnumerator9")))

(event Input|EnhancedActionEvents|EnhancedInputActionIA_Visu_StickLeft_Press
  (params (ActionValue :type Boolean) (ElapsedSeconds :type Float%20%28double-precision%29) (TriggeredSeconds :type Float%20%28double-precision%29) (InputAction :type Input%20Action%20Object%20Reference :default "/Game/ControllerInputVisualizer/Inputs/IA_Visu_StickLeft_Press.IA_Visu_StickLeft_Press"))
  ;[0 0 0 0.33 50] ControllerVisualizer Debug
  ;;[0.1729 0.2596 1 0.33] Stick Presses
  (:Started
    (Default|ReceiveInputVisualizationDataButton (Variables|DebugMenu|GetController%20Input%20Visualizer) true "NewEnumerator12"))
  (:Completed
    (Default|ReceiveInputVisualizationDataButton (Variables|DebugMenu|GetController%20Input%20Visualizer) false "NewEnumerator12")))

(event Input|EnhancedActionEvents|EnhancedInputActionIA_Visu_StickRight_Press
  (params (ActionValue :type Boolean) (ElapsedSeconds :type Float%20%28double-precision%29) (TriggeredSeconds :type Float%20%28double-precision%29) (InputAction :type Input%20Action%20Object%20Reference :default "/Game/ControllerInputVisualizer/Inputs/IA_Visu_StickRight_Press.IA_Visu_StickRight_Press"))
  ;[0 0 0 0.33 50] ControllerVisualizer Debug
  ;;[0.1729 0.2596 1 0.33] Stick Presses
  (:Started
    (Default|ReceiveInputVisualizationDataButton (Variables|DebugMenu|GetController%20Input%20Visualizer) true "NewEnumerator13"))
  (:Completed
    (Default|ReceiveInputVisualizationDataButton (Variables|DebugMenu|GetController%20Input%20Visualizer) false "NewEnumerator13")))

(event Input|EnhancedActionEvents|EnhancedInputActionIA_Throw
  (params (ActionValue :type Boolean) (ElapsedSeconds :type Float%20%28double-precision%29) (TriggeredSeconds :type Float%20%28double-precision%29) (InputAction :type Input%20Action%20Object%20Reference :default "/Game/_GameManager/Inputs/Actions/IA_Throw.IA_Throw"))
  ;[0.15 0.15 0.15 0.5] Weapon Input Actions
  (bind _asbp_chara_systems (Utilities|Casting|CastToBP_CharaSystems (Pawn|GetControlledPawn)))
  (Default|ThrowWeapon (Variables|/Game/PlayerCharacter/BP_CharaSystems.BP_CharaSystems_C|GetAC_Weapon_User _asbp_chara_systems)))

(event Input|EnhancedActionEvents|EnhancedInputActionIA_Dash
  (params (ActionValue :type Boolean) (ElapsedSeconds :type Float%20%28double-precision%29) (TriggeredSeconds :type Float%20%28double-precision%29) (InputAction :type Input%20Action%20Object%20Reference :default "/Game/_GameManager/Inputs/Actions/IA_Dash.IA_Dash"))
  (bind _playercharacterref (Variables|Default|GetPlayerCharacterRef))
  (bind _playercharacterref_2 (Variables|Default|GetPlayerCharacterRef))
  (bind _returnvalue (Transformation|GetVelocity _playercharacterref))
  (bind _combatfeel (Variables|/Script/FTJ_Proto.Game_Character|GetCombatFeel _playercharacterref))
  (bind (_dashdistance _delaybetweentwodash) (Utilities|Struct|BreakUCombatFeel _combatfeel))
  (bind _returnvalue_2 (* _returnvalue _dashdistance))
  ;[1 0.05 1] Dash
  (if (Variables|Dash|GetbCanDash)
    (Variables|Dash|SetbCanDash false)
    (if (<= (Math|Vector|VectorLength _returnvalue) 1.0)
      ;;[0.25 0.25 0.25] No Input Dash
      (Variables|/Script/Engine.MovementComponent|SetVelocity (Variables|/Script/Engine.Character|GetCharacterMovement _playercharacterref_2) (* (Transformation|GetActorForwardVector) (* (* (Utilities|Struct|BreakUCombatFeel (Variables|/Script/FTJ_Proto.Game_Character|GetCombatFeel _playercharacterref_2)) -1.0) 5e+02)))
      (else
        (Character|LaunchCharacter _playercharacterref (Math|Vector|MakeVector (.x _returnvalue_2) (.y _returnvalue_2) 0.0) true true)))
    (Utilities|FlowControl|Delay _delaybetweentwodash)
    (Variables|Dash|SetbCanDash true)))

(event Input|EnhancedActionEvents|EnhancedInputActionIA_180Turn
  (params (ActionValue :type Boolean) (ElapsedSeconds :type Float%20%28double-precision%29) (TriggeredSeconds :type Float%20%28double-precision%29) (InputAction :type Input%20Action%20Object%20Reference :default "/Game/_GameManager/Inputs/Actions/IA_180Turn.IA_180Turn"))
  (bind _returnvalue (Pawn|GetControlRotation :!class /Script/Engine.Controller))
  (bind _180_rotation (Variables|180Rotation|Get180_Rotation))
  (bind _returnvalue_2 (* _180_rotation -1.0))
  (bind _returnvalue_3 (+ (.yaw _returnvalue) _180_rotation))
  (bind _returnvalue_4 (< (.yaw _returnvalue) 0.0))
  (bind _returnvalue_5 (Math|Rotator|MakeRotator (.roll _returnvalue) (.pitch _returnvalue) _returnvalue_3))
  (bind _returnvalue_6 (+ (.yaw _returnvalue) _returnvalue_2))
  (bind _returnvalue_7 (Math|Rotator|MakeRotator (.roll _returnvalue) (.pitch _returnvalue) _returnvalue_6))
  (bind _returnvalue_8 (select _returnvalue_4 _returnvalue_7 _returnvalue_5))
  (bind (_roll _pitch _yaw) (Math|Rotator|BreakRotator _returnvalue_8))
  ;[0.2 1 0.2] 180 Rotation
  (if (Variables|180Rotation|GetbCan180Rota)
    (Variables|180Rotation|SetbCan180Rota false)
    (Components|Movement|StopMovementImmediately (Variables|/Script/Engine.Character|GetCharacterMovement (Variables|Default|GetPlayerCharacterRef)))
    (bind _output_get (Variables|180Rotation|SetTemp%20Rota (Math|Rotator|MakeRotator _roll _pitch (select (>= _yaw 3.6e+02) (- _yaw 3.6e+02) (select (<= _yaw 0.0) (+ _yaw 3.6e+02) _yaw)))))
    (bind _rota_speed (Timeline|Timeline PlayFromStart)
      (:Update
        (Pawn|SetControlRotation (Math|Rotator|Lerp(Rotator) (Pawn|GetControlRotation :!class /Script/Engine.Controller) _output_get _rota_speed)))
      (:Finished
        (Variables|180Rotation|SetbCan180Rota true)))))

(event Input|EnhancedActionEvents|EnhancedInputActionIA_Visu_DPad_Right
  (params (ActionValue :type Boolean) (ElapsedSeconds :type Float%20%28double-precision%29) (TriggeredSeconds :type Float%20%28double-precision%29) (InputAction :type Input%20Action%20Object%20Reference :default "/Game/ControllerInputVisualizer/Inputs/IA_Visu_DPad_Right.IA_Visu_DPad_Right"))
  ;[0 0 0 0.33 50] ControllerVisualizer Debug
  ;;[0.3557 1 0.4036 0.33] DPad
  (:Started
    (Default|ReceiveInputVisualizationDataButton (Variables|DebugMenu|GetController%20Input%20Visualizer) true "NewEnumerator2"))
  (:Completed
    (Default|ReceiveInputVisualizationDataButton (Variables|DebugMenu|GetController%20Input%20Visualizer) false "NewEnumerator2")))

(event Input|EnhancedActionEvents|EnhancedInputActionIA_Visu_DPad_Top
  (params (ActionValue :type Boolean) (ElapsedSeconds :type Float%20%28double-precision%29) (TriggeredSeconds :type Float%20%28double-precision%29) (InputAction :type Input%20Action%20Object%20Reference :default "/Game/ControllerInputVisualizer/Inputs/IA_Visu_DPad_Top.IA_Visu_DPad_Top"))
  ;[0 0 0 0.33 50] ControllerVisualizer Debug
  ;;[0.3557 1 0.4036 0.33] DPad
  (:Started
    (Default|ReceiveInputVisualizationDataButton (Variables|DebugMenu|GetController%20Input%20Visualizer) true "NewEnumerator3"))
  (:Completed
    (Default|ReceiveInputVisualizationDataButton (Variables|DebugMenu|GetController%20Input%20Visualizer) false "NewEnumerator3")))

(event Input|EnhancedActionEvents|EnhancedInputActionIA_Visu_FaceButton_Bottom
  (params (ActionValue :type Boolean) (ElapsedSeconds :type Float%20%28double-precision%29) (TriggeredSeconds :type Float%20%28double-precision%29) (InputAction :type Input%20Action%20Object%20Reference :default "/Game/ControllerInputVisualizer/Inputs/IA_Visu_FaceButton_Bottom.IA_Visu_FaceButton_Bottom"))
  ;[0 0 0 0.33 50] ControllerVisualizer Debug
  ;;[1 0.5477 0.8376 0.33] Face Button
  (:Started
    (Default|ReceiveInputVisualizationDataButton (Variables|DebugMenu|GetController%20Input%20Visualizer) true "NewEnumerator4"))
  (:Completed
    (Default|ReceiveInputVisualizationDataButton (Variables|DebugMenu|GetController%20Input%20Visualizer) false "NewEnumerator4")))

(event EventBeginPlay
  (Input|AddMappingContext (PlayerController|LocalPlayerSubsystems|GetEnhancedInputLocalPlayerSubsystem) "/Game/ControllerInputVisualizer/Inputs/IMC_ControllerVisualizer.IMC_ControllerVisualizer" 1 "(bIgnoreAllPressedKeysUntilRelease=True,bForceImmediately=False,bNotifyUserSettings=False)")
  (CallFunction|GenerateWidget)
  ;[0.15 0.15 0.15 0.5] Viewport Setup
  (bind _ashud_in_game (Utilities|Casting|CastToHUD_InGame (HUD|GetHUD)))
  (Variables|Ref|SetRef%20HUD%20InGame _ashud_in_game)
  (Utilities|FlowControl|Sequence
    (:then_0
      (bind _asgi_systems (Utilities|Casting|CastToGI_Systems (Game|GetGameInstance)))
      (Variables|Ref|SetAs%20GI%20Systems _asgi_systems)
      (Default|StartTimer (Variables|Ref|GetAs%20GI%20Systems))
      (bind _returnvalue (UserInterface|CreateWidget "/Game/UI/WBP_Timer.WBP_Timer_C"))
      (Variables|Widget|SetTimerWidget _returnvalue)
      (UserInterface|Viewport|AddtoViewport (Variables|Widget|GetTimerWidget) 0))
    (:then_1
      (bind _returnvalue_2 (UserInterface|CreateWidget (Variables|Default|GetwDebugWidget)))
      (bind _output_get (Variables|Default|SetMyDebugMenu _returnvalue_2))
      (UserInterface|Viewport|AddtoViewport _output_get 0)
      (Widget|SetVisibility _output_get "Collapsed"))))

(event EventTick
  (params (DeltaSeconds :type Float%20%28single-precision%29))
  (bind _as_gi_systems (Variables|Ref|GetAs%20GI%20Systems)
    (:then
      (Default|RunTimer _as_gi_systems DeltaSeconds)
      ;[0.15 0 0 0.5] Debug
      (CallFunction|SendControllerVisualizerData))
    (:else)))

(event Input|KeyboardEvents|DebugKeyR
  (params (Key :type Key%20Structure :default "None") (ActionValue :type Input%20Action%20Value%20Structure))
  ;[1 0 1] Debug
  (:Released
    (bind _returnvalue (Game|GetCurrentLevelName true))
    (Game|OpenLevel(byName) (Utilities|String|StringToName _returnvalue))))

(event Input|KeyboardEvents|NumPadFour
  (params (Key :type Key%20Structure :default "None"))
  (:Pressed
    (bind _isa (Utilities|FlowControl|FlipFlop)
      (:A
        (Widget|SetVisibility (Variables|DebugMenu|GetDebugMenu) "Visible"))
      (:B
        (Widget|SetVisibility (Variables|DebugMenu|GetDebugMenu) "Hidden")))
    (Variables|Default|SetbShowMouseCursor _isa)
    (Utilities|Struct|SetmembersinUAimAssistFeel (Variables|/Script/FTJ_Proto.AimComponent_Base|GetAimFeel (Variables|/Script/FTJ_Proto.Game_Character|GetAimComponent (Variables|Default|GetPlayerCharacterRef))) _isa)
    (Class|PlayerController|InitializeVarswithCameraFeelStruct)))

(event Input|GamepadEvents|GamepadDPadLeft
  (params (Key :type Key%20Structure :default "None"))
  (:Pressed
    (bind _isa (Utilities|FlowControl|FlipFlop)
      (:A
        (Widget|SetVisibility (Variables|DebugMenu|GetDebugMenu) "Visible"))
      (:B
        (Widget|SetVisibility (Variables|DebugMenu|GetDebugMenu) "Hidden")))
    (Variables|Default|SetbShowMouseCursor _isa)
    (Utilities|Struct|SetmembersinUAimAssistFeel (Variables|/Script/FTJ_Proto.AimComponent_Base|GetAimFeel (Variables|/Script/FTJ_Proto.Game_Character|GetAimComponent (Variables|Default|GetPlayerCharacterRef))) _isa)
    (Class|PlayerController|InitializeVarswithCameraFeelStruct)))

(event Input|GamepadEvents|GamepadDPadDown
  (params (Key :type Key%20Structure :default "None"))
  ;[1 0 1] Debug
  (:Released
    (bind _isa (Utilities|FlowControl|FlipFlop)
      (:A
        _)
      (:B
        _))
    (Utilities|Struct|SetmembersinUCameraFeel (Variables|Default|GetCameraFeel) _isa)))

(fn ConstructionScript)

(fn DecreaseSound
  (bind _ref_hud_ingame (Variables|Ref|GetRef%20HUD%20InGame))
  (bind _ref_pausemenu (Variables|/Game/UI/HUD_InGame.HUD_InGame_C|GetRef%20PauseMenu _ref_hud_ingame))
  (bind _wbp_settingscontent (Variables|/Game/UI/PauseMenu/WBP_PauseMenu.WBP_PauseMenu_C|GetWBP_SettingsContent _ref_pausemenu))
  ;[0.2089 0.8021 0.3296 0.5] Sound Less Button
  (bind _output_get (Variables|/Game/UI/MainMenu/WBP_SettingsContent.WBP_SettingsContent_C|SetSoundValue _wbp_settingscontent (Math|Float|Clamp(Float) (- (Variables|/Game/UI/MainMenu/WBP_SettingsContent.WBP_SettingsContent_C|GetSoundValue _wbp_settingscontent) 0.1))))
  (Variables|/Game/UI/MainMenu/WBP_SettingsContent.WBP_SettingsContent_C|SetSoundValue_Text _wbp_settingscontent (Utilities|Text|ToText(Float) (* _output_get 1e+02) "HalfToEven")))

(fn IncreaseSound
  (bind _ref_hud_ingame (Variables|Ref|GetRef%20HUD%20InGame))
  (bind _ref_pausemenu (Variables|/Game/UI/HUD_InGame.HUD_InGame_C|GetRef%20PauseMenu _ref_hud_ingame))
  (bind _wbp_settingscontent (Variables|/Game/UI/PauseMenu/WBP_PauseMenu.WBP_PauseMenu_C|GetWBP_SettingsContent _ref_pausemenu))
  ;[0.2089 0.8021 0.3296 0.5] Sound More Button
  (bind _output_get (Variables|/Game/UI/MainMenu/WBP_SettingsContent.WBP_SettingsContent_C|SetSoundValue _wbp_settingscontent (Math|Float|Clamp(Float) (+ (Variables|/Game/UI/MainMenu/WBP_SettingsContent.WBP_SettingsContent_C|GetSoundValue _wbp_settingscontent) 0.1))))
  (Variables|/Game/UI/MainMenu/WBP_SettingsContent.WBP_SettingsContent_C|SetSoundValue_Text _wbp_settingscontent (Utilities|Text|ToText(Float) (* _output_get 1e+02) "HalfToEven")))

(fn DecreaseXSens
  (bind _ref_hud_ingame (Variables|Ref|GetRef%20HUD%20InGame))
  (bind _ref_pausemenu (Variables|/Game/UI/HUD_InGame.HUD_InGame_C|GetRef%20PauseMenu _ref_hud_ingame))
  (bind _wbp_settingscontent (Variables|/Game/UI/PauseMenu/WBP_PauseMenu.WBP_PauseMenu_C|GetWBP_SettingsContent _ref_pausemenu))
  ;[0.3673 0.8021 0.2882 0.5] Horizontal Sensitivity Less Button
  (bind _output_get (Variables|/Game/UI/MainMenu/WBP_SettingsContent.WBP_SettingsContent_C|SetXSensiValue _wbp_settingscontent (Math|Float|Clamp(Float) (- (Variables|/Game/UI/MainMenu/WBP_SettingsContent.WBP_SettingsContent_C|GetXSensiValue _wbp_settingscontent) 0.1))))
  (Variables|/Game/UI/MainMenu/WBP_SettingsContent.WBP_SettingsContent_C|SetXSensiValue_Text _wbp_settingscontent (Utilities|Text|ToText(Float) (* _output_get 1e+02) "HalfToEven")))

(fn IncreaseXSens
  (bind _ref_hud_ingame (Variables|Ref|GetRef%20HUD%20InGame))
  (bind _ref_pausemenu (Variables|/Game/UI/HUD_InGame.HUD_InGame_C|GetRef%20PauseMenu _ref_hud_ingame))
  (bind _wbp_settingscontent (Variables|/Game/UI/PauseMenu/WBP_PauseMenu.WBP_PauseMenu_C|GetWBP_SettingsContent _ref_pausemenu))
  ;[0.3673 0.8021 0.2882 0.5] Horizontal Sensitivity More Button
  (bind _output_get (Variables|/Game/UI/MainMenu/WBP_SettingsContent.WBP_SettingsContent_C|SetXSensiValue _wbp_settingscontent (Math|Float|Clamp(Float) (+ (Variables|/Game/UI/MainMenu/WBP_SettingsContent.WBP_SettingsContent_C|GetXSensiValue _wbp_settingscontent) 0.1))))
  (Variables|/Game/UI/MainMenu/WBP_SettingsContent.WBP_SettingsContent_C|SetXSensiValue_Text _wbp_settingscontent (Utilities|Text|ToText(Float) (* _output_get 1e+02) "HalfToEven")))

(fn DecreaseYSens
  (bind _ref_hud_ingame (Variables|Ref|GetRef%20HUD%20InGame))
  (bind _ref_pausemenu (Variables|/Game/UI/HUD_InGame.HUD_InGame_C|GetRef%20PauseMenu _ref_hud_ingame))
  (bind _wbp_settingscontent (Variables|/Game/UI/PauseMenu/WBP_PauseMenu.WBP_PauseMenu_C|GetWBP_SettingsContent _ref_pausemenu))
  ;[0.3381 0.5625 0.1934 0.5] Vertical Sensitivity Less Button
  (bind _output_get (Variables|/Game/UI/MainMenu/WBP_SettingsContent.WBP_SettingsContent_C|SetYSensiValue _wbp_settingscontent (Math|Float|Clamp(Float) (- (Variables|/Game/UI/MainMenu/WBP_SettingsContent.WBP_SettingsContent_C|GetYSensiValue _wbp_settingscontent) 0.1))))
  (Variables|/Game/UI/MainMenu/WBP_SettingsContent.WBP_SettingsContent_C|SetYSensiValue_Text _wbp_settingscontent (Utilities|Text|ToText(Float) (* _output_get 1e+02) "HalfToEven")))

(fn IncreaseYsens
  (bind _ref_hud_ingame (Variables|Ref|GetRef%20HUD%20InGame))
  (bind _ref_pausemenu (Variables|/Game/UI/HUD_InGame.HUD_InGame_C|GetRef%20PauseMenu _ref_hud_ingame))
  (bind _wbp_settingscontent (Variables|/Game/UI/PauseMenu/WBP_PauseMenu.WBP_PauseMenu_C|GetWBP_SettingsContent _ref_pausemenu))
  ;[0.3542 0.5625 0.2197 0.5] Horizontal Sensitivity More Button
  (bind _output_get (Variables|/Game/UI/MainMenu/WBP_SettingsContent.WBP_SettingsContent_C|SetYSensiValue _wbp_settingscontent (Math|Float|Clamp(Float) (+ (Variables|/Game/UI/MainMenu/WBP_SettingsContent.WBP_SettingsContent_C|GetYSensiValue _wbp_settingscontent) 0.1))))
  (Variables|/Game/UI/MainMenu/WBP_SettingsContent.WBP_SettingsContent_C|SetYSensiValue_Text _wbp_settingscontent (Utilities|Text|ToText(Float) (* _output_get 1e+02) "HalfToEven")))

(fn GenerateWidget
  (Utilities|FlowControl|Sequence
    (:then_0
      ;[0.15 0.15 0.15 0.5] Debug Menu
      (bind _returnvalue (UserInterface|CreateWidget "/Game/IA_System/Viewport/WBP_DebugMenu.WBP_DebugMenu_C"))
      (bind _output_get (Variables|DebugMenu|SetDebugMenu _returnvalue))
      (UserInterface|Viewport|AddtoViewport _output_get 0)
      (Widget|SetVisibility _output_get "Hidden"))
    (:then_1
      ;[0.15 0.15 0.15 0.5] Debug Parameters
      (bind _returnvalue_2 (UserInterface|CreateWidget "/Game/IA_System/Viewport/WBP_DebugParameters.WBP_DebugParameters_C"))
      (bind _output_get_2 (Variables|DebugMenu|SetDebugParameter _returnvalue_2))
      (UserInterface|Viewport|AddtoViewport _output_get_2 0)
      (Widget|SetVisibility _output_get_2 "Hidden"))
    (:then_2
      ;[0.15 0.15 0.15 0.5] Debug Player
      (bind _returnvalue_3 (UserInterface|CreateWidget "/Game/IA_System/Viewport/WBP_DebugPlayer.WBP_DebugPlayer_C"))
      (bind _output_get_3 (Variables|DebugMenu|SetDebugPlayer _returnvalue_3))
      (UserInterface|Viewport|AddtoViewport _output_get_3 0)
      (Widget|SetVisibility _output_get_3 "Hidden"))
    (:then_3
      ;[0.15 0.15 0.15 0.5] Debug Level
      (bind _returnvalue_4 (UserInterface|CreateWidget "/Game/IA_System/Viewport/WBP_DebugLevel.WBP_DebugLevel_C"))
      (bind _output_get_4 (Variables|DebugMenu|SetDebugLevel _returnvalue_4))
      (UserInterface|Viewport|AddtoViewport _output_get_4 0)
      (Widget|SetVisibility _output_get_4 "Hidden"))
    (:then_4
      ;[0.15 0.15 0.15 0.5] Debug 3C
      (bind _returnvalue_5 (UserInterface|CreateWidget "/Game/IA_System/Viewport/WBP_Debug3CParam.WBP_Debug3CParam_C"))
      (bind _output_get_5 (Variables|DebugMenu|SetDebug3C _returnvalue_5))
      (UserInterface|Viewport|AddtoViewport _output_get_5 0)
      (Widget|SetVisibility _output_get_5 "Hidden"))
    (:then_5
      ;[0.15 0.15 0.15 0.5] Debug EnemyAI
      (bind _returnvalue_6 (UserInterface|CreateWidget "/Game/IA_System/Viewport/WBP_DebugEnemyAI.WBP_DebugEnemyAI_C"))
      (bind _output_get_6 (Variables|DebugMenu|SetDebugEnemyAI _returnvalue_6))
      (UserInterface|Viewport|AddtoViewport _output_get_6 0)
      (Widget|SetVisibility _output_get_6 "Hidden"))
    (:then_6
      ;[0.15 0.15 0.15 0.5] Debug Weapon
      (bind _returnvalue_7 (UserInterface|CreateWidget "/Game/IA_System/Viewport/WBP_DebugWeapon.WBP_DebugWeapon_C"))
      (bind _output_get_7 (Variables|DebugMenu|SetDebugWeapon _returnvalue_7))
      (UserInterface|Viewport|AddtoViewport _output_get_7 0)
      (Widget|SetVisibility _output_get_7 "Hidden"))
    (:then_7
      ;[0.15 0.15 0.15 0.5] Debug Input
      (bind _returnvalue_8 (UserInterface|CreateWidget "/Game/ControllerInputVisualizer/WBP_ControllerInputsVisualizer.WBP_ControllerInputsVisualizer_C"))
      (bind _output_get_8 (Variables|DebugMenu|SetController%20Input%20Visualizer _returnvalue_8))
      (UserInterface|Viewport|AddtoViewport _output_get_8 0)
      (Widget|SetVisibility _output_get_8 "Hidden"))
    (:then_8
      ;[0.15 0.15 0.15 0.5] Debug Aim
      (bind _returnvalue_9 (UserInterface|CreateWidget "/Game/IA_System/Viewport/WBP_DebugAim.WBP_DebugAim_C"))
      (bind _output_get_9 (Variables|Ref|SetDebugAim _returnvalue_9))
      (UserInterface|Viewport|AddtoViewport _output_get_9 0)
      (Widget|SetVisibility _output_get_9 "Hidden"))))