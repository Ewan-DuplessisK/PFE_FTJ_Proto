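; Enemy pooling manager that pre-spawns enemies for the level's wave managers.
; InitializePoolSize scans every BP_WaveManager's waves and spawn groups, mapping each enemy class to the largest group count gathered so far plus a buffer.
; A tick later, PopulatePool spawns them at an offset pool position, marks them unused, reports misplaced spawns and registers them by class.
; PooledActorRequest simply passes through to the parent implementation.
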(event `self.InitializePoolSize`
  (bind _outactors (`GameplayStatics.GetAllActorsOfClass` "/Game/_GameManager/WaveManager/BP_WaveManager.BP_WaveManager_C"))
  (bind _output_get (set `self.Wave Managers` _outactors))
  (for _array_element _output_get
    (for _array_element_2 (`/Game/_GameManager/WaveManager/BP_WaveManager.Waves` _array_element)
      (for _array_element_3 (`/Game/_GameManager/WaveManager/PDA_Wave.Spawn Groups` _array_element_2)
        (bind (_enemyclass _enemycount) (break `/Game/_GameManager/WaveManager/Data/ST_Spawn_Group` _array_element_3))
        (`KismetArrayLibrary.Array_Add` (`self.Temp Amount`) _enemycount)
        (`KismetArrayLibrary.Array_AddUnique` (`self.TempClassesArray`) _enemyclass))
      (for _array_element_4 (`self.TempClassesArray`)
        (`BlueprintMapLibrary.Map_Add` (`self.PoolSizeMap`) _array_element_4 (+ (`.MaxValue` (`KismetMathLibrary.MaxOfIntArray` (`self.Temp Amount`))) (`self.Enemy Amount Buffer`))))))
  (`KismetSystemLibrary.DelayUntilNextTick`)
  (`KismetArrayLibrary.Array_Clear` (`self.TempClassesArray`))
  (`self.PopulatePool`))

(event `self.PopulatePool`
  (bind _temppoolarray (`self.TempPoolArray`))
  (bind _tempclassesarray (`self.TempClassesArray`))
  (bind _returnvalue (+ (`self.PoolSpawnPosition`) (`self.Enemy Position Offset`)))
  (bind (_keypin _valuepin) (`|MapForEach` (`self.PoolSizeMap`))
    (:`then`
      (set `self.Is pool Populated` false)
      (`KismetArrayLibrary.Array_AddUnique` (`self.TempClassesArray`) _keypin)
      (for _ (range (+ _valuepin 1))
        (bind _returnvalue_2 (`|SpawnActorFromClass` _keypin (`KismetMathLibrary.MakeTransform` _returnvalue) "AlwaysSpawn" "MultiplyWithRoot" null null))
        (`Enemy_Base.SetInUse` _returnvalue_2 false)
        (`KismetArrayLibrary.Array_AddUnique` (`self.TempPoolArray`) _returnvalue_2)
        (if (not (== (`self.K2_GetActorLocation` _returnvalue_2) _returnvalue :`ErrorTolerance` 10.0))
          (`KismetSystemLibrary.PrintString` (`KismetStringLibrary.Concat_StrStr` "Spawn FAILED | " (`KismetSystemLibrary.GetDisplayName` _returnvalue_2)) true true (struct :`R` 1.0 :`G` 0.272152 :`A` 1.0) 5.0)))
      (`self.AddTempToPool` _tempclassesarray _temppoolarray)
      (`KismetArrayLibrary.Array_Clear` _tempclassesarray)
      (`KismetArrayLibrary.Array_Clear` _temppoolarray))
    (:`CompletedPin`
      (set `self.Is pool Populated` true))))

(fn `PooledActorRequest`
  (params (Class :type "Enemy_Base Class Reference") (Num :type Integer))
  (returns (ReturnValue :type "PoolRequestResponce Structure"))
  (bind _returnvalue (`parent.PooledActorRequest` Class Num))
  (if (`.Success` (break `PoolRequestResponce` _returnvalue))
    _
    (else
      _))
  (return _returnvalue))

(fn `UserConstructionScript`)