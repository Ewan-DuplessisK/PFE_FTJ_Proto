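; BP_Wave_Starter is a trigger volume that launches an enemy or gameplay wave when the player enters it.
; On BeginPlay it caches the player, the pooling manager and, if not already set, the wave manager.
; The first player overlap polls until the pool is populated, then calls LaunchWave with its WaveIndex and destroys itself.
; The construction script sizes the box from BoxSize.
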(event `self.ReceiveBeginPlay`
  (`KismetSystemLibrary.Delay` 0.2)
  (bind _outactors (`GameplayStatics.GetAllActorsOfClass` "/Game/_GameManager/Pooling_Manager/BP_Pooling_Manager.BP_Pooling_Manager_C"))
  (set `self.Pooling Manager Ref` (`|GetArrayItem` _outactors))
  (bind _asbp_player (cast `/Game/Characters/Player/Blueprints/BP_Player` (`GameplayStatics.GetPlayerCharacter` 0)))
  (set `self.Player Ref` _asbp_player)
  (`self.Wave Manager Ref`
    (:`then`)
    (:`else`
      (bind _outactors_2 (`GameplayStatics.GetAllActorsOfClass` "/Game/_GameManager/WaveManager/BP_WaveManager.BP_WaveManager_C"))
      (set `self.Wave Manager Ref` (`|GetArrayItem` _outactors_2)))))

(event `self.Box.OnComponentBeginOverlap`
  (params (OverlappedComponent :type "PrimitiveComponent Object Reference") (OtherActor :type "Actor Object Reference") (OtherComp :type "PrimitiveComponent Object Reference") (OtherBodyIndex :type Integer) (bFromSweep :type Boolean) (SweepResult :type "HitResult Structure (by ref)"))
  (if (== (`self.Player Ref`) OtherActor)
    (`/Engine/EditorBlueprintResources/StandardMacros.DoOnce` false
      (:`Completed`
        (bind _pooling_manager_ref (`self.Pooling Manager Ref`)
          (:`then`
            (if (`/Game/_GameManager/Pooling_Manager/BP_Pooling_Manager.Is pool Populated` _pooling_manager_ref) :!label _label
              (bind _wave_manager_ref (`self.Wave Manager Ref`)
                (:`then`
                  (`WaveManager.LaunchWave` _wave_manager_ref (`self.Wave Index`))
                  (`KismetSystemLibrary.DelayUntilNextTick`)
                  (`self.K2_DestroyActor`))
                (:`else`))
              (else
                (`KismetSystemLibrary.Delay` 0.3)
                (goto _label))))
          (:`else`))))))

(fn `UserConstructionScript`
  (`BoxComponent.SetBoxExtent` (`self.Box`) (`self.Box_Size`) true))