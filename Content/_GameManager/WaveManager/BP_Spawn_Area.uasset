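; Spawn area actor, filed under the wave manager, that supplies random spawn points around its SpawnRange sphere.
; The construction script applies SpawnRangeRadius to the sphere, so the area can be resized in the editor.
; GetRandomPointsInArea returns one point offset by random polar terms at a fixed height above the center.
; X and Y roll radius and angle independently, so points can land outside the circle.
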(fn `Get Random Points In Area`
  (returns (`Spawn Point` :type "Vector Structure"))
  (bind _spawn_range (`self.Spawn Range`))
  (bind _returnvalue (`KismetMathLibrary.DegreesToRadians` (`KismetMathLibrary.RandomFloatInRange` 0.0 360.0)))
  (bind (_returnvalue_x _returnvalue_y _returnvalue_z) (`KismetMathLibrary.BreakVector` (`SceneComponent.K2_GetComponentLocation` _spawn_range)))
  (bind _returnvalue_2 (`KismetMathLibrary.RandomFloatInRange` 0.0 (`SphereComponent.GetScaledSphereRadius` _spawn_range)))
  (return (`KismetMathLibrary.MakeVector` (+ (* _returnvalue_2 (`KismetMathLibrary.Cos` _returnvalue)) _returnvalue_x) (+ (* (`KismetMathLibrary.Sin` _returnvalue) _returnvalue_2) _returnvalue_y) (+ _returnvalue_z 90.0))))

(fn `UserConstructionScript`
  ;[0 0.15 0.15] Make it Modifiable in Editor
  (`SphereComponent.SetSphereRadius` (`self.Spawn Range`) (`self.Spawn Range Radius`) true))