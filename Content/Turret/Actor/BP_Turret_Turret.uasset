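; Turret actor that layers VFX and Wwise audio onto show, hide, pre-shoot, shoot, hit and destroyed events.
; Audio runs through a turret audio component and an Ak component toggled around several posts.
; Hits drive an emissive flash through a timeline on a dynamic material.
; Destruction notifies any owning arena, awards score, disables the warning effect and spawns Niagara decal and breakup effects, feeding the latter breakable-prop data.
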(event `self.ReceiveBeginPlay`
  (`ActorComponent.Deactivate` (`self.Ak_Turret`))
  (bind _returnvalue (`PrimitiveComponent.CreateDynamicMaterialInstance` (`self.Mesh`) 0 null "None"))
  (set `self.Dynamic Material` _returnvalue))

(event `self.OnTurretShow`
  (bind _ak_turret (`self.Ak_Turret`))
  (`ActorComponent.Activate` (`self.ShowEffect`) false)
  (`ActorComponent.Activate` _ak_turret false)
  (`AkGameObject.PostAkEvent` :`self` _ak_turret :`AkEvent` "/Game/WwiseAudio/Events/Default_Work_Unit/ENEMIES/TURRET/Turret_Appear.Turret_Appear")
  (`ActorComponent.Deactivate` _ak_turret))

(event `self.OnTurretPreShoot`
  (if (not (`self.WarningDisabled`))
    (`ActorComponent.Activate` (`self.WarningFX`) true)
    ;[0.7708 0.1766 0.7483 0.5] Audio Charge
    (`/Game/Audio/AC_Turret_Audio.AudioCharge` (`self.AC_Turret_Audio`))))

(event `self.OnTurretShoot`
  (`ActorComponent.Activate` (`self.ShootEffect`) false)
  (`ActorComponent.Activate` (`self.ShootMuzzleFX`) true)
  (`ActorComponent.Activate` (`self.Ak_Turret`) true)
  ;[0.7708 0.1766 0.7483 0.5] Audio Shoot
  (`/Game/Audio/AC_Turret_Audio.AudioShoot` (`self.AC_Turret_Audio`) (`self.Ak_Turret`))
  (`ActorComponent.Deactivate` (`self.Ak_Turret`)))

(event `self.OnTurretDestroyed`
  (bind _mesh (`self.Mesh`))
  (bind _arenaref (`self.ArenaRef`))
  (bind _returnvalue (`SceneComponent.K2_GetComponentRotation` _mesh))
  (bind _returnvalue_2 (`SceneComponent.K2_GetComponentLocation` _mesh))
  (`/Engine/EditorBlueprintResources/StandardMacros.IsValid` _arenaref ; If Turret isn't in an arena, ignore the BPI Event
    (:`Is Valid`
      (message `/Game/BPs/BPI_Arena.RobotKilled` _arenaref) ; Called in BP_Arena when needed
    )
    (:`Is Not Valid`
      _))
  (`FTJ_ScoringSystem_Score.IncreaseWithText` (subsystem `/Game/CppSystems/ScoringSystem/Public/Blueprint/BP_ScoringSystem_Score`) (`KismetMathLibrary.Conv_IntToDouble` 100) 0.5 false (`|FormatText` "Broke Turret"))
  (`ActorComponent.Activate` (`self.Ak_Turret`) true)
  ;[0.7708 0.1766 0.7483 0.5] Audio Destroyed
  (`/Game/Audio/AC_Turret_Audio.AudioDestroyed` (`self.AC_Turret_Audio`) (`self.Ak_Turret`))
  (`ActorComponent.Deactivate` (`self.Ak_Turret`))
  (`ActorComponent.Deactivate` (`self.WarningFX`))
  (set `self.WarningDisabled` true)
  (`NiagaraFunctionLibrary.SpawnSystemAtLocation` (`self.VFX BOOM Decal`) _returnvalue_2 _returnvalue)
  (bind _returnvalue_3 (`NiagaraFunctionLibrary.SpawnSystemAtLocation` (`self.VFX Props Break`) _returnvalue_2 _returnvalue))
  (bind _output_get (set `self.PropsBreakSystem` _returnvalue_3))
  (`/Engine/EditorBlueprintResources/StandardMacros.IsValid` _output_get
    (:`Is Valid`
      (`NiagaraComponent.SetVariableInt` _output_get "SmokeCount" 0)
      (`/Game/VFX/Blueprint/BPFL_FX_DataTable_To_BreakableProp.SendBreakablePropDataToNiagara` (`self.DT_Positions`) _output_get (`self.Array Mesh Renderer`) (stale _fx_material) :!label _label))
    (:`Is Not Valid`
      (bind _fx_material (`self.FX_Material`)
        (:`then`
          (goto _label))
        (:`else`
          _))))
  (bind _destructioneffect (`self.DestructionEffect`)
    (:`then`
      (`ActorComponent.Activate` _destructioneffect false))
    (:`else`)))

(event `/Game/BPs/BPI_Arena.Arena`
  (params (RefArena :type "/Game/BPs/Arena/BP_Arena Object Reference"))
  ;[0 0.5158 1 0.5] ARENA REFERENCE
  (set `self.ArenaRef` RefArena))

(event `self.OnTurretHit`
  ;[0.7708 0.1766 0.7483 0.5] Audio damaged
  (`/Game/Audio/AC_Turret_Audio.AudioTakeDamage` (`self.AC_Turret_Audio`))
  (`ActorComponent.Activate` (`self.HitEffect`) false)
  (bind (_direction _newtrack_0) (`Timeline|Timeline` :!via `PlayFromStart`)
    (:`Update`
      (`MaterialInstanceDynamic.SetScalarParameterValue` (`self.Dynamic Material`) "Emissive_Hit" _newtrack_0))))

(event `self.OnTurretHide`
  (bind _ak_turret (`self.Ak_Turret`))
  (`ActorComponent.Activate` _ak_turret false)
  (`AkGameObject.PostAkEvent` :`self` _ak_turret :`AkEvent` "/Game/WwiseAudio/Events/Default_Work_Unit/ENEMIES/TURRET/Turret_Disappear.Turret_Disappear")
  (`ActorComponent.Deactivate` _ak_turret))

(fn `UserConstructionScript`
  (`parent.UserConstructionScript`))