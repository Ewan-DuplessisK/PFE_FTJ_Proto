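; BP_Exit is a breakable exit sign with a pulsing spotlight.
; A self-retriggering timeline with FlipFlop ping-pongs the light intensity while intact.
; The first hit from a Heavy, Medium or Light tagged actor breaks it, awarding score, playing Wwise audio, spawning VFX and swapping the mesh.
; Breaking stops the pulse and starts a second ping-pong timeline that tilts the sign and drives a dimmer light.
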(event `self.ReceiveBeginPlay`
  ; Defautl behaviour
  (`self.Event Light anim`))

(event `Event Light anim`
  ; Defautl behaviour
  ;; Light Anim
  (if (not (`self.Is Broken`))
    (`/Engine/EditorBlueprintResources/StandardMacros.FlipFlop`
      (:`A`
        (bind (_direction _alpha) (`Timeline|Anim` :!label _label)
          (:`Update`
            (`LightComponent.SetIntensity` (`self.SpotLight`) (`KismetMathLibrary.Lerp` 0.0 160.0 _alpha)))
          (:`Finished`
            (`self.Event Light anim`))))
      (:`B`
        (goto _label :!via `Reverse`)))))

(event `Force Stop Anim`
  ; Defautl behaviour
  ;; Light Anim
  (goto _label :!via `Stop`))

(event `HitInterface.GetHit`
  (params (Damage :type "Float (single-precision)") (HitStunDuration :type "Float (single-precision)") (KnockbackVector :type "Vector Structure") (InvincibilityTime :type "Float (single-precision)") (SourceActor :type "Actor Object Reference"))
  ; Hit Event
  (if (or (`self.ActorHasTag` SourceActor "Heavy") (`self.ActorHasTag` SourceActor "Medium") (`self.ActorHasTag` SourceActor "Light"))
    (if (not (`self.Is Broken`))
      (set `self.Is Broken` true)
      (`/Engine/EditorBlueprintResources/StandardMacros.DoOnce` false
        (:`Completed`
          (`self.Destroyed`)
          (`FTJ_ScoringSystem_Score.IncreaseWithText` (subsystem `/Game/CppSystems/ScoringSystem/Public/Blueprint/BP_ScoringSystem_Score`) (`KismetMathLibrary.Conv_IntToDouble` 10) 0.2 false (`|FormatText` "Broke Exit"))
          (`AkGameObject.PostAkEvent` :`self` (`self.Ak_Security`) :`AkEvent` "/Game/WwiseAudio/Events/Default_Work_Unit/SFX/SFX_GLOBAL/SFX_DESTRUCTION/SFX_Metal_Destruction.SFX_Metal_Destruction")
          (`StaticMeshComponent.SetStaticMesh` (`self.Sm_Exit`) "/Game/Environment/Office/Meshes/WallAssets/SM_Sign_Exit_01_Broken.SM_Sign_Exit_01_Broken"))))))

(event `Destroyed`
  (bind _vfx_spawn (`self.VFX Spawn`))
  (bind _vfx_spawn_2 (`self.VFX Spawn`))
  ;[0 1 1 0.5] Sound When Hit
  (`AkGameObject.PostAkEvent` :`self` (`self.Ak_Security`) :`AkEvent` "/Game/WwiseAudio/Events/Default_Work_Unit/SFX/SFX_GLOBAL/SFX_DESTRUCTION/SFX_Metal_Destruction.SFX_Metal_Destruction")
  ;[0 1 1] VFX
  (`NiagaraFunctionLibrary.SpawnSystemAtLocation` (`self.VFX When Hit`) (`SceneComponent.K2_GetComponentLocation` _vfx_spawn_2) (`SceneComponent.K2_GetComponentRotation` _vfx_spawn_2) (/ (`self.GetActorScale3D`) 12.0))
  (`NiagaraFunctionLibrary.SpawnSystemAtLocation` "/Game/VFX/Niagara/Sparks/NS_Burst_Spark_Loop.NS_Burst_Spark_Loop" (`SceneComponent.K2_GetComponentLocation` _vfx_spawn) (`SceneComponent.K2_GetComponentRotation` _vfx_spawn))
  (`self.Force Stop Anim`)
  (`KismetSystemLibrary.DelayUntilNextTick`)
  (`self.Anim Destroyed Event`))

(event `Anim Destroyed Event`
  ;[0 1 1] Anim
  (`/Engine/EditorBlueprintResources/StandardMacros.FlipFlop`
    (:`A`
      (bind (_direction _rotation _light) (`Timeline|Anim Destroyed` :!via `PlayFromStart` :!label _label_2)
        (:`Update`
          (`SceneComponent.K2_SetRelativeRotation` (`self.Sm_Exit`) (`KismetMathLibrary.RLerp` (struct) (struct :`Pitch` -45.0) _rotation) false false)
          (`LightComponent.SetIntensity` (`self.SpotLight`) (`KismetMathLibrary.Lerp` 0.0 30.0 _light)))
        (:`Finished`
          (`self.Anim Destroyed Event`))))
    (:`B`
      (goto _label_2 :!via `ReverseFromEnd`))))

(fn `Update Life`)

(fn `UserConstructionScript`)