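; A door actor that can be launched as a physics object and knock dummies and other doors into motion.
; Its Launched event flags it as launched, turns on mesh physics and applies the force as a velocity-change impulse.
; While launched, overlaps with unlaunched dummies or doors call their Launched event with a scaled-down copy of its velocity, then slow the door, allowing chain reactions.
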(event `Launched`
  (params (Force :type "Vector Structure"))
  (bind _doormesh (`self.DoorMesh`))
  (set `self.isLaunched` true)
  (`PrimitiveComponent.SetSimulatePhysics` _doormesh true)
  (`PrimitiveComponent.AddImpulse` _doormesh Force "None" true))

(event `self.OverlapPhysics.OnComponentBeginOverlap`
  (params (OverlappedComponent :type "PrimitiveComponent Object Reference") (OtherActor :type "Actor Object Reference") (OtherComp :type "PrimitiveComponent Object Reference") (OtherBodyIndex :type Integer) (bFromSweep :type Boolean) (SweepResult :type "HitResult Structure (by ref)"))
  (bind _returnvalue (`self.GetVelocity`))
  (bind _returnvalue_2 (* _returnvalue 0.8))
  ; Physics enabled objects collisions
  ; If the object is moving and not detecting itself
  (if (`self.isLaunched`)
    (if (!= OtherActor self)
      ; Colliding with an enemy
      (bind _asbp_dummy (cast `/Game/Systems_Integration/BP_Dummy` OtherActor)
        (:`then`
          (if (not (`/Game/Systems_Integration/BP_Dummy.isLaunched` _asbp_dummy))
            (`/Game/Systems_Integration/BP_Dummy.Launched` _asbp_dummy _returnvalue_2)
            ; Reduce actor speed after transmitting force
            (`PrimitiveComponent.SetAllPhysicsLinearVelocity` (`self.DoorMesh`) (* _returnvalue 0.5) false :!label _label)))
        (:`CastFailed`
          ; Colliding with a door
          (bind _asbp_kickable_door (cast `/Game/Systems_Integration/BP_KickableDoor` OtherActor))
          (if (not (`/Game/Systems_Integration/BP_KickableDoor.isLaunched` _asbp_kickable_door))
            (`self.Launched` _asbp_kickable_door _returnvalue_2)
            (goto _label)))))))

(fn `UserConstructionScript`)