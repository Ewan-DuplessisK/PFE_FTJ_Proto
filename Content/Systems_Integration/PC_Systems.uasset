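; First-person player controller that maps Enhanced Input to movement, look and BP_CharaSystems actions: fire, throw and kick.
; BeginPlay applies pitch limits, FOV and tilt settings from a camera-feel struct.
; Move and look Y input accumulate camera roll, which Tick clamps and decays over the control rotation.
; Interact temporarily messages the first overlapping actor, and D-pad down toggles the vertical look inversion flag.
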(event `self.ReceiveTick`
  (params (DeltaSeconds :type "Float (single-precision)"))
  (`self.Head Tilt` DeltaSeconds))

(event `self.ReceiveBeginPlay`
  (bind _returnvalue (`GameplayStatics.GetPlayerCameraManager` 0))
  (bind ((`FOVTarget_54_748119344E827DE77056228505A02BA1` _fovtarget) (`FOVInterpSpeed_58_A7D04A59425E5006DF4BF8859724B2D1` _fovinterpspeed) (`FOVSwitchSpeed_56_7A1CC80441B1BE04A27391862602A262` _fovswitchspeed) (`TitRecoverySpeed_41_B0EAD35C44C2B8DC530A72B308D0893B` _titrecoveryspeed) (`TiltClamp_51_1A1E3FEB4354BFAA12EEA98BBA7D8D3B` _tiltclamp) (`MaxTilt_40_48D4C2F74564D063DEBC7ABA5BB316FE` _maxtilt)) (break `/Game/DataAssets/Data_3C/S_FPSCameraFeel` (`self.Camera Feel Structure Ref`)))
  (bind ((`FOVTarget_54_748119344E827DE77056228505A02BA1` _fovtarget_2) (`FOVInterpSpeed_58_A7D04A59425E5006DF4BF8859724B2D1` _fovinterpspeed_2) (`FOVSwitchSpeed_56_7A1CC80441B1BE04A27391862602A262` _fovswitchspeed_2) (`InvertCam_28_90E7021E4B9690B321581A938CF1278B` _invertcam) (`HorizontalCamSpeed_48_BCC115954F2DC5CE029858B577AE2287` _horizontalcamspeed) (`VerticalCamSpeed_47_BDA38A3643667DFE78A0778FF1A6268E` _verticalcamspeed) (`ViewPitchMin_34_1401A7A94B9759766D93A8BF0EDF6337` _viewpitchmin) (`ViewPitchMax_35_D2DEF8154FD9D617C127778BFC7FEC8E` _viewpitchmax)) (break `/Game/DataAssets/Data_3C/S_FPSCameraFeel` (`self.Camera Feel Structure Ref`)))
  (bind _asbp_chara_systems (cast `/Game/Systems_Integration/BP_CharaSystems` (`GameplayStatics.GetPlayerPawn` 0) :!pure true))
  ;[0.5 0.5 1] Add IMC
  (`EnhancedInputSubsystemInterface.AddMappingContext` (subsystem `EnhancedInputLocalPlayerSubsystem`) "/Game/Systems_Integration/Inputs/IMC_Systems.IMC_Systems" 0 (struct))
  ;[0.005 0.005 0.005] Clamp Camera
  (set `PlayerCameraManager.ViewPitchMin` _viewpitchmin _returnvalue)
  (set `PlayerCameraManager.ViewPitchMax` _viewpitchmax _returnvalue)
  ;[0.25 0.25 0.25] Camera Settings from Struct ("S_FPSCameraFeel")
  (`CameraComponent.SetFieldOfView` (`/Game/Systems_Integration/BP_CharaSystems.Camera` _asbp_chara_systems) (`.FOV_5_3BBB83674770A4A3F1B4E99A3A546ABD` (break `/Game/DataAssets/Data_3C/S_FPSCameraFeel` (`self.Camera Feel Structure Ref`))))
  (set `self.Player Ref` _asbp_chara_systems)
  (set `self.Tilt Recover Speed` _titrecoveryspeed)
  (set `self.Max Tilt` _maxtilt))

(event `EnhancedInput|/Game/Systems_Integration/Inputs/Actions/IA_Move`
  (params (ActionValue :type "Vector2D Structure") (ElapsedSeconds :type "Float (double-precision)") (TriggeredSeconds :type "Float (double-precision)") (InputAction :type "InputAction Object Reference" :default "/Game/Systems_Integration/Inputs/Actions/IA_Move.IA_Move"))
  (bind _returnvalue (`self.K2_GetPawn`))
  (bind _returnvalue_2 (`self.GetControlRotation`))
  ;[0.5 0.5 0.5] Basic Movement
  ;;[1 0 0] Movement
  (:`Triggered`
    (`Pawn.AddMovementInput` _returnvalue (`KismetMathLibrary.GetForwardVector` _returnvalue_2) ActionValue_X false) ; Forward
    (`Pawn.AddMovementInput` _returnvalue (`KismetMathLibrary.GetRightVector` _returnvalue_2) ActionValue_Y false) ; Right
    ;;[0.65 0 0.65] Camera Tilt (For Movement)
    (set `self.Tilt` (+ ActionValue_Y (`self.Tilt`)))))

(event `EnhancedInput|/Game/Systems_Integration/Inputs/Actions/IA_Look`
  (params (ActionValue :type "Vector2D Structure") (ElapsedSeconds :type "Float (double-precision)") (TriggeredSeconds :type "Float (double-precision)") (InputAction :type "InputAction Object Reference" :default "/Game/Systems_Integration/Inputs/Actions/IA_Look.IA_Look"))
  (bind ((`FOVTarget_54_748119344E827DE77056228505A02BA1` _fovtarget) (`FOVInterpSpeed_58_A7D04A59425E5006DF4BF8859724B2D1` _fovinterpspeed) (`FOVSwitchSpeed_56_7A1CC80441B1BE04A27391862602A262` _fovswitchspeed) (`HorizontalCamSpeed_48_BCC115954F2DC5CE029858B577AE2287` _horizontalcamspeed) (`VerticalCamSpeed_47_BDA38A3643667DFE78A0778FF1A6268E` _verticalcamspeed)) (break `/Game/DataAssets/Data_3C/S_FPSCameraFeel` (`self.Camera Feel Structure Ref`)))
  (bind _returnvalue (* ActionValue_Y _verticalcamspeed))
  ;[0.5 0.5 0.5] Basic Movement
  ;;[0.025 0.65 1] Look
  (:`Triggered`
    (`self.AddYawInput` (* ActionValue_X _horizontalcamspeed)) ; Roll on X
    (if (`self.Inverted Cam`)
      (`self.AddPitchInput` _returnvalue) ; Roll on Y
      (else
        (`self.AddPitchInput` (* _returnvalue -1.0)) ; Invert Roll on Y
      ))
    ;;[0.65 0 0.65] Camera Tilt (For Look)
    (set `self.Tilt` (+ ActionValue_Y (`self.Tilt`)))))

(event `Head Tilt`
  (params (`Delta Time` :type "Float (double-precision)"))
  (bind _player_ref (`self.Player Ref`))
  (bind _tilt (`self.Tilt`))
  (bind _camera (`/Game/Systems_Integration/BP_CharaSystems.Camera` _player_ref))
  (bind _returnvalue (- _tilt (* _tilt (`self.Tilt Recover Speed`) `Delta Time`)))
  ;[0.75 0.45 0.15] Head Tilt
  (`/Engine/EditorBlueprintResources/StandardMacros.IsValid` _player_ref
    (:`Is Valid`
      (set `self.Tilt` (select `bool` (< _returnvalue 0.0) :`false` (`KismetMathLibrary.FClamp` _returnvalue 0.0 (`self.Max Tilt`)) :`true` (`KismetMathLibrary.FClamp` _returnvalue (* (`self.Max Tilt`) -1.0) 0.0)))
      (`SceneComponent.K2_SetWorldRotation` _camera (`self.GetControlRotation`) false false)
      (`SceneComponent.K2_AddRelativeRotation` _camera (`KismetMathLibrary.MakeRotator` (`self.Tilt`)) false false))))

(event `EnhancedInput|/Game/Systems_Integration/Inputs/Actions/IA_Fire`
  (params (ActionValue :type Boolean) (ElapsedSeconds :type "Float (double-precision)") (TriggeredSeconds :type "Float (double-precision)") (InputAction :type "InputAction Object Reference" :default "/Game/Systems_Integration/Inputs/Actions/IA_Fire.IA_Fire"))
  (:`Triggered`
    (bind _asbp_chara_systems (cast `/Game/Systems_Integration/BP_CharaSystems` (`self.K2_GetPawn`)))
    (bind _currentweapon (`/Game/Systems_Integration/BP_CharaSystems.CurrentWeapon` _asbp_chara_systems)
      (:`then`
        (`/Game/Systems_Integration/BP_CharaSystems.Raycast Damage` _asbp_chara_systems (`/Game/Developers/ISh/Weapon/BP_WeaponBase_COMP.Range` _currentweapon) (`/Game/Developers/ISh/Weapon/BP_WeaponBase_COMP.Range Damage` _currentweapon)))
      (:`else`))))

(event `EnhancedInput|/Game/Systems_Integration/Inputs/Actions/IA_Throw`
  (params (ActionValue :type Boolean) (ElapsedSeconds :type "Float (double-precision)") (TriggeredSeconds :type "Float (double-precision)") (InputAction :type "InputAction Object Reference" :default "/Game/Systems_Integration/Inputs/Actions/IA_Throw.IA_Throw"))
  (:`Triggered`
    (bind _asbp_chara_systems (cast `/Game/Systems_Integration/BP_CharaSystems` (`self.K2_GetPawn`)))
    (`/Game/Systems_Integration/BP_CharaSystems.Throw` _asbp_chara_systems)))

(event `EnhancedInput|/Game/Systems_Integration/Inputs/Actions/IA_Kick`
  (params (ActionValue :type Boolean) (ElapsedSeconds :type "Float (double-precision)") (TriggeredSeconds :type "Float (double-precision)") (InputAction :type "InputAction Object Reference" :default "/Game/Systems_Integration/Inputs/Actions/IA_Kick.IA_Kick"))
  (:`Triggered`
    (bind _asbp_chara_systems (cast `/Game/Systems_Integration/BP_CharaSystems` (`self.K2_GetPawn`)))
    (`/Game/Systems_Integration/BP_CharaSystems.Kick` _asbp_chara_systems)))

(event `EnhancedInput|/Game/Systems_Integration/Inputs/Actions/IA_Interact`
  (params (ActionValue :type Boolean) (ElapsedSeconds :type "Float (double-precision)") (TriggeredSeconds :type "Float (double-precision)") (InputAction :type "InputAction Object Reference" :default "/Game/Systems_Integration/Inputs/Actions/IA_Interact.IA_Interact"))
  (bind _overlappingactors (`self.GetOverlappingActors` (`self.K2_GetPawn`) null))
  (:`Triggered`
    (`KismetSystemLibrary.PrintString` (`KismetStringLibrary.Conv_IntToString` (`KismetArrayLibrary.Array_Length` _overlappingactors)))
    (message `/Game/Developers/ISh/Pickup/BPI_Interact.Interact` (`|GetArrayItem` _overlappingactors) (cast `/Game/Systems_Integration/BP_CharaSystems` (`self.K2_GetPawn`) :!pure true))))

(event `Key|Gamepad_DPad_Down`
  (params (Key :type "Key Structure"))
  (:`Released`
    (bind _isa (`/Engine/EditorBlueprintResources/StandardMacros.FlipFlop`)
      (:`A`
        _)
      (:`B`
        _))
    (set `self.Inverted Cam` _isa)))

(fn `UserConstructionScript`)