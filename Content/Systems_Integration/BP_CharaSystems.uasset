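; Player character that integrates kick, weapon equip and throw, hitscan damage and an enemy-grab QTE.
; Movement and kick tuning come from structs; sphere-trace kicks launch dummies and doors, and weapons are socket-attached components that respawn as pickups when dropped.
; Overlapping an enemy swaps the input mapping context and starts timers draining health and QTE progress.
; Enough presses restore input, launch the player free and release the enemy after a delay.
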(event `self.ReceiveBeginPlay`
  (bind _capsulecomponent (`self.CapsuleComponent`))
  (bind (_gravity _walkspeed _runspeed _lineardamping _angulardamping) (break `/Game/_3C/Data/S_PlayerFeel` (`self.Player Feel Structure Ref`)))
  ;[0.025 0.75 0.75] Custom Game Feel set trough a Structure ("S_PlayerFeel")
  (set `CharacterMovementComponent.GravityScale` _gravity (`self.CharacterMovement`))
  (set `CharacterMovementComponent.MaxWalkSpeed` _walkspeed (`self.CharacterMovement`))
  (set `self.Run Speed` _runspeed)
  (`PrimitiveComponent.SetLinearDamping` _capsulecomponent _lineardamping)
  (`PrimitiveComponent.SetAngularDamping` _capsulecomponent _angulardamping)
  (bind _returnvalue (`|CreateWidget` "/Game/UI/W_PlayerLife.W_PlayerLife_C"))
  (`UserWidget.AddToViewport` _returnvalue 0)
  (set `self.PlayerLife Current` (`self.PlayerLife Max`)))

(event `Kick`
  (bind _returnvalue (`self.K2_GetActorLocation`))
  (bind (_returnvalue_x _returnvalue_y) (`KismetMathLibrary.BreakVector` (`self.GetActorForwardVector`)))
  (bind (_combatfeelstructref_kickforce _combatfeelstructref_kicklength) (break `/Game/_3C/Data_3C/S_CombatFeel` (`self.CombatFeelStructRef`)))
  (bind _combatfeelstructref_kickforce_2 (break `/Game/_3C/Data_3C/S_CombatFeel` (`self.CombatFeelStructRef`)))
  (bind _returnvalue_2 (+ (* (`KismetMathLibrary.MakeVector` _returnvalue_x _returnvalue_y) (`KismetMathLibrary.MakeVector` (.x _combatfeelstructref_kickforce_2) (.y _combatfeelstructref_kickforce_2))) (`KismetMathLibrary.MakeVector` 0.0 0.0 (.z _combatfeelstructref_kickforce_2))))
  ;[0 0.4323 0.113 0.5] Kick System
  (bind _outhit (`KismetSystemLibrary.SphereTraceSingleForObjects` :`Start` _returnvalue :`End` (+ _returnvalue (* (`SceneComponent.GetForwardVector` (`self.Camera`)) _combatfeelstructref_kicklength)) :`Radius` 50.0 :`ObjectTypes` (`|MakeArray` "ObjectTypeQuery3" "ObjectTypeQuery7" :!type "EObjectTypeQuery Enum") :`DrawDebugType` "Persistent"))
  (bind (_bblockinghit _binitialoverlap _time _distance _location _impactpoint _normal _impactnormal _physmat _hitactor) (`GameplayStatics.BreakHitResult` _outhit))
  ;; Kick Enemy
  (bind _asbp_dummy (cast `/Game/CombatSystem/BP_Dummy` _hitactor)
    (:`then`
      (`/Game/CombatSystem/BP_Dummy.Launched` _asbp_dummy _returnvalue_2))
    (:`CastFailed`
      ;; Kick door
      (bind _asbp_kickable_door (cast `/Game/CombatSystem/BP_KickableDoor` _hitactor))
      (`/Game/CombatSystem/BP_KickableDoor.Launched` _asbp_kickable_door _returnvalue_2))))

(event `Throw`
  (bind _currentweapon (`self.CurrentWeapon`)
    (:`then`
      (bind _returnvalue (`|SpawnActorFromClass` (`/Game/Developers/ISh/Weapon/BP_WeaponBase_COMP.Pickup Class` _currentweapon) (`KismetMathLibrary.MakeTransform` (`self.K2_GetActorLocation`) (`self.K2_GetActorRotation`)) "AdjustIfPossibleButAlwaysSpawn" "MultiplyWithRoot" null null))
      (`ActorComponent.K2_DestroyComponent` (`self.CurrentWeapon`))
      (`PrimitiveComponent.AddImpulse` (`/Game/Developers/ISh/Pickup/BP_PickupBase.Cube` _returnvalue) (* (`SceneComponent.GetForwardVector` (`self.Camera`)) (`self.ThrowForce`)) "None" false))
    (:`else`
      (`KismetSystemLibrary.PrintString` "not valid"))))

(event `SpawnWeapon`
  (params (PickUpClass :type "/Game/Developers/ISh/Weapon/BP_WeaponBase_COMP Class Reference") (PickUpLocation :type "Vector Structure"))
  (bind _currentweapon (`self.CurrentWeapon`))
  (bind _currentweapon_2 (`self.CurrentWeapon`)
    (:`then`
      (`|SpawnActorFromClass` (`/Game/Developers/ISh/Weapon/BP_WeaponBase_COMP.Pickup Class` _currentweapon_2) (`KismetMathLibrary.MakeTransform` (+ PickUpLocation (0.0 0.0 10.0))) "Undefined" "MultiplyWithRoot" null null)
      (`ActorComponent.K2_DestroyComponent` _currentweapon_2))
    (:`else`
      _))
  (bind _returnvalue (`|AddComponentByClass` PickUpClass))
  (bind _output_get (set `self.CurrentWeapon` _returnvalue))
  (`SceneComponent.K2_AttachToComponent` _output_get (`self.Mesh`) (`/Game/Developers/ISh/Weapon/BP_WeaponBase_COMP.Socket Name` _output_get) "SnapToTarget" "SnapToTarget" "SnapToTarget" true)
  (`KismetSystemLibrary.PrintString` (`KismetStringLibrary.Concat_StrStr` "Equipped: " (`KismetSystemLibrary.GetDisplayName` _output_get)))
  (`SceneComponent.K2_SetRelativeTransform` _currentweapon (`/Game/Developers/ISh/Weapon/BP_WeaponBase_COMP.Transform` _currentweapon) false false))

(event `self.CapsuleComponent.OnComponentBeginOverlap`
  (params (OverlappedComponent :type "PrimitiveComponent Object Reference") (OtherActor :type "Actor Object Reference") (OtherComp :type "PrimitiveComponent Object Reference") (OtherBodyIndex :type Integer) (bFromSweep :type Boolean) (SweepResult :type "HitResult Structure (by ref)"))
  ;[0.4329 0 1 0.5] QTE Behavior
  ;; Enemy Hits Player
  (if (`self.ActorHasTag` OtherActor "Enemy")
    (set `self.Is Hit ?` true)
    (set `self.Enemy` (cast `/Game/CombatSystem/BP_Dummy` OtherActor :!pure true))
    (`/Game/CombatSystem/BP_Dummy.QTE Begin` (`self.Enemy`))
    (bind _returnvalue (`|CreateWidget` "/Game/UI/W_QTE.W_QTE_C"))
    (`UserWidget.AddToViewport` _returnvalue 0)
    (`self.Switch Input Event`) ; Change input to stop any other commands than the QTE needs
    (`self.HealthQTE`) ; Reduce Health when in QTE
    (bind _returnvalue_2 (`KismetSystemLibrary.K2_SetTimerDelegate` (delegate `HealthQTE`) 0.1 true)) ; Loop "Health QTE" after a certain amount of time
    (set `self.QTE Health Timer` _returnvalue_2)
    (bind _returnvalue_3 (`KismetSystemLibrary.K2_SetTimerDelegate` (delegate `QTE Charge`) 0.1 true)) ; Loop "QTE Charge" after a certain amount of time
    (set `self.NewVar` _returnvalue_3)
    (`KismetSystemLibrary.PrintString` "QTE !!")))

(event `EnhancedInput|/Game/FirstPerson/Input/Actions/IA_QTE`
  (params (ActionValue :type Boolean) (ElapsedSeconds :type "Float (double-precision)") (TriggeredSeconds :type "Float (double-precision)") (InputAction :type "InputAction Object Reference" :default "/Game/FirstPerson/Input/Actions/IA_QTE.IA_QTE"))
  ;[0.4329 0 1 0.5] QTE Behavior
  ;; QTE Necessary Hit
  (:`Started`
    (set `self.QTE Current` (+ (`self.QTE Current`) 1.25))
    (if (>= (`self.QTE Current`) (`self.QTE Max`))
      (`self.QTE End Event`))))

(event `HealthQTE`
  ;[0.4329 0 1 0.5] QTE Behavior
  ;;[0.1667 0.1667 0.1667] Health decreases when in QTE
  (if (and (`self.Is Hit ?`) (<= (`self.QTE Current`) (`self.QTE Max`)))
    (set `self.PlayerLife Current` (- (`self.PlayerLife Current`) 1))))

(event `QTE Charge`
  ;[0.4329 0 1 0.5] QTE Behavior
  ;; Reduce QTE Bar With Time
  (set `self.QTE Current` (- (`self.QTE Current`) 0.1)))

(event `Switch Input Event`
  (bind _returnvalue (pcsubsystem `EnhancedInputLocalPlayerSubsystem` (`GameplayStatics.GetPlayerController` 0)))
  ;[0.4329 0 1 0.5] QTE Behavior
  ;; Input Mapping Swap + QTE End Event
  (`/Engine/EditorBlueprintResources/StandardMacros.IsValid` _returnvalue
    (:`Is Valid`
      (if (`self.Is Hit ?`)
        ;;; Change IMC from Default to QTE
        (`EnhancedInputSubsystemInterface.RemoveMappingContext` _returnvalue "/Game/Systems_Integration/Inputs/IMC_Systems.IMC_Systems" (struct))
        (`EnhancedInputSubsystemInterface.AddMappingContext` _returnvalue "/Game/FirstPerson/Input/IMC_QTE.IMC_QTE" 0 (struct))))))

(event `QTE End Event`
  (bind _enemy (`self.Enemy`))
  (bind _returnvalue (pcsubsystem `EnhancedInputLocalPlayerSubsystem` (`GameplayStatics.GetPlayerController` 0)))
  ;[0.4329 0 1 0.5] QTE Behavior
  ;; Input Mapping Swap + QTE End Event
  (`KismetSystemLibrary.K2_PauseTimerHandle` (`self.QTE Health Timer`))
  (set `self.QTE Current` 0.0) ; Reset QTE necessary input to complete
  ;;;[1 1 1 0.5] Change IMC from QTE to Default
  (`EnhancedInputSubsystemInterface.RemoveMappingContext` _returnvalue "/Game/FirstPerson/Input/IMC_QTE.IMC_QTE" (struct))
  (`EnhancedInputSubsystemInterface.AddMappingContext` _returnvalue "/Game/Systems_Integration/Inputs/IMC_Systems.IMC_Systems" 0 (struct))
  (`Widget.RemoveFromParent` (stale `self.CapsuleComponent.OnComponentBeginOverlap` _returnvalue)) ; Remove QTE UI
  (`self.LaunchCharacter` (-500.0 500.0 500.0)) ; Push Player from the enemy who grabbed him
  (`KismetSystemLibrary.PrintString` "You are free !")
  (`KismetSystemLibrary.Delay` 3.0) ; Time before enemy reactivate
  (`/Engine/EditorBlueprintResources/StandardMacros.IsValid` _enemy
    (:`Is Valid`
      (`/Game/CombatSystem/BP_Dummy.QTE End` _enemy)
      (set `self.Is Hit ?` false) ; Define Player invicibility after QTE end
    )))

(fn `Raycast Damage`
  (params (Range :type "Float (double-precision)") (Damage :type "Float (double-precision)"))
  (bind (_returnvalue_location _returnvalue_rotation) (`KismetMathLibrary.BreakTransform` (`SceneComponent.K2_GetComponentToWorld` (`self.Camera`))))
  (bind _returnvalue (+ _returnvalue_location (0.0 0.0 -2.0)))
  (bind _outhit (`KismetSystemLibrary.LineTraceSingle` :`Start` _returnvalue :`End` (+ _returnvalue (* (`KismetMathLibrary.GetForwardVector` _returnvalue_rotation) Range)) :`TraceChannel` "TraceTypeQuery2" :`bTraceComplex` true :`DrawDebugType` "ForDuration"))
  (`/Engine/EditorBlueprintResources/StandardMacros.IsValid` (`.HitActor` (`GameplayStatics.BreakHitResult` _outhit))
    (:`Is Valid`
      (`GameplayStatics.ApplyDamage` (`.HitActor` (`GameplayStatics.BreakHitResult` _outhit)) Damage))))

(fn `UserConstructionScript`)