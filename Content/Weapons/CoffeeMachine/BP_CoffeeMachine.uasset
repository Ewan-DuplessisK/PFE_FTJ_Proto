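; Coffee machine weapon Blueprint that adds its own animated feedback on top of its parent weapon class.
; The AddFeedbacks override calls the parent, then a timeline interpolates the static mesh's relative location and rotation between two hard-coded poses.
; When that finishes, a short delay leads into a second timeline that moves the Piston component along its local Z offset.
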(event `self.ReceiveBeginPlay`)

(event `self.AddFeedbacks`
  (`parent.AddFeedbacks`)
  (bind (_direction _location _rotation) (`Timeline|Weapon Anim` :!via `PlayFromStart`)
    (:`Update`
      (`SceneComponent.K2_SetRelativeLocationAndRotation` (`self.StaticMesh`) (`KismetMathLibrary.VLerp` (25.0 9.0 -7.0) (8.0 9.0 -7.0) _location) (`KismetMathLibrary.RLerp` (struct :`Pitch` -59.0 :`Yaw` -81.0 :`Roll` -100.0) (struct :`Pitch` -44.0 :`Yaw` -37.0 :`Roll` -135.0) _rotation) false false))
    (:`Finished`
      (`KismetSystemLibrary.Delay` 0.2)
      (bind (_direction_2 _location_2) (`Timeline|Timeline` :!via `PlayFromStart`)
        (:`Update`
          (`SceneComponent.K2_SetRelativeLocationAndRotation` :`self` (`self.Piston`) :`NewLocation` (`KismetMathLibrary.VLerp` (0.0 0.0 0.0) (0.0 0.0 20.0) _location_2)))))))

(fn `UserConstructionScript`
  (`parent.UserConstructionScript`))