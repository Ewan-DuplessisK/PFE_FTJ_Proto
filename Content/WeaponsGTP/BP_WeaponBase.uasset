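; Base weapon actor that the player can pick up, drop and throw, with empty use and feedback events.
; Its pickup sphere registers it with BP_CharaSystems and shows a screen-space name prompt, dimmed unless it is the closest weapon.
; Pickup and drop toggle collision and set or clear the player's held weapon.
; When thrown, overlapping an enemy deals damage and destroys the weapon; UpdateWidget forwards ammo or durability to the player's ammo widget.
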(event `self.ReceiveBeginPlay`
  (bind _widgetcomp (`self.WidgetComp`))
  (bind _returnvalue (`|CreateWidget` "/Game/Usables_System/Interactable/WBP_Interactable.WBP_Interactable_C"))
  (`WidgetComponent.SetWidget` _widgetcomp _returnvalue)
  (`WidgetComponent.SetWidgetSpace` _widgetcomp "Screen")
  (`SceneComponent.SetVisibility` _widgetcomp false false)
  (set `/Game/Usables_System/Interactable/WBP_Interactable.Title` (`self.WeaponName`) (cast `/Game/Usables_System/Interactable/WBP_Interactable` (`WidgetComponent.GetWidget` _widgetcomp) :!pure true))
  (if (`KismetTextLibrary.EqualEqual_TextText` (`self.Type`) (`self.DefText`))
    (`KismetSystemLibrary.PrintString` "Weapon Type is \"None\"" true true (struct :`R` 1.0 :`A` 1.0) 60.0)))

(event `self.ReceiveTick`
  (params (DeltaSeconds :type "Float (single-precision)"))
  (if (`KismetArrayLibrary.Array_IsNotEmpty` (`PrimitiveComponent.GetOverlappingActors` (`self.PickupSphere`) "/Game/PlayerCharacter/BP_CharaSystems.BP_CharaSystems_C"))
    (`UserWidget.SetColorAndOpacity` (`WidgetComponent.GetWidget` (`self.WidgetComp`)) (make `LinearColor` 1.0 1.0 1.0 (`KismetMathLibrary.SelectFloat` 1.0 0.3 (== (`/Game/PlayerCharacter/BP_CharaSystems.ClosestWeapon` (cast `/Game/PlayerCharacter/BP_CharaSystems` (`GameplayStatics.GetPlayerPawn` 0) :!pure true)) self))))))

(event `self.PickupSphere.OnComponentBeginOverlap`
  (params (OverlappedComponent :type "PrimitiveComponent Object Reference") (OtherActor :type "Actor Object Reference") (OtherComp :type "PrimitiveComponent Object Reference") (OtherBodyIndex :type Integer) (bFromSweep :type Boolean) (SweepResult :type "HitResult Structure (by ref)"))
  (bind _returnvalue (`GameplayStatics.GetPlayerPawn` 0))
  (if (== OtherActor _returnvalue)
    (`KismetArrayLibrary.Array_AddUnique` (`/Game/PlayerCharacter/BP_CharaSystems.Overlaping` (cast `/Game/PlayerCharacter/BP_CharaSystems` _returnvalue :!pure true)) self)
    (`SceneComponent.SetVisibility` (`self.WidgetComp`) true true)
    (elif (`self.ThrownState`)
      (bind _asenemy_base (cast `Enemy_Base` OtherActor))
      (`Enemy_Base.Damaged` _asenemy_base (`KismetMathLibrary.Conv_IntToDouble` (`self.DamageThrow`)) (0.0 0.0 0.0))
      (`KismetSystemLibrary.DelayUntilNextTick`)
      (`self.K2_DestroyActor`))))

(event `self.PickupSphere.OnComponentEndOverlap`
  (params (OverlappedComponent :type "PrimitiveComponent Object Reference") (OtherActor :type "Actor Object Reference") (OtherComp :type "PrimitiveComponent Object Reference") (OtherBodyIndex :type Integer))
  (bind _returnvalue (`GameplayStatics.GetPlayerPawn` 0))
  (if (== _returnvalue OtherActor)
    (`KismetArrayLibrary.Array_RemoveItem` (`/Game/PlayerCharacter/BP_CharaSystems.Overlaping` (cast `/Game/PlayerCharacter/BP_CharaSystems` _returnvalue :!pure true)) self :!label _label)
    (`SceneComponent.SetVisibility` (`self.WidgetComp`) false true)))

(event `OnPickup`
  (bind _widgetcomp (`self.WidgetComp`))
  (`|ExecutionSequence`
    (:`then_0`
      (goto _label))
    (:`then_1`
      (`PrimitiveComponent.SetCollisionEnabled` (`self.PickupSphere`) "NoCollision")
      (`PrimitiveComponent.SetCollisionEnabled` (`self.StaticMesh`) "NoCollision")
      (`SceneComponent.SetVisibility` _widgetcomp false true)
      (`PrimitiveComponent.SetCollisionEnabled` _widgetcomp "NoCollision")
      (set `/Game/PlayerCharacter/BP_CharaSystems.HeldWeapon` self (cast `/Game/PlayerCharacter/BP_CharaSystems` (`GameplayStatics.GetPlayerPawn` 0) :!pure true)))))

(event `OnDrop`
  (`PrimitiveComponent.SetCollisionEnabled` (`self.PickupSphere`) "QueryOnly")
  (`PrimitiveComponent.SetCollisionEnabled` (`self.StaticMesh`) "QueryAndPhysics")
  (`PrimitiveComponent.SetCollisionEnabled` (`self.WidgetComp`) "QueryOnly")
  (set `/Game/PlayerCharacter/BP_CharaSystems.HeldWeapon` null (cast `/Game/PlayerCharacter/BP_CharaSystems` (`GameplayStatics.GetPlayerPawn` 0) :!pure true)))

(event `UseWeapon`)

(event `WeaponFeedback`)

(event `UpdateWidget`
  (params (`Ammo/Durability` :type Integer))
  (`/Game/UI/W_Ammo.SetCurrentAmmo` (`/Game/PlayerCharacter/BP_CharaSystems.AmmoWidgetRef` (cast `/Game/PlayerCharacter/BP_CharaSystems` (`GameplayStatics.GetPlayerPawn` 0) :!pure true)) `Ammo/Durability`))

(fn `UserConstructionScript`)