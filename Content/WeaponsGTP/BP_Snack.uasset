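; BP_Snack is a health pickup that heals the player character when the player pawn overlaps its Pickup component.
; The overlap fires once, calls Heal on BP_CharaSystems, then adds the snack's Health value to PlayerLifeCurrent, capped at PlayerLifeMax.
; The actor destroys itself after a short delay.
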(event `self.Pickup.OnComponentBeginOverlap`
  (params (OverlappedComponent :type "PrimitiveComponent Object Reference") (OtherActor :type "Actor Object Reference") (OtherComp :type "PrimitiveComponent Object Reference") (OtherBodyIndex :type Integer) (bFromSweep :type Boolean) (SweepResult :type "HitResult Structure (by ref)"))
  (bind _returnvalue (`GameplayStatics.GetPlayerPawn` 0))
  (bind _asbp_chara_systems (cast `/Game/PlayerCharacter/BP_CharaSystems` _returnvalue :!pure true))
  (bind _playerlife_max (`/Game/PlayerCharacter/BP_CharaSystems.PlayerLife Max` _asbp_chara_systems))
  (bind _returnvalue_2 (+ (`/Game/PlayerCharacter/BP_CharaSystems.PlayerLife Current` _asbp_chara_systems) (`self.Health`)))
  (if (== OtherActor _returnvalue)
    (`/Engine/EditorBlueprintResources/StandardMacros.DoOnce` false
      (:`Completed`
        (`/Game/PlayerCharacter/BP_CharaSystems.Heal` _asbp_chara_systems)
        (if (> _returnvalue_2 _playerlife_max)
          (set `/Game/PlayerCharacter/BP_CharaSystems.PlayerLife Current` _playerlife_max _asbp_chara_systems)
          (else
            (set `/Game/PlayerCharacter/BP_CharaSystems.PlayerLife Current` _returnvalue_2 _asbp_chara_systems)))
        (`KismetSystemLibrary.Delay` 0.2)
        (`self.K2_DestroyActor`)))))

(fn `UserConstructionScript`)