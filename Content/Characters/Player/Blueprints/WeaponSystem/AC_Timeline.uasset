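; Actor component in the player weapon system that acts as a reusable timeline, playing a float curve at a signed speed.
; Play optionally swaps the curve, sets speed and direction, enables component tick and fires OnStart from the current time clamped to the curve's range.
; Tick advances time and broadcasts the sampled value, stopping when clamped time stops changing, then firing OnTick and OnEnd with a time-range bound as Value.
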(event `self.ReceiveTick`
  (params (DeltaSeconds :type "Float (single-precision)"))
  (bind _current_time (`self.Current Time`))
  (bind _current_time_2 (`self.Current Time`))
  (bind (_mintime _maxtime) (`CurveBase.GetTimeRange` (`self.Curve`)))
  (bind (_mintime_2 _maxtime_2) (`CurveBase.GetTimeRange` (`self.Curve`)))
  (bind _returnvalue (`KismetMathLibrary.SelectFloat` _mintime_2 _maxtime_2 (< (`self.Speed`) 0.0)))
  (bind _returnvalue_2 (`KismetMathLibrary.FClamp` (+ _current_time (* DeltaSeconds (`self.Speed`))) _mintime _maxtime))
  (if (`self.Playing`)
    (if (== _current_time _returnvalue_2)
      (bind _output_get (set `self.Playing` false))
      (`self.SetComponentTickEnabled` _output_get)
      (`self.OnTick` _current_time_2 _returnvalue)
      (`self.OnEnd` _current_time_2 _returnvalue)
      (else
        (set `self.Current Time` _returnvalue_2)
        (set `self.Value` (`self.Get Value`))
        (`self.OnTick` (`self.Current Time`) (`self.Value`))))))

(event `Play`
  (params (Curve :type "CurveFloat Object Reference") (Speed :type "Float (double-precision)" :default 1.0) (Reversed :type Boolean))
  (bind _curve (`self.Curve`))
  (bind (_mintime _maxtime) (`CurveBase.GetTimeRange` _curve))
  (bind _returnvalue (`KismetMathLibrary.FClamp` (`self.Current Time`) _mintime _maxtime))
  (`/Engine/EditorBlueprintResources/StandardMacros.IsValid` Curve
    (:`Is Valid`
      (set `self.Curve` Curve))
    (:`Is Not Valid`
      _))
  (set `self.Speed` (* Speed (`KismetMathLibrary.SelectFloat` -1.0 1.0 Reversed)))
  (bind _output_get (set `self.Playing` true))
  (`self.SetComponentTickEnabled` _output_get)
  (set `self.Current Time` _returnvalue)
  (`self.OnStart` _returnvalue (`CurveFloat.GetFloatValue` _curve _returnvalue)))

(fn `Get Value`
  (returns (Value :type "Float (single-precision)"))
  (return (`CurveFloat.GetFloatValue` (`self.Curve`) (`self.Current Time`))))