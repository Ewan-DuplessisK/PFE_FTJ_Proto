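; Player interaction component that tracks nearby AC_Interactable components and triggers interaction with the closest one.
; Owner overlap events maintain the candidate list and toggle passive highlights.
; Tick picks the candidate nearest a point ahead of the owner along control rotation, using squared distance, and highlights it actively.
; The Interact input action messages that target with the owner, then calls a handleInteract event that only holds a disabled debug print.
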(event `OnActorBeginOverlap_Event`
  (params (OverlappedActor :type "Actor Object Reference") (OtherActor :type "Actor Object Reference"))
  (bind _returnvalue (`Actor.GetComponentByClass` OtherActor "/Game/Characters/Player/Blueprints/WeaponSystem/Interactable/AC_Interactable.AC_Interactable_C"))
  ; Bind Overlapping array to Actor's Overlap begin/end events
  (`/Engine/EditorBlueprintResources/StandardMacros.IsValid` _returnvalue
    (:`Is Valid`
      (if (`/Game/Characters/Player/Blueprints/WeaponSystem/Interactable/AC_Interactable.Interactable?` _returnvalue)
        (`KismetArrayLibrary.Array_AddUnique` (`self.overlappings`) _returnvalue)
        (`/Game/Characters/Player/Blueprints/WeaponSystem/Interactable/AC_Interactable.Highlight` _returnvalue true true)))))

(event `self.ReceiveBeginPlay`
  (bind _returnvalue (`self.GetOwner`))
  ; Add Map Ctx          To be removed, only IMC_Systems should be used, and it already has IA_Interact -Ewan
  ;; char
  (bind _ascharacter (cast `Character` (`self.GetOwner`)))
  (bind _output_get (set `self.сharacter` _ascharacter))
  ;; ctrl
  (bind _asplayer_controller (cast `PlayerController` (`Pawn.GetController` _output_get)))
  (set `self.playerController` _asplayer_controller)
  ; Bind Overlapping array to Actor's Overlap begin/end events
  (`|ExecutionSequence`
    (:`then_0`
      (add `Actor.OnActorBeginOverlap` _returnvalue (delegate `OnActorBeginOverlap_Event`)))
    (:`then_1`
      (add `Actor.OnActorEndOverlap` _returnvalue (delegate `OnActorEndOverlap_Event`)))))

(event `EnhancedInput|/Game/Characters/Player/Blueprints/WeaponSystem/Interactable/Inputs/X_IA_I_Interact`
  (params (ActionValue :type Boolean) (ElapsedSeconds :type "Float (double-precision)") (TriggeredSeconds :type "Float (double-precision)") (InputAction :type "InputAction Object Reference" :default "/Game/Characters/Player/Blueprints/WeaponSystem/Interactable/Inputs/X_IA_I_Interact.X_IA_I_Interact"))
  ; Keymapping
  (:`Started`
    (`self.IA Interact`)))

(event `OnActorEndOverlap_Event`
  (params (OverlappedActor :type "Actor Object Reference") (OtherActor :type "Actor Object Reference"))
  (bind _returnvalue (`Actor.GetComponentByClass` OtherActor "/Game/Characters/Player/Blueprints/WeaponSystem/Interactable/AC_Interactable.AC_Interactable_C"))
  (bind _overlappings (`self.overlappings`))
  ; Bind Overlapping array to Actor's Overlap begin/end events
  (`/Engine/EditorBlueprintResources/StandardMacros.IsValid` _returnvalue
    (:`Is Valid`
      (`KismetArrayLibrary.Array_RemoveItem` _overlappings _returnvalue)
      (`KismetSystemLibrary.PrintString` (`KismetStringLibrary.Concat_StrStr` "Length: " (`KismetStringLibrary.Conv_IntToString` (`KismetArrayLibrary.Array_Length` _overlappings :!enabledstate Disabled) :!enabledstate Disabled) " Left -> " (`KismetSystemLibrary.GetDisplayName` _returnvalue :!enabledstate Disabled) :!enabledstate Disabled) :!enabledstate Disabled)
      (`/Game/Characters/Player/Blueprints/WeaponSystem/Interactable/AC_Interactable.Highlight` _returnvalue false true))))

(event `IA Interact`
  (bind _closest_interactable (`self.closest interactable`))
  ; Interact w the nearest actor
  (`/Engine/EditorBlueprintResources/StandardMacros.IsValid` _closest_interactable
    (:`Is Valid`
      (message `/Game/Characters/Player/Blueprints/WeaponSystem/Interactable/BPI_Interact.Interact` _closest_interactable (`self.GetOwner`))
      (`self.handle Interact` _closest_interactable))))

(event `handle Interact`
  (params (Interactable :type "/Game/Characters/Player/Blueprints/WeaponSystem/Interactable/AC_Interactable Object Reference"))
  (`KismetSystemLibrary.PrintString` "handle Interactable!" :!enabledstate Disabled))

(event `self.ReceiveTick`
  (params (DeltaSeconds :type "Float (single-precision)"))
  (bind _closest_interactable (`self.closest interactable`))
  (bind _interactable (`self.Find Closest In Overlappings` (`self.Get Interaction Location`)))
  ; Set nearest and highlight
  (`KismetSystemLibrary.DelayUntilNextTick` :!label _label)
  (`/Engine/EditorBlueprintResources/StandardMacros.IsValid` _interactable
    (:`Is Valid`
      (`/Game/Characters/Player/Blueprints/WeaponSystem/Interactable/AC_Interactable.Highlight` _interactable true false)
      (`/Engine/EditorBlueprintResources/StandardMacros.IsValid` _closest_interactable
        (:`Is Valid`
          (if (not (== _closest_interactable _interactable))
            (`/Game/Characters/Player/Blueprints/WeaponSystem/Interactable/AC_Interactable.Highlight` _closest_interactable (`KismetArrayLibrary.Array_Contains` (`self.overlappings`) _closest_interactable) true)
            (set `self.closest interactable` _interactable :!label _label_2)))
        (:`Is Not Valid`
          (goto _label_2))))
    (:`Is Not Valid`
      (set `self.closest interactable` null))))

(event `Update Closest`
  ; Set nearest and highlight
  (goto _label))

(fn `Find Closest In Overlappings`
  (params (Location :type "Vector Structure"))
  (returns (Interactable :type "/Game/Characters/Player/Blueprints/WeaponSystem/Interactable/AC_Interactable Object Reference"))
  (locals (Closest :type "/Game/Characters/Player/Blueprints/WeaponSystem/Interactable/AC_Interactable Object Reference") (`Closest Dist` :type "Float (double-precision)" :default 9999999.0))
  (bind _overlappings (`self.overlappings`))
  (if (== (`KismetArrayLibrary.Array_Length` _overlappings) 1)
    (return (`|GetArrayItem` _overlappings))
    (else
      (for _array_element (`self.overlappings`)
        (`/Engine/EditorBlueprintResources/StandardMacros.IsValid` _array_element
          (:`Is Valid`
            (bind _returnvalue (- (`Actor.K2_GetActorLocation` (`self.GetOwner` _array_element)) Location))
            (bind _returnvalue_2 (`KismetMathLibrary.Dot_VectorVector` _returnvalue _returnvalue))
            (if (and (`/Game/Characters/Player/Blueprints/WeaponSystem/Interactable/AC_Interactable.Interactable?` _array_element) (< _returnvalue_2 (`local.Closest Dist`)))
              (set `local.Closest Dist` _returnvalue_2)
              (set `local.Closest` _array_element)))))
      (return (`local.Closest`)))))

(fn `Get Interaction Location`
  (returns (Location :type "Vector Structure"))
  (bind (_returnvalue_location _returnvalue_rotation) (`KismetMathLibrary.BreakTransform` (`Actor.GetTransform` (`self.GetOwner`))))
  (bind _returnvalue_location_2 (`KismetMathLibrary.BreakTransform` (`Actor.GetTransform` (`self.GetOwner`))))
  (bind _returnvalue (+ _returnvalue_location_2 (`KismetMathLibrary.GreaterGreater_VectorRotator` (100.0 0.0 0.0) (`Controller.GetControlRotation` (`GameplayStatics.GetPlayerController` 0)))))
  (`KismetSystemLibrary.DrawDebugLine` _returnvalue_location _returnvalue (struct :`R` 1.0 :`G` 0.29348 :`B` 0.430497 :`A` 1.0) 0.1 1.0 :!enabledstate Disabled)
  (return _returnvalue))