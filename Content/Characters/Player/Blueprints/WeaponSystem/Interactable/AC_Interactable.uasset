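; Actor component that makes its owner interactable, with a screen-space prompt, a pickup overlap sphere and a highlight, and fires OnInteract when used.
; On BeginPlay it builds all three around the owner's static mesh, centering widget and scale-compensated sphere on its center of mass.
; Highlight shows the widget, dimmed when passive, and toggles the overlay material through its max draw distance.
; Disabling interaction clears the highlight.
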(event `self.ReceiveBeginPlay`
  (set `self.mesh` (`Actor.GetComponentByClass` (`self.GetOwner`) "/Script/Engine.StaticMeshComponent"))
  (`self.Add Widget`)
  (`self.Add Overlap Collision`)
  (`self.Add Highlight Material`))

(event `/Game/Characters/Player/Blueprints/WeaponSystem/Interactable/BPI_Interact.Interact`
  (params (Character :type "Actor Object Reference"))
  (`self.On Interact` null))

(fn `Add Highlight Material`
  (bind _mesh (`self.mesh`))
  (bind (_returnvalue_x _returnvalue_y _returnvalue_z) (`KismetMathLibrary.BreakVector` (`SceneComponent.K2_GetComponentScale` (`self.mesh`))))
  (`MeshComponent.SetOverlayMaterialMaxDrawDistance` _mesh -0.01)
  (`/Engine/EditorBlueprintResources/StandardMacros.IsValid` (`MeshComponent.GetOverlayMaterial` _mesh)
    (:`Is Not Valid`
      (bind _returnvalue (`KismetMaterialLibrary.CreateDynamicMaterialInstance` (`self.Highlight Material`)))
      (`MaterialInstanceDynamic.SetScalarParameterValue` _returnvalue "Line Thickness" (/ (+ _returnvalue_x _returnvalue_y _returnvalue_z) 3.0) :!enabledstate Disabled)
      (`MeshComponent.SetOverlayMaterial` (`self.mesh`) _returnvalue))))

(fn `Add Overlap Collision`
  (returns (Collision :type "SphereComponent Object Reference"))
  (bind _returnvalue (`|AddComponentByClass` :`self` (`self.GetOwner`) :`Class` "/Script/Engine.SphereComponent"))
  (bind _output_get (set `self.collision` _returnvalue))
  (`SceneComponent.K2_AttachToComponent` _returnvalue (`self.mesh`) "owm" "KeepRelative" "KeepRelative" "KeepRelative" true)
  (`SceneComponent.K2_SetRelativeLocation` _output_get (`self.Get Relative Center of Mass`) false false)
  (`SceneComponent.SetRelativeScale3D` _returnvalue (/ (1.0 1.0 1.0) (`SceneComponent.RelativeScale3D` (`self.mesh`))))
  (`SphereComponent.SetSphereRadius` _returnvalue (`self.Collision Radius`) true)
  (`PrimitiveComponent.SetCollisionProfileName` _returnvalue "WeaponPickup" true)
  (return _returnvalue))

(fn `Add Widget`
  (bind _returnvalue (`self.GetOwner`))
  (bind _player_controller (`/Game/Characters/Player/Blueprints/WeaponSystem/Interactable/FL_Common.Player's Controller` _returnvalue))
  (bind _returnvalue_2 (`|AddComponentByClass` :`self` _returnvalue :`Class` "/Game/Characters/Player/Blueprints/WeaponSystem/Interactable/AC_InteractableWidget.AC_InteractableWidget_C"))
  (bind _output_get (set `self.widget comp` _returnvalue_2))
  (`SceneComponent.K2_SetRelativeLocation` _output_get (`self.Get Relative Center of Mass`) false false)
  (bind _returnvalue_3 (`|CreateWidget` (`self.Widget Class`) _player_controller))
  (bind _aswbp_interactable (cast `/Game/Characters/Player/Blueprints/WeaponSystem/Interactable/WBP_Interactable` _returnvalue_3))
  (bind _output_get_2 (set `self.widget` _aswbp_interactable))
  (`WidgetComponent.SetWidget` _returnvalue_2 _output_get_2)
  (`WidgetComponent.SetWidgetSpace` _returnvalue_2 "Screen")
  (`SceneComponent.SetVisibility` _output_get false false)
  (set `/Game/Characters/Player/Blueprints/WeaponSystem/Interactable/WBP_Interactable.Title` (`self.Title`) (`self.widget`)))

(fn `Get Relative Center of Mass`
  (returns (Location :type "Vector Structure"))
  (bind _mesh (`self.mesh`))
  (return (- (`PrimitiveComponent.GetCenterOfMass` _mesh "None") (`SceneComponent.K2_GetComponentLocation` _mesh))))

(fn `Highlight`
  (params (State :type Boolean :default true) (Passive :type Boolean :default true))
  (bind _widget_comp (`self.widget comp`))
  (if (not (== State (`self.lastState`)))
    (`KismetSystemLibrary.PrintString` (`KismetStringLibrary.Concat_StrStr` "Highlight: " (`KismetStringLibrary.Conv_BoolToString` State) " -> " (`KismetSystemLibrary.GetDisplayName` (`self.GetOwner`))) true true (struct :`G` 0.66 :`B` 1.0 :`A` 1.0) 5.0 :!enabledstate Disabled))
  (set `self.lastState` State)
  (`MeshComponent.SetOverlayMaterialMaxDrawDistance` (`self.mesh`) (`KismetMathLibrary.SelectFloat` 5000.0 -0.01 (and State (not Passive))))
  (`SceneComponent.SetVisibility` _widget_comp State false)
  (if State
    (`UserWidget.SetColorAndOpacity` (`WidgetComponent.GetWidget` _widget_comp) (make `LinearColor` 1.0 1.0 1.0 (`KismetMathLibrary.SelectFloat` 0.3 1.0 Passive)))))

(fn `Set Interactable`
  (params (`Interactable?` :type Boolean))
  (bind _output_get (set `self.Interactable?` `Interactable?`))
  (if (not _output_get)
    (`self.Highlight` false)))