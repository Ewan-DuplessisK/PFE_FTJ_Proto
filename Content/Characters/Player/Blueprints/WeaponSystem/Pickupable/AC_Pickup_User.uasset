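; Player pickup component that extends an interaction-user component to handle picking up and dropping AC_Pickupable items.
; Interacting with a pickupable disables its interactability, clears it from overlap and closest-target tracking, and adds it to Inventory if inventoryable.
; Dropping re-enables interaction.
; Helper functions detach an item in world space, re-registering it if still overlapping the owner, and disable its mesh physics and collision.
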(event `self.handle Interact`
  (params (Interactable :type "/Game/Characters/Player/Blueprints/WeaponSystem/Interactable/AC_Interactable Object Reference"))
  (`parent.handle Interact` Interactable)
  (bind _asac_pickupable (cast `/Game/Characters/Player/Blueprints/WeaponSystem/Pickupable/AC_Pickupable` Interactable))
  (`self.handle Pickup` _asac_pickupable))

(event `handle Pickup`
  (params (Pickupable :type "/Game/Characters/Player/Blueprints/WeaponSystem/Pickupable/AC_Pickupable Object Reference"))
  (`/Game/Characters/Player/Blueprints/WeaponSystem/Interactable/AC_Interactable.Set Interactable` Pickupable false)
  (`KismetArrayLibrary.Array_RemoveItem` (`self.overlappings`) Pickupable)
  (set `self.closest interactable` null)
  (if (`/Game/Characters/Player/Blueprints/WeaponSystem/Pickupable/AC_Pickupable.Inventoryable?` Pickupable)
    (`KismetArrayLibrary.Array_Add` (`self.Inventory`) Pickupable)))

(event `handle Drop`
  (params (Target :type "/Game/Characters/Player/Blueprints/WeaponSystem/Interactable/AC_Interactable Object Reference"))
  (`/Game/Characters/Player/Blueprints/WeaponSystem/Interactable/AC_Interactable.Set Interactable` Target true))

(fn `$ Detach It`
  (params (`AC Interactable` :type "/Game/Characters/Player/Blueprints/WeaponSystem/Interactable/AC_Interactable Object Reference"))
  (bind _returnvalue (`self.GetOwner` `AC Interactable`))
  (`Actor.K2_DetachFromActor` _returnvalue "KeepWorld" "KeepWorld" "KeepRelative")
  (if (`Actor.IsOverlappingActor` _returnvalue (`self.GetOwner`))
    (`KismetArrayLibrary.Array_Add` (`self.overlappings`) `AC Interactable`)))

(fn `$ Disable Its Physics`
  (params (`AC Interactable` :type "/Game/Characters/Player/Blueprints/WeaponSystem/Interactable/AC_Interactable Object Reference"))
  (bind _mesh (`/Game/Characters/Player/Blueprints/WeaponSystem/Interactable/AC_Interactable.mesh` `AC Interactable`))
  (`PrimitiveComponent.SetSimulatePhysics` _mesh false)
  (`PrimitiveComponent.SetEnableGravity` _mesh false)
  (`PrimitiveComponent.SetCollisionEnabled` _mesh "NoCollision"))