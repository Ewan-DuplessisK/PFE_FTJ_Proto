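; Weapon component on a weapon actor that tracks ammo or durability, drives melee, ranged and throw attacks, and shows ammo in a title widget.
; A data asset supplies stats, combo infos whose cooldowns gate attacks, and projectile classes.
; Ranged shots spawn scattered projectiles at the muzzle socket, while empty weapons can request a throw.
; Throwing adds a projectile component that re-arming tries to remove, marked as buggy.
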(event `self.ReceiveBeginPlay`
  (`parent.ReceiveBeginPlay`)
  (`self.Bind Events`)
  (`self.Save Last Prefs`)
  ; Set default Asset Ammo if this Ammo is -1 (default var)
  (if (< (`self.Current Ammo`) 0.0)
    (bind _output_get (set `self.Current Ammo` (`/Game/Characters/Player/Blueprints/WeaponSystem/Weapon/DA_Weapon_Base.Ammo` (`self.Data Asset`)))))
  (`self.Set Widget Title` "" (`KismetStringLibrary.Conv_DoubleToString` _output_get)))

(event `Bind Events`
  (add `self.On Armed` (delegate `On Armed_Event`))
  (add `self.On Throwed` (delegate `On Throwed_Event`)))

(event `On Armed_Event` :!signature `self.On Armed`
  (params (`AC Weapon User` :type "/Game/Characters/Player/Blueprints/WeaponSystem/Weapon/AC_Weapon_User Object Reference"))
  (bind _ac_throw_projectile (`self.AC Throw Projectile`)
    (:`then`
      ; BUG: cant destroy :( reactivation doesnt work too
      (`self.SetActive` _ac_throw_projectile false false)
      (`self.Deactivate` _ac_throw_projectile)
      (`self.K2_DestroyComponent` _ac_throw_projectile)
      (set `self.AC Throw Projectile` null))
    (:`else`)))

(event `On Throwed_Event` :!signature `self.On Throwed`
  (params (`AC Weapon User` :type "/Game/Characters/Player/Blueprints/WeaponSystem/Weapon/AC_Weapon_User Object Reference"))
  (`|ExecutionSequence`
    (:`then_0`
      ; BUG: cant destroy :( reactivation doesnt work too
      (bind _returnvalue (`|AddComponentByClass` (`self.GetOwner`) (`/Game/Characters/Player/Blueprints/WeaponSystem/Weapon/DA_Weapon_Base.AC Throw Projectile Class` (`self.Data Asset`))))
      (set `self.AC Throw Projectile` _returnvalue))
    (:`then_1`
      (bind _output_get (set `self.Current Ammo` (- (`self.Current Ammo`) 1.0)))
      (`self.Set Widget Title` "" (`KismetStringLibrary.Conv_DoubleToString` _output_get)))))

(fn `$ Attacking _ Melee Hit Someone`
  (`self.$ Decrease Ammo`))

(fn `$ Attacking _ Pre`
  (params (`AC Weapon User` :type "/Game/Characters/Player/Blueprints/WeaponSystem/Weapon/AC_Weapon_User Object Reference"))
  (returns (`Allow Attack` :type Boolean) (Throw :type Boolean))
  (locals (_Cooldown :type Boolean) (_NoAmmo :type Boolean))
  (bind _returnvalue (> (`self.Current Ammo`) 0.0))
  (if (> (- (`KismetSystemLibrary.GetGameTimeInSeconds`) (`.Cooldown_5_5657D8CB423FA11F1D2B669BCEAA1958` (break `/Game/Characters/Player/Blueprints/S_ComboAttackInfo` (`self.Get Combo Attack Info`)))) (`self.lastAttackTime`))
    (set `self.lastAttackTime` (`KismetSystemLibrary.GetGameTimeInSeconds`))
    (return _returnvalue (and (not _returnvalue) (`/Game/Characters/Player/Blueprints/WeaponSystem/Weapon/DA_Weapon_Base.Throw when Empty?` (`self.Data Asset`))))
    (else
      (return false false))))

(fn `$ Attacking _ Ranged`
  (`self.$ Decrease Ammo`)
  (for _ (range (`/Game/Characters/Player/Blueprints/WeaponSystem/Weapon/DA_Weapon_Base.Projectiles Number` (`self.Data Asset`)))
    (bind _returnvalue (`|SpawnActorFromClass` (`/Game/Characters/Player/Blueprints/WeaponSystem/Weapon/DA_Weapon_Base.Projectile Class` (`self.Data Asset`)) (`KismetMathLibrary.MakeTransform` (`self.Get Projectile Spawn Transform`) (`self.Scatter Projectile Dir` (`.Rot` (`/Game/Characters/Player/Blueprints/WeaponSystem/Weapon/AC_Weapon_User.Get Aiming Dir` (`self.Get Last AC Weapon User`) (`self.Get Projectile Spawn Transform`))))) "AdjustIfPossibleButAlwaysSpawn" "OverrideRootScale" (`self.GetOwner`) (`GameplayStatics.GetPlayerPawn` 0)))
    (set `/Game/Characters/Player/Blueprints/WeaponSystem/Weapon/BP_Weapon_Projectile_Base.weaponData` (`self.Data Asset`) _returnvalue)
    (`/Game/Characters/Player/Blueprints/WeaponSystem/Weapon/BP_Weapon_Projectile_Base.Fire!` _returnvalue))
  (`|ExecutionSequence`
    (:`then_0`
      (bind _asbp_weapon_base (cast `/Game/Characters/Player/Blueprints/WeaponSystem/Weapon/BP_Weapon_Base` (`self.GetOwner`))
        (:`then`
          (`/Game/Characters/Player/Blueprints/WeaponSystem/Weapon/BP_Weapon_Base.AddFeedbacks` _asbp_weapon_base))
        (:`CastFailed`
          (`KismetSystemLibrary.PrintString` "[Weapon_User] Ranged, Weapon Actor cast fail"))))
    (:`then_1`
      (`GameplayStatics.PlaySoundAtLocation` (`/Game/Characters/Player/Blueprints/WeaponSystem/Weapon/DA_Weapon_Base.Sound` (`self.Data Asset`)) (`self.Get Projectile Spawn Transform`) (struct) 1.0 1.0 0.0 null null null null))))

(fn `$ Decrease Ammo`
  (returns (Ammo :type "Float (double-precision)"))
  (bind _output_get (set `self.Current Ammo` (- (`self.Current Ammo`) (`KismetMathLibrary.SelectFloat` 0.0 1.0 (`/Game/Characters/Player/Blueprints/WeaponSystem/Weapon/AC_Weapon_User.TEST Infinite Durability` (`self.Get Last AC Weapon User`))))))
  (`self.Set Widget Title` "" (`KismetMathLibrary.SelectString` (`KismetStringLibrary.Conv_DoubleToString` _output_get) "" (> _output_get 0.0)))
  (return (`self.Current Ammo`)))

(fn `$ Throwing`
  (`|ExecutionSequence`))

(fn `Get Combo Attack Info`
  (returns (`Combo Attack Info` :type "/Game/Characters/Player/Blueprints/S_ComboAttackInfo Structure (by ref)") (`Attack Type` :type "/Game/Characters/Enemies/Blueprints/E_AttackTypes Enum") (`Combo Count` :type Integer))
  (bind _ac_weapon_user (`self.Get Last AC Weapon User`))
  (bind _combo_hit_infos (`/Game/Characters/Player/Blueprints/WeaponSystem/Weapon/DA_Weapon_Base.Combo Hit Infos` (`self.Data Asset`)))
  (bind _combo_count (`/Game/Characters/Player/Blueprints/WeaponSystem/Weapon/AC_Weapon_User.Combo Count` _ac_weapon_user))
  (if (`/Game/Characters/Player/Blueprints/WeaponSystem/Weapon/AC_Weapon_User.Combo Launcher` _ac_weapon_user)
    (return (`/Game/Characters/Player/Blueprints/WeaponSystem/Weapon/DA_Weapon_Base.Combo Launcher Info` (`self.Data Asset`)) "NewEnumerator3" (`/Game/Characters/Player/Blueprints/WeaponSystem/Weapon/AC_Weapon_User.Combo Count` _ac_weapon_user))
    (elif (>= _combo_count (`KismetArrayLibrary.Array_Length` _combo_hit_infos))
      (return (`/Game/Characters/Player/Blueprints/WeaponSystem/Weapon/DA_Weapon_Base.Combo Finisher Info` (`self.Data Asset`)) "NewEnumerator4" _combo_count)
      (else
        (return (`|GetArrayItem` _combo_hit_infos _combo_count) "NewEnumerator2" _combo_count)))))

(fn `Get Cooldown`
  (returns (Allowed :type Boolean) (`Since Allowed` :type "Float (double-precision)") (Duration :type "Float (double-precision)") (Remaining :type "Float (double-precision)"))
  (bind _combo_attack_info (`self.Get Combo Attack Info`))
  (bind _returnvalue (`KismetSystemLibrary.GetGameTimeInSeconds`))
  (bind _lastattacktime (`self.lastAttackTime`))
  (bind _returnvalue_2 (- _returnvalue (`.Cooldown_5_5657D8CB423FA11F1D2B669BCEAA1958` (break `/Game/Characters/Player/Blueprints/S_ComboAttackInfo` _combo_attack_info))))
  (bind _returnvalue_3 (- _returnvalue_2 _lastattacktime))
  (return (<= _returnvalue_2 _lastattacktime) _returnvalue_3 (`.Cooldown_5_5657D8CB423FA11F1D2B669BCEAA1958` (break `/Game/Characters/Player/Blueprints/S_ComboAttackInfo` _combo_attack_info)) (`KismetMathLibrary.FMax` (- _returnvalue_3 _returnvalue))))

(fn `Get Last AC Weapon User`
  (returns (`AC Weapon User` :type "/Game/Characters/Player/Blueprints/WeaponSystem/Weapon/AC_Weapon_User Object Reference"))
  (return (`Actor.GetComponentByClass` (`GameplayStatics.GetPlayerPawn` 0) "/Game/Characters/Player/Blueprints/WeaponSystem/Weapon/AC_Weapon_User.AC_Weapon_User_C")))

(fn `Get Last Prefs`
  (returns (`Init Prefs` :type "/Game/Characters/Player/Blueprints/WeaponSystem/Weapon/private/F_Weapon_Prefs Structure"))
  (return (`self.lastPrefs`)))

(fn `Get Projectile Spawn Transform`
  (returns (Location :type "Vector Structure") (Rotation :type "Rotator Structure") (`Return Value Scale` :type "Vector Structure"))
  (bind (_returnvalue_location _returnvalue_rotation _returnvalue_scale) (`KismetMathLibrary.BreakTransform` (`SceneComponent.GetSocketTransform` (`self.mesh`) "WeaponMuzzle" "RTS_World")))
  (return _returnvalue_location _returnvalue_rotation _returnvalue_scale))

(fn `Save Last Prefs`
  (bind _returnvalue (`Actor.GetComponentByClass` (`self.GetOwner` self) "/Script/Engine.MeshComponent"))
  (set `self.lastPrefs` (make `/Game/Characters/Player/Blueprints/WeaponSystem/Weapon/private/F_Weapon_Prefs` (`PrimitiveComponent.GetCollisionEnabled` _returnvalue) (`PrimitiveComponent.IsGravityEnabled` _returnvalue) (`SceneComponent.IsAnySimulatingPhysics` _returnvalue) (`PrimitiveComponent.GetCollisionProfileName` _returnvalue))))

(fn `Scatter Projectile Dir`
  (params (`In Rot` :type "Rotator Structure"))
  (returns (Rot :type "Rotator Structure"))
  (bind _projectiles_scattering (`/Game/Characters/Player/Blueprints/WeaponSystem/Weapon/DA_Weapon_Base.Projectiles Scattering` (`self.Data Asset`)))
  (return (`KismetMathLibrary.SelectRotator` (`KismetMathLibrary.Conv_VectorToRotator` (`KismetMathLibrary.RandomUnitVectorInConeInDegrees` (`KismetMathLibrary.Conv_RotatorToVector` `In Rot`) _projectiles_scattering)) `In Rot` (> _projectiles_scattering 0.0))))

(fn `Set Widget Title`
  (params (Name :type String) (Info :type String))
  (bind _widget (`self.widget`))
  (bind _returnvalue (`KismetMathLibrary.SelectString` (`KismetStringLibrary.Conv_NameToString` (`/Game/Characters/Player/Blueprints/WeaponSystem/Weapon/DA_Weapon_Base.Name` (`self.Data Asset`))) "" (== (`KismetStringLibrary.Len` Name) 0)))
  (if (`KismetStringLibrary.IsEmpty` Info)
    (set `/Game/Characters/Player/Blueprints/WeaponSystem/Interactable/WBP_Interactable.Title` (`KismetTextLibrary.Conv_StringToText` _returnvalue) _widget)
    (else
      (set `/Game/Characters/Player/Blueprints/WeaponSystem/Interactable/WBP_Interactable.Title` (`KismetTextLibrary.Conv_StringToText` (`KismetStringLibrary.Concat_StrStr` _returnvalue " - " Info)) _widget))))