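; Base projectile actor for the player weapon system that launches on fire and reports hits to the actors it strikes.
; It stores the passed weapon data, though applying bounciness and speed from it is disabled, and Fire activates the projectile movement.
; On hit it switches to a post-hit gravity scale, plays the ranged hit sound and sends the hit with weapon and user only once per actor, tracked in a set.
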(event `Set Weapon Data`
  (params (weaponData :type "/Game/Characters/Player/Blueprints/WeaponSystem/Weapon/DA_Weapon_Base Object Reference"))
  (bind _projectilemovement (`self.ProjectileMovement` :!enabledstate Disabled))
  (bind _weapondata (`self.weaponData` :!enabledstate Disabled))
  (bind _velocity (`/Game/Characters/Player/Blueprints/WeaponSystem/Weapon/DA_Weapon_Base.Velocity` _weapondata :!enabledstate Disabled))
  (set `self.weaponData` weaponData)
  (set `ProjectileMovementComponent.Bounciness` (`/Game/Characters/Player/Blueprints/WeaponSystem/Weapon/DA_Weapon_Base.Bounciness` _weapondata :!enabledstate Disabled) _projectilemovement :!enabledstate Disabled)
  (set `ProjectileMovementComponent.InitialSpeed` _velocity _projectilemovement :!enabledstate Disabled)
  (set `MovementComponent.Velocity` (* (1.0 0.0 0.0) _velocity) _projectilemovement :!enabledstate Disabled))

(event `Fire!`
  (`ActorComponent.SetActive` (`self.ProjectileMovement`) true false))

(event `self.ReceiveHit`
  (params (MyComp :type "PrimitiveComponent Object Reference") (Other :type "Actor Object Reference") (OtherComp :type "PrimitiveComponent Object Reference") (bSelfMoved :type Boolean) (HitLocation :type "Vector Structure") (HitNormal :type "Vector Structure") (NormalImpulse :type "Vector Structure") (Hit :type "HitResult Structure (by ref)"))
  (bind _ac_weapon (`self.AC Weapon`))
  (`|ExecutionSequence`
    (:`then_0`
      (set `ProjectileMovementComponent.ProjectileGravityScale` (`self.PostHit GravityScale`) (`self.ProjectileMovement`)))
    (:`then_1`
      (`GameplayStatics.PlaySoundAtLocation` (`/Game/Characters/Player/Blueprints/WeaponSystem/Weapon/DA_Weapon_Base.Range Hit Sound` (`self.weaponData`)) HitLocation (struct) 1.0 1.0 0.0 null null null null))
    (:`then_2`
      (bind _uniq (`/Game/Characters/Player/Blueprints/WeaponSystem/Interactable/FL_Common.Add to Set Uniq` (`self.hittedActors`) Other))
      (if _uniq
        (message `/Game/Characters/Player/Blueprints/WeaponSystem/Weapon/BPI_Weapon_Hitting.Take Weapon Range Hit` Other Hit _ac_weapon (`/Game/Characters/Player/Blueprints/WeaponSystem/Weapon/AC_Weapon.Get Last AC Weapon User` _ac_weapon))))))

(fn `UserConstructionScript`)