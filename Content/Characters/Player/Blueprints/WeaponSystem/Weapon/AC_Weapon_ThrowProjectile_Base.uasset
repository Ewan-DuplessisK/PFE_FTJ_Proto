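; AC_Weapon_ThrowProjectile_Base is a base component that handles hit detection for a thrown weapon projectile.
; On BeginPlay it binds to the owner's mesh component hit event.
; While active, each hit actor is added to a unique set, and a first-time hit sends it a weapon throwing hit message with the hit result and weapon component.
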(event `self.ReceiveTick`
  (params (DeltaSeconds :type "Float (single-precision)"))
  (`parent.ReceiveTick` DeltaSeconds))

(event `self.ReceiveBeginPlay`
  (`parent.ReceiveBeginPlay`)
  (add `PrimitiveComponent.OnComponentHit` (`Actor.GetComponentByClass` (`self.GetOwner`) "/Script/Engine.MeshComponent") (delegate `OnComponentHit_Event`)))

(event `OnComponentHit_Event`
  (params (HitComponent :type "PrimitiveComponent Object Reference") (OtherActor :type "Actor Object Reference") (OtherComp :type "PrimitiveComponent Object Reference") (NormalImpulse :type "Vector Structure") (Hit :type "HitResult Structure (by ref)"))
  (if (`self.IsActive`)
    (bind _uniq (`/Game/Characters/Player/Blueprints/WeaponSystem/Interactable/FL_Common.Add to Set Uniq` (`self.hittedActors`) OtherActor))
    (if _uniq
      (message `/Game/Characters/Player/Blueprints/WeaponSystem/Weapon/BPI_Weapon_Hitting.Take Weapon Throwing Hit` OtherActor Hit (`self.AC Weapon`) null))))