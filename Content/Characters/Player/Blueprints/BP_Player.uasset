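; First-person player character with dash, stun, kick, health-costing desperation sphere and camera-shake hit reactions.
; BeginPlay copies DataAssetPlayer tuning into variables and Feel structs, and caches the PC_Systems controller used for stun UI.
; Attack, throw and weapon scrolling go through ACWeaponUser, whose pre-attack event sphere-traces ahead to warn enemies.
; Timelines drive dash FOV, stun overlay, placeholder kick animation, sphere growth and forward movement during combo hits.
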(event OnComponentBeginOverlap(Sphere_Desperation)
  (params (OverlappedComponent :type Primitive%20Component%20Object%20Reference) (OtherActor :type Actor%20Object%20Reference) (OtherComp :type Primitive%20Component%20Object%20Reference) (OtherBodyIndex :type Integer) (bFromSweep :type Boolean) (SweepResult :type Hit%20Result%20Structure%20%28by%20ref%29))
  (bind _asbp_enemy (Utilities|Casting|CastToBP_Enemy OtherActor))
  (Utilities|FlowControl|DoOnce false :!label _label
    (:Completed
      (Default|GetHit _asbp_enemy (Variables|DataAsset|GetDesperation_Damage) 0.0 (* (Math|Vector|Normalize (- (Transformation|GetActorLocation OtherActor) (Transformation|GetActorLocation))) (* (Variables|DataAsset|GetDesperation_Force) 2.0)) 0.0)
      (Utilities|FlowControl|Delay 0.2)
      (goto _label Reset))))

(event Custom|AttacksCancel
  ;[0.15 0.15 0.15 0.5] Cancel attacks
  (Variables|Punch|Count|SetAttackType "NewEnumerator0")
  (Transformation|SetRelativeTransform (Variables|Default|GetKick_PlaceHolder) (Math|Transform|MakeTransform "0.000000,-40.000000,0.000000" "0.000000,-90.000000,0.000000" "1.000000,1.000000,1.000000") false false))

(event Custom|DesperationSphere
  (bind _sphere_desperation (Variables|Default|GetSphere_Desperation))
  (bind _sphere_desperation_2 (Variables|Default|GetSphere_Desperation))
  ;[1 0 0.8901 0.5] Despe Attack
  (if (> (Variables|Default|GetCurrentHealth) (Variables|DataAsset|GetDesperation_HP_Removal))
    (Components|Sphere|SetSphereRadius _sphere_desperation_2 0.0 true)
    ;;[0.1151 1 0.001055] Sphere Visibility
    (Rendering|SetVisibility _sphere_desperation_2 true false)
    (Variables|Default|SetCurrentHealth (- (Variables|Default|GetCurrentHealth) (Variables|DataAsset|GetDesperation_HP_Removal)))
    (bind _tl_growsphere (Timeline|SphereSizeGrowth PlayFromStart)
      (:Update
        (Components|Sphere|SetSphereRadius _sphere_desperation (Math|Float|Lerp 0.0 (Variables|DataAsset|GetDesperation_Size) _tl_growsphere) true))
      (:Finished
        (Utilities|FlowControl|Delay (Variables|DataAsset|GetDesperation_Sphere_Time))
        ;;[0.1151 1 0.001055] Sphere Visibility
        (Rendering|SetVisibility _sphere_desperation false false)))))

(event Custom|GetHit
  (params (RawDamage :type Integer) (HitStunDuration :type Float%20%28double-precision%29) (KnockbackVector :type Vector) (InvincibilityTime :type Float%20%28double-precision%29))
  (bind _returnvalue (Game|GetPlayerController 0))
  (if (<= (Variables|Default|GetInvincibilityTime) 0.0)
    (Utilities|FlowControl|Sequence
      (:then_0
        (Variables|Default|SetCurrentHealth (- (Variables|Default|GetCurrentHealth) RawDamage))
        (Variables|Default|SetInvincibilityTime InvincibilityTime))
      (:then_1
        ;[0 1 1] Feedbacks (hit)
        (Game|Feedback|ClientStartCameraShake _returnvalue "/Game/VFX/Blueprint/BP_FX_CameraShake_Impact_Strong.BP_FX_CameraShake_Impact_Strong_C" 1.0 "CameraLocal" "0, 0, 0")
        (Game|Feedback|PlayDynamicForceFeedback _returnvalue 1.0 0.2 true true true true)))))

(event Custom|Pre%20Attack%20Hit%20Notify
  (bind _capsulecomponent (Variables|Default|GetCapsuleComponent))
  (bind _returnvalue (Transformation|GetWorldLocation _capsulecomponent))
  ;[0 1 0] Pre Attack Hit Notify
  (bind _outhit (Collision|SphereTraceForObjects _returnvalue (+ _returnvalue (* (Math|Vector|GetForwardVector (Transformation|GetWorldRotation _capsulecomponent)) 6.5e+02)) 75.0 (Utilities|Array|MakeArray "ObjectTypeQuery3") false (Utilities|Array|MakeArray self) "ForDuration"))
  (bind _asbp_enemy (Utilities|Casting|CastToBP_Enemy (.HitActor (Collision|BreakHitResult _outhit))))
  (Default|PreAttackHit _asbp_enemy))

(event Custom|Start%20FOV
  ;[0 1 1] FOV Change For Dash
  (if (not (Variables|Dash|FOVEffect|GetHas%20Applied%20FOV))
    (Variables|Dash|FOVEffect|SetHas%20Applied%20FOV true)
    (Variables|Dash|FOVEffect|SetOld%20FOV (Variables|/Script/Engine.CameraComponent|GetFieldOfView (Variables|Default|GetFirstPersonCameraComponent)))
    (bind (_direction _fov_alpha) (Timeline|T_FOV Play)
      (:Update
        (Camera|SetFieldOfView (Variables|Default|GetFirstPersonCameraComponent) (Math|Float|Lerp (Variables|Dash|FOVEffect|GetOld%20FOV) (Variables|DataAsset|GetDash_Fov) _fov_alpha)))
      (:Finished
        (if (Utilities|Enum|Equal(Enum) _direction "Backward")
          (Variables|Dash|FOVEffect|SetHas%20Applied%20FOV false))))))

(event Custom|StunState
  (bind _pc_systems (Variables|Refs|GetPC%20Systems))
  (bind _charactermovement (Variables|Character|GetCharacterMovement))
  (bind _stunwidget (Variables|/Game/_GameManager/PC_Systems.PC_Systems_C|GetStunWidget _pc_systems))
  ;[0.15 0.15 0.15 0.5] Stun State
  (Variables|Default|SetbCanDash false)
  (Components|Movement|StopMovementImmediately _charactermovement)
  (Variables|/Script/Engine.CharacterMovementComponent|SetMaxWalkSpeed _charactermovement 0.0)
  (bind _opacity_value (Timeline|StunState_TL PlayFromStart)
    (:Update
      (Widget|SetRenderOpacity _stunwidget 1.0)
      (Rendering|Material|SetScalarParameterValue (Variables|/Game/UI/WBP_Stun.WBP_Stun_C|GetDynamicMat _stunwidget) "Anim" _opacity_value :!class /Script/Engine.MaterialInstanceDynamic))
    (:Finished
      (Variables|/Script/Engine.CharacterMovementComponent|SetMaxWalkSpeed (Variables|Character|GetCharacterMovement) (Variables|DataAsset|GetMax_Walk_Speed%20))
      (Widget|SetRenderOpacity _stunwidget 0.0)
      (Variables|Default|SetbCanDash true))))

(event Custom|Player_DesperationAttack
  (CallFunction|DesperationSphere))

(event Custom|Stop%20FOV
  ;[0 1 1] FOV Change For Dash
  (if (Variables|Dash|FOVEffect|GetHas%20Applied%20FOV)
    (bind (_direction _fov_alpha) (Timeline|T_FOV Reverse)
      (:Update
        (Camera|SetFieldOfView (Variables|Default|GetFirstPersonCameraComponent) (Math|Float|Lerp (Variables|Dash|FOVEffect|GetOld%20FOV) (Variables|DataAsset|GetDash_Fov) _fov_alpha)))
      (:Finished
        (if (Utilities|Enum|Equal(Enum) _direction "Backward")
          (Variables|Dash|FOVEffect|SetHas%20Applied%20FOV false))))))

(event Custom|Animation%20Move%20Lock
  (params (Lock :type Boolean))
  ;[0 1 1] Feedbacks (Movement restriction during attack animations)
  (if Lock
    ;;[0.15 0.15 0.15 0.5] Temporary full lock
    (Pawn|Components|CharacterMovement|DisableMovement (Variables|Character|GetCharacterMovement))
    (else
      (Pawn|Components|CharacterMovement|SetMovementMode (Variables|Character|GetCharacterMovement) "MOVE_Walking" 0))))

(event Custom|Animation%20Auto%20Movement
  ;[0 1 1] Feedbacks (Auto move during Attacks)
  (switch int (Variables|Punch|Count|GetSuccess%20Attack%20Count)
    (:0
      (bind _newtrack_0 (Timeline|T_Hit1Move PlayFromStart)
        (:Update
          (Variables|/Script/Engine.MovementComponent|SetVelocity (Variables|Character|GetCharacterMovement) (Math|Vector|MakeVector (.x (* (Transformation|GetActorForwardVector) (* _newtrack_0 (Variables|Default|GetAttack%20Movement%20Distance)))) (.y (* (Transformation|GetActorForwardVector) (* _newtrack_0 (Variables|Default|GetAttack%20Movement%20Distance)))) (.z (Variables|/Script/Engine.MovementComponent|GetVelocity (Variables|Character|GetCharacterMovement))))))
        (:Finished
          (Development|PrintString "HIT01"))))
    (:1
      (bind _newtrack_0_2 (Timeline|T_Hit2Move PlayFromStart)
        (:Update
          (Variables|/Script/Engine.MovementComponent|SetVelocity (Variables|Character|GetCharacterMovement) (Math|Vector|MakeVector (.x (* (Transformation|GetActorForwardVector) (* _newtrack_0_2 (Variables|Default|GetAttack%20Movement%20Distance)))) (.y (* (Transformation|GetActorForwardVector) (* _newtrack_0_2 (Variables|Default|GetAttack%20Movement%20Distance)))) (.z (Variables|/Script/Engine.MovementComponent|GetVelocity (Variables|Character|GetCharacterMovement))))))
        (:Finished
          (Development|PrintString "HIT02" true true "(R=1.000000,G=0.063134,B=0.000000,A=1.000000)"))))
    (:2
      (bind _newtrack_0_3 (Timeline|Timeline PlayFromStart)
        (:Update
          (Variables|/Script/Engine.MovementComponent|SetVelocity (Variables|Character|GetCharacterMovement) (Math|Vector|MakeVector (.x (* (Transformation|GetActorForwardVector) (* _newtrack_0_3 (Variables|Default|GetAttack%20Movement%20Distance)))) (.y (* (Transformation|GetActorForwardVector) (* _newtrack_0_3 (Variables|Default|GetAttack%20Movement%20Distance)))) (.z (Variables|/Script/Engine.MovementComponent|GetVelocity (Variables|Character|GetCharacterMovement))))))
        (:Finished
          (Development|PrintString "HIT03" true true "(R=0.946139,G=0.000000,B=1.000000,A=1.000000)"))))
    (:3
      (switch Utilities|FlowControl|Switch|SwitchonE_AttackTypes (Variables|Punch|Count|GetAttackType)
        (:NewEnumerator3
          (Timeline|T_LauncherMove PlayFromStart))
        (:NewEnumerator4
          (Timeline|T_FinisherMove PlayFromStart))))))

(event Input|EnhancedActionEvents|EnhancedInputActionIA_Dash
  (params (ActionValue :type Boolean) (ElapsedSeconds :type Float%20%28double-precision%29) (TriggeredSeconds :type Float%20%28double-precision%29) (InputAction :type Input%20Action%20Object%20Reference :default "/Game/_GameManager/Inputs/Actions/IA_Dash.IA_Dash"))
  (bind _returnvalue (Class|Pawn|GetLastMovementInputVector))
  (bind _charactermovement (Variables|Character|GetCharacterMovement))
  (bind _charactermovement_2 (Variables|Character|GetCharacterMovement))
  (bind _dash_distance (Variables|DataAsset|GetDash_Distance))
  (bind _returnvalue_2 (* _dash_distance 1e+01))
  ;[1 0 0.5] Dash
  (if (Variables|Default|GetbCanDash)
    (CallFunction|AttacksCancel)
    ;[1 0 0 0.5] Debug
    (Variables|Dash|SetDashStartLocation (Transformation|GetWorldLocation (Variables|Default|GetCapsuleComponent)))
    (Variables|Dash|SetDashStartFrame (Utilities|GetFrameCount))
    (Variables|Default|SetbCanDash false)
    (Variables|Default|SetisDashing true)
    (Variables|Dash|SetOld%20Velocity (Variables|/Script/Engine.MovementComponent|GetVelocity _charactermovement))
    (Variables|Dash|SetOld%20Ground%20Friction (Variables|/Script/Engine.CharacterMovementComponent|GetGroundFriction _charactermovement))
    (Variables|/Script/Engine.CharacterMovementComponent|SetGroundFriction _charactermovement 0.0)
    (if (Math|Vector|VectorIsNearlyZero _returnvalue)
      (Variables|/Script/Engine.MovementComponent|SetVelocity _charactermovement (* (* (Transformation|GetActorForwardVector) -1.0) _returnvalue_2))
      (else
        (Variables|/Script/Engine.MovementComponent|SetVelocity _charactermovement (* (Math|Vector|Normalize _returnvalue) _returnvalue_2))))
    (CallFunction|StartFOV)
    (Utilities|FlowControl|Delay (Variables|DataAsset|GetDash_Duration))
    (CallFunction|StopFOV)
    (Variables|Default|SetisDashing false)
    (Variables|/Script/Engine.CharacterMovementComponent|SetGroundFriction _charactermovement_2 (Variables|Dash|GetOld%20Ground%20Friction))
    (Variables|/Script/Engine.MovementComponent|SetVelocity _charactermovement_2 (Variables|Dash|GetOld%20Velocity))
    ;[1 0 0 0.5] Debug
    (Development|PrintText (Utilities|Text|FormatText "Dash distance : {dis} meters; duration : {tim} frames" (/ (Math|Vector|Distance(Vector) (Transformation|GetWorldLocation (Variables|Default|GetCapsuleComponent)) (Variables|Dash|GetDashStartLocation)) 1e+02) (- (Utilities|GetFrameCount) (Variables|Dash|GetDashStartFrame))) true true "(R=0.000000,G=0.660000,B=1.000000,A=1.000000)" 5.0)
    (Utilities|FlowControl|Delay (Variables|DataAsset|GetDash_Cooldown))
    (Variables|Default|SetbCanDash true)))

(event EventBeginPlay
  (Utilities|FlowControl|Sequence
    (:then_0
      (CallFunction|WeaponBeginPlay))
    (:then_1
      (DataAsset|SetDataAsset)
      (DataAsset|ApplyModifDataAsset))
    (:then_2
      (Variables|Default|SetCurrentHealth (Variables|DataAsset|GetMax_HP))
      (bind _aspc_systems (Utilities|Casting|CastToPC_Systems (Pawn|GetController)))
      (Variables|Refs|SetPC%20Systems _aspc_systems))
    (:then_3
      (Camera|SetFieldOfView (Variables|Default|GetFirstPersonCameraComponent) (Variables|DataAsset|GetCurrent_Fov)))))

(event EventKickFeedback
  (params (Location :type Vector :default "0, 0, 0") (HitEnemy :type Actor%20Object%20Reference))
  ;[0 1 1 0.5] Kick Feedback
  (Game|Feedback|ClientPlayForceFeedback (Game|GetPlayerController 0) "/Game/_GameManager/Feedbacks/FFB_Kick.FFB_Kick" "None" false false false)
  (Utilities|IsValid HitEnemy
    (:Is%20Valid
      (bind _asbp_enemy (Utilities|Casting|CastToBP_Enemy HitEnemy))
      (Class|EnemyBase|Kicked _asbp_enemy (* (Transformation|GetActorForwardVector) (.x (.KickForce (Utilities|Struct|BreakUCombatFeel (Variables|Default|GetCombatFeel))))) (Transformation|GetActorLocation)))
    (:Is%20Not%20Valid
      _))
  (Components|Timeline|SetPlayRate (Variables|Default|GetT_Kick) (/ 1.0 (Variables|Kick|GetKickAnimDuration)))
  (Utilities|FlowControl|DelayUntilNextTick)
  (bind (_direction _kick_length_transition _kick_rotate_transition) (Timeline|T_Kick PlayFromStart)
    (:Update
      (Transformation|SetRelativeScale3D (Variables|Default|GetKick_PlaceHolder) (Math|Vector|MakeVector 1.0 1.0 (Math|Float|Lerp 1.0 (/ (Math|Vector|Distance(Vector) Location (Transformation|GetActorLocation)) 95.0) _kick_length_transition)))
      (bind _result (Math|Float|NegateFloat (Math|Float|Lerp 0.0 (+ (.pitch (Transformation|GetWorldRotation (Variables|Default|GetFirstPersonCameraComponent))) 1e+02) _kick_rotate_transition))
        (:%20%20
          (Transformation|SetRelativeRotation (Variables|Default|GetKick_PlaceHolder) (Math|Rotator|MakeRotator _result 0.0 -9e+01) false false))))))

(event EventTick
  (params (DeltaSeconds :type Float%20%28single-precision%29)))

(event Input|KeyboardEvents|DebugKeyU
  (params (Key :type Key%20Structure) (ActionValue :type Input%20Action%20Value%20Structure))
  (:Pressed
    (CallFunction|StunState)))

(event Custom|Player_HitFinisher
  (bind _ac_weapon_user (Variables|Default|GetAC_Weapon_User))
  ;[0.15 0.15 0.15 0.5] Attacks
  (Default|IAAttackStarted _ac_weapon_user false)
  ;;[0.15 0.15 0.15 0.5] move to AC WUSER
  (Variables|Punch|Count|SetAttackType (Variables|/Game/Characters/Player/Blueprints/WeaponSystem/Weapon/AC_Weapon_User.AC_Weapon_User_C|GetCombo%20Attack%20Type _ac_weapon_user))
  (Variables|Weapons|SetAttackingMelee%20Anim (.attackanimation (Variables|/Game/Characters/Player/Blueprints/WeaponSystem/Weapon/AC_Weapon_User.AC_Weapon_User_C|GetCombo%20Attack%20Info _ac_weapon_user))))

(event Custom|Player_Launcher
  (bind _ac_weapon_user (Variables|Default|GetAC_Weapon_User))
  ;[0.15 0.15 0.15 0.5] Attacks
  (Default|IAAttackStarted _ac_weapon_user true)
  ;;[0.15 0.15 0.15 0.5] move to AC WUSER
  (Variables|Punch|Count|SetAttackType (Variables|/Game/Characters/Player/Blueprints/WeaponSystem/Weapon/AC_Weapon_User.AC_Weapon_User_C|GetCombo%20Attack%20Type _ac_weapon_user))
  (Variables|Weapons|SetAttackingMelee%20Anim (.attackanimation (Variables|/Game/Characters/Player/Blueprints/WeaponSystem/Weapon/AC_Weapon_User.AC_Weapon_User_C|GetCombo%20Attack%20Info _ac_weapon_user))))

(event Custom|WeaponScroll
  (params (ActionValue :type Float%20%28double-precision%29))
  ;[0.15 0.15 0.15 0.5] Weapon Scroll
  (Default|ScrollWeaponSlot (Variables|Default|GetAC_Weapon_User) (Math|Float|Truncate ActionValue)))

(event Custom|Player_Throw_Start
  ;[0.15 0.15 0.15 0.5] Throw
  (Default|IAAimingStart (Variables|Default|GetAC_Weapon_User)))

(event Custom|Player_Throw_End
  (bind _ac_weapon_user (Variables|Default|GetAC_Weapon_User))
  ;[0.15 0.15 0.15 0.5] Throw
  (Default|IAThrow _ac_weapon_user)
  (Default|IAAimEnd _ac_weapon_user))

(event Custom|Weapon%20Begin%20Play
  ;[0.15 0.15 0.15 0.5] Attacks
  (EventDispatchers|AssignOnAttackPre (Variables|Default|GetAC_Weapon_User) (delegate Custom|OnAttackPre_Event)))

(event Custom|OnAttackPre_Event
  (params (AC%20Weapon :type AC%20Weapon%20Object%20Reference))
  ;[0.15 0.15 0.15 0.5] Attacks
  (CallFunction|PreAttackHitNotify))

(fn ConstructionScript)

(fn SetSpeed/Accel/RotaRate
  (params (Max%20Walk%20Speed :type Float%20%28double-precision%29) (Max%20Acceleration :type Float%20%28double-precision%29) (Rotation%20Rate :type Rotator))
  (bind _charactermovement (Variables|Character|GetCharacterMovement))
  (Variables|/Script/Engine.CharacterMovementComponent|SetMaxWalkSpeed _charactermovement Max%20Walk%20Speed)
  (Variables|/Script/Engine.CharacterMovementComponent|SetMaxAcceleration _charactermovement Max%20Acceleration)
  (Variables|/Script/Engine.CharacterMovementComponent|SetRotationRate _charactermovement Rotation%20Rate))

(fn SetDataAsset
  (bind _data_asset_player (Variables|DataAsset|GetData_Asset_Player))
  (bind _data_asset_player_2 (Variables|DataAsset|GetData_Asset_Player))
  (Utilities|FlowControl|Sequence
    (:then_0
      (Variables|DataAsset|SetPlayer_State (Variables|/Game/_GameManager/Data_Assets/Data_3C/PDA_Player.PDA_Player_C|GetPlayer_State _data_asset_player_2))
      (bind _output_get (Variables|DataAsset|SetMax_HP (Variables|/Game/_GameManager/Data_Assets/Data_3C/PDA_Player.PDA_Player_C|GetMax_HP _data_asset_player_2)))
      (Variables|DataAsset|SetCurrentHP _output_get)
      (Variables|DataAsset|SetCurrent_Fov (Variables|/Game/_GameManager/Data_Assets/Data_3C/PDA_Player.PDA_Player_C|GetCurrent_FOV _data_asset_player_2))
      (bind _output_get_2 (Variables|/Script/Engine.CharacterMovementComponent|SetMaxWalkSpeed (Variables|Character|GetCharacterMovement) (Variables|/Game/_GameManager/Data_Assets/Data_3C/PDA_Player.PDA_Player_C|GetMax_Walk_Speed _data_asset_player_2)))
      (Variables|DataAsset|SetMax_Walk_Speed%20 _output_get_2)
      (Variables|DataAsset|SetMin_Walk_Speed%20 (Variables|/Game/_GameManager/Data_Assets/Data_3C/PDA_Player.PDA_Player_C|GetMin_Walk_Speed _data_asset_player_2))
      (Variables|DataAsset|SetKick_Length (Variables|/Game/_GameManager/Data_Assets/Data_3C/PDA_Player.PDA_Player_C|GetKick_Length _data_asset_player_2))
      (Variables|DataAsset|SetKick_Force (Variables|/Game/_GameManager/Data_Assets/Data_3C/PDA_Player.PDA_Player_C|GetKick_Force _data_asset_player_2)))
    (:then_1
      (Variables|DataAsset|SetKick_Damage (Variables|/Game/_GameManager/Data_Assets/Data_3C/PDA_Player.PDA_Player_C|GetKick_Damage _data_asset_player))
      (Variables|DataAsset|SetDash_Distance (Variables|/Game/_GameManager/Data_Assets/Data_3C/PDA_Player.PDA_Player_C|GetDash_Distance _data_asset_player))
      (Variables|DataAsset|SetDash_Fov (Variables|/Game/_GameManager/Data_Assets/Data_3C/PDA_Player.PDA_Player_C|GetDash_FOV _data_asset_player))
      (Variables|DataAsset|SetDash_Duration (Variables|/Game/_GameManager/Data_Assets/Data_3C/PDA_Player.PDA_Player_C|GetDash_Duration _data_asset_player))
      (Variables|DataAsset|SetDash_Cooldown (Variables|/Game/_GameManager/Data_Assets/Data_3C/PDA_Player.PDA_Player_C|GetDash_Cooldown _data_asset_player))
      (Variables|DataAsset|SetDesperation_Size (Variables|/Game/_GameManager/Data_Assets/Data_3C/PDA_Player.PDA_Player_C|GetDesperation_Size _data_asset_player))
      (Variables|DataAsset|SetDesperation_Sphere_Time (Variables|/Game/_GameManager/Data_Assets/Data_3C/PDA_Player.PDA_Player_C|GetDesperation_Sphere_Time_Activated _data_asset_player))
      (Variables|DataAsset|SetDesperation_Force (Variables|/Game/_GameManager/Data_Assets/Data_3C/PDA_Player.PDA_Player_C|GetDesperation_Force _data_asset_player))
      (Variables|DataAsset|SetDesperation_Damage (Variables|/Game/_GameManager/Data_Assets/Data_3C/PDA_Player.PDA_Player_C|GetDesperation_Damage _data_asset_player))
      (Variables|DataAsset|SetDesperation_HP_Removal (Variables|/Game/_GameManager/Data_Assets/Data_3C/PDA_Player.PDA_Player_C|GetDesperation_HP_Removal _data_asset_player)))
    (:then_2
      (Variables|DataAsset|SetCamera_Invert (Variables|/Game/_GameManager/Data_Assets/Data_3C/PDA_Player.PDA_Player_C|GetCamera_Invert _data_asset_player))
      (Variables|DataAsset|SetCamera_Horizontal_Speed (Variables|/Game/_GameManager/Data_Assets/Data_3C/PDA_Player.PDA_Player_C|GetCamera_Horizontal_Speed _data_asset_player))
      (Variables|DataAsset|SetCamera_Vertical_Speed (Variables|/Game/_GameManager/Data_Assets/Data_3C/PDA_Player.PDA_Player_C|GetCamera_Vertical_Speed _data_asset_player))
      (Variables|DataAsset|SetCamera_View_Pitch_Min (Variables|/Game/_GameManager/Data_Assets/Data_3C/PDA_Player.PDA_Player_C|GetCamera_View_Pitch_Min _data_asset_player))
      (Variables|DataAsset|SetCamera_View_Pitch_Max (Variables|/Game/_GameManager/Data_Assets/Data_3C/PDA_Player.PDA_Player_C|GetCamera_View_Pitch_Max _data_asset_player)))))

(fn GetIsThrowing?
  (return (Variables|/Game/Characters/Player/Blueprints/WeaponSystem/Weapon/AC_Weapon_User.AC_Weapon_User_C|GetIs%20Throwing (Variables|Default|GetAC_Weapon_User))))

(fn GetWeaponUser
  (return (Variables|Default|GetAC_Weapon_User)))

(fn ApplyModifDataAsset
  (Utilities|FlowControl|Sequence
    (:then_0
      (Utilities|Struct|SetmembersinUPlayerFeel (Variables|Default|GetPlayerFeel) (Variables|DataAsset|GetMax_Walk_Speed%20)))
    (:then_1
      (Utilities|Struct|SetmembersinUCombatFeel (Variables|Default|GetCombatFeel) (Variables|DataAsset|GetKick_Force) (Variables|DataAsset|GetKick_Length) (Variables|DataAsset|GetKick_Damage)))
    (:then_2
      (Utilities|Struct|SetmembersinUCameraFeel (Variables|Default|GetCameraFeel) (Variables|DataAsset|GetCurrent_Fov) (Variables|DataAsset|GetDash_Fov) (Variables|DataAsset|GetCamera_Invert) (Variables|DataAsset|GetCamera_Horizontal_Speed) (Variables|DataAsset|GetCamera_Vertical_Speed) (Variables|DataAsset|GetCamera_View_Pitch_Min) (Variables|DataAsset|GetCamera_View_Pitch_Max)))))