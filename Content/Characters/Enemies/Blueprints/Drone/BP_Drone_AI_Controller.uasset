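; AI controller for the drone enemy that starts the BT_Drone behavior tree on BeginPlay.
; RotatetoTarget uses a timeline to lerp its own rotation toward a target along the shortest path, with pitch zeroed.
; Timeline play rate is rotation speed divided by the initial yaw difference, so larger turns take longer.
; When the timeline finishes, it calls OnRotatedToTarget with the target.
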(event `self.ReceiveBeginPlay`
  (`self.RunBehaviorTree` "/Game/Characters/Enemies/Blueprints/Drone/BT_Drone.BT_Drone"))

(event `Rotate to Target`
  (params (Target :type "Actor Object Reference"))
  (bind _returnvalue (`self.K2_GetActorRotation`))
  (bind _rotator (`/Game/BPs/Other/FL_Common.Get Direction` self Target))
  (bind (_returnvalue_roll _returnvalue_pitch _returnvalue_yaw) (`KismetMathLibrary.BreakRotator` (`KismetMathLibrary.NormalizedDeltaRotator` _returnvalue _rotator)))
  ; time
  (`TimelineComponent.SetPlayRate` (`self.Timeline`) (/ (`self.Rotate To Target Speed`) (`KismetMathLibrary.Abs` _returnvalue_yaw)))
  ; anim
  (bind (_direction _newtrack_0) (`Timeline|Timeline` :!via `PlayFromStart`)
    (:`Update`
      (`self.K2_SetActorRotation` (`KismetMathLibrary.RLerp` (`KismetMathLibrary.MakeRotator` (.roll _returnvalue) 0.0 (.yaw _returnvalue)) (`KismetMathLibrary.MakeRotator` (.roll _rotator) 0.0 (.yaw _rotator)) _newtrack_0 true)))
    (:`Finished`
      (`self.On Rotated To Target` Target))))

(fn `UserConstructionScript`)