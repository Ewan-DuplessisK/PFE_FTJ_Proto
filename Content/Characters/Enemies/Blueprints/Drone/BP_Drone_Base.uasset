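; Base drone enemy that patrols a spline, arms itself with suckable props and launches them at the player.
; A looping timer feeds the closest-first, line-of-sight prop search into the Blackboard, while AI perception supplies the player target.
; Grabbed props attach to the muzzle socket until a montage notify fires them with predicted, slightly randomized velocity.
; Hits set stun time and flash the material; stun or death drops the prop.
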(event `Possees`
  (`PlayerController.SetViewTargetWithBlend` (`GameplayStatics.GetPlayerController` 0) self 0.0 "VTBlend_Linear" 0.0 false))

(event `self.ReceiveBeginPlay`
  (`self.Init Vars`)
  (bind _returnvalue (`KismetSystemLibrary.K2_SetTimerDelegate` (delegate `Find Armable Prop - LOOP`) 0.2 true))
  (set `self.Find Armable Timer` _returnvalue)
  (add `self.On Stunned` (delegate `On Stunned_Event`))
  (bind _returnvalue_2 (`PrimitiveComponent.CreateDynamicMaterialInstance` (`self.Mesh`) 0 null "None"))
  (set `self.Dynamic Material` _returnvalue_2))

(event `On Stunned_Event` :!signature `self.On Stunned`
  (params (Phase :type "Float (double-precision)"))
  (`self.Drop Armed`))

(event `Attack Target`
  (params (Target :type "Actor Object Reference"))
  (`self.Rotate to Target` Target)
  (`TimelineComponent.SetTimelineFinishedFunc` (`self.Timeline`) (delegate `On Rotate To Target_Event`)))

(event `On Rotate To Target_Event`
  (`self.Shoot` null))

(event `Rotate to Target`
  (params (Target :type "Actor Object Reference"))
  (bind _returnvalue (`self.K2_GetActorRotation`))
  (bind _rotator (`/Game/BPs/Other/FL_Common.Get Direction` self Target))
  (bind (_returnvalue_roll _returnvalue_pitch _returnvalue_yaw) (`KismetMathLibrary.BreakRotator` (`KismetMathLibrary.NormalizedDeltaRotator` _returnvalue _rotator)))
  ; time
  (`TimelineComponent.SetPlayRate` (`self.Timeline`) (/ (`self.Rotate To Target Speed`) (`KismetMathLibrary.Abs` _returnvalue_yaw)))
  ; anim
  (bind (_direction _newtrack_0) (`Timeline|Timeline` :!via `PlayFromStart`)
    (:`Update`
      (`self.K2_SetActorRotation` (`KismetMathLibrary.RLerp` (`KismetMathLibrary.MakeRotator` (.roll _returnvalue) 0.0 (.yaw _returnvalue)) (`KismetMathLibrary.MakeRotator` (.roll _rotator) 0.0 (.yaw _rotator)) _newtrack_0 true)))
    (:`Finished`
      (`self.On Rotated To Target` Target))))

(event `Find Armable Prop - LOOP`
  (bind _actor (`self.Find ArmableProp`))
  ; Find Armable Prop - LOOP (TODO: remake async task)
  (`self.Has Armed Prop`
    (:`No`
      (`/Engine/EditorBlueprintResources/StandardMacros.IsValid` _actor
        (:`Is Valid`
          _)
        (:`Is Not Valid`
          _))
      (`BlackboardComponent.SetValueAsObject` (`self.Blackboard`) "Found Armable Prop" _actor))))

(event `self.AIPerception.OnTargetPerceptionUpdated`
  (params (Actor :type "Actor Object Reference") (Stimulus :type "AIStimulus Structure"))
  (bind (_age _expirationage _strength _stimuluslocation _receiverlocation _tag _bsuccessfullysensed) (break `AIStimulus` Stimulus))
  (`/Game/BPs/Other/ML_Object.If is Player` Actor
    (:`Yes`
      (`BlackboardComponent.SetValueAsObject` (`self.Blackboard`) "Target to Attack" (`KismetMathLibrary.SelectObject` Actor null _bsuccessfullysensed))
      (`KismetSystemLibrary.PrintString` (`KismetStringLibrary.Concat_StrStr` "Sensed: " (`KismetStringLibrary.Conv_BoolToString` _bsuccessfullysensed))))))

(event `Shoot`
  (params (TargetActor :type "Actor Object Reference"))
  (bind _armedprop (`self.ArmedProp`))
  (`AIController.K2_SetFocus` (`self.AI`) TargetActor)
  (`|PlayMontage` (`self.Mesh`) "/Game/Characters/Enemies/Meshes/Drone/Animations/AS_Drone_Anim_Attack_Montage.AS_Drone_Anim_Attack_Montage" 1.0 0.0 "None"
    (:`then`
      (`self.On Attack` TargetActor -1.0))
    (:`OnCompleted`
      (`self.On Attack` null 1.0))
    (:`OnNotifyBegin`
      (`self.On Attack` TargetActor)
      (bind _outlaunchvelocity (`GameplayStatics.SuggestProjectileVelocity_MovingTarget` (`SceneComponent.K2_GetComponentLocation` (`SuckablePropParent.StaticMeshComp` (`self.ArmedProp`))) TargetActor (0.0 0.0 0.0) 0.0 (`KismetMathLibrary.RandomFloatInRange` 0.3 0.7) "None"))
      (`self.K2_DetachFromActor` _armedprop "KeepRelative" "KeepRelative" "KeepRelative")
      (`/Game/BPs/VacuumProps/BP_SuckableProp.SetReadyToShootAsEnemy` _armedprop)
      (`PrimitiveComponent.SetPhysicsLinearVelocity` (`SuckablePropParent.StaticMeshComp` _armedprop) (+ _outlaunchvelocity (`KismetMathLibrary.RandomUnitVectorInConeInDegrees` _outlaunchvelocity 2.0)) false "None")
      (set `SuckablePropParent.Damage` (`self.Damage`) (`self.ArmedProp`))
      (set `self.ArmedProp` null)
      (`BlackboardComponent.SetValueAsBool` (`self.Blackboard`) "Has Armed Prop" false)
      (`AIController.K2_ClearFocus` (`self.AI`)))))

(event `/Game/Characters/Enemies/Blueprints/Drone/BPI_Bot.On Stance Change`
  (params (Stance :type "/Game/Characters/Enemies/Blueprints/Drone/E_Bot_Stance Enum" :default "NewEnumerator3") (Value :type "Float (double-precision)"))
  ; draft
  (switch `/Game/Characters/Enemies/Blueprints/Drone/E_Bot_Stance` Stance
    (:`NewEnumerator6`
      (`self.Drop Armed`))))

(event `HitInterface.GetHit`
  (params (Damage :type "Float (single-precision)") (HitStunDuration :type "Float (single-precision)") (KnockbackVector :type "Vector Structure") (InvincibilityTime :type "Float (single-precision)") (SourceActor :type "Actor Object Reference"))
  (`BlackboardComponent.SetValueAsFloat` (`self.Blackboard`) "Is Stunned" (+ (`KismetSystemLibrary.GetGameTimeInSeconds`) (`self.Stun Duration`)))
  (`HealthInterface.RemoveHealth` Damage)
  (`self.On Take Damage`)
  (`self.Feedback Shader`))

(event `Feedback Shader`
  (bind (_direction _newtrack_0) (`Timeline|TL_Hit_ShaderAnim` :!via `PlayFromStart`)
    (:`Update`
      (`MaterialInstanceDynamic.SetScalarParameterValue` (`self.Dynamic Material`) "Emissive_Hit" _newtrack_0))))

(event `self.ReceiveEndPlay`
  (params (EndPlayReason :type "EEndPlayReason Enum" :default "Destroyed")))

(event `HealthInterface.RemoveHealth`
  (params (Damage :type "Float (single-precision)") (EnemyRef :type "Actor Object Reference"))
  (bind _output_get (set `self.CurrentHealth` (- (`self.CurrentHealth`) Damage)))
  (if (<= _output_get 0.0)
    (`self.Drop Armed`)
    (bind _armedprop (`self.ArmedProp`)
      (:`then`
        (`SuckablePropParent.WakeUp` _armedprop)
        (set `self.ArmedProp` null))
      (:`else`
        _))
    (`KismetSystemLibrary.K2_ClearAndInvalidateTimerHandle` (`self.Find Armable Timer`))
    (`KismetSystemLibrary.Delay` 0.2)
    (`self.K2_DestroyActor`)))

(fn `Arm ArmableProp`
  (params (`Armed Prop` :type "SuckablePropParent Object Reference"))
  (`self.K2_SetActorRelativeTransform` `Armed Prop` (`self.Arming Transform`) false true)
  (`self.K2_AttachToComponent` `Armed Prop` (`self.Mesh`) "MuzzleSocket" "KeepRelative" "KeepRelative" "KeepRelative" true)
  (bind _output_get (set `self.ArmedProp` `Armed Prop`))
  (`/Game/BPs/VacuumProps/BP_SuckableProp.Sleep` _output_get)
  (`SuckablePropParent.SetHoldingActor` _output_get self)
  (`BlackboardComponent.SetValueAsObject` (`self.Blackboard`) "Found Armable Prop" null)
  (`BlackboardComponent.SetValueAsBool` (`self.Blackboard`) "Has Armed Prop" true))

(fn `Drop Armed`
  (bind _armedprop (`self.ArmedProp`))
  (`/Engine/EditorBlueprintResources/StandardMacros.IsValid` _armedprop
    (:`Is Valid`
      (`self.K2_DetachFromActor` _armedprop "KeepWorld" "KeepWorld" "KeepWorld")
      (set `SuckablePropParent.HoldingActor` null _armedprop)
      (set `SuckablePropParent.EnemyAttack` false _armedprop)
      (`/Game/BPs/VacuumProps/BP_SuckableProp.WakeUp` _armedprop)
      (set `self.ArmedProp` null)
      (`BlackboardComponent.SetValueAsBool` (`self.Blackboard`) "Has Armed Prop" false))))

(fn `Find ArmableProp`
  (returns (Actor :type "Actor Object Reference"))
  (bind _returnvalue (`self.K2_GetActorLocation`))
  (bind (_outhits _returnvalue_2) (`KismetSystemLibrary.SphereTraceMultiForObjects` _returnvalue _returnvalue (`self.Sight Radius`) (`|MakeArray` "ObjectTypeQuery23" :!type "EObjectTypeQuery Enum")))
  (if _returnvalue_2
    (bind (_outarray _returnvalue_3) (`StaticFunctions.SortHitsByDistance` _outhits))
    (for _array_element _returnvalue_3
      (bind (_bblockinghit _binitialoverlap _time _distance _location _impactpoint _normal _impactnormal _physmat _hitactor) (`GameplayStatics.BreakHitResult` _array_element))
      (bind (_outhit _returnvalue_4) (`KismetSystemLibrary.LineTraceSingleForObjects` (`self.K2_GetActorLocation`) _location (`|MakeArray` "ObjectTypeQuery1" "ObjectTypeQuery2" :!type "EObjectTypeQuery Enum") false (`|MakeArray` _hitactor) "ForDuration"))
      (if (not _returnvalue_4)
        (break)))
    (return _hitactor)
    (else
      (return null))))

(fn `Grab ArmableProp`
  (params (Armable :type "Actor Object Reference"))
  (bind _assuckable_prop_parent (cast `SuckablePropParent` Armable))
  (`self.Arm ArmableProp` _assuckable_prop_parent)
  (`BlackboardComponent.SetValueAsBool` (`self.Blackboard`) "Has Armed Prop" true))

(fn `Init Vars`
  (bind _spline_to_patrol (`self.Spline to Patrol`))
  (bind _returnvalue (`AIBlueprintHelperLibrary.GetAIController` (`self.GetController`)))
  (set `self.AI` _returnvalue)
  (set `self.Blackboard` (`AIBlueprintHelperLibrary.GetBlackboard` _returnvalue))
  (`BlackboardComponent.SetValueAsObject` (`self.Blackboard`) "Spline to Patrol" _spline_to_patrol)
  (`self.Set Closest Spline If Missing`)
  (set `/Game/BPs/AC_PatrolAlongSpline.Patrol Spline` _spline_to_patrol (`self.AC_PatrolAlongSpline`))
  (`BlackboardComponent.SetValueAsFloat` (`self.Blackboard`) "Attack Cooldown" (`self.Attack Cooldown`)))

(fn `Search for ArmableProp3`
  (returns (`Moving to Armable` :type Boolean))
  (bind _returnvalue (`self.K2_GetActorLocation`))
  (`|ExecutionSequence`
    (:`then_1`
      (bind (_outhit _returnvalue_2) (`KismetSystemLibrary.SphereTraceSingleForObjects` _returnvalue _returnvalue (`self.Sight Radius`) (`|MakeArray` "ObjectTypeQuery13" :!type "EObjectTypeQuery Enum")))
      (if _returnvalue_2
        (bind _returnvalue_3 (`AIController.MoveToLocation` (`self.AI`) (+ (`self.K2_GetActorLocation` (`.HitActor` (`GameplayStatics.BreakHitResult` _outhit))) (0.0 0.0 100.0)) -1.0 true false false false null false))
        (switch `EPathFollowingRequestResult` _returnvalue_3
          (:`Failed`
            (return false))
          (:`AlreadyAtGoal`
            (`self.Grab ArmableProp` null))
          (:`RequestSuccessful`
            (return true)))
        (else
          (return false))))))

(fn `Set Closest Spline If Missing`
  (`self.Spline to Patrol`
    (:`then`)
    (:`else`
      (bind _outactors (`GameplayStatics.GetAllActorsOfClass` "/Game/Characters/Enemies/Blueprints/BP_PatrolSpline.BP_PatrolSpline_C"))
      (if (`KismetArrayLibrary.Array_IsNotEmpty` _outactors)
        (bind _closest (`/Game/BPs/Other/FL_Common.Find Closest Actor` _outactors (`self.K2_GetActorLocation`) 1000.0))
        (bind _asbp_patrol_spline (cast `/Game/Characters/Enemies/Blueprints/BP_PatrolSpline` _closest)
          (:`then`
            (set `self.Spline to Patrol` _asbp_patrol_spline))
          (:`CastFailed`
            (`KismetSystemLibrary.PrintText` (`|FormatText` "!!! {n} doesnt have BP_PatrolSpline" (`KismetSystemLibrary.GetDisplayName` self)) :!label _label)))
        (else
          (goto _label))))))

(fn `Spawn ArmableProp`
  (returns (Armable :type "SuckablePropParent Object Reference"))
  (bind _returnvalue (`|SpawnActorFromClass` "/Game/BPs/VacuumProps/BP_SuckableProp.BP_SuckableProp_C" (`KismetMathLibrary.MakeTransform` (0.0 0.0 0.0)) "AdjustIfPossibleButAlwaysSpawn" "OverrideRootScale" self null))
  (return _returnvalue))

(fn `UserConstructionScript`)