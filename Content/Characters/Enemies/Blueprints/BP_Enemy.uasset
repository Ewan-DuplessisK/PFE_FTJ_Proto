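; Pooled enemy character, tuned from DT_Enemy, that competes for space around the player through a combat grid.
; Looping timers claim approach slots, sometimes displacing other creatures, and randomly choose between guarding and requesting an attack slot.
; Attack only traces toward the player, without applying damage.
; Hits trigger knockback and feedback, pre-attack signals can trigger an evade dash whose chance rises after each failure, and death returns it to the pool.
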(event `self.ReceiveBeginPlay`
  (`|ExecutionSequence`
    (:`then_0`
      (bind _asaic_fthis_job (cast `/Game/_GameManager/AIC_FThisJob` (`self.GetController`)))
      (set `self.AIControllerRef` _asaic_fthis_job)
      (`KismetSystemLibrary.DelayUntilNextTick`)
      (set `self.Player` (cast `/Game/Characters/Player/Blueprints/BP_Player` (`GameplayStatics.GetPlayerCharacter` 0) :!pure true))
      (`self.Set Values from DataTable`)
      (set `self.PlayerGrid` (`/Game/Characters/Player/Blueprints/BP_Player.BP_CombatManager_Grid_SC` (`self.Player`)))
      (bind _returnvalue (`GameplayStatics.GetActorOfClass` "/Game/_GameManager/Pooling_Manager/BP_Pooling_Manager.BP_Pooling_Manager_C"))
      (`/Engine/EditorBlueprintResources/StandardMacros.IsValid` _returnvalue
        (:`Is Valid`
          (bind _output_get (set `self.Pool` _returnvalue))
          (bind _output_get_2 (set `self.EmptyGoal` (`self.K2_GetActorLocation` _output_get)))
          (set `self.Goal` _output_get_2)
          (`self.UpdatePosition`)
          (`self.Start Timers`)
          (set `self.Dodge Chance Current` (`self.DodgeChance`)))
        (:`Is Not Valid`
          (`KismetSystemLibrary.PrintString` "BP_Enemy couldn't get a valid BP_PoolingManager" true true (struct :`R` 1.0 :`A` 1.0) 20.0))))
    (:`then_1`
      (bind _outactors (`GameplayStatics.GetAllActorsOfClass` "/Script/BlockoutToolsPlugin.BlockoutToolsParent"))
      (set `self.Blockout ref` (`|GetArrayItem` _outactors)))))

(event `self.ReceiveTick`
  (params (DeltaSeconds :type "Float (single-precision)"))
  (bind _invincibilitytime (`self.InvincibilityTime`))
  (bind _getupdelaycurrent (`self.GetUpDelayCurrent`))
  (`|ExecutionSequence`
    (:`then_0`
      (if (> _getupdelaycurrent 0.0)
        (bind _output_get (set `self.GetUpDelayCurrent` (- _getupdelaycurrent DeltaSeconds)))
        (if (<= _output_get 0.0)
          (set `self.CanGetUp` true))))
    (:`then_1`
      (if (> _invincibilitytime 0.0)
        (bind _output_get_2 (set `self.InvincibilityTime` (- _invincibilitytime DeltaSeconds)))
        (if (<= _output_get_2 0.0)
          (set `self.CanBeDamaged` true))))))

(event `/Game/Characters/Player/Blueprints/WeaponSystem/Weapon/BPI_Weapon_Hitting.Take Weapon Melee Hit`
  (params (Hit :type "HitResult Structure") (`AC Weapon` :type "/Game/Characters/Player/Blueprints/WeaponSystem/Weapon/AC_Weapon Object Reference") (`AC Weapon User` :type "/Game/Characters/Player/Blueprints/WeaponSystem/Weapon/AC_Weapon_User Object Reference"))
  (bind _returnvalue (`self.K2_GetActorLocation`))
  (bind _returnvalue_2 (`GameplayStatics.GetPlayerController` 0))
  (bind _data_asset (`/Game/Characters/Player/Blueprints/WeaponSystem/Weapon/AC_Weapon.Data Asset` `AC Weapon`))
  ; Get Hit
  (`|ExecutionSequence`
    (:`then_0`
      (bind _output_get (set `self.HitType` (`/Game/Characters/Player/Blueprints/BP_Player.AttackType` (`self.Player`))))
      (if (`|EnumEquality` _output_get "NewEnumerator3")
        (set `self.GetUpDelayCurrent` (`self.GetUpDelayBase`))
        (set `self.CanGetUp` false))
      (`self.GetHit` (`/Game/Characters/Player/Blueprints/WeaponSystem/Weapon/DA_Weapon_Base.Damage` _data_asset) 0.0 (* (`self.GetActorForwardVector` (`ActorComponent.GetOwner` `AC Weapon User`)) (`/Game/Characters/Player/Blueprints/WeaponSystem/Weapon/DA_Weapon_Base.Melee Impulse` _data_asset))))
    (:`then_1`
      ;;[0 1 1] Feedbacks (hit melee)
      (`PlayerController.ClientStartCameraShake` :`self` _returnvalue_2 :`Shake` "/Game/VFX/Blueprint/BP_FX_CameraShake_Impact_Strong.BP_FX_CameraShake_Impact_Strong_C")
      (`|ExecutionSequence`
        (:`then_0`
          (`PlayerController.PlayDynamicForceFeedback` _returnvalue_2 1.0 0.2 true true true true))
        (:`then_1`
          (bind _returnvalue_3 (`NiagaraFunctionLibrary.SpawnSystemAtLocation` "/Game/VFX/Niagara/Text/NS_Text_BONK.NS_Text_BONK" (+ _returnvalue (* (- _returnvalue (`self.K2_GetActorLocation` (`ActorComponent.GetOwner` `AC Weapon User`))) 0.25))))
          (`KismetSystemLibrary.Delay` 0.7)
          (`ActorComponent.K2_DestroyComponent` _returnvalue_3))))))

(event `self.GetHit`
  (params (Damage :type "Float (single-precision)") (HitStunDuration :type "Float (single-precision)") (KnockbackVector :type "Vector Structure") (InvincibilityTime :type "Float (single-precision)") (SourceActor :type "Actor Object Reference"))
  ; Get Hit
  (if (<= (`self.InvincibilityTime`) 0.0)
    (if (`self.IsGuarding?`)
      (`|ExecutionSequence`
        (:`then_0`
          ;;[1 0 0] Change for something controllable
          (`self.LaunchCharacter` (* KnockbackVector 0.5))
          (`FTJ_CombatManager_Creature.TryDeregisterAttack` (`self.Creature`) (`self.PlayerGrid`) :!label _label)
          (set `self.IsAttacking?` false)
          (set `self.CanAct` false)
          (if (<= (`FTJ_CharaBase.CurrentHealth` (`self.Player`)) 0.0)
            (`self.Death`)))
        (:`then_1`
          ;;[0 1 1] Feedbacks (guard)
          (`GameplayStatics.PlaySoundAtLocation` "/Game/_GameManager/Feedbacks/Sounds/A_Hurt_Enemy_5_Cue.A_Hurt_Enemy_5_Cue" (`self.K2_GetActorLocation`) (struct) 1.0 1.0 0.0 null null null null)))
      (else
        (set `FTJ_CharaBase.CurrentHealth` (- (`self.CurrentHealth`) Damage) (`self.Player`))
        (set `self.InvincibilityTime` InvincibilityTime)
        (`|ExecutionSequence`
          (:`then_0`
            (`self.LaunchCharacter` KnockbackVector)
            (goto _label))
          (:`then_1`
            ;;[0 1 1] Feedbacks (hurt)
            (`GameplayStatics.PlaySoundAtLocation` "/Game/_GameManager/Feedbacks/Sounds/A_Hurt_Enemy_5_Cue.A_Hurt_Enemy_5_Cue" (`self.K2_GetActorLocation`) (struct) 1.0 1.0 0.0 null null null null)))))))

(event `KickedInterface.Kicked`
  (params (KickVector :type "Vector Structure") (PlayerPosition :type "Vector Structure") (Damage :type "Float (single-precision)"))
  (bind _returnvalue (`self.K2_GetActorLocation`))
  ; Get Hit
  (set `self.HitType` "NewEnumerator6")
  (`|ExecutionSequence`
    (:`then_0`
      (`self.LaunchCharacter` KickVector))
    (:`then_1`
      ;;[0 1 1] Feedbacks (kicked)
      (bind _returnvalue_2 (`NiagaraFunctionLibrary.SpawnSystemAtLocation` "/Game/VFX/Niagara/Text/NS_Text_WHACK.NS_Text_WHACK" (+ _returnvalue (* (- _returnvalue (0.0 0.0 0.0)) 0.25))))
      (`GameplayStatics.PlaySoundAtLocation` "/Game/_GameManager/Feedbacks/Sounds/A_Hurt_Enemy_5_Cue.A_Hurt_Enemy_5_Cue" _returnvalue (struct) 1.0 1.0 0.0 null null null null)
      (`KismetSystemLibrary.Delay` 0.7)
      (`ActorComponent.K2_DestroyComponent` _returnvalue_2))))

(event `/Game/Characters/Player/Blueprints/WeaponSystem/Weapon/BPI_Weapon_Hitting.Take Weapon Throwing Hit`
  (params (Hit :type "HitResult Structure") (`AC Weapon` :type "/Game/Characters/Player/Blueprints/WeaponSystem/Weapon/AC_Weapon Object Reference") (`AC Weapon User` :type "/Game/Characters/Player/Blueprints/WeaponSystem/Weapon/AC_Weapon_User Object Reference"))
  ; Get Hit
  (`KismetSystemLibrary.PrintString` (`KismetStringLibrary.Concat_StrStr` "Throw: " (`KismetSystemLibrary.GetObjectName` self))))

(event `Death`
  ; Get Hit
  (`KismetSystemLibrary.Delay` 1.0)
  (`self.SetInUse` false)
  (`PoolingManager.HandOverActor` (`self.Pool`) self))

(event `PreAttackHit`
  (bind _dodge_chance_current (`self.Dodge Chance Current`))
  ; Input read for Dash
  (if (<= (`KismetMathLibrary.RandomFloatInRange` 0.0 1.0) _dodge_chance_current)
    (set `self.Dodge Chance Current` (`self.DodgeChance`))
    (`self.EvadeDash` (`KismetMathLibrary.Normal` (- (`self.K2_GetActorLocation` (`self.Player`)) (`self.K2_GetActorLocation`))))
    (`FTJ_CombatManager_CreatureBase.TryDeregisterApproach` (`self.Creature`) (`self.PlayerGrid`))
    (else
      (set `self.Dodge Chance Current` (`KismetMathLibrary.FMin` (+ _dodge_chance_current (`self.DodgeIncrease`)) 1.0)))))

(event `EvadeDash`
  (params (Direction :type "Vector Structure"))
  (bind _charactermovement (`self.CharacterMovement`))
  (bind _charactermovement_2 (`self.CharacterMovement`))
  (bind _returnvalue (* (`self.Dash Length`) 10.0))
  ;[1 0 0.5] Dash
  (if (`self.bCanDash`)
    (set `self.bCanDash` false)
    (set `self.isDashing` true)
    (set `self.Old Velocity` (`MovementComponent.Velocity` _charactermovement))
    (set `self.Old Ground Friction` (`CharacterMovementComponent.GroundFriction` _charactermovement))
    (set `CharacterMovementComponent.GroundFriction` 0.0 _charactermovement)
    (if (`KismetMathLibrary.Vector_IsNearlyZero` Direction)
      (set `MovementComponent.Velocity` (* (* (`self.GetActorForwardVector`) -1.0) _returnvalue) _charactermovement)
      (else
        (set `MovementComponent.Velocity` (* Direction _returnvalue) _charactermovement)))
    (`KismetSystemLibrary.Delay` (`self.Dash Duration`))
    (set `self.isDashing` false)
    (set `CharacterMovementComponent.GroundFriction` (`self.Old Ground Friction`) _charactermovement_2)
    (set `MovementComponent.Velocity` (`self.Old Velocity`) _charactermovement_2)
    (`KismetSystemLibrary.Delay` (`self.Dash CD`))
    (set `self.bCanDash` true)))

(event `self.SetInUse`
  (params (InUse :type Boolean))
  (if InUse
    (`self.Start Timers`)
    (else
      (`KismetSystemLibrary.K2_ClearAndInvalidateTimerHandle` (`self.MoveTimerHandle`))
      (`KismetSystemLibrary.K2_ClearAndInvalidateTimerHandle` (`self.AttackTimerHandle`))))
  (`parent.SetInUse` InUse))

(event `Start Timers`
  (bind _returnvalue (`KismetSystemLibrary.K2_SetTimerDelegate` (delegate `UpdatePosition`) (`self.UpdatePositionRepeatTime`) true true))
  (set `self.MoveTimerHandle` _returnvalue)
  (bind _returnvalue_2 (`KismetSystemLibrary.K2_SetTimerDelegate` (delegate `ChooseMove`) (`self.Attack/GuardRepeatTime`) true true))
  (set `self.AttackTimerHandle` _returnvalue_2))

(event `UpdatePosition`
  (bind _playergrid (`self.PlayerGrid`))
  (bind _returnvalue (`FTJ_CombatManager_Grid.GetDeregisteringSlot` _playergrid (`self.Creature`)))
  (bind _asbp_enemy (cast `/Game/Characters/Enemies/Blueprints/BP_Enemy` (`ActorComponent.GetOwner` (`self.CurrentCreature`)) :!pure true))
  (bind (_output_creature _output_approachweight) (break `FTJ_CombatManager_SlotBase` (`|GetArrayItem` _returnvalue)))
  ; Slot Approach and Attack
  (if (`self.isDashing`)
    _
    (elif (<= (`KismetMathLibrary.Vector_Distance` (`self.Goal`) (`self.K2_GetActorLocation` (`self.Player`))) (* (`FTJ_CombatManager_GridBase.ApproachRadius` (`self.PlayerGrid`)) 1.1))
      (if (`KismetMathLibrary.Vector_IsNearlyZero` (- (`self.Goal`) (`SceneComponent.K2_GetComponentLocation` (`self.CapsuleComponent`))) 50.0)
        (set `self.CanAct` true)
        (else
          (set `self.Goal` (`self.EmptyGoal`) :!label _label)
          (bind (_outspot _returnvalue_2) (`FTJ_CombatManager_CreatureBase.TryRegisterApproach` (`self.Creature`) _playergrid))
          (switch `EFTJ_CombatManager_ApproachRegistrationResult` _returnvalue_2
            (:`Success`
              (bind _output_get (set `self.Goal` _outspot))
              (`KismetSystemLibrary.DrawDebugLine` (`self.K2_GetActorLocation`) _output_get (struct :`B` 1.0 :`A` 1.0) 0.1)
              (`CharacterMovementComponent.SetMovementMode` (`self.CharacterMovement`) "MOVE_Walking" 0)
              (`AIController.MoveToLocation` (`self.AIControllerRef`) _output_get -1.0 true true false true null true))
            (:`ApproachCapacityIsTooLow`
              (`MovementComponent.StopMovementImmediately` (`self.CharacterMovement`) :!label _label_2)
              (set `self.Goal` (`self.EmptyGoal`))
              (if (!= (`KismetArrayLibrary.Array_Length` _returnvalue) 0)
                (`/Engine/EditorBlueprintResources/StandardMacros.IsValid` _output_creature
                  (:`Is Valid`
                    (bind _output_get_2 (set `self.CurrentCreature` _output_creature))
                    (if (>= (+ _output_approachweight (`FTJ_CombatManager_GridBase.ApproachCapacity` (`self.PlayerGrid`))) (`FTJ_CombatManager_CreatureBase.ApproachWeight` (`self.Creature`)))
                      (bind _returnvalue_3 (`FTJ_CombatManager_CreatureBase.TryDeregisterApproach` _output_get_2 (`self.PlayerGrid`)))
                      (switch `EFTJ_CombatManager_ApproachDeregistrationResult` _returnvalue_3
                        (:`Success`
                          (set `/Game/Characters/Enemies/Blueprints/BP_Enemy.Goal` (`self.EmptyGoal`) _asbp_enemy)
                          (`MovementComponent.StopMovementImmediately` (`Character.CharacterMovement` _asbp_enemy))
                          (bind _outspot_2 (`FTJ_CombatManager_CreatureBase.TryRegisterApproach` (`self.Creature`) (`self.PlayerGrid`)))
                          (bind _output_get_3 (set `self.Goal` _outspot_2))
                          (`KismetSystemLibrary.DrawDebugLine` (`self.K2_GetActorLocation`) _output_get_3 (struct :`G` 1.0 :`A` 1.0) 0.1)
                          (`CharacterMovementComponent.SetMovementMode` (`self.CharacterMovement`) "MOVE_Walking" 0)
                          (`AIController.MoveToLocation` (`self.AIControllerRef`) _output_get_3 -1.0 true true false true null true))))))))
            (:`GridHasNoMoreSlots`
              (goto _label_2))
            (:`OccupiedSlotIsInvalidNow`
              (`MovementComponent.StopMovementImmediately` (`self.CharacterMovement`))
              (set `self.Goal` (`self.EmptyGoal`))
              (`FTJ_CombatManager_CreatureBase.TryDeregisterApproach` (`self.Creature`) (`self.PlayerGrid`))))))
      (else
        (`FTJ_CombatManager_CreatureBase.TryDeregisterApproach` (`self.Creature`) (`self.PlayerGrid`))
        (goto _label)))))

(event `ChooseMove`
  (if (`self.CanAct`)
    (set `self.CanAct` false)
    (if (<= (`KismetMathLibrary.RandomFloat`) (`self.GuardChance`))
      (bind _returnvalue (`FTJ_CombatManager_Creature.TryRegisterAttack` (`self.Creature`) (`self.PlayerGrid`) 1))
      (switch `EFTJ_CombatManager_AttackRegistrationResult` _returnvalue
        (:`Success`
          (set `self.IsGuarding?` false)
          (`self.Attack`))
        (:`CreatureIsNotOnGrid`
          (`FTJ_CombatManager_CreatureBase.TryDeregisterApproach` (`self.Creature`) (`self.PlayerGrid`) :!label _label_3)
          (set `self.Goal` (`self.EmptyGoal`)))
        (:`AttackCapacityIsTooLow`
          (set `self.IsGuarding?` true)
          (goto _label_3))
        (:`CreatureNeedsToBeCloser`
          (goto _label_3)))
      (else
        (set `self.IsGuarding?` true)))))

(event `Attack`
  (bind _returnvalue (`self.K2_GetActorLocation`))
  (bind _returnvalue_2 (`self.K2_GetActorLocation` (`self.Player`)))
  ; Attack
  (set `self.IsAttacking?` true)
  (`self.K2_SetActorRotation` (`KismetMathLibrary.FindLookAtRotation` _returnvalue _returnvalue_2))
  (bind (_outhits _returnvalue_3) (`KismetSystemLibrary.SphereTraceMultiForObjects` _returnvalue _returnvalue_2 10.0 (`|MakeArray` "ObjectTypeQuery3" :!type "EObjectTypeQuery Enum") false (`|MakeArray` (`self.Blockout ref`) :!type "Actor Object Reference") "ForDuration"))
  (if _returnvalue_3
    (for _array_element _outhits
      (if (`self.ActorHasTag` (`.HitActor` (`GameplayStatics.BreakHitResult` _array_element)) "Player")
        _))
    (`KismetSystemLibrary.Delay` 3.0)
    (`FTJ_CombatManager_Creature.TryDeregisterAttack` (`self.Creature`) (`self.PlayerGrid`))
    (set `self.IsAttacking?` false)))

(fn `Set Values from DataTable`
  (bind _charactermovement (`self.CharacterMovement`))
  (bind _returnvalue (`|GetDataTableRow` "/Game/_GameManager/Data_Assets/Data_3C/DT_Enemy.DT_Enemy" "EnemyBase")
    (:`then`
      (bind (_maxwalkspeed _maxacceleration _startingdodgechance _dodgechanceincrease _getupdelay _basicattackdamage _positionrefreshrate _attacktryrefreshrate _guardchance _dashduration _dashcooldown _dashlength) (break `/Game/_GameManager/Data_Assets/Data_3C/S_Enemy` _returnvalue))
      (set `CharacterMovementComponent.MaxWalkSpeed` _maxwalkspeed _charactermovement)
      (set `CharacterMovementComponent.MaxAcceleration` _maxacceleration _charactermovement)
      (set `self.DodgeChance` _startingdodgechance)
      (set `self.DodgeIncrease` _dodgechanceincrease)
      (set `self.GetUpDelayBase` _getupdelay)
      (set `self.AttackDamageTMP` _basicattackdamage)
      (set `self.UpdatePositionRepeatTime` _positionrefreshrate)
      (set `self.Attack/GuardRepeatTime` _attacktryrefreshrate)
      (set `self.GuardChance` _guardchance)
      (set `self.Dash Duration` _dashduration)
      (set `self.Dash CD` _dashcooldown)
      (set `self.Dash Length` _dashlength))))

(fn `UserConstructionScript`)