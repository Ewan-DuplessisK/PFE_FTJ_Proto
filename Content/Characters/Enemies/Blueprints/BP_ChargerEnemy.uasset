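; BP_ChargerEnemy is an enemy that charges at the player's last sighted position and deals damage on impact.
; PawnSensing sight stores the pawn's location, then after a short wind-up starts a SimpleMoveToLocation charge that ends on a timer.
; While nothing is seen, Tick turns it toward the stored location, which player noises also update.
; Hits on Player-tagged actors during a charge send GetHitMessage; Kicked is empty.
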(event `self.ReceiveTick`
  (params (DeltaSeconds :type "Float (single-precision)"))
  (if (not (`self.PlayerSeen`))
    (`self.K2_SetActorRotation` (`KismetMathLibrary.RInterpTo_Constant` (`self.K2_GetActorRotation`) (`KismetMathLibrary.FindLookAtRotation` (`self.K2_GetActorLocation`) (`self.PlayerLocationSeen`)) DeltaSeconds (`self.RotationRate`)))))

(event `self.PawnSensing.OnSeePawn`
  (params (Pawn :type "Pawn Object Reference"))
  (set `self.PlayerSeen` true)
  (set `self.PlayerLocationSeen` (`self.K2_GetActorLocation` Pawn))
  (`KismetSystemLibrary.Delay` 0.5)
  (`AIBlueprintHelperLibrary.SimpleMoveToLocation` (`self.GetController`) (`self.PlayerLocationSeen`))
  (set `self.IsCharging` true)
  (`KismetSystemLibrary.Delay` 2.0)
  (set `self.PlayerSeen` false)
  (set `self.IsCharging` false))

(event `self.PawnSensing.OnHearNoise`
  (params (Instigator :type "Pawn Object Reference") (Location :type "Vector Structure (by ref)") (Volume :type "Float (single-precision)"))
  (if (`self.ActorHasTag` Instigator "Player")
    (set `self.PlayerLocationSeen` Location)))

(event `self.ReceiveHit`
  (params (MyComp :type "PrimitiveComponent Object Reference") (Other :type "Actor Object Reference") (OtherComp :type "PrimitiveComponent Object Reference") (bSelfMoved :type Boolean) (HitLocation :type "Vector Structure") (HitNormal :type "Vector Structure") (NormalImpulse :type "Vector Structure") (Hit :type "HitResult Structure (by ref)"))
  (if (and (`self.ActorHasTag` Other "Player") (`self.IsCharging`))
    (message `HitInterface.GetHit` Other (`self.Damage`) 0.0 (0.0 0.0 0.0) 0.0 self)))

(event `KickedInterface.Kicked`
  (params (KickVector :type "Vector Structure") (PlayerPosition :type "Vector Structure")))

(fn `UserConstructionScript`)