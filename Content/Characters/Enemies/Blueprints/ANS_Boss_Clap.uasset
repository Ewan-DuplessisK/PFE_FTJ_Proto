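; Anim notify state that handles hit detection for the boss's clap attack.
; Each tick it sphere-traces for pawns at the left and right clap sockets, ignoring the mesh owner.
; When a trace hits an actor tagged Player, it calls CloseAttack on a BP_ChargerEnemy found by class lookup rather than on the owner.
; When the notify ends, it calls ResetPunch on every BP_ChargerEnemy in the world.
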(fn `Received_NotifyEnd`
  (params (MeshComp :type "SkeletalMeshComponent Object Reference") (Animation :type "AnimSequenceBase Object Reference") (EventReference :type "AnimNotifyEventReference Structure (by ref)"))
  (returns (ReturnValue :type Boolean))
  (bind _outactors (`GameplayStatics.GetAllActorsOfClass` MeshComp "/Game/Characters/Enemies/Blueprints/BP_ChargerEnemy.BP_ChargerEnemy_C"))
  (for _array_element _outactors
    (`/Game/Characters/Enemies/Blueprints/BP_ChargerEnemy.ResetPunch` _array_element))
  (return true))

(fn `Received_NotifyTick`
  (params (MeshComp :type "SkeletalMeshComponent Object Reference") (Animation :type "AnimSequenceBase Object Reference") (FrameDeltaTime :type "Float (single-precision)") (EventReference :type "AnimNotifyEventReference Structure (by ref)"))
  (returns (ReturnValue :type Boolean))
  (bind _returnvalue (`SceneComponent.GetSocketLocation` MeshComp "ClapR_Socket"))
  (bind _returnvalue_2 (`SceneComponent.GetSocketLocation` MeshComp "ClapL_Socket"))
  (bind _array (`|MakeArray` "ObjectTypeQuery3" :!type "EObjectTypeQuery Enum"))
  (bind _array_2 (`|MakeArray` (`ActorComponent.GetOwner` MeshComp)))
  (bind _outhits (`KismetSystemLibrary.SphereTraceMultiForObjects` MeshComp _returnvalue_2 _returnvalue_2 50.0 _array false _array_2))
  (for _array_element _outhits
    (bind (_bblockinghit _binitialoverlap _time _distance _location _impactpoint _normal _impactnormal _physmat _hitactor) (`GameplayStatics.BreakHitResult` _array_element))
    (if (`Actor.ActorHasTag` _hitactor "Player")
      (bind _returnvalue_3 (`GameplayStatics.GetActorOfClass` _hitactor "/Game/Characters/Enemies/Blueprints/BP_ChargerEnemy.BP_ChargerEnemy_C"))
      (`/Game/Characters/Enemies/Blueprints/BP_ChargerEnemy.CloseAttack` _returnvalue_3)
      (break)))
  (bind _outhits_2 (`KismetSystemLibrary.SphereTraceMultiForObjects` MeshComp _returnvalue _returnvalue 50.0 _array false _array_2))
  (for _array_element_2 _outhits_2
    (bind (_bblockinghit_2 _binitialoverlap_2 _time_2 _distance_2 _location_2 _impactpoint_2 _normal_2 _impactnormal_2 _physmat_2 _hitactor_2) (`GameplayStatics.BreakHitResult` _array_element_2))
    (if (`Actor.ActorHasTag` _hitactor_2 "Player")
      (bind _returnvalue_4 (`GameplayStatics.GetActorOfClass` _hitactor_2 "/Game/Characters/Enemies/Blueprints/BP_ChargerEnemy.BP_ChargerEnemy_C"))
      (`/Game/Characters/Enemies/Blueprints/BP_ChargerEnemy.CloseAttack` _returnvalue_4)
      (break)))
  (return true))