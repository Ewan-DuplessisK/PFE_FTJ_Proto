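; Enemy drone that patrols along a spline and hurls a carried physics prop at the player, spawning one at start if unarmed.
; PawnSensing sightings halt the patrol; an armed drone turns via timeline and launches the detached prop using predicted moving-target velocity with random flight time.
; An unarmed drone sphere-traces for props, flies toward the hit without pathfinding, attaches it if already there, or resumes patrol when none is found.
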(event `self.ReceiveBeginPlay`
  (set `self.AI` (`AIBlueprintHelperLibrary.GetAIController` (`self.GetController`)))
  (`KismetSystemLibrary.Delay` 2.0)
  (`|ExecutionSequence`
    (:`then_0`
      (set `PawnSensingComponent.SightRadius` (`self.Sight Radius`) (`self.PawnSensing`)))
    (:`then_1`
      (`self.Has Armed Prop`
        (:`Yes`
          _)
        (:`No`
          (bind _armable (`self.Spawn ArmableProp`))
          (`self.Arm ArmableProp` _armable)))
      (`/Game/BPs/AC_PatrolAlongSpline.Start Patrol` (`self.AC_PatrolAlongSpline`)))))

(event `self.ReceiveTick`
  (params (DeltaSeconds :type "Float (single-precision)")))

(event `self.PawnSensing.OnSeePawn`
  (params (Pawn :type "Pawn Object Reference"))
  (`/Game/BPs/Other/ML_Object.If is Player` Pawn
    (:`Yes`
      (set `self.Current Attack Target` Pawn)
      (`/Game/BPs/AC_PatrolAlongSpline.Stop Patrol` (`self.AC_PatrolAlongSpline`))
      (`self.Has Armed Prop`
        (:`Yes`
          (`self.Attack Target` Pawn))
        (:`No`
          (`self.Search for ArmableProp`
            (:`Nothing Found`
              (`/Game/BPs/AC_PatrolAlongSpline.Start Patrol` (`self.AC_PatrolAlongSpline`)))))))))

(event `Attack Target`
  (params (Target :type "Actor Object Reference"))
  (`self.Rotate to Target` Target)
  (`self.Shoot`))

(event `Rotate to Target`
  (params (Target :type "Actor Object Reference"))
  (bind (_direction _newtrack_0) (`Timeline|Timeline` :!via `PlayFromStart`)
    (:`Update`
      (`self.K2_SetActorRotation` (`KismetMathLibrary.RLerp` (`self.K2_GetActorRotation`) (`/Game/BPs/Other/FL_Common.Get Direction` self Target) _newtrack_0)))))

(fn `Arm ArmableProp`
  (params (`Armed Prop` :type "/Game/BPs/VacuumProps/BP_SuckableProp Object Reference"))
  (`self.K2_SetActorRelativeLocation` `Armed Prop` (`self.Arming Location`) false false)
  (`self.K2_AttachToActor` `Armed Prop` self "None" "KeepRelative" "KeepRelative" "KeepRelative" true)
  (set `self.ArmedProp` `Armed Prop`))

(fn `Grab ArmableProp`
  (params (Armable :type "Actor Object Reference"))
  (bind _asbp_suckable_prop (cast `/Game/BPs/VacuumProps/BP_SuckableProp` Armable))
  (`self.Arm ArmableProp` _asbp_suckable_prop))

(fn `Search for ArmableProp3`
  (returns (`Moving to Armable` :type Boolean))
  (bind _returnvalue (`self.K2_GetActorLocation`))
  (`|ExecutionSequence`
    (:`then_1`
      (bind (_outhit _returnvalue_2) (`KismetSystemLibrary.SphereTraceSingleForObjects` _returnvalue _returnvalue (`self.Sight Radius`) (`|MakeArray` "ObjectTypeQuery13" :!type "EObjectTypeQuery Enum")))
      (if _returnvalue_2
        (bind (_bblockinghit _binitialoverlap _time _distance _location _impactpoint _normal _impactnormal _physmat _hitactor) (`GameplayStatics.BreakHitResult` _outhit))
        (bind _returnvalue_3 (`KismetStringLibrary.Concat_StrStr` "2: " (`KismetSystemLibrary.GetDisplayName` _hitactor)))
        (`KismetSystemLibrary.PrintString` _returnvalue_3 true true (struct :`G` 0.66 :`B` 1.0 :`A` 1.0) 2.0 (`KismetStringLibrary.Conv_StringToName` _returnvalue_3))
        (bind _returnvalue_4 (`AIController.MoveToLocation` (`self.AI`) (+ (`self.K2_GetActorLocation` _hitactor) (0.0 0.0 100.0)) -1.0 true false false false null false))
        (switch `EPathFollowingRequestResult` _returnvalue_4
          (:`Failed`
            (return false))
          (:`AlreadyAtGoal`
            (`self.Grab ArmableProp` null))
          (:`RequestSuccessful`
            (return true)))
        (else
          (return false))))))

(fn `Shoot`
  (bind _armedprop (`self.ArmedProp`))
  (bind _outlaunchvelocity (`GameplayStatics.SuggestProjectileVelocity_MovingTarget` (`SceneComponent.K2_GetComponentLocation` (`/Game/BPs/VacuumProps/BP_SuckableProp.StaticMesh` (`self.ArmedProp`))) (`GameplayStatics.GetPlayerPawn` 0) (0.0 0.0 0.0) 0.0 (`KismetMathLibrary.RandomFloatInRange` 0.3 0.7) "None"))
  (`self.K2_DetachFromActor` _armedprop "KeepRelative" "KeepRelative" "KeepRelative")
  (`/Game/BPs/VacuumProps/BP_SuckableProp.Activate` _armedprop false)
  (`PrimitiveComponent.AddImpulse` (`/Game/BPs/VacuumProps/BP_SuckableProp.StaticMesh` _armedprop) _outlaunchvelocity "None" true)
  (set `self.ArmedProp` null))

(fn `Spawn ArmableProp`
  (returns (Armable :type "/Game/BPs/VacuumProps/BP_SuckableProp Object Reference"))
  (bind _returnvalue (`|SpawnActorFromClass` (`self.ArmedProp Class`) (`KismetMathLibrary.MakeTransform` (`self.Arming Location`)) "AdjustIfPossibleButAlwaysSpawn" "OverrideRootScale" self null null))
  (return _returnvalue))

(fn `UserConstructionScript`)