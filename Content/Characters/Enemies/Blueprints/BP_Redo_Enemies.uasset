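; Base melee enemy character that chases the player, attacks in range and awards score when hit or killed.
; BeginPlay secures an AI controller, loads DT_Enemy stats and starts looping Move and Attack timers, with attacks using sphere traces.
; Hit, guard and kick events launch the character with feedback; only RemoveHealth triggers Death, while GetHit subtracts health directly.
; Pooling and prop-collision logic is disconnected, and Tick countdowns subtract zero.
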(event `self.ReceiveBeginPlay`
  (bind (_asbp_player _bsuccess) (cast `/Game/Characters/Player/Blueprints/BP_Player` (`GameplayStatics.GetPlayerCharacter` 0) :!pure true))
  (`|ExecutionSequence`
    (:`then_0`
      (bind _asaic_fthis_job (cast `/Game/_GameManager/AIC_FThisJob` (`self.GetController`))
        (:`then`
          (set `self.AIControllerRef` _asaic_fthis_job))
        (:`CastFailed`
          ; Safety when dynamically spawning enemy
          (`KismetSystemLibrary.PrintString` "Enemy Failed to cast AI Controller" true true (struct :`R` 1.0 :`A` 1.0) 20.0)
          (bind _returnvalue (`|SpawnActorFromClass` "/Game/_GameManager/AIC_FThisJob.AIC_FThisJob_C" (`KismetMathLibrary.MakeTransform` (0.0 0.0 0.0)) "Undefined" "MultiplyWithRoot" null null))
          (bind _output_get (set `self.AIControllerRef` _returnvalue))
          (`Controller.Possess` _output_get self)
          (`KismetSystemLibrary.PrintString` "Enemy Possessed by new AI Controller" true true (struct :`G` 1.0 :`A` 1.0) 20.0)))
      (`KismetSystemLibrary.DelayUntilNextTick`)
      (if _bsuccess
        (set `self.Player` _asbp_player)
        (else
          (`KismetSystemLibrary.PrintString` "Enemy Failed to get Player" true true (struct :`R` 1.0 :`A` 1.0) 20.0)))
      (`self.Set Values from DataTable`)
      (set `self.PlayerGrid` (`/Game/Characters/Player/Blueprints/BP_Player.BP_CombatManager_Grid_SC` (`self.Player`))))
    (:`then_1`
      (if (not (`self.TEST Not Moving`))
        (`KismetSystemLibrary.K2_SetTimerDelegate` (delegate `Move`) 0.1 true true)
        (`KismetSystemLibrary.K2_SetTimerDelegate` (delegate `Attack`) 2.0 true true)))))

(event `Move`
  ; Move towards Player
  (if (`self.TEST Not Moving`)
    _
    (elif (`self.CanMove?`)
      (if (not (<= (`KismetMathLibrary.VSize` (- (`self.K2_GetActorLocation` (`self.Player`)) (`self.K2_GetActorLocation`))) (`self.Approach distance`)))
        (`AIController.MoveToActor` (`self.AIControllerRef`) (`self.Player`) (- (`self.Approach distance`) 90.0) true true true null true)))))

(event `Attack`
  (bind _returnvalue (`self.K2_GetActorLocation`))
  (bind _returnvalue_2 (`self.K2_GetActorLocation` (`self.Player`)))
  (if (<= (`KismetMathLibrary.VSize` (- (`self.K2_GetActorLocation` (`self.Player`)) (`self.K2_GetActorLocation`))) (`self.Approach distance`))
    (set `self.IsAttacking?` true)
    (`self.K2_SetActorRotation` (`KismetMathLibrary.FindLookAtRotation` _returnvalue _returnvalue_2))
    (bind (_outhits _returnvalue_3) (`KismetSystemLibrary.SphereTraceMultiForObjects` _returnvalue _returnvalue_2 10.0 (`|MakeArray` "ObjectTypeQuery3" :!type "EObjectTypeQuery Enum") false (`|MakeArray` null :!type "Actor Object Reference") "ForDuration"))
    (if _returnvalue_3
      (for _array_element _outhits
        (bind (_bblockinghit _binitialoverlap _time _distance _location _impactpoint _normal _impactnormal _physmat _hitactor) (`GameplayStatics.BreakHitResult` _array_element))
        (if (`self.ActorHasTag` _hitactor "Player")
          (message `HitInterface.GetHit` _hitactor (`KismetMathLibrary.Conv_IntToDouble` (`self.AttackDamageTMP`)) 0.0 (0.0 0.0 0.0) 0.0 self)
          (break)))
      (`KismetSystemLibrary.Delay` 1.5)
      (set `self.IsAttacking?` false))))

(event `self.ReceiveTick`
  (params (DeltaSeconds :type "Float (single-precision)"))
  (bind _invincibilitytime (`self.InvincibilityTime`))
  (bind _getupdelaycurrent (`self.GetUpDelayCurrent`))
  (`|ExecutionSequence`
    (:`then_0`
      (if (> _getupdelaycurrent 0.0)
        (bind _output_get (set `self.GetUpDelayCurrent` (- _getupdelaycurrent 0.0)))
        (if (<= _output_get 0.0)
          (set `self.CanGetUp` true))))
    (:`then_1`
      (if (> _invincibilitytime 0.0)
        (bind _output_get_2 (set `self.InvincibilityTime` (- _invincibilitytime 0.0)))
        (if (<= _output_get_2 0.0)
          (set `self.CanBeDamaged` true))))))

(event `/Game/Characters/Player/Blueprints/WeaponSystem/Weapon/BPI_Weapon_Hitting.Take Weapon Melee Hit`
  (params (Hit :type "HitResult Structure") (`AC Weapon` :type "/Game/Characters/Player/Blueprints/WeaponSystem/Weapon/AC_Weapon Object Reference") (`AC Weapon User` :type "/Game/Characters/Player/Blueprints/WeaponSystem/Weapon/AC_Weapon_User Object Reference"))
  (bind _returnvalue (`self.K2_GetActorLocation`))
  (bind _returnvalue_2 (`GameplayStatics.GetPlayerController` 0))
  (`|ExecutionSequence`
    (:`then_0`
      (bind _output_get (set `self.HitType` (`/Game/Characters/Player/Blueprints/BP_Player.AttackType` (`self.Player`))))
      (if (`|EnumEquality` _output_get "NewEnumerator3")
        (set `self.GetUpDelayCurrent` (`self.GetUpDelayBase`))
        (set `self.CanGetUp` false)))
    (:`then_1`
      ;[0 1 1] Feedbacks (hit melee)
      (`PlayerController.ClientStartCameraShake` :`self` _returnvalue_2 :`Shake` "/Game/VFX/Blueprint/BP_FX_CameraShake_Impact_Strong.BP_FX_CameraShake_Impact_Strong_C")
      (`|ExecutionSequence`
        (:`then_0`
          (`PlayerController.PlayDynamicForceFeedback` _returnvalue_2 1.0 0.2 true true true true))
        (:`then_1`
          (bind _returnvalue_3 (`NiagaraFunctionLibrary.SpawnSystemAtLocation` "/Game/VFX/Niagara/Text/NS_Text_BONK.NS_Text_BONK" (+ _returnvalue (* (- _returnvalue (`self.K2_GetActorLocation` (`ActorComponent.GetOwner` `AC Weapon User`))) 0.25))))
          (`KismetSystemLibrary.Delay` 0.7)
          (`ActorComponent.K2_DestroyComponent` _returnvalue_3))))))

(event `HitInterface.GetHit`
  (params (Damage :type "Float (single-precision)") (HitStunDuration :type "Float (single-precision)") (KnockbackVector :type "Vector Structure") (InvincibilityTime :type "Float (single-precision)") (SourceActor :type "Actor Object Reference"))
  ; Get Hit
  (if (<= (`self.InvincibilityTime`) 0.0)
    (if (`self.IsGuarding?`)
      (`|ExecutionSequence`
        (:`then_0`
          ;;[1 0 0] Change for something controllable
          (`self.LaunchCharacter` (* KnockbackVector 0.5))
          (set `self.IsAttacking?` false :!label _label)
          (set `self.CanAct` false)
          (`self.Player`
            (:`then`
              (`FTJ_ScoringSystem_Score.IncreaseWithText` (subsystem `/Game/CppSystems/ScoringSystem/Public/Blueprint/BP_ScoringSystem_Score`) 10 0 (`|FormatText` "Hit Enemy")))
            (:`else`)))
        (:`then_1`
          ;;[0 1 1] Feedbacks (guard)
          (`GameplayStatics.PlaySoundAtLocation` "/Game/_GameManager/Feedbacks/Sounds/A_Hurt_Enemy_5_Cue.A_Hurt_Enemy_5_Cue" (`self.K2_GetActorLocation`) (struct) 1.0 1.0 0.0 null null null null)))
      (else
        (set `self.CurrentHealth` (- (`self.CurrentHealth`) Damage))
        (set `self.InvincibilityTime` InvincibilityTime)
        (`|ExecutionSequence`
          (:`then_0`
            (`self.LaunchCharacter` KnockbackVector)
            (goto _label))
          (:`then_1`
            ;;[0 1 1] Feedbacks (hurt)
            (`GameplayStatics.PlaySoundAtLocation` "/Game/_GameManager/Feedbacks/Sounds/A_Hurt_Enemy_5_Cue.A_Hurt_Enemy_5_Cue" (`self.K2_GetActorLocation`) (struct) 1.0 1.0 0.0 null null null null)))))))

(event `KickedInterface.Kicked`
  (params (KickVector :type "Vector Structure") (PlayerPosition :type "Vector Structure"))
  (bind _returnvalue (`self.K2_GetActorLocation`))
  ; Get Hit
  (set `self.HitType` "NewEnumerator6")
  (`|ExecutionSequence`
    (:`then_0`
      (set `self.CanMove?` false)
      (`self.LaunchCharacter` KickVector)
      (`KismetSystemLibrary.Delay` 1.5)
      (set `self.CanMove?` true))
    (:`then_1`
      ;;[0 1 1] Feedbacks (kicked)
      (bind _returnvalue_2 (`NiagaraFunctionLibrary.SpawnSystemAtLocation` "/Game/VFX/Niagara/Text/NS_Text_WHACK.NS_Text_WHACK" (+ _returnvalue (* (- _returnvalue (0.0 0.0 0.0)) 0.25))))
      (`GameplayStatics.PlaySoundAtLocation` "/Game/_GameManager/Feedbacks/Sounds/A_Hurt_Enemy_5_Cue.A_Hurt_Enemy_5_Cue" _returnvalue (struct) 1.0 1.0 0.0 null null null null)
      (`KismetSystemLibrary.Delay` 0.7)
      (`ActorComponent.K2_DestroyComponent` _returnvalue_2))))

(event `Death`
  ; Get Hit
  (`SceneComponent.SetVisibility` (`self.DeathWidget`) true false)
  (`KismetSystemLibrary.Delay` 1.0)
  (`SceneComponent.SetVisibility` (`self.DeathWidget`) true false)
  (`self.Player`
    (:`then`
      (`FTJ_ScoringSystem_Score.IncreaseWithText` (subsystem `/Game/CppSystems/ScoringSystem/Public/Blueprint/BP_ScoringSystem_Score`) 50 0 (`|FormatText` "Killed Enemy"))
      (`self.K2_DestroyActor`))
    (:`else`)))

(event `HealthInterface.AddHealth`
  (params (Amount :type "Float (single-precision)"))
  (set `self.CurrentHealth` (`KismetMathLibrary.FClamp` (+ (`self.CurrentHealth`) 0.0) 0.0 (`self.MaxHealth`))))

(event `HealthInterface.RemoveHealth`
  (params (Damage :type "Float (single-precision)") (EnemyRef :type "Actor Object Reference"))
  (bind _output_get (set `self.CurrentHealth` (`KismetMathLibrary.FClamp` (- (`self.CurrentHealth`) Damage) 0.0 (`self.MaxHealth`))))
  (if (<= _output_get 0.0)
    (`self.Death`)))

(event `/Game/Characters/Player/Blueprints/WeaponSystem/Weapon/BPI_Weapon_Hitting.Take Weapon Throwing Hit`
  (params (Hit :type "HitResult Structure") (`AC Weapon` :type "/Game/Characters/Player/Blueprints/WeaponSystem/Weapon/AC_Weapon Object Reference") (`AC Weapon User` :type "/Game/Characters/Player/Blueprints/WeaponSystem/Weapon/AC_Weapon_User Object Reference"))
  (`KismetSystemLibrary.PrintString` (`KismetStringLibrary.Concat_StrStr` "Throw: " (`KismetSystemLibrary.GetObjectName` self))))

(event `self.ReceiveHit`
  (params (MyComp :type "PrimitiveComponent Object Reference") (Other :type "Actor Object Reference") (OtherComp :type "PrimitiveComponent Object Reference") (bSelfMoved :type Boolean) (HitLocation :type "Vector Structure") (HitNormal :type "Vector Structure") (NormalImpulse :type "Vector Structure") (Hit :type "HitResult Structure (by ref)"))
  (`|ExecutionSequence`
    (:`then_0`
      ; Vacuum Props
      (`/Engine/EditorBlueprintResources/StandardMacros.IsValid` Other
        (:`Is Valid`
          (`/Engine/EditorBlueprintResources/StandardMacros.IsValid` (`self.GetComponentByClass` Other "/Game/CppSystems/Prop/Public/ActorComponent/BP_Prop_PhysicsReactingCompBase_AC.BP_Prop_PhysicsReactingCompBase_AC_C")))))
    (:`then_1`
      ; Kickable Props
      (`/Engine/EditorBlueprintResources/StandardMacros.IsValid` Other
        (:`Is Valid`
          (`/Engine/EditorBlueprintResources/StandardMacros.IsValid` (`self.GetComponentByClass` Other "/Game/CppSystems/Prop/Public/ActorComponent/BP_Prop_PhysicsKickableCompBase_AC.BP_Prop_PhysicsKickableCompBase_AC_C")))))))

(fn `Set Values from DataTable`
  (bind _charactermovement (`self.CharacterMovement`))
  (bind _returnvalue (`|GetDataTableRow` "/Game/_GameManager/Data_Assets/Data_3C/DT_Enemy.DT_Enemy" "RedoEnemy")
    (:`then`
      (bind (_maxwalkspeed _maxacceleration _startingdodgechance _dodgechanceincrease _getupdelay _basicattackdamage _positionrefreshrate _attacktryrefreshrate _guardchance _dashduration _dashcooldown _dashlength) (break `/Game/_GameManager/Data_Assets/Data_3C/S_Enemy` _returnvalue))
      (set `CharacterMovementComponent.MaxWalkSpeed` _maxwalkspeed _charactermovement)
      (set `CharacterMovementComponent.MaxAcceleration` _maxacceleration _charactermovement)
      (set `self.DodgeChance` _startingdodgechance)
      (set `self.DodgeIncrease` _dodgechanceincrease)
      (set `self.GetUpDelayBase` _getupdelay)
      (set `self.AttackDamageTMP` _basicattackdamage)
      (set `self.GuardChance` _guardchance)
      (set `self.Dash Duration` _dashduration)
      (set `self.Dash CD` _dashcooldown)
      (set `self.Dash Length` _dashlength))))

(fn `UserConstructionScript`)