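; BP_CombatChara is a combat character with kick and throwable mechanics.
; Kick sphere-traces forward from KickPoint and launches a hit BP_Dummy or BP_KickableDoor along the facing direction.
; GetThrowable attaches a small sphere mesh to the right-hand socket of ArmsMesh as ThrowPoint.
; Predict runs a projectile path prediction from that socket, feeds the points into a spline and adds spline mesh segments along the arc.
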(event `Kick`
  (bind _returnvalue (`SceneComponent.K2_GetComponentLocation` (`self.KickPoint`)))
  (bind _returnvalue_2 (+ (* (`self.GetActorForwardVector`) 2500.0) (0.0 0.0 150.0)))
  (bind _outhit (`KismetSystemLibrary.SphereTraceSingleForObjects` :`Start` _returnvalue :`End` (+ _returnvalue (* (`self.GetActorForwardVector`) 200.0)) :`ObjectTypes` (`|MakeArray` "ObjectTypeQuery3" "ObjectTypeQuery7" :!type "EObjectTypeQuery Enum") :`DrawDebugType` "Persistent"))
  (bind (_bblockinghit _binitialoverlap _time _distance _location _impactpoint _normal _impactnormal _physmat _hitactor) (`GameplayStatics.BreakHitResult` _outhit))
  (bind _asbp_dummy (cast `/Game/CombatSystem/BP_Dummy` _hitactor)
    (:`then`
      (`/Game/CombatSystem/BP_Dummy.Launched` _asbp_dummy _returnvalue_2))
    (:`CastFailed`
      (bind _asbp_kickable_door (cast `/Game/CombatSystem/BP_KickableDoor` _hitactor))
      (`/Game/CombatSystem/BP_KickableDoor.Launched` _asbp_kickable_door _returnvalue_2))))

(event `GetThrowable`
  (bind _returnvalue (`AddComponent|NODE_AddStaticMeshComponent-0` :`bManualAttachment` true))
  (set `self.ThrowPoint` _returnvalue)
  (`SceneComponent.K2_AttachToComponent` _returnvalue (`self.ArmsMesh`) "hand_r" "KeepRelative" "KeepRelative" "KeepRelative" true)
  (`StaticMeshComponent.SetStaticMesh` _returnvalue "/Game/StarterContent/Shapes/Shape_Sphere.Shape_Sphere")
  (`SceneComponent.SetWorldScale3D` _returnvalue (0.3 0.3 0.3)))

(event `Predict`
  (bind _spline (`self.Spline`))
  (`KismetArrayLibrary.Array_Clear` (`self.SplineMesh`))
  (`SplineComponent.ClearSplinePoints` (`self.Spline`) true)
  (bind _returnvalue (`GameplayStatics.GetActorOfClass` "BP_CombatChara_C"))
  (bind (_outhit _outpathpositions) (`GameplayStatics.Blueprint_PredictProjectilePath_ByObjectType` (`SceneComponent.GetSocketLocation` (`self.ArmsMesh`) "hand_r") (* (`self.LaunchVelocity`) (`self.GetActorForwardVector`)) true 30.0 (`|MakeArray` "ObjectTypeQuery1" "ObjectTypeQuery3" :!type "EObjectTypeQuery Enum") false (`|MakeArray` _returnvalue :!type "Actor Object Reference")))
  (for _array_element _outpathpositions
    (`SplineComponent.AddSplinePoint` _spline _array_element "World" true))
  (for _index (range 1 (+ (`SplineComponent.GetNumberOfSplinePoints` _spline) 1))
    (bind _returnvalue_2 (`AddComponent|NODE_AddSplineMeshComponent-0`))
    (`KismetArrayLibrary.Array_Add` (`self.SplineMesh`) _returnvalue_2)
    (bind (_location _tangent) (`SplineComponent.GetLocationAndTangentAtSplinePoint` _spline _index "World"))
    (bind (_location_2 _tangent_2) (`SplineComponent.GetLocationAndTangentAtSplinePoint` _spline (+ _index 1) "World"))
    (`SplineMeshComponent.SetStartAndEnd` _returnvalue_2 _location _tangent (`KismetMathLibrary.VLerp` _location _location_2 0.5) (`KismetMathLibrary.VLerp` _tangent _tangent_2 0.5) true)))

(fn `UserConstructionScript`)