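; BP_BaseThrowable is a base throwable actor for the combat system that builds a trajectory preview, while its Throw event is an empty stub.
; Predict traces a projectile path from LaunchVelocity against WorldStatic and Pawn objects, ignoring BP_CombatChara, and feeds the positions into a spline.
; It adds spline mesh segments ending halfway to the next point.
; Each call clears the mesh array without destroying earlier components.
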(event `Throw`)

(event `Predict`
  (bind _spline (`self.Spline`))
  (`KismetArrayLibrary.Array_Clear` (`self.SplineMesh`))
  (`SplineComponent.ClearSplinePoints` (`self.Spline`) true)
  (bind _returnvalue (`GameplayStatics.GetActorOfClass` "/Game/CombatSystem/BP_CombatChara.BP_CombatChara_C"))
  (bind (_outhit _outpathpositions) (`GameplayStatics.Blueprint_PredictProjectilePath_ByObjectType` (`self.K2_GetActorLocation`) (`self.LaunchVelocity`) true 30.0 (`|MakeArray` "ObjectTypeQuery1" "ObjectTypeQuery3" :!type "EObjectTypeQuery Enum") false (`|MakeArray` _returnvalue :!type "Actor Object Reference")))
  (for _array_element _outpathpositions
    (`SplineComponent.AddSplinePoint` _spline _array_element "World" true))
  (for _index (range 1 (+ (`SplineComponent.GetNumberOfSplinePoints` _spline) 1))
    (bind _returnvalue_2 (`AddComponent|NODE_AddSplineMeshComponent-0`))
    (`KismetArrayLibrary.Array_Add` (`self.SplineMesh`) _returnvalue_2)
    (bind (_location _tangent) (`SplineComponent.GetLocationAndTangentAtSplinePoint` _spline _index "World"))
    (bind (_location_2 _tangent_2) (`SplineComponent.GetLocationAndTangentAtSplinePoint` _spline (+ _index 1) "World"))
    (`SplineMeshComponent.SetStartAndEnd` _returnvalue_2 _location _tangent (`KismetMathLibrary.VLerp` _location _location_2 0.5) (`KismetMathLibrary.VLerp` _tangent _tangent_2 0.5) true)))

(fn `UserConstructionScript`)