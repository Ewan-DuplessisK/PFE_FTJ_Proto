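; An enemy prop Blueprint that flies along world X and destroys itself after striking an actor that has a prop component.
; Tick applies a constant, mass-independent acceleration to its physics mesh.
; On hit, it prints a debug string and forwards the contact to the other actor's FTJ_Prop_PropComp through CallReversedHit, with an empty trait array.
; That hit sets a flag, so destruction happens in Tick rather than inside the hit event.
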(event `self.ReceiveTick`
  (params (DeltaSeconds :type "Float (single-precision)"))
  (`PrimitiveComponent.AddForce` (`self.StaticMeshComponent`) (15000.0 0.0 0.0) "None" true)
  (if (`self.WillBeDestroyed`)
    (`self.K2_DestroyActor`)))

(event `self.StaticMeshComponent.OnComponentHit`
  (params (HitComponent :type "PrimitiveComponent Object Reference") (OtherActor :type "Actor Object Reference") (OtherComp :type "PrimitiveComponent Object Reference") (NormalImpulse :type "Vector Structure") (Hit :type "HitResult Structure (by ref)"))
  (bind _returnvalue (`self.GetComponentByClass` OtherActor "/Script/FThisJob.FTJ_Prop_PropComp"))
  (`/Engine/EditorBlueprintResources/StandardMacros.IsValid` OtherActor
    (:`Is Valid`
      (`KismetSystemLibrary.PrintString` "_BP_Prop_Enemy")
      (`/Engine/EditorBlueprintResources/StandardMacros.IsValid` _returnvalue
        (:`Is Valid`
          (`FTJ_Prop_PropCompBase.CallReversedHit` _returnvalue OtherComp self HitComponent NormalImpulse Hit (`|MakeArray`))
          (set `self.WillBeDestroyed` true))))))

(fn `UserConstructionScript`
  (`parent.UserConstructionScript`))