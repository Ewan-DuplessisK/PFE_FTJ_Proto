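; Player controller that drives the score system's timer and its on-screen display.
; On BeginPlay it caches the GI_ScoreSystem game instance, starts its timer, adds the IMC_Score input context and shows the WBP_Timer widget.
; Tick passes delta time to the game instance's RunTimer, so the timer logic lives there rather than in the controller.
; Releasing the IA_PauseTimer input calls PauseTimer on the game instance.
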(event `self.ReceiveBeginPlay`
  (bind _asgi_score_system (cast `/Game/Score_system/GI_ScoreSystem` (`GameplayStatics.GetGameInstance`)))
  (set `self.As GI Score System` _asgi_score_system)
  (`/Game/Score_system/GI_ScoreSystem.StartTimer` (`self.As GI Score System`))
  (`EnhancedInputSubsystemInterface.AddMappingContext` (subsystem `EnhancedInputLocalPlayerSubsystem`) "/Game/Score_system/Inputs/IMC_Score.IMC_Score" 0 (struct))
  (bind _returnvalue (`|CreateWidget` "/Game/Score_system/WBP_Timer.WBP_Timer_C"))
  (set `self.TimerWidget` _returnvalue)
  (`UserWidget.AddToViewport` (`self.TimerWidget`) 0))

(event `self.ReceiveTick`
  (params (DeltaSeconds :type "Float (single-precision)"))
  (bind _as_gi_score_system (`self.As GI Score System`)
    (:`then`
      (`/Game/Score_system/GI_ScoreSystem.RunTimer` _as_gi_score_system DeltaSeconds))
    (:`else`)))

(event `EnhancedInput|/Game/Score_system/Inputs/Actions/IA_PauseTimer`
  (params (ActionValue :type Boolean) (ElapsedSeconds :type "Float (double-precision)") (TriggeredSeconds :type "Float (double-precision)") (InputAction :type "InputAction Object Reference" :default "/Game/Score_system/Inputs/Actions/IA_PauseTimer.IA_PauseTimer"))
  (:`Completed`
    (bind _asgi_score_system (cast `/Game/Score_system/GI_ScoreSystem` (`GameplayStatics.GetGameInstance`)))
    (`/Game/Score_system/GI_ScoreSystem.PauseTimer` _asgi_score_system)))

(fn `UserConstructionScript`)