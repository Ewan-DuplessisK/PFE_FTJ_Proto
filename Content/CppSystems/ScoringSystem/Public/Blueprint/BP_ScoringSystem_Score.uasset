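; Scoring system Blueprint that bridges score, multiplier and gauge logic to the scoring widget owned by PC_Systems.
; IncreasewithText applies gains through Increase, then refreshes the widget's texts, gauge, rank image (fixed DT_Ranks row "1") and added-score popup.
; An empty gauge triggers a delayed reverse animation that hides the display.
; Higher and lower transitions play level-change animations, while the trance transition is empty.
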(event `self.InitializeBlueprint`
  (`parent.InitializeBlueprint`))

(event `InitWorldContext`
  (params (Controller :type "PlayerController Object Reference"))
  (bind _aspc_systems (cast `/Game/_GameManager/PC_Systems` Controller))
  (set `self.As PC Systems` _aspc_systems))

(event `self.DeinitializeBlueprint`
  (`parent.DeinitializeBlueprint`))

(event `self.OnTransitionedTrance`
  (params (bInEntered :type Boolean)))

(event `self.IncreaseWithText`
  (params (InScoreIncrease :type "Float (single-precision)") (InGaugeIncrease :type "Float (single-precision)") (bInIsMultiplierIgnored :type Boolean) (InMessage :type "Text (by ref)"))
  (bind _wbp_scoring (`/Game/_GameManager/PC_Systems.WBP Scoring` (`self.As PC Systems`)))
  (bind _wbp_scoring_2 (`/Game/_GameManager/PC_Systems.WBP Scoring` (`self.As PC Systems`)))
  ; Score display + update
  (`self.As PC Systems`
    (:`then`
      (if (not (`self.bIsScoreIncreasing`))
        (`UserWidget.PlayAnimation` _wbp_scoring_2 (`/Game/UI/Menus/InGameMenu/WBP_Scoring.DisplayScoreAnimation` _wbp_scoring_2) 0.0 1 "Forward" 1.0 false)
        (set `self.bIsScoreIncreasing` true))
      (`self.Increase` InScoreIncrease InGaugeIncrease bInIsMultiplierIgnored)
      ;;[0.1519 0.849 0.383] UI changement
      (`UserWidget.PlayAnimation` _wbp_scoring (`/Game/UI/Menus/InGameMenu/WBP_Scoring.MultiplierBarFillingAnimation` _wbp_scoring) 0.0 1 "Forward" 1.0 false)
      (`UserWidget.PlayAnimation` _wbp_scoring (`/Game/UI/Menus/InGameMenu/WBP_Scoring.ScoreFillingAnimation` _wbp_scoring) 0.0 1 "Forward" 1.0 false)
      (`/Game/UI/Menus/InGameMenu/WBP_Scoring.SetTextScore` _wbp_scoring (`KismetMathLibrary.FTrunc` (`self.Score`)))
      (`/Game/UI/Menus/InGameMenu/WBP_Scoring.SetTextMultiplier` _wbp_scoring (`self.GetMultiplier`))
      (`/Game/UI/Menus/InGameMenu/WBP_Scoring.SetGaugeBar` _wbp_scoring (`self.GetGauge`))
      (set `/Game/UI/Menus/InGameMenu/WBP_Scoring.AlreadyVisible` true _wbp_scoring)
      (bind _returnvalue (`|GetDataTableRow` "/Game/_GameManager/Data_Assets/Scoring/DT_Ranks.DT_Ranks" "1")
        (:`then`
          (`/Game/UI/Menus/InGameMenu/WBP_Scoring.SetRankNameImage` _wbp_scoring (`.RankNames_17_708FD1F1417D7E2C85B76C96870D6B20` (break `/Game/_GameManager/Data_Assets/Scoring/ST_RankRow` _returnvalue)) (`.ColoRankNames_16_5DE520C04B9FBFA644866A8A3349F955` (break `/Game/_GameManager/Data_Assets/Scoring/ST_RankRow` _returnvalue))))
        (:`RowNotFound`
          (`/Game/UI/Menus/InGameMenu/WBP_Scoring.SetRankNameImage` :`self` _wbp_scoring :`RankText` "/Game/UI/Textures/T_Scoring_Multiplier_S.T_Scoring_Multiplier_S")))
      (`/Game/UI/Menus/InGameMenu/WBP_Scoring.SpawnAddingScore` _wbp_scoring (`KismetMathLibrary.FTrunc` InScoreIncrease))
      (add `/Game/UI/Menus/InGameMenu/WBP_Scoring.GaugeIsZero` (`/Game/_GameManager/PC_Systems.WBP Scoring` (`self.As PC Systems`)) (delegate `HideScore`)))
    (:`else`)))

(event `HideScore`
  (bind _wbp_scoring (`/Game/_GameManager/PC_Systems.WBP Scoring` (`self.As PC Systems`)))
  (set `/Game/UI/Menus/InGameMenu/WBP_Scoring.AlreadyVisible` false _wbp_scoring)
  (`KismetSystemLibrary.Delay` (`self.As PC Systems`) 2.0)
  (`UserWidget.PlayAnimationReverse` _wbp_scoring (`/Game/UI/Menus/InGameMenu/WBP_Scoring.DisplayScoreAnimation` _wbp_scoring) 1.0 false)
  (`KismetSystemLibrary.Delay` (`self.As PC Systems`) 0.35)
  (set `self.bIsScoreIncreasing` false))

(event `self.OnTransitionedHigher`
  (bind _wbp_scoring (`/Game/_GameManager/PC_Systems.WBP Scoring` (`self.As PC Systems`)))
  (`UserWidget.PlayAnimation` _wbp_scoring (`/Game/UI/Menus/InGameMenu/WBP_Scoring.ScoreSupLevelAnimation` _wbp_scoring) 0.0 1 "Forward" 1.0 false)
  (`UserWidget.PlayAnimation` _wbp_scoring (`/Game/UI/Menus/InGameMenu/WBP_Scoring.MultiplierBarSupLevelAnimation` _wbp_scoring) 0.0 1 "Forward" 1.0 false :!label _label))

(event `self.OnTransitionedLower`
  (goto _label))