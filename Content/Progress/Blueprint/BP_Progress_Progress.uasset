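; BP_Progress_Progress is a progress manager with Initialize/Deinitialize hooks that drives dialogue display and the end screen for a given player controller.
; Dialogue looks up rows in DT_Dialogues and sends them to the in-game or cinematic widget, while EndText collapses the cinematic box.
; ForceEnd pushes the HUD_Game end screen with score and rank texture.
; A looping one-second timer calls an empty Update, and a duck-color loop is left unconnected.
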(event `self.InitializeBlueprint`
  (`parent.InitializeBlueprint`)
  (`KismetSystemLibrary.K2_SetTimer` null "Update" 1.0 true true))

(event `self.DeinitializeBlueprint`
  (`parent.DeinitializeBlueprint`))

(event `Dialogue`
  (params (PlayerController :type "/Game/_GameManager/PC_Systems Object Reference") (RowName :type Name) (`In Game Dialogue` :type Boolean))
  (bind _wbp_dialogue_cinematic (`/Game/_GameManager/PC_Systems.WBP Dialogue Cinematic` PlayerController))
  (bind _wbp_dialogue_in_game (`/Game/_GameManager/PC_Systems.WBP Dialogue in Game` PlayerController))
  (if `In Game Dialogue`
    (bind _returnvalue (`|GetDataTableRow` "/Game/_GameManager/Data_Assets/Dialogues/DT_Dialogues.DT_Dialogues" RowName)
      (:`then`
        (`/Game/UI/Menus/InGameMenu/WBP_Dialogue_In_Game.DisplayDialogue` _wbp_dialogue_in_game _returnvalue)
        (set `/Game/UI/Menus/InGameMenu/WBP_Dialogue_In_Game.CurrentIndex` 0 _wbp_dialogue_in_game)))
    (else
      (bind _returnvalue_2 (`|GetDataTableRow` "/Game/_GameManager/Data_Assets/Dialogues/DT_Dialogues.DT_Dialogues" RowName)
        (:`then`
          (`/Game/UI/Menus/InGameMenu/WBP_Dialogue_Cinematic.DisplayDialogue` _wbp_dialogue_cinematic _returnvalue_2)
          (set `/Game/UI/Menus/InGameMenu/WBP_Dialogue_Cinematic.CurrentIndex` 0 _wbp_dialogue_cinematic))))))

(event `End Text`
  (params (PlayerController :type "/Game/_GameManager/PC_Systems Object Reference"))
  (`/Game/UI/Menus/InGameMenu/WBP_Dialogue_Cinematic.CollapsedDialogueBox` (`/Game/_GameManager/PC_Systems.WBP Dialogue Cinematic` PlayerController)))

(event `Force End`
  (params (PlayerController :type "/Game/_GameManager/PC_Systems Object Reference") (Score :type Integer) (RankTexture :type "Texture2D Object Reference"))
  (bind _ashud_game (cast `/Game/UI/HUD_Game` (`PlayerController.GetHUD` PlayerController)))
  (bind _returnvalue (`GameHUD.GetEndScreenClass` _ashud_game))
  (`BaseHUD.PushWidget` _ashud_game _returnvalue)
  (bind _wbp_endscreen (`/Game/UI/HUD_Game.WBP_EndScreen` _ashud_game))
  (`/Game/UI/Menus/InGameMenu/WBP_EndScreen.ShowEndScreen` _wbp_endscreen)
  (`/Game/UI/Menus/InGameMenu/WBP_EndScreen.SetAllDisplay` _wbp_endscreen Score RankTexture 0.0 null null 0 null null 0))

(fn `Update`)